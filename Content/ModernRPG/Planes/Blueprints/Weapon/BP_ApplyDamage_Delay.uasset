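; Delayed explosion actor for the plane weapon system that deals radial damage at its location once ActivateTime elapses after BeginPlay.
; A server event applies damage with the ATGM damage type, crediting Driver as causer and the owning pawn's controller as instigator.
; The owner's child actors are gathered from its ChildActorComponents and ignored by the blast.
; An Activate-All event then triggers the particle and audio effects.
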(event Custom|Activate%20-%20All
  (Components|Activation|Activate (Variables|Default|GetParticleSystem) false)
  (Components|Activation|Activate (Variables|Default|GetAudio) false))

(event Custom|Activate%20-%20Server
  (Game|Damage|ApplyRadialDamage (Variables|Default|GetDamage) (Transformation|GetActorLocation) 3e+03 "/Game/ModernRPG/General/Blueprints/DamageTypes/BPDT_ATGM.BPDT_ATGM_C" (CallFunction|GetChildActors) (Variables|Default|GetDriver) (Pawn|GetController (.AsPawn (Utilities|Casting|CastToPawn (Components|GetOwner)))) false "ECC_GameTraceChannel4")
  (CallFunction|Activate-All))

(event EventBeginPlay
  (Utilities|FlowControl|Delay (Variables|Default|GetActivateTime))
  (CallFunction|Activate-Server))

(fn ConstructionScript)

(fn GetChildActors
  (for _array_element (Actor|GetComponentsByClass (Components|GetOwner) "/Script/Engine.ChildActorComponent")
    (Utilities|Array|Add (LocalVariables|GetChildArray) (Variables|/Script/Engine.ChildActorComponent|GetChildActor _array_element)))
  (return (LocalVariables|GetChildArray)))