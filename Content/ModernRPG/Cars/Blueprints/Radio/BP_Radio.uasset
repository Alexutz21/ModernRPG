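; BP_Radio is a car radio that plays media-source stations and shows the current one on a widget component.
; Stations are data table row handles, cycled with wraparound and opened on a MediaPlayer only if the source is playable.
; A media sound component is added at BeginPlay, with volume set through an SCM_Radio sound mix override on SC_Radio.
; Turning on creates the WB_Radio display, and stopping closes the player and clears it.
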(event EventBeginPlay
  (bind _aswb_radio (Utilities|Casting|CastToWB_Radio (UserInterface|GetUserWidgetObject (Variables|Default|GetWB_Radio))))
  (Variables|/Game/ModernRPG/Cars/Blueprints/Radio/WB_Radio.WB_Radio_C|SetInternetRadio_BP _aswb_radio self)
  (AddComponent|AddMediaSoundComponent false)
  (Class|GameplayStatics|SetBaseSoundMix "/Game/ModernRPG/Cars/Blueprints/Radio/SCM_Radio.SCM_Radio"))

(fn ConstructionScript)

(fn NextStation
  (Media|MediaPlayer|Close (Variables|Default|GetMediaPlayer) :!class /Script/MediaAssets.MediaPlayer)
  (bind _returnvalue (Class|MediaPlayer|CanPlaySource (Variables|Default|GetMediaPlayer) (Utilities|Struct|BreakS_Radio (CallFunction|GetSRadio (Utilities|Array|Get(acopy) (Variables|Default|GetRadios) (Math|Integer|%(Integer) (+ (Variables|Default|GetStationIndex) 1) (Utilities|Array|Length (Variables|Default|GetRadios))))))))
  (if _returnvalue
    (Variables|Default|SetStationIndex (Math|Integer|%(Integer) (+ (Variables|Default|GetStationIndex) 1) (Utilities|Array|Length (Variables|Default|GetRadios))))
    (CallFunction|NewStation)))

(fn PreviousStation
  (Media|MediaPlayer|Close (Variables|Default|GetMediaPlayer) :!class /Script/MediaAssets.MediaPlayer)
  (bind _returnvalue (Class|MediaPlayer|CanPlaySource (Variables|Default|GetMediaPlayer) (Utilities|Struct|BreakS_Radio (CallFunction|GetSRadio (Utilities|Array|Get(acopy) (Variables|Default|GetRadios) (select (< (- (Variables|Default|GetStationIndex) 1) 0) (Utilities|Array|LastIndex (Variables|Default|GetRadios)) (- (Variables|Default|GetStationIndex) 1)))))))
  (if _returnvalue
    (Variables|Default|SetStationIndex (select (< (- (Variables|Default|GetStationIndex) 1) 0) (Utilities|Array|LastIndex (Variables|Default|GetRadios)) (- (Variables|Default|GetStationIndex) 1)))
    (CallFunction|NewStation)))

(fn PlayRadio
  (Media|MediaPlayer|Play (Variables|Default|GetMediaPlayer) :!class /Script/MediaAssets.MediaPlayer))

(fn StopRadio
  (bind _wb_radioref (Variables|Default|GetWB_RadioRef))
  (Media|MediaPlayer|Close (Variables|Default|GetMediaPlayer) :!class /Script/MediaAssets.MediaPlayer)
  (Utilities|IsValid _wb_radioref
    (:Is%20Valid
      (Default|TurnOffRadio _wb_radioref))
    (:Is%20Not%20Valid
      _))
  (UserInterface|SetWidget (Variables|Default|GetWB_Radio) 0))

(fn TurnonRadio
  (CallFunction|ChangeVolumeRadio (Variables|Default|GetVolumeLevel))
  (bind _returnvalue (UserInterface|CreateWidget "/Game/ModernRPG/Cars/Blueprints/Radio/WB_Radio.WB_Radio_C"))
  (bind _output_get (Variables|Default|SetWB_RadioRef _returnvalue))
  (UserInterface|SetWidget (Variables|Default|GetWB_Radio) _output_get)
  (Default|TurnonRadio (Variables|Default|GetWB_RadioRef))
  (CallFunction|NewStation))

(fn NewStation
  (bind _stationindex (Variables|Default|GetStationIndex))
  (bind _radios (Variables|Default|GetRadios))
  (bind _output (Utilities|Array|Get(acopy) _radios _stationindex))
  (bind _out_row (CallFunction|GetSRadio _output))
  (bind _mediasource (Utilities|Struct|BreakS_Radio _out_row))
  (Utilities|IsValid (Variables|Default|GetWB_RadioRef)
    (:Is%20Valid
      (bind _returnvalue (Class|MediaPlayer|CanPlaySource (Variables|Default|GetMediaPlayer) _mediasource))
      (if _returnvalue
        (Media|MediaPlayer|OpenSource (Variables|Default|GetMediaPlayer) _mediasource)
        (Default|UpdateStationName (Variables|Default|GetWB_RadioRef) (Utilities|Array|Get(acopy) (Variables|Default|GetRadios) (Variables|Default|GetStationIndex)))))))

(fn ChangeVolumeRadio
  (params (VolumeLevel :type Float%20%28double-precision%29))
  (Variables|Default|SetVolumeLevel VolumeLevel)
  (Audio|SetSoundMixClassOverride "/Game/ModernRPG/Cars/Blueprints/Radio/SCM_Radio.SCM_Radio" "/Game/ModernRPG/Cars/Blueprints/Radio/SC_Radio.SC_Radio" (Variables|Default|GetVolumeLevel) 1.0 1.0 true))

(fn GetSRadio
  (params (DataTableRowHandle :type Data%20Table%20Row%20Handle%20Structure%20%28by%20ref%29))
  (bind (_datatable _rowname) (Utilities|Struct|BreakDataTableRowHandle DataTableRowHandle))
  (bind _returnvalue (Utilities|GetDataTableRow _datatable _rowname)
    (:then
      (return _returnvalue))))