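; Actor component that sets up grenade throw prediction for its owning actor by giving it a spline predictor actor.
; On BeginPlay it gets the throw prediction reference from the owner and, if valid, spawns BP_PredicateSpline at that world transform.
; The spawned actor is owned by the same owner, stored as Predicate and attached to it with location snapped and rotation and scale kept relative.
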(event Custom|SpawnPredi%20-%20OC
  ;[1 1 1] Initialize Component
  (bind _grenadethrowpred (Class|BPISkillSystem|GrenadeThrowPred(Message) (Components|GetOwner)))
  (Utilities|IsValid _grenadethrowpred
    (:Is%20Valid
      (bind _returnvalue (Game|SpawnActorfromClass "/Game/ModernRPG/ModernSkillTree/Blueprint/BP_PredicateSpline.BP_PredicateSpline_C" (Transformation|GetWorldTransform _grenadethrowpred) "Undefined" (Components|GetOwner) false "0.000000,0.000000,0.000000" 0))
      (Variables|Default|SetPredicate _returnvalue)
      (Transformation|AttachActorToActor (Variables|Default|GetPredicate) (Components|GetOwner) "None" "SnapToTarget" "KeepRelative" "KeepRelative" true))))

(event EventBeginPlay
  ;[1 1 1] Initialize Component
  (CallFunction|SpawnPredi-OC))