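; BP_PredicateSpline is an actor that previews a grenade throw arc for its owning character while throwing is active.
; Each tick it predicts a projectile path from a component supplied by the owner, launched along control rotation.
; When the trace hits, it rebuilds the spline and its spline meshes from the path points and moves a marker sphere to the end.
; Ending the throw disables tick and clears the preview.
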(event Custom|Throwing-OC
  (params (Throwing :type Boolean))
  (bind _output_get (Variables|Default|SetThrowing Throwing))
  (Actor|Tick|SetActorTickEnabled _output_get)
  (if _output_get
    (CallFunction|StartWork)
    (else
      (CallFunction|DestroyPrediction))))

(event Custom|StartWork
  (bind (_start _velocity) (CallFunction|GetPositions))
  (bind _spline (Variables|Default|GetSpline))
  (bind (_outhit _outpathpositions _outlasttracedestination _returnvalue) (Class|GameplayStatics|BlueprintPredictProjectilePathbyTraceChannel _start _velocity true 0.0 "ECC_Camera" false (Utilities|Array|MakeArray (Components|GetOwner)) "None" 0.0 15.0 3.0))
  (Rendering|SetVisibility (Variables|Default|GetSphere) _returnvalue false)
  (if _returnvalue
    (Utilities|FlowControl|Sequence
      (:then_0
        (Variables|Default|SetArrayLocations _outpathpositions)
        (Spline|ClearSplinePoints (Variables|Default|GetSpline) true)
        (if (Utilities|Array|IsValidIndex (Variables|Default|GetSplineMeshes))
          (for _array_element (Variables|Default|GetSplineMeshes)
            (Components|DestroyComponent _array_element))
          (Utilities|Array|Clear (Variables|Default|GetSplineMeshes)))
        (for (_array_element_2 _array_index) (Variables|Default|GetArrayLocations)
          (Spline|AddSplinePointatIndex (Variables|Default|GetSpline) _array_element_2 _array_index "World" true))
        (for _index (range 0 (- (Spline|GetNumberOfSplinePoints (Variables|Default|GetSpline)) 2))
          (bind _returnvalue_2 (AddComponent|AddSplineMeshComponent true))
          (Utilities|Array|Add (Variables|Default|GetSplineMeshes) _returnvalue_2)
          (SplineMesh|SetStartandEnd _returnvalue_2 (.Location (Spline|GetLocationandTangentatSplinePoint _spline _index "World")) (.Tangent (Spline|GetLocationandTangentatSplinePoint _spline _index "World")) (.Location (Spline|GetLocationandTangentatSplinePoint _spline (+ _index 1) "World")) (.Tangent (Spline|GetLocationandTangentatSplinePoint _spline (+ _index 1) "World")) true :!class /Script/Engine.SplineMeshComponent)))
      (:then_1
        (Transformation|SetWorldLocation (Variables|Default|GetSphere) _outlasttracedestination false true)))))

(event Custom|DestroyPrediction
  (if (Utilities|Array|IsValidIndex (Variables|Default|GetSplineMeshes))
    (for _array_element (Variables|Default|GetSplineMeshes)
      (Components|DestroyComponent _array_element))
    (Rendering|SetVisibility (Variables|Default|GetSphere) false false)
    (Utilities|Array|Clear (Variables|Default|GetSplineMeshes))
    (Utilities|Array|Clear (Variables|Default|GetArrayLocations))))

(event EventTick
  (params (DeltaSeconds :type Float%20%28single-precision%29))
  (if (Variables|Default|GetThrowing)
    (CallFunction|StartWork)))

(fn ConstructionScript)

(fn GetPositions
  (bind _returnvalue (Components|GetOwner))
  (bind _ascharacter (Utilities|Casting|CastToCharacter _returnvalue))
  (bind _returnvalue_2 (Pawn|GetControlRotation _ascharacter :!class /Script/Engine.Pawn))
  (bind _returnvalue_3 (Math|Vector|GetForwardVector _returnvalue_2))
  (bind _grenadethrowpred (Class|BPISkillSystem|GrenadeThrowPred(Message) (Components|GetOwner)))
  (return (+ (Transformation|GetWorldLocation _grenadethrowpred) (* _returnvalue_3 5e+01)) (* _returnvalue_3 2e+03)))