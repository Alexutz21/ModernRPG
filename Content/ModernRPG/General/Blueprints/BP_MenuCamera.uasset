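; BP_MenuCamera is a menu camera actor that fakes a camera animation by drifting back and forth between two poses.
; StartAnimation, called on BeginPlay, caches the camera's relative transform, enables tick and opens a gate; StopAnimation reverses the latter two.
; Each tick lerps location and rotation toward NextCameraPoint by a fixed, frame-rate-dependent alpha step, flipping direction near either end.
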(event Custom|StartAnimation
  (bind _nextcamerapoint (Variables|Default|GetNextCameraPoint))
  (bind _cameracomponent (Variables|CameraActor|GetCameraComponent))
  ;[1 1 1] Emulationg of a camera animation
  (Variables|Default|SetStartLocation (Variables|/Script/Engine.SceneComponent|GetRelativeLocation _cameracomponent))
  (Variables|Default|SetStartRotation (Variables|/Script/Engine.SceneComponent|GetRelativeRotation _cameracomponent))
  (Actor|Tick|SetActorTickEnabled true)
  (Utilities|FlowControl|Gate true) ; enters at Open
)

(event Custom|StopAnimation
  (bind _nextcamerapoint (Variables|Default|GetNextCameraPoint))
  ;[1 1 1] Emulationg of a camera animation
  (Actor|Tick|SetActorTickEnabled false)
  (Utilities|FlowControl|Gate true) ; enters at Close
)

(event EventBeginPlay
  ;[1 1 1] Emulationg of a camera animation
  (CallFunction|StartAnimation))

(event EventTick
  (params (DeltaSeconds :type Float%20%28single-precision%29))
  (bind _nextcamerapoint (Variables|Default|GetNextCameraPoint))
  ;[1 1 1] Emulationg of a camera animation
  (Utilities|FlowControl|Gate true
    (:Exit
      (Variables|Default|SetCurrentAlpha (+ (Variables|Default|GetCurrentAlpha) (* 0.0005 (select (Variables|Default|GetReversed) -1.0 1.0))))
      (Transformation|SetRelativeLocationAndRotation (Variables|CameraActor|GetCameraComponent) (Math|Vector|Lerp(Vector) (Variables|Default|GetStartLocation) (Variables|/Script/Engine.SceneComponent|GetRelativeLocation _nextcamerapoint) (Variables|Default|GetCurrentAlpha)) (Math|Rotator|Lerp(Rotator) (Variables|Default|GetStartRotation) (Variables|/Script/Engine.SceneComponent|GetRelativeRotation _nextcamerapoint) (Variables|Default|GetCurrentAlpha)) false false)
      (if (or (>= (Variables|Default|GetCurrentAlpha) 0.95) (<= (Variables|Default|GetCurrentAlpha) 0.0))
        (Variables|Default|SetReversed (not (Variables|Default|GetReversed)))))))

(fn ConstructionScript)