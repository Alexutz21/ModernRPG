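; Target indicator Blueprint for the RL weapon, hosting an indicator widget through its WBMark widget component.
; On BeginPlay it casts the component's widget to WB_RLIndicator, then passes it a reference to itself and its DistanceCurve.
; PlayFirstAnimation and PlayCloseAnimation are placeholders here that only return zero.
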(event EventBeginPlay
  (bind _output_get (Variables|Default|SetWB (Variables|Default|GetWB_Mark)))
  (bind _aswb_rlindicator (Utilities|Casting|CastToWB_RLIndicator (UserInterface|GetUserWidgetObject _output_get)))
  (bind _output_get_2 (Variables|Default|SetRL _aswb_rlindicator))
  (Variables|/Game/ModernRPG/General/GUI/Widgets/TargetIndicator/WB_RLIndicator.WB_RLIndicator_C|SetOwnerBP_RL _output_get_2 self)
  (Variables|/Game/ModernRPG/General/GUI/Widgets/TargetIndicator/WB_RLIndicator.WB_RLIndicator_C|SetDistanceCurve (Variables|Default|GetRL) (Variables|Setup|GetDistanceCurve)))

(fn ConstructionScript)

(fn PlayCloseAnimation
  (return 0.0))

(fn PlayFirstAnimation
  (return 0.0))