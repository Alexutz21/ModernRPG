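; BP_WeaponBullet is a weapon bullet actor that destroys itself on hitting anything but its owner.
; If enabled, it first pushes physics-simulating components with a velocity-scaled impulse.
; Helpers filter out self and owner-related targets, look up decal and sound by surface, and spawn jittered metal sparks, though the event graph calls none.
; A large shared vehicle/weapon interface is mostly stubbed, apart from returns like parent owner and fixed shell damage.
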(event Collision|EventHit
  (params (MyComp :type Primitive%20Component%20Object%20Reference) (Other :type Actor%20Object%20Reference) (OtherComp :type Primitive%20Component%20Object%20Reference) (bSelfMoved :type Boolean) (HitLocation :type Vector :default "0, 0, 0") (HitNormal :type Vector :default "0, 0, 0") (NormalImpulse :type Vector :default "0, 0, 0") (Hit :type Hit%20Result%20Structure%20%28by%20ref%29))
  ;[1 1 1] Hit someone
  (if (!= Other (Components|GetOwner))
    _
    (else
      (Utilities|IsValid Other
        (:Is%20Not%20Valid
          _))))
  (Utilities|IsValid OtherComp
    (:Is%20Valid
      (if (Physics|IsSimulatingPhysics OtherComp "None")
        (if (Variables|Default|GetShouldAddImpulse)
          (Physics|AddImpulseatLocation OtherComp (* (Transformation|GetVelocity) 1e+02) (Transformation|GetActorLocation) "None")
          (Actor|DestroyActor)
          (else
            (Actor|DestroyActor :!label _label)))
        (else
          (goto _label))))))

(fn ConstructionScript)

(fn NotSelfandOwner
  (params (Primitive :type Primitive%20Component%20Object%20Reference))
  (return (Math|Boolean|ANDBoolean (!= (Variables|Default|GetOverlappedCache) (Game|GetInstigator)) (!= (Variables|Default|GetOverlappedCache) self) (!= Primitive (Variables|MyProjectile|GetCollisionComponent)) (!= (Utilities|GetClass (Variables|Default|GetOverlappedCache)) (Utilities|GetClass self)))))

(fn IsItTarget
  (params (Primitive :type Primitive%20Component%20Object%20Reference) (InputPin :type Actor%20Object%20Reference))
  (bind _owner (Class|BPIVehicles|GetParentOwner(Message) InputPin))
  (bind _owner_2 (Class|BPIVehicles|GetParentOwner(Message) (Components|GetOwner)))
  (if (Math|Boolean|ANDBoolean (CallFunction|NotSelfandOwner Primitive) (!= _owner _owner_2) true)
    (return true)
    (else
      (return false))))

(fn GetImpactData
  (params (B :type EPhysicalSurface%20Enum :default "SurfaceType_Default"))
  (bind _outrownames (DataTable|GetDataTableRowNames (Variables|Default|GetImpactDataTAble)))
  (for _array_element _outrownames
    (bind _returnvalue (Utilities|GetDataTableRow (Variables|Default|GetImpactDataTAble) _array_element)
      (:then
        (if (Utilities|Enum|Equal(Enum) (.Surface (Utilities|Struct|BreakS_ImpactData _returnvalue)) B)
          (return (.Decal (Utilities|Struct|BreakS_ImpactData _returnvalue)) (.Sound (Utilities|Struct|BreakS_ImpactData _returnvalue))))))))

(fn SpawnHitEmitter
  (params (Location :type Vector) (Material :type Physical%20Material%20Object%20Reference))
  (bind _returnvalue (Math|Conversions|RotationFromXVector Location))
  (bind (_roll _pitch _yaw) (Math|Rotator|BreakRotator _returnvalue))
  (Effects|SpawnEmitteratLocation "/Game/ModernRPG/Particles/P_Metal.P_Metal" Location (Math|Rotator|MakeRotator (Math|Random|RandomFloatinRange (+ _roll 7.0) (- _roll 7.0)) (Math|Random|RandomFloatinRange (+ _pitch 7.0) (- _pitch 7.0)) (Math|Random|RandomFloatinRange (+ _yaw 7.0) (- _yaw 7.0))))
  (return))

(fn GetSmokeSettings0
  (return ""))

(fn GetCannonSettings0
  (return ""))

(fn GetMinigunSettings0
  (return ""))

(fn BulletDamage
  (return 0.0))

(fn CanHit
  (return false))

(fn CanShot?
  (return false))

(fn GetMinigunShellPlace
  (return 0))

(fn GetTankSettings
  (return ""))

(fn GetActiveCamera
  (return "NewEnumerator0"))

(fn GetAllWeapons
  (return "NewEnumerator0"))

(fn GetArrowBarrel
  (return 0))

(fn GetArrowMinigun
  (return 0))

(fn GetArrowSmoke
  (return 0))

(fn GetAudioAmmunitionExplosion
  (return 0))

(fn GetBarrel
  (return 0))

(fn GetBlackboardRef
  (return 0))

(fn GetBody
  (return 0 0))

(fn GetBodyCamera
  (return 0))

(fn GetBreakThroughSound
  (return 0))

(fn GetCameraAimInside
  (return 0))

(fn GetCameraMinigun
  (return 0))

(fn GetCameraTurret
  (return 0))

(fn GetCannonSettings
  (return ""))

(fn GetCannonSound
  (return 0))

(fn GetCountOfCannonShells
  (return 0))

(fn GetCountOfMachineGun
  (return 0))

(fn GetCountOfMinigunShells
  (return 0))

(fn GetCountOfShells
  (return 0))

(fn GetCountOfSmokes
  (return 0))

(fn GetDefaultAim
  (return 0))

(fn GetDemoSkeletalMeshes
  (return 0 0 0 0 0 0))

(fn GetDestroyedTankParticle
  (return 0))

(fn GetDestroyedTankSmokeParticle
  (return 0))

(fn GetDetectionDistance[Fighter]
  (return 0.0))

(fn GetDriver
  (return 0))

(fn GetDriverInside
  (return 0))

(fn GetDriverPlace
  (return 0))

(fn GetExpInfo
  (return 0.0 0.0))

(fn GetForward/SideSpeed
  (return 0.0 0.0 0.0))

(fn GetHealth
  (return 0.0 0.0))

(fn GetHeight
  (return 0.0))

(fn GetHitDecalClass
  (return 0))

(fn GetHitWidget
  (return 0))

(fn GetLastActiveWeapon
  (return "NewEnumerator0"))

(fn GetLastWheels
  (return 0))

(fn GetLeftWheels
  (return 0))

(fn GetMainCamera
  (return 0))

(fn GetMainShotParticle
  (return 0))

(fn GetMainSpringArm
  (return 0))

(fn GetMaxSpeed
  (return 0.0))

(fn GetMinigunAim
  (return 0))

(fn GetMinigunSettings
  (return ""))

(fn GetMiniGunTurret
  (return 0))

(fn GetMinimapArrow
  (return 0))

(fn GetParentOwner
  (return (Components|GetOwner)))

(fn GetPassengers
  (return 0))

(fn GetPawnType
  (return "NewEnumerator3"))

(fn GetPlaceforAmmunitionExplosionParticle
  (return 0))

(fn GetPlaneSettings
  (return ""))

(fn GetPointtoShot
  (return 0))

(fn GetPredictAim
  (return 0))

(fn GetReloadTime
  (return 0.0))

(fn GetRicochetSound
  (return 0))

(fn GetRightWheels
  (return 0))

(fn GetSecondShotParticle
  (return 0))

(fn GetShellDamage
  (return 1e+01))

(fn GetShotAudio
  (return 0))

(fn GetSmokeSettings
  (return ""))

(fn GetSpeed
  (return 0.0))

(fn GetSplineL
  (return 0))

(fn GetSplineR
  (return 0))

(fn GetSusp
  (return 0))

(fn GetSuspensions
  (return 0))

(fn GetTarget
  (return 0))

(fn GetTeam
  (return "NewEnumerator2"))

(fn GetTrackL
  (return 0))

(fn GetTrackR
  (return 0))

(fn GetTurret
  (return 0))

(fn GetVehicleHealthInfo
  (return ""))

(fn GetWBTank
  (return 0))

(fn HitCharacterVelocity
  (return 0.0 0))

(fn IamParent
  (return false))

(fn IsAI
  (return false))

(fn IsAiming
  (return false))

(fn IsBOMBLOAD
  (return false))

(fn IsComponentAllright
  (return false))

(fn IsDestroyed
  (return false))

(fn IsDrone
  (return false))

(fn IsHeatTrap
  (return false))

(fn IsItTrack
  (return false))

(fn IsShell
  (return false))

(fn IsSiucideMode
  (return false))

(fn IsTank
  (return false))

(fn IsTankActive
  (return false))

(fn IsTankValid
  (return false))

(fn IsVehicleActive
  (return false))

(fn IsVehicleTarget
  (return false))

(fn NoImpulse
  (return false))

(fn PlaceforShotSound
  (return 0))

(fn PointtoMove
  (return false))

(fn Sensible
  (return false))

(fn TankStarted
  (return false))

(fn TypeOfShell
  (return "NewEnumerator6"))