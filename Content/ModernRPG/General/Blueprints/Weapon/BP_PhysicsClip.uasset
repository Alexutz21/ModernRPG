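; BP_PhysicsClip is a weapon clip actor that displays a given mesh, either as a short-lived physics prop or without collision.
; A server event forwards initialization to an all-clients event, which sets the mesh and physics state.
; Simulated clips expire after a few seconds, while others have collision disabled.
; Materials come from the mesh's defaults or a supplied array, and an impulse node is left unconnected.
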(event Custom|Initialize%20-ALL
  (params (NewMesh :type Static%20Mesh%20Object%20Reference) (bSimulate :type Boolean) (Materials :type Array%20of%20Material%20Instance%20Object%20References) (DefaultMaterial :type Boolean))
  ;[1 1 1] Initialzie
  (Utilities|FlowControl|Sequence
    (:then_0
      (Components|StaticMesh|SetStaticMesh (Variables|Default|GetStaticMesh) NewMesh)
      (Physics|SetSimulatePhysics (Variables|Default|GetStaticMesh) bSimulate)
      (if bSimulate
        (Actor|SetLifeSpan 3.0)
        (else
          (Collision|SetCollisionEnabled (Variables|Default|GetStaticMesh) "NoCollision"))))
    (:then_1
      (if DefaultMaterial
        (for (_array_element _array_index) (Variables|/Script/Engine.StaticMesh|GetStaticMaterials NewMesh)
          (Rendering|Material|SetMaterial (Variables|Default|GetStaticMesh) _array_index (Utilities|Struct|BreakStaticMaterial _array_element)))
        (else
          (for (_ _array_index_2) (Rendering|Material|GetMaterials (Variables|Default|GetStaticMesh))
            (if (Utilities|Array|IsValidIndex Materials _array_index_2)
              (Rendering|Material|SetMaterial (Variables|Default|GetStaticMesh) _array_index_2 (Utilities|Array|Get(acopy) Materials _array_index_2)))))))))

(event Custom|InitializeClip%20-Server
  (params (NewMesh :type Static%20Mesh%20Object%20Reference) (bSimulate :type Boolean) (Materials :type Array%20of%20Material%20Instance%20Object%20References) (DefaultMaterial :type Boolean))
  ;[1 1 1] Initialzie
  (CallFunction|Initialize-ALL NewMesh bSimulate Materials DefaultMaterial))

(fn ConstructionScript)