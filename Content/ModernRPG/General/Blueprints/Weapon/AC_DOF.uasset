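; AC_DOF is a weapon-related component that switches camera depth of field between first-person and third-person settings.
; InitializeCamera stores the passed-in camera for later use.
; SetFPPDOF zeroes aperture and focus distance, while SetTPPDOF applies the configured TPP values.
; Both write the aperture F-stop and focal distance into that camera's post-process settings when it is valid.
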(event Custom|InitializeCamera
  (params (FirstPersonCamera :type Camera%20Component%20Object%20Reference))
  ;[1 1 1] Initialize Camera
  (Variables|Default|SetFirstPersonCamera FirstPersonCamera)
  (Variables|Default|SetRememberMainCamera FirstPersonCamera))

(event Custom|SetFPPDOF
  (bind _remembermaincamera (Variables|Default|GetRememberMainCamera))
  ;[1 1 1] Set DOF
  (Variables|Default|SetDOF%20Aperture 0.0)
  (Variables|Default|SetFocusLocation 0.0)
  (Utilities|IsValid _remembermaincamera
    (:Is%20Valid
      (bind _structout (Utilities|Struct|SetmembersinPostProcessSettings (Variables|/Script/Engine.CameraComponent|GetPostProcessSettings _remembermaincamera) (Variables|Default|GetDOF%20Aperture) (Variables|Default|GetFocusLocation)))
      (Variables|/Script/Engine.CameraComponent|SetPostProcessSettings (Variables|Default|GetRememberMainCamera) _structout))))

(event Custom|SetTPPDOF
  (bind _remembermaincamera (Variables|Default|GetRememberMainCamera))
  ;[1 1 1] Set DOF TPP
  (Variables|Default|SetDOF%20Aperture (Variables|Default|GetTPP%20DOF))
  (Variables|Default|SetFocusLocation (Variables|Default|GetTPP%20Focus))
  (Utilities|IsValid _remembermaincamera
    (:Is%20Valid
      (bind _structout (Utilities|Struct|SetmembersinPostProcessSettings (Variables|/Script/Engine.CameraComponent|GetPostProcessSettings _remembermaincamera) (Variables|Default|GetDOF%20Aperture) (Variables|Default|GetFocusLocation)))
      (Variables|/Script/Engine.CameraComponent|SetPostProcessSettings (Variables|Default|GetRememberMainCamera) _structout))))