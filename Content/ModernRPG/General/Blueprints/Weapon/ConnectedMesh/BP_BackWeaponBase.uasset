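; BP_BackWeaponBase is a base Blueprint for a cosmetic weapon, by its name the one shown on a character's back.
; Initialize sets the skeletal weapon mesh and materials, then attaches a default clip mesh at the given socket.
; Modifications spawn as collision-free static mesh components on weapon sockets, tracked in a map by type.
; A Patronage (magazine) modification clears the default clip, and removing it restores that clip.
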(event Custom|SetModifications
  (params (Skeletal :type Static%20Mesh%20Object%20Reference) (SocketName :type Name) (Type :type E_ModifiablePart%20Enum :default "NewEnumerator0"))
  (bind _returnvalue (AddComponent|AddStaticMeshComponent false))
  (Collision|SetCollisionEnabled _returnvalue "NoCollision")
  (CallFunction|SetModificationsALL Skeletal SocketName _returnvalue Type))

(event Custom|Initialize
  (params (Skeletal :type Skeletal%20Mesh%20Object%20Reference) (Materials :type Array%20of%20Material%20Instance%20Object%20References) (Clip :type Static%20Mesh%20Object%20Reference) (Socket :type Name))
  (Variables|Default|SetSkeletal Skeletal)
  (Variables|Default|SetMaterials Materials)
  (Variables|Default|SetClip Clip)
  (Variables|Default|SetSocket Socket)
  (CallFunction|SetDefaultPatronage)
  (Class|SkinnedMeshComponent|SetSkeletalMesh (Variables|Default|GetWeaponMesh) (Variables|Default|GetSkeletal) true)
  (for (_array_element _array_index) (Variables|Default|GetMaterials)
    (Rendering|Material|SetMaterial (Variables|Default|GetWeaponMesh) _array_index _array_element)))

(event Custom|RemoveModification
  (params (Key :type E_ModifiablePart%20Enum%20%28by%20ref%29 :default "NewEnumerator0"))
  (bind _modifications (Variables|Default|GetModifications))
  (bind (_value _returnvalue) (Utilities|Map|Find _modifications Key))
  (if _returnvalue
    (Components|DestroyComponent _value)
    (Utilities|Map|Remove (Variables|Default|GetModifications) Key)
    (if (Utilities|Enum|Equal(Enum) Key (Variables|Default|GetPatronage))
      (CallFunction|SetDefaultPatronage))))

(event Custom|SetDefaultPatronage
  (Components|StaticMesh|SetStaticMesh (Variables|Default|GetClipMesh) (Variables|Default|GetClip))
  (Transformation|AttachComponentToComponent (Variables|Default|GetClipMesh) (Variables|Default|GetWeaponMesh) (Variables|Default|GetSocket) "KeepRelative" "KeepRelative" "KeepRelative" true)
  (Collision|SetCollisionEnabled (Variables|Default|GetClipMesh) "NoCollision")
  (for (_array_element _array_index) (Variables|Default|GetClipMaterials)
    (Rendering|Material|SetMaterial (Variables|Default|GetClipMesh) _array_index _array_element)))

(event Custom|SetModificationsALL
  (params (InputPin :type Static%20Mesh%20Object%20Reference) (InputPin2 :type Name) (Target :type Static%20Mesh%20Component%20Object%20Reference) (InputPin3 :type E_ModifiablePart%20Enum :default "NewEnumerator0"))
  (Components|StaticMesh|SetStaticMesh Target InputPin)
  (Transformation|AttachComponentToComponent Target (Variables|Default|GetWeaponMesh) InputPin2 "KeepRelative" "KeepRelative" "KeepRelative" true)
  (Collision|SetCollisionEnabled Target "NoCollision")
  (Utilities|Map|Add (Variables|Default|GetModifications) InputPin3 Target)
  (if (Utilities|Enum|Equal(Enum) InputPin3 (Variables|Default|GetPatronage))
    (Components|StaticMesh|SetStaticMesh (Variables|Default|GetClipMesh) 0)))

(fn ConstructionScript)