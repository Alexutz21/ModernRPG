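; BP_ConnectedArmor is an equipment actor that attaches armor meshes to its owning character's body mesh.
; It sets its static and skeletal meshes on initialization, using master pose so the skeletal mesh follows the body's animation.
; Take and remove events move it between main and back sockets, while detach events destroy it.
; CheckState reports whether the owner is in certain weapon states or has a blocked weapon.
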(event Custom|InitializeCustom
  (params (Socket :type Name) (BackSocket :type Name) (NewStaticMesh :type Static%20Mesh%20Object%20Reference) (Skeletal%20Mesh :type Skeletal%20Mesh%20Object%20Reference))
  ;[1 1 1] Inialize
  (Variables|Default|SetSocket Socket)
  (Variables|Default|SetBackSocket BackSocket)
  (bind _output_get (Variables|Default|SetNewStaticMesh NewStaticMesh))
  (Components|StaticMesh|SetStaticMesh (Variables|Default|GetStaticMesh) _output_get)
  (CallFunction|AttachActor)
  (Class|SkinnedMeshComponent|SetSkeletalMesh (Variables|Default|GetSkeletalMesh) Skeletal%20Mesh true)
  (CallFunction|SetSkeletal Skeletal%20Mesh))

(event Custom|AttachToCustomSocket
  (params (SocketName :type Name))
  ;[1 1 1] Attach to custom socket
  (bind _bodymesh (CallFunction|GetCharacterSkeleton (Components|GetOwner)))
  (Transformation|AttachComponentToComponent _bodymesh SocketName "KeepRelative" "KeepRelative" "KeepRelative" true))

(event Custom|SetSkeletal
  (params (NewMesh :type Skeletal%20Mesh%20Object%20Reference))
  (Class|SkinnedMeshComponent|SetSkeletalMesh (Variables|Default|GetSkeletalMesh) NewMesh true)
  (bind _bodymesh (CallFunction|GetCharacterSkeleton (Components|GetOwner)))
  (Class|SkinnedMeshComponent|SetMasterPoseComponent (Variables|Default|GetSkeletalMesh) _bodymesh true))

(event Custom|TakeItem
  ;[1 1 1] Toggle Item
  (CallFunction|AttachtoCustomSocket (Variables|Default|GetSocket))
  (Variables|Default|SetItemRemoved true))

(event Custom|RemoveItem
  ;[1 1 1] Toggle Item
  (CallFunction|AttachtoCustomSocket (Variables|Default|GetBackSocket))
  (Variables|Default|SetItemRemoved false))

(event Custom|Detach%20-ALL
  ;[1 1 1] Detach
  (Transformation|DetachFromActor "KeepWorld" "KeepWorld" "KeepWorld")
  (Actor|DestroyActor))

(event Custom|InitialzieSockets
  (params (Socket :type Name) (BackSocket :type Name) (Type :type E_ItemType%20Enum :default "NewEnumerator0"))
  ;[1 1 1] Initialize Sockets
  (Variables|Default|SetSocket Socket)
  (Variables|Default|SetBackSocket BackSocket)
  (CallFunction|AttachActor))

(event Custom|Detach%20-Server
  ;[1 1 1] Detach
  (CallFunction|Detach-ALL))

(event Custom|AttachActor
  ;[1 1 1] Attach Process
  (bind _bodymesh (CallFunction|GetCharacterSkeleton (Components|GetOwner)))
  (Transformation|AttachComponentToComponent _bodymesh (Variables|Default|GetSocket) "KeepRelative" "KeepRelative" "KeepRelative" true)
  (if (Utilities|IsValidClass (.AnimBP (Utilities|Struct|BreakS_SecondaryInventoryInfoF (Variables|Default|GetBagInfo))))
    (Class|SkeletalMeshComponent|SetAnimClass (Variables|Default|GetSkeletalMesh))))

(event EventBeginPlay
  ;[1 1 1] Begin play
  (bind _bodymesh (CallFunction|GetCharacterSkeleton (Components|GetOwner)))
  (Class|SkinnedMeshComponent|SetMasterPoseComponent (Variables|Default|GetSkeletalMesh) _bodymesh true))

(fn ConstructionScript)

(fn GetUsedSceneComponent
  (return (Variables|Default|GetSkeletalMesh)))

(fn CheckState
  (bind _returnvalue (Components|GetOwner))
  (bind _returnvalue_2 (Actor|GetComponentbyClass _returnvalue "/Game/ModernRPG/General/Blueprints/ActorComponents/Character/State/AC_PlayerCurrentState.AC_PlayerCurrentState_C"))
  (bind _currentstate (Variables|/Game/ModernRPG/General/Blueprints/ActorComponents/Character/State/AC_PlayerCurrentState.AC_PlayerCurrentState_C|GetCurrentState _returnvalue_2))
  (Utilities|IsValid _returnvalue
    (:Is%20Valid
      (return (Math|Boolean|ORBoolean (== _currentstate (Utilities|Enum|LiteralenumE_WeaponState "NewEnumerator0")) (== _currentstate (Utilities|Enum|LiteralenumE_WeaponState "NewEnumerator2")) (== _currentstate (Utilities|Enum|LiteralenumE_WeaponState "NewEnumerator1")) (.BlockedWeapon (Default|GetBlockInformation (Actor|GetComponentbyClass (Components|GetOwner) "/Game/ModernRPG/General/Blueprints/ActorComponents/Weapon/AC_WeaponBlock.AC_WeaponBlock_C"))))))))