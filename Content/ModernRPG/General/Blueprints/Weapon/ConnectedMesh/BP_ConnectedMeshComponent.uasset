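; Weapon mesh actor that attaches to the owning character's body, switching between active and back sockets when taken or removed.
; It sets meshes and materials from supplied data, and routes clip setup, clip removal and detach-destroy through Server/All events.
; It manages the aim camera and scope render target, and relays aim, zoom and laser toggles to modification actors.
; Laser targeting picks weapon-component or laser-forward traces by aim and movement state.
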(event Custom|InitializeCustom
  (params (Socket :type Name) (BackSocket :type Name) (NewStaticMesh :type Static%20Mesh%20Object%20Reference) (Skeletal%20Mesh :type Skeletal%20Mesh%20Object%20Reference) (Type :type E_ItemType%20Enum :default "NewEnumerator0") (Materials :type Array%20of%20Material%20Instance%20Object%20References))
  ;[1 1 1] Initialize
  (Variables|Default|SetSocket Socket)
  (Variables|Default|SetBackSocket BackSocket)
  (bind _output_get (Variables|Default|SetNewStaticMesh NewStaticMesh))
  (Components|StaticMesh|SetStaticMesh (Variables|Default|GetStaticMesh) _output_get)
  (Variables|Default|SetType Type)
  (CallFunction|AttachActor)
  (Class|SkinnedMeshComponent|SetSkeletalMesh (Variables|Default|GetSkeletalMesh) Skeletal%20Mesh true)
  (CallFunction|InitializeClip-Server (.Clip (Utilities|Struct|BreakS_Appearance (Utilities|Struct|BreakS_Weapon (CallFunction|GetItemInfo)))))
  (for (_array_element _array_index) Materials
    (Rendering|Material|SetMaterial (Variables|Default|GetSkeletalMesh) _array_index _array_element)))

(event Custom|AttachToCustomSocket
  (params (SocketName :type Name))
  ;[1 1 1] Attach to custom socket
  (bind _ascharacter (Utilities|Casting|CastToCharacter (Components|GetOwner)))
  (bind _bodymesh (CallFunction|GetCharacterSkeleton _ascharacter))
  (Transformation|AttachComponentToComponent _bodymesh SocketName "KeepRelative" "KeepRelative" "KeepRelative" true))

(event Custom|InitializeClip%20-ALL
  (params (NewMesh :type Static%20Mesh%20Object%20Reference))
  ;[1 1 1] Handle Clip
  (Utilities|IsValid (Variables|Default|GetClip)
    (:Is%20Valid
      (Components|StaticMesh|SetStaticMesh (Variables|Default|GetClip) NewMesh)
      (Transformation|AttachComponentToComponent (Variables|Default|GetClip) (Variables|Default|GetSkeletalMesh) "Clip" "SnapToTarget" "SnapToTarget" "KeepRelative" true))))

(event Custom|UpdateCameraSettings
  (params (Transform :type Transform) (DOF :type S%20DOF%20Settings%20Structure) (InFieldOfView :type Float%20%28double-precision%29) (HasAdditionalScope :type Boolean))
  (bind (_aperturef_stop _focaldistance) (Utilities|Struct|BreakS_DOF_Settings DOF))
  ;[1 1 1] Update Camera Setttings
  (if HasAdditionalScope
    (Transformation|SetRelativeTransform (Variables|Default|GetAimCamera) Transform false true))
  (Utilities|Struct|SetmembersinPostProcessSettings (Variables|/Script/Engine.CameraComponent|GetPostProcessSettings (CallFunction|PGetActiveCamera)) _aperturef_stop _focaldistance)
  (Camera|SetFieldOfView (Variables|Default|GetAimCamera) InFieldOfView))

(event Custom|RemoveClipSM%20-%20All
  (bind _clip (Variables|Default|GetClip))
  ;[1 1 1] Handle Clip
  (Utilities|IsValid _clip
    (:Is%20Valid
      (Components|DestroyComponent _clip))))

(event Custom|RemoveClipSM%20-%20Server
  ;[1 1 1] Handle Clip
  (CallFunction|RemoveClipSM-All))

(event Custom|RemoveClip
  ;[1 1 1] Handle Clip
  (Networking|SwitchHasAuthority
    (:Authority
      (CallFunction|RemoveClipSM-All))
    (:Remote
      (CallFunction|RemoveClipSM-Server))))

(event Custom|SetMaterials
  (params (Array :type Array%20of%20Material%20Instance%20Object%20References))
  ;[1 1 1] Set Materials to All
  (for (_array_element _array_index) Array
    (Rendering|Material|SetMaterial (Variables|Default|GetSkeletalMesh) _array_index _array_element)))

(event Custom|ControlAim
  (params (TurnOn :type Boolean) (ModificationScope? :type Boolean) (AimBlendTime :type Float%20%28double-precision%29))
  ;[1 1 1] Zoom Process
  (if (not (not ModificationScope?))
    (CallFunction|SendMessagetoScopeModifications TurnOn AimBlendTime)))

(event Custom|AttachActor
  ;[1 1 1] Attach Process
  (bind _ascharacter (Utilities|Casting|CastToCharacter (Components|GetOwner)))
  (bind _bodymesh (CallFunction|GetCharacterSkeleton _ascharacter))
  (Transformation|AttachComponentToComponent _bodymesh (Variables|Default|GetSocket) "KeepRelative" "KeepRelative" "KeepRelative" true))

(event Custom|ControlLaser%20-%20ALL
  (params (bNewVisibility :type Boolean))
  ;[1 1 1] We decided not to replicate the laser because event tick + multiplayer is a very bad idea
  (bind _output_get (Variables|Default|SetbLaser (stale Custom|ControlLaserVisibility bNewVisibility)))
  (CallFunction|SendMessagetoLaserModifications _output_get))

(event Custom|ControlLaserVisibility
  (params (bNewVisibility :type Boolean))
  ;[1 1 1] We decided not to replicate the laser because event tick + multiplayer is a very bad idea
  (bind _output_get (Variables|Default|SetbLaser bNewVisibility))
  (CallFunction|SendMessagetoLaserModifications _output_get))

(event Custom|ControlLaser%20-%20Server
  (params (bNewVisibility :type Boolean))
  ;[1 1 1] We decided not to replicate the laser because event tick + multiplayer is a very bad idea
  (CallFunction|ControlLaser-ALL bNewVisibility))

(event Custom|TakeItem
  ;[1 1 1] Toggle Item
  (CallFunction|AttachtoCustomSocket (Variables|Default|GetSocket))
  (Variables|Default|SetItemRemoved true))

(event Custom|RemoveItem
  ;[1 1 1] Toggle Item
  (CallFunction|AttachtoCustomSocket (Variables|Default|GetBackSocket))
  (Variables|Default|SetItemRemoved false))

(event Custom|Detach%20-ALL
  ;[1 1 1] Detach
  (Transformation|DetachFromActor "KeepWorld" "KeepWorld" "KeepWorld")
  (Actor|DestroyActor))

(event Custom|InitialzieSockets
  (params (Socket :type Name) (BackSocket :type Name) (Type :type E_ItemType%20Enum :default "NewEnumerator0") (MaterialInstance :type Array%20of%20Material%20Instance%20Object%20References) (FirstTime :type Boolean))
  ;[1 1 1] Initialize Sockets
  (Variables|Default|SetSocket Socket)
  (Variables|Default|SetBackSocket BackSocket)
  (Variables|Default|SetType Type)
  (CallFunction|AttachActor)
  (Utilities|FlowControl|Delay (select FirstTime 2.0 0.0))
  (for (_array_element _array_index) MaterialInstance
    (Rendering|Material|SetMaterial (Variables|Default|GetSkeletalMesh) _array_index _array_element))
  (CallFunction|SetMaterials MaterialInstance))

(event Custom|Detach%20-Server
  ;[1 1 1] Detach
  (CallFunction|Detach-ALL))

(event Custom|InitializeClip%20-Server
  (params (NewMesh :type Static%20Mesh%20Object%20Reference))
  ;[1 1 1] Handle Clip
  (CallFunction|InitializeClip-ALL NewMesh))

(event Custom|Zoom
  (params (InFieldOfView :type Float%20%28double-precision%29) (ModificationScope? :type Boolean))
  ;[1 1 1] Zoom Process
  (if (not (not ModificationScope?))
    (CallFunction|SendMessagetoScopeModificationsZoom InFieldOfView)))

(event EventBeginPlay
  (bind _info (CallFunction|GetItemInfo))
  (bind _weapon_characteristics (Utilities|Struct|BreakS_Weapon _info))
  (bind _haslaser (Utilities|Struct|BreakS_WeaponCharacteristics _weapon_characteristics))
  ;[1 1 1] Begin play
  (Utilities|FlowControl|Sequence
    (:then_0
      (CallFunction|InitializeClip-Server (.Clip (Utilities|Struct|BreakS_Appearance (Utilities|Struct|BreakS_Weapon (CallFunction|GetItemInfo))))))
    (:then_1
      (Variables|Default|SetHasLaser _haslaser)
      (if (not _haslaser)
        (Components|DestroyComponent (Variables|Default|GetNS_Laser))))
    (:then_2
      (CallFunction|AttachActor))))

(fn ConstructionScript)

(fn GetUsedSceneComponent
  (return (Variables|Default|GetSkeletalMesh)))

(fn CheckState
  (bind _returnvalue (Components|GetOwner))
  (bind _returnvalue_2 (Actor|GetComponentbyClass _returnvalue "/Game/ModernRPG/General/Blueprints/ActorComponents/Character/State/AC_PlayerCurrentState.AC_PlayerCurrentState_C"))
  (bind _currentstate (Variables|/Game/ModernRPG/General/Blueprints/ActorComponents/Character/State/AC_PlayerCurrentState.AC_PlayerCurrentState_C|GetCurrentState _returnvalue_2))
  (Utilities|IsValid _returnvalue
    (:Is%20Valid
      (return (Math|Boolean|ORBoolean (== _currentstate (Utilities|Enum|LiteralenumE_WeaponState "NewEnumerator0")) (== _currentstate (Utilities|Enum|LiteralenumE_WeaponState "NewEnumerator2")) (== _currentstate (Utilities|Enum|LiteralenumE_WeaponState "NewEnumerator1")) (.BlockedWeapon (Default|GetBlockInformation (Actor|GetComponentbyClass (Components|GetOwner) "/Game/ModernRPG/General/Blueprints/ActorComponents/Weapon/AC_WeaponBlock.AC_WeaponBlock_C"))))))))

(fn GetLocationfromWeapon
  (bind _fromaimcamera (CallFunction|LaseratCenter))
  (bind _returnvalue (Components|GetOwner))
  (bind _returnvalue_2 (Components|GetOwner))
  (bind _returnvalue_3 (Components|GetOwner))
  (bind _returnvalue_4 (Components|GetOwner))
  (bind _ns_laser (Variables|Default|GetNS_Laser))
  (bind _returnvalue_5 (Actor|GetComponentbyClass _returnvalue_2 "/Script/Engine.CharacterMovementComponent"))
  (bind _returnvalue_6 (Actor|GetComponentbyClass _returnvalue_4 "/Game/ModernRPG/General/Blueprints/ActorComponents/Weapon/AC_Aiming.AC_Aiming_C"))
  (bind _returnvalue_7 (Actor|GetComponentbyClass _returnvalue_2 "/Game/ModernRPG/General/Blueprints/ActorComponents/Character/State/AC_PlayerCurrentState.AC_PlayerCurrentState_C"))
  (bind _returnvalue_8 (Actor|GetComponentbyClass _returnvalue "/Game/ModernRPG/General/Blueprints/ActorComponents/Weapon/AC_Weapon.AC_Weapon_C"))
  (bind _returnvalue_9 (Actor|GetComponentbyClass _returnvalue_3 "/Game/ModernRPG/General/Blueprints/ActorComponents/Weapon/AC_Weapon.AC_Weapon_C"))
  (bind _returnvalue_10 (Transformation|GetWorldLocation _ns_laser))
  (bind _returnvalue_11 (select _fromaimcamera "NewEnumerator0" "NewEnumerator1"))
  (bind (_startlocation _endlocation) (Default|LASERGetTraceVectors _returnvalue_8 _returnvalue_11))
  (bind (_startlocation_2 _endlocation_2) (Default|LASERGetTraceVectors _returnvalue_9 "NewEnumerator0"))
  (bind _currentstate (Variables|/Game/ModernRPG/General/Blueprints/ActorComponents/Character/State/AC_PlayerCurrentState.AC_PlayerCurrentState_C|GetCurrentState _returnvalue_7))
  (bind _movementmode (Variables|/Script/Engine.CharacterMovementComponent|GetMovementMode _returnvalue_5))
  (Utilities|IsValid _returnvalue_2
    (:Is%20Valid
      (Utilities|IsValid (Actor|GetComponentbyClass _returnvalue_2 "/Game/ModernRPG/General/Blueprints/ActorComponents/Weapon/AC_Aiming.AC_Aiming_C")
        (:Is%20Valid
          (Utilities|IsValid _returnvalue_7
            (:Is%20Valid
              (if (Math|Boolean|ANDBoolean (and (Utilities|Enum|NotEqual(Enum) _currentstate "NewEnumerator1") (Utilities|Enum|NotEqual(Enum) _currentstate "NewEnumerator2")) (Utilities|Enum|Equal(Enum) (Variables|/Game/ModernRPG/General/Blueprints/ActorComponents/SpeedChange/AC_SpeedChange.AC_SpeedChange_C|GetCurrentWalkState (Actor|GetComponentbyClass _returnvalue_2 "/Game/ModernRPG/General/Blueprints/ActorComponents/SpeedChange/AC_SpeedChange.AC_SpeedChange_C")) "NewEnumerator3") (Math|Boolean|ANDBoolean (Utilities|Enum|NotEqual(Enum) _movementmode "MOVE_Falling") (Utilities|Enum|NotEqual(Enum) _movementmode "MOVE_Swimming") (Utilities|Enum|NotEqual(Enum) _movementmode "MOVE_Flying")))
                (bind (_outhit _returnvalue_12) (Collision|LineTraceByChannel _startlocation _endlocation "TraceTypeQuery1" false (Utilities|Array|MakeArray self (Components|GetOwner)) "None" true "(R=0.069618,G=0.000000,B=1.000000,A=1.000000)" "(R=0.855045,G=1.000000,B=0.000000,A=1.000000)" 0.5))
                (if _returnvalue_12
                  (return _returnvalue_12 (.Location (Collision|BreakHitResult _outhit)) (.Location (Collision|BreakHitResult _outhit)))
                  (else
                    (return _returnvalue_12 (.TraceEnd (Collision|BreakHitResult _outhit)) (.TraceEnd (Collision|BreakHitResult _outhit)))))
                (else
                  (if (and (Default|Aiming? _returnvalue_6) (Default|Scopable _returnvalue_6))
                    _
                    (elif (and (Default|Aiming? (Actor|GetComponentbyClass (Components|GetOwner) "/Game/ModernRPG/General/Blueprints/ActorComponents/Weapon/AC_Aiming.AC_Aiming_C")) (not (Default|IsThirdPerson (Actor|GetComponentbyClass (Components|GetOwner) "/Game/ModernRPG/General/Blueprints/ActorComponents/Weapon/AC_Aiming.AC_Aiming_C"))))
                      _
                      (else
                        (bind (_outhit_2 _returnvalue_13) (Collision|LineTraceByChannel _returnvalue_10 (+ _returnvalue_10 (* (Math|Vector|GetRightVector _ns_laser) 10000)) "TraceTypeQuery1" false (Utilities|Array|MakeArray self (Components|GetOwner)) "None"))
                        (if _returnvalue_13
                          (return true (.Location (Collision|BreakHitResult _outhit_2)) (.Location (Collision|BreakHitResult _outhit_2)))
                          (else
                            (return true (.TraceEnd (Collision|BreakHitResult _outhit_2)) (.TraceEnd (Collision|BreakHitResult _outhit_2))))))))
                  (bind (_outhit_3 _returnvalue_14) (Collision|LineTraceByChannel _startlocation_2 _endlocation_2 "TraceTypeQuery1" false (Utilities|Array|MakeArray self (Components|GetOwner)) "None" true "(R=0.069618,G=0.000000,B=1.000000,A=1.000000)" "(R=0.855045,G=1.000000,B=0.000000,A=1.000000)" 0.5))
                  (if _returnvalue_14
                    (return _returnvalue_14 (.Location (Collision|BreakHitResult _outhit_3)) (.Location (Collision|BreakHitResult _outhit_3)))
                    (else
                      (return _returnvalue_14 (.TraceEnd (Collision|BreakHitResult _outhit_3)) (.TraceEnd (Collision|BreakHitResult _outhit_3))))))))))))))

(fn GetStart/End
  (bind _returnvalue (Components|GetOwner))
  (bind _returnvalue_2 (Actor|GetComponentbyClass _returnvalue "/Game/ModernRPG/General/Blueprints/ActorComponents/Weapon/AC_Aiming.AC_Aiming_C"))
  (bind _camera (Variables|/Game/ModernRPG/General/Blueprints/ActorComponents/Weapon/AC_Aiming.AC_Aiming_C|GetCamera _returnvalue_2))
  (bind _returnvalue_3 (Transformation|GetWorldLocation _camera))
  (Utilities|IsValid _returnvalue
    (:Is%20Valid
      (Utilities|IsValid _camera
        (:Is%20Valid
          (return _returnvalue_3 (+ _returnvalue_3 (* (Math|Vector|GetForwardVector _camera) 2e+04))))))))

(fn DebugLaser
  (Rendering|Debug|DrawDebugBox "0, 0, 0" "50.000000,50.000000,50.000000" "(R=1.000000,G=0.130695,B=0.000000,A=1.000000)" "0, 0, 0" 0.0 0.0)
  (Rendering|Debug|DrawDebugBox (Transformation|GetWorldLocation (Variables|Default|GetNS_Laser)) "50.000000,50.000000,50.000000" "(R=1.000000,G=0.130695,B=0.000000,A=1.000000)" "0, 0, 0" 0.0 0.0))

(fn GetItemInfo
  (return (Variables|Default|GetInfo)))

(fn PGetActiveCamera
  (return (Variables|Default|GetAimCamera)))

(fn GetSKtoHide
  (bind _bodyskeletal (Class|BPIAI|GetBody(Message) (Components|GetOwner)))
  (return (Variables|Default|GetSkeletalMesh) _bodyskeletal))

(fn ControlLaser
  (bind (_block _returnvalue _location) (CallFunction|GetLocationfromWeapon))
  (if (Variables|Default|GetHasLaser)
    (return _block _returnvalue _location)))

(fn CreateRT
  (params (Target :type Scene%20Capture%20Component%202D%20Object%20Reference))
  (Utilities|IsValid Target
    (:Is%20Valid
      (bind _returnvalue (Rendering|CreateRenderTarget2D 1300 1300 "RTF_RGBA16f"))
      (bind _output_get (Variables|/Script/Engine.SceneCaptureComponent2D|SetTextureTarget Target _returnvalue))
      (Utilities|IsValid (Variables|Default|GetDynamicMaterial)
        (:Is%20Valid
          (Rendering|Material|SetTextureParameterValue (Variables|Default|GetDynamicMaterial) "Render" (Variables|/Script/Engine.SceneCaptureComponent2D|GetTextureTarget Target))
          (return))
        (:Is%20Not%20Valid
          (bind _returnvalue_2 (Rendering|Material|CreateDynamicMaterialInstance "/Game/ModernRPG/Shooter/Materials/Combat/Aim/Scope/MI_RT_Scope.MI_RT_Scope" "None" "None" :!class /Script/Engine.KismetMaterialLibrary))
          (Variables|Default|SetDynamicMaterial _returnvalue_2)
          (Rendering|Material|SetTextureParameterValue (Variables|Default|GetDynamicMaterial) "Render" _output_get)
          (return))))
    (:Is%20Not%20Valid
      (return))))

(fn SendMessagetoScopeModifications
  (params (Start :type Boolean) (AimBlendTime :type Float%20%28double-precision%29))
  (for _array_element (Variables|/Game/ModernRPG/General/Blueprints/ActorComponents/InteractActors/AC_EquipmentHandler.AC_EquipmentHandler_C|GetINV_Equipment (Actor|GetComponentbyClass (Components|GetOwner) "/Game/ModernRPG/General/Blueprints/ActorComponents/InteractActors/AC_EquipmentHandler.AC_EquipmentHandler_C"))
    (for _array_element_2 (Utilities|Struct|BreakS_InvItemDyn _array_element)
      (Class|BPIComponents|AimControl(Message) (.Actor (Utilities|Struct|BreakS_ModificationDynamic _array_element_2)) Start AimBlendTime)))
  (return))

(fn SendMessagetoScopeModificationsZoom
  (params (NewParam :type Float%20%28double-precision%29))
  (for _array_element (Variables|/Game/ModernRPG/General/Blueprints/ActorComponents/InteractActors/AC_EquipmentHandler.AC_EquipmentHandler_C|GetINV_Equipment (Actor|GetComponentbyClass (Components|GetOwner) "/Game/ModernRPG/General/Blueprints/ActorComponents/InteractActors/AC_EquipmentHandler.AC_EquipmentHandler_C"))
    (for _array_element_2 (Utilities|Struct|BreakS_InvItemDyn _array_element)
      (Utilities|IsValid (Utilities|Struct|BreakS_ModificationDynamic _array_element_2)
        (:Is%20Valid
          (Default|ZoomControl (Utilities|Struct|BreakS_ModificationDynamic _array_element_2) NewParam)))))
  (return))

(fn LaseratCenter
  (if (Default|Aiming? (Actor|GetComponentbyClass (Components|GetOwner) "/Game/ModernRPG/General/Blueprints/ActorComponents/Weapon/AC_Aiming.AC_Aiming_C"))
    (if (Default|IsThirdPerson (Actor|GetComponentbyClass (Components|GetOwner) "/Game/ModernRPG/General/Blueprints/ActorComponents/Weapon/AC_Aiming.AC_Aiming_C"))
      (if (Default|Scopable (Actor|GetComponentbyClass (Components|GetOwner) "/Game/ModernRPG/General/Blueprints/ActorComponents/Weapon/AC_Aiming.AC_Aiming_C"))
        (return true)
        (else
          (return false)))
      (else
        (return true)))
    (else
      (return false))))

(fn SendMessagetoLaserModifications
  (params (Start :type Boolean))
  (bind _returnvalue (Components|GetOwner))
  (bind _returnvalue_2 (Actor|GetComponentbyClass _returnvalue "/Game/ModernRPG/General/Blueprints/ActorComponents/InteractActors/AC_EquipmentHandler.AC_EquipmentHandler_C"))
  (bind _inv_equipment (Variables|/Game/ModernRPG/General/Blueprints/ActorComponents/InteractActors/AC_EquipmentHandler.AC_EquipmentHandler_C|GetINV_Equipment _returnvalue_2))
  (if (> (Utilities|Array|Length _inv_equipment) 0)
    (for _array_element _inv_equipment
      (for _array_element_2 (Utilities|Struct|BreakS_InvItemDyn _array_element)
        (Utilities|IsValid (.Actor (Utilities|Struct|BreakS_ModificationDynamic _array_element_2))
          (:Is%20Valid
            (Default|LaserControl (.Actor (Utilities|Struct|BreakS_ModificationDynamic _array_element_2)) Start)))))
    (return)))