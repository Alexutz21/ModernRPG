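; BP_SimpleAttach is a simple weapon-system attachment that shows a static or skeletal mesh on a socket of its owning character.
; Initialize stores the socket and static mesh, then applies both supplied meshes to its mesh components.
; If the owner is a Character, it looks up the character skeleton and attaches to the body mesh at that socket, keeping relative transforms.
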(event Custom|Initialize
  (params (Socket :type Name) (NewStaticMesh :type Static%20Mesh%20Object%20Reference) (Skeletal%20Mesh :type Skeletal%20Mesh%20Object%20Reference))
  (Variables|Settings|SetSocket Socket)
  (bind _output_get (Variables|Default|SetNewStaticMesh NewStaticMesh))
  (Components|StaticMesh|SetStaticMesh (Variables|Default|GetStaticMesh) _output_get)
  (Class|SkinnedMeshComponent|SetSkeletalMesh (Variables|Default|GetSkeletalMesh) Skeletal%20Mesh true)
  (bind _ascharacter (Utilities|Casting|CastToCharacter (Components|GetOwner)))
  (bind _bodymesh (CallFunction|GetCharacterSkeleton _ascharacter))
  (Transformation|AttachComponentToComponent _bodymesh (Variables|Settings|GetSocket) "KeepRelative" "KeepRelative" "KeepRelative" true))

(event EventBeginPlay)

(fn ConstructionScript)