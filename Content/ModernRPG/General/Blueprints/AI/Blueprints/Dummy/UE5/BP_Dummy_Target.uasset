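; BP_Dummy_Target is a UE5 dummy AI character, apparently a practice target, built on a parent AI Blueprint.
; It hides the inherited Stats component at BeginPlay and overrides the behavior and target-selection events with empty bodies, so it adds no AI logic.
; The construction script applies two mesh materials, while overrides report it as AI and return a fixed skeleton type.
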(event EventSetBehavior
  (params (State :type E_StateAI%20Enum :default "NewEnumerator0"))
  ;[1 1 1] Initialzie
)

(event EventBeginPlay
  (bind _stats (Variables|Default|GetStats))
  ;[1 1 1] Initialzie
  (|CallParentFunction)
  (Rendering|SetVisibility _stats false false)
  (Development|SetHiddeninGame _stats true false))

(event EventSetNewTarget
  (params (Target :type Actor%20Object%20Reference) (Stimulus :type AI%20Stimulus%20Structure))
  ;[1 1 1] Initialzie
)

(fn ConstructionScript
  (|CallParentFunction)
  (Rendering|Material|SetMaterial (Variables|Character|GetMesh) 0 (Utilities|Array|Get(acopy) (Variables|Settings|GetMaterials)))
  (Rendering|Material|SetMaterial (Variables|Character|GetMesh) 1 (Utilities|Array|Get(acopy) (Variables|Settings|GetMaterials) 1)))

(fn IsAI
  (return true))

(fn IsUsingAlternativeSkeleton?
  (return "NewEnumerator0"))