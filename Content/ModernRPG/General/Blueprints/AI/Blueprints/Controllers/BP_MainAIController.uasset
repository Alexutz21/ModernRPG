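; Main AI controller that relays perception events to its pawn and re-evaluates the pawn's current target.
; Perception memory is cleared shortly after BeginPlay, then updates reach living pawns as new-target messages through interface calls.
; CheckTarget reads the blackboard target, removing it if dead.
; If the living target's first stimulus is successfully sensed, a retriggerable SenseTime delay precedes a behavior change.
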(event OnTargetPerceptionUpdated(AIPerception)
  (params (Actor :type Actor%20Object%20Reference) (Stimulus :type AI%20Stimulus%20Structure))
  (bind _returnvalue (Pawn|GetControlledPawn))
  ;[1 1 1] Perveption Update
  (bind _result (Class|BPICharacter|IsAlive?(Message) _returnvalue))
  (if _result
    (Class|BPIAI|SetNewTarget(Message) _returnvalue Actor Stimulus)))

(event Custom|CheckTarget
  (bind _self self)
  (bind _returnvalue (AI|GetBlackboard _self))
  ;[1 1 1] Remove target is sense time is over
  (Utilities|IsValid _returnvalue
    (:Is%20Valid
      (bind _asactor (Utilities|Casting|CastToActor (AI|Components|Blackboard|GetValueasObject _returnvalue (Variables|Default|GetTarget))))
      (if (Utilities|DoesObjectImplementInterface _asactor "/Game/ModernRPG/General/Blueprints/Interfaces/BP_I_Character.BP_I_Character_C")
        (bind _result (Class|BPICharacter|IsAlive?(Message) _asactor))
        (if _result
          (bind _info (Class|AIPerceptionComponent|GetActorsPerception (Variables|Default|GetAIPerception) _asactor))
          (if (.bSuccessfullySensed (Utilities|Struct|BreakAIStimulus (Utilities|Array|Get(acopy) (.LastSensedStimuli (Utilities|Struct|BreakActorPerceptionBlueprintInfo _info)))))
            (Utilities|FlowControl|RetriggerableDelay (Variables|Default|GetSenseTime))
            (Class|BPIAI|SetBehavior(Message) (Pawn|GetControlledPawn) "NewEnumerator11"))
          (else
            (Class|BPIAI|RemoveTarget(Message) (Pawn|GetControlledPawn))))))))

(event EventBeginPlay
  ;[1 1 1] Activate perception after BT spawn
  (Utilities|FlowControl|Delay 3.0)
  (Class|AIPerceptionComponent|ForgetAll (Variables|Default|GetAIPerception)))

(fn ConstructionScript)