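; BP_Projectile is a projectile actor from the AI folder that damages living characters it touches.
; On sphere overlap it casts to Character, accepts only capsule component overlaps, and checks IsAliveMessage before applying Damage and destroying itself.
; Any blocking hit on the sphere also destroys the projectile without dealing damage.
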(event OnComponentHit(Sphere)
  (params (HitComponent :type Primitive%20Component%20Object%20Reference) (OtherActor :type Actor%20Object%20Reference) (OtherComp :type Primitive%20Component%20Object%20Reference) (NormalImpulse :type Vector :default "0, 0, 0") (Hit :type Hit%20Result%20Structure%20%28by%20ref%29))
  ;[1 1 1] On actor overlapped by something
  (Actor|DestroyActor))

(event OnComponentBeginOverlap(Sphere)
  (params (OverlappedComponent :type Primitive%20Component%20Object%20Reference) (OtherActor :type Actor%20Object%20Reference) (OtherComp :type Primitive%20Component%20Object%20Reference) (OtherBodyIndex :type Integer) (bFromSweep :type Boolean) (SweepResult :type Hit%20Result%20Structure%20%28by%20ref%29))
  ;[1 1 1] On actor overlapped by something
  (bind _ascharacter (Utilities|Casting|CastToCharacter OtherActor))
  (if (== OtherComp (Variables|/Script/Engine.Character|GetCapsuleComponent _ascharacter))
    (bind _result (Class|BPICharacter|IsAlive?(Message) _ascharacter))
    (if _result
      (Game|Damage|ApplyDamage _ascharacter (Variables|Default|GetDamage) 0 0)
      (Actor|DestroyActor))))

(fn ConstructionScript)