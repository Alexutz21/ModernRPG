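; Explosive barrel actor with a configurable mesh that blows up once upon receiving any, point or radial damage.
; The explosion routes through server and all-client events, with player 0's character set as owner on BeginPlay.
; It hides the mesh, applies full grenade-type radial damage and plays camera shake, Niagara and sound effects.
; After a short delay, it adds a radial force component, fires an impulse and destroys itself.
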(event Custom|Explode
  ;[1 1 1] Replicate Explosion Event
  (Utilities|FlowControl|DoOnce false
    (:Completed
      (CallFunction|Explode-Server))))

(event Custom|Explode%20-Server
  ;[1 1 1] Replicate Explosion Event
  (CallFunction|Explode-ALL))

(event Custom|Explode%20-ALL
  ;[1 1 1] Explode Event
  (Rendering|SetVisibility (Variables|Components|GetStaticMesh) false false)
  (Game|Damage|ApplyRadialDamage (Variables|Settings|GetDamage) (+ (Transformation|GetActorLocation) "0, 0,50.000000") (Variables|Settings|GetRadius) "/Game/ModernRPG/General/Blueprints/DamageTypes/BPDT_Grenade.BPDT_Grenade_C" 0 self (Game|GetPlayerController 0) true "ECC_WorldStatic")
  (Camera|PlayWorldCameraShake (Variables|Settings|GetCameraShake) (Transformation|GetActorLocation) 0.0 4e+03 1e+01)
  (Niagara|SpawnSystematLocation (Variables|Settings|GetNiagaraSystemExplosion) (Transformation|GetActorLocation))
  (Audio|PlaySoundatLocation (Variables|Settings|GetExplosionSound) (Transformation|GetActorLocation) "0, 0, 0" 1.0 1.0 0.0 0 0 0 0)
  (Utilities|FlowControl|Delay 0.15)
  (CallFunction|DestroyBarrel))

(event Custom|DestroyBarrel
  ;[1 1 1] Destroy
  (bind _returnvalue (AddComponent|AddRadialForceComponent false))
  (bind _output_get (Variables|Default|Setforce _returnvalue))
  (Utilities|IsValid _output_get
    (:Is%20Valid
      (Class|RadialForceComponent|FireImpulse (Variables|Default|Getforce)))
    (:Is%20Not%20Valid
      _))
  (Actor|DestroyActor)
  (Variables|Default|SetDestroyed true))

(event EventBeginPlay
  ;[1 1 1] Set server as owner
  (Actor|SetOwner (Game|GetPlayerCharacter 0)))

(event Game|Damage|EventPointDamage
  (params (Damage :type Float%20%28single-precision%29) (DamageType :type Damage%20Type%20Object%20Reference) (HitLocation :type Vector :default "0, 0, 0") (HitNormal :type Vector :default "0, 0, 0") (HitComponent :type Primitive%20Component%20Object%20Reference) (BoneName :type Name :default "None") (ShotFromDirection :type Vector :default "0, 0, 0") (InstigatedBy :type Controller%20Object%20Reference) (DamageCauser :type Actor%20Object%20Reference) (HitInfo :type Hit%20Result%20Structure%20%28by%20ref%29))
  ;[1 1 1] Explode on getting any damage
  (CallFunction|Explode))

(event Game|Damage|EventAnyDamage
  (params (Damage :type Float%20%28single-precision%29) (DamageType :type Damage%20Type%20Object%20Reference) (InstigatedBy :type Controller%20Object%20Reference) (DamageCauser :type Actor%20Object%20Reference))
  ;[1 1 1] Explode on getting any damage
  (CallFunction|Explode))

(event Game|Damage|EventRadialDamage
  (params (DamageReceived :type Float%20%28single-precision%29) (DamageType :type Damage%20Type%20Object%20Reference) (Origin :type Vector :default "0, 0, 0") (HitInfo :type Hit%20Result%20Structure%20%28by%20ref%29) (InstigatedBy :type Controller%20Object%20Reference) (DamageCauser :type Actor%20Object%20Reference))
  ;[1 1 1] Explode on getting any damage
  (CallFunction|Explode))

(fn ConstructionScript
  (Components|StaticMesh|SetStaticMesh (Variables|Components|GetStaticMesh) (Variables|Settings|GetMesh)))