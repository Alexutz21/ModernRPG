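; BP_Spawner is an enemy spawner that releases endless timed waves, starting on BeginPlay.
; Each wave has its own delay and list of enemy classes, read from EnemiesInformation by the current wave index.
; A one-shot timer spawns each listed enemy at a random navigable point within the Sphere's radius, then advances the wave and re-arms.
; The index is clamped, so the last entry repeats indefinitely.
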(event Custom|SpawnWave
  (bind _sphere (Variables|Default|GetSphere))
  (for _array_element (.enemeis (CallFunction|GetEnemiesInfo))
    (Game|SpawnActorfromClass _array_element (Math|Conversions|ToTransform(Vector) (.RandomLocation (Class|NavigationSystemV1|GetRandomPointinNavigableRadius (Transformation|GetWorldLocation _sphere) (Components|Sphere|GetScaledSphereRadius _sphere) 0 0))) "Undefined" 0 0))
  (Math|Integer|IncrementInt (Variables|Default|GetCurrentWave)
    (:%20%20
      (CallFunction|SpawnEnemeis))))

(event Custom|SpawnEnemeis
  (Utilities|Time|SetTimerbyEvent (delegate Custom|SpawnWave) (.spawndelay (CallFunction|GetEnemiesInfo))))

(event EventBeginPlay
  (CallFunction|SpawnEnemeis))

(fn ConstructionScript)

(fn GetEnemiesInfo
  (bind _enemiesinformation (Variables|Default|GetEnemiesInformation))
  (return (Utilities|Array|Get(acopy) _enemiesinformation (Math|Integer|Clamp(Integer) (Variables|Default|GetCurrentWave) 0 (Utilities|Array|LastIndex _enemiesinformation)))))