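; Actor component that manages quick-use slots for consumables (heal, food, water), tracking assigned inventory items and mirroring them in main UI widgets.
; Using an item applies an instant stat change or queues a regeneration slot, then removes one from inventory.
; A server-to-all montage uses notifies to attach a prop, play sound and destroy the prop.
; Slots save to a BP_SaveUsables save game and reload after a delayed BeginPlay.
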(event Custom|ReplicateSound%20-ALL
  (params (Sound :type Sound%20Base%20Object%20Reference) (Location :type Vector))
  ;[1 1 1] Play Replicated Eat Sound
  (Audio|PlaySoundatLocation Sound Location "0, 0, 0" 1.0 1.0 0.0 0 0 0 0))

(event Custom|SetUsableItem
  (params (InventorySlot :type WB%20Inventory%20Slot%20Object%20Reference) (Index :type Integer) (InventoryWidget :type WB%20Inventory%20Object%20Reference))
  (bind _item2 (Variables|/Game/ModernRPG/General/GUI/Widgets/Inventory/InventorySlot/WB_InventorySlot.WB_InventorySlot_C|GetItem2 InventorySlot))
  (bind _row (Utilities|Struct|BreakS_InvItemDyn _item2))
  (bind _armor (CallFunction|GetUsableInfo _row))
  (bind _type (Utilities|Struct|BreakS_UsableItem _armor))
  ;[1 1 1] Initialize Usable Item in Menu
  (CallFunction|RemoveUsableType _type)
  (bind _returnvalue (Utilities|Array|Add (Variables|Default|GetUsables) (Utilities|Struct|MakeS_SaveUsables (Variables|/Game/ModernRPG/General/GUI/Widgets/Inventory/WB_Inventory.WB_Inventory_C|GetCurrentInventory InventoryWidget) Index _type)))
  (Default|InitialzieUsable (Default|GetUsableWidget (Variables|Default|GetMainUI) (CallFunction|TranslateUsable _type)) _item2 Index InventoryWidget InventorySlot (.RowName (Utilities|Struct|BreakDataTableRowHandle _row)) _returnvalue))

(event Custom|UseItemFromInventory
  (params (Type :type WB%20Inventory%20Slot%20Object%20Reference) (Item :type S%20Inv%20Item%20Dyn%20Structure%20%28by%20ref%29) (InputPin :type Integer) (Target :type WB%20Inventory%20Object%20Reference))
  (bind _currentinventory (Variables|/Game/ModernRPG/General/GUI/Widgets/Inventory/WB_Inventory.WB_Inventory_C|GetCurrentInventory Target))
  ;[1 1 1] Remove Item From Inventory On Used
  (CallFunction|OnItemUsed Item)
  (Variables|Default|SetDeleteUsableType (.Type (Utilities|Struct|BreakS_UsableItem (CallFunction|GetUsableInfo (.Row (Utilities|Struct|BreakS_InvItemDyn Item))))))
  (if (<= (.Amount (Utilities|Struct|BreakS_InvItemDyn (Utilities|Array|Get(acopy) (Variables|/Game/ModernRPG/General/Blueprints/ActorComponents/Character/Inventory/AC_Inventory.AC_Inventory_C|GetInventory _currentinventory) InputPin))) 1)
    (CallFunction|RemoveUsableType (Variables|Default|GetDeleteUsableType)))
  (Default|RemoveItem _currentinventory InputPin 1))

(event Custom|ReplicateSound
  (params (Sound :type Sound%20Base%20Object%20Reference) (Location :type Vector))
  ;[1 1 1] Play Replicated Eat Sound
  (if (Ability|HasAuthority (Components|GetOwner))
    (CallFunction|ReplicateSound-ALL Sound Location)
    (else
      (CallFunction|ReplicateSound-Server Sound Location))))

(event Custom|ReplicateSound%20-Server
  (params (Sound :type Sound%20Base%20Object%20Reference) (Location :type Vector))
  ;[1 1 1] Play Replicated Eat Sound
  (CallFunction|ReplicateSound-ALL Sound Location))

(event Custom|PlayMontage%20-%20Server
  (params (MontageToPlay :type Anim%20Montage%20Object%20Reference) (Sound :type Sound%20Base%20Object%20Reference) (Actor :type Actor%20Class%20Reference) (SocketName :type Name))
  ;[1 1 1] On used - Play montage
  (CallFunction|PlayMontage-ALL MontageToPlay Sound Actor SocketName))

(event Custom|UseItem
  (params (Type :type E_UsableType%20Enum :default "NewEnumerator0"))
  (bind _mainui (Variables|Default|GetMainUI))
  (bind _array_element (Default|GetUsableWidget _mainui Type))
  (bind _inventorywidget (Variables|/Game/ModernRPG/General/GUI/Widgets/Inventory/QuickUse/WB_QuickUse.WB_QuickUse_C|GetInventoryWidget _array_element))
  (bind _index (Variables|/Game/ModernRPG/General/GUI/Widgets/Inventory/QuickUse/WB_QuickUse.WB_QuickUse_C|GetIndex _array_element))
  (bind _item (Variables|/Game/ModernRPG/General/GUI/Widgets/Inventory/QuickUse/WB_QuickUse.WB_QuickUse_C|GetItem _array_element))
  (bind _currentinventory (Variables|/Game/ModernRPG/General/GUI/Widgets/Inventory/WB_Inventory.WB_Inventory_C|GetCurrentInventory _inventorywidget))
  ;[1 1 1] Use Item
  (Utilities|IsValid _array_element
    (:Is%20Valid
      (if (Variables|/Game/ModernRPG/General/GUI/Widgets/Inventory/QuickUse/WB_QuickUse.WB_QuickUse_C|GetAvailable _array_element)
        (Utilities|IsValid _inventorywidget
          (:Is%20Valid
            (Variables|Default|SetDeleteUsableType (.Type (Utilities|Struct|BreakS_UsableItem (CallFunction|GetUsableInfo (.Row (Utilities|Struct|BreakS_InvItemDyn _item))))))
            (CallFunction|OnItemUsed _item)
            (Utilities|IsValid _currentinventory
              (:Is%20Valid
                (if (<= (.Amount (Utilities|Struct|BreakS_InvItemDyn (Utilities|Array|Get(acopy) (Variables|/Game/ModernRPG/General/Blueprints/ActorComponents/Character/Inventory/AC_Inventory.AC_Inventory_C|GetInventory _currentinventory) _index))) 1)
                  (CallFunction|RemoveUsableType (Variables|Default|GetDeleteUsableType)))
                (bind _removed_all (Default|RemoveItem _currentinventory _index 1))
                (if (not _removed_all)
                  (Default|RemoveOne _array_element))))))))))

(event Custom|PlayMontage%20-%20ALL
  (params (MontageToPlay :type Anim%20Montage%20Object%20Reference) (Sound :type Sound%20Base%20Object%20Reference) (Actor :type Actor%20Class%20Reference) (SocketName :type Name))
  ;[1 1 1] On used - Play montage
  (bind _defaultbodymesh (Class|BPIAI|GetDemoSkeletalMeshes(Message) (Components|GetOwner)))
  (bind _notifyname (Animation|Montage|PlayMontage _defaultbodymesh MontageToPlay)
    (:OnNotifyBegin
      (CallFunction|PassEvent _notifyname Sound Actor SocketName))))

(event EventBeginPlay
  ;[1 1 1] Initialize Component
  (Utilities|FlowControl|Delay 3.0)
  (Variables|Default|SetMainUI (Variables|/Game/ModernRPG/General/Blueprints/DialoguesQuests/WidgetHandler/AC_MainWidgetHandler.AC_MainWidgetHandler_C|GetCastedMainUI (Actor|GetComponentbyClass (Components|GetOwner) "/Game/ModernRPG/General/Blueprints/DialoguesQuests/WidgetHandler/AC_MainWidgetHandler.AC_MainWidgetHandler_C")))
  (Utilities|FlowControl|Delay 0.2)
  (CallFunction|LoadUsable))

(fn OnItemUsed
  (params (Item :type S%20Inv%20Item%20Dyn%20Structure%20%28by%20ref%29))
  (bind _row (Utilities|Struct|BreakS_InvItemDyn Item))
  (bind _returnvalue (Components|GetOwner))
  (bind _row_2 (Utilities|Struct|BreakS_InvItemDyn Item))
  (bind _row_3 (Utilities|Struct|BreakS_InvItemDyn Item))
  (bind _armor (CallFunction|GetUsableInfo _row))
  (bind (_type _usetype _value) (Utilities|Struct|BreakS_UsableItem _armor))
  (bind _out_row (CallFunction|GetItemInfo _row_3))
  (bind _armor_2 (CallFunction|GetUsableInfo _row_2))
  (bind (_actortoconnect _sockets) (Utilities|Struct|BreakS_InventoryItem _out_row))
  (bind (_usesound _usemontage) (Utilities|Struct|BreakS_UsableItem _armor_2))
  (bind _component (CallFunction|GetCharacteristicbyType _returnvalue _type))
  (Utilities|FlowControl|Sequence
    (:then_0
      (switch Utilities|FlowControl|Switch|SwitchonE_UseType _usetype
        (:NewEnumerator0
          (Default|AddRegenerationSlot (Variables|/Game/ModernRPG/General/GUI/Widgets/WB_MainUI.WB_MainUI_C|GetWB_UsableBar (Variables|Default|GetMainUI)) (.Texture (Utilities|Struct|BreakS_InventorySlot (.InvTexture (Utilities|Struct|BreakS_InventoryItem (CallFunction|GetItemInfo _row))))) (CallFunction|GetUsableInfo (Utilities|Struct|BreakS_InvItemDyn Item)) _component))
        (:NewEnumerator1
          (Default|ModifyStat _component _value true))))
    (:then_1
      (Utilities|IsValid _usemontage
        (:Is%20Valid
          (CallFunction|PlayMontage-Server _usemontage _usesound _actortoconnect (Utilities|Struct|BreakS_ItemSockets _sockets)))))))

(fn SaveUsable
  (bind _returnvalue (SaveGame|DoesSaveGameExist (Variables|Default|GetUsable)))
  (if _returnvalue
    (bind _returnvalue_2 (SaveGame|LoadGamefromSlot (Variables|Default|GetUsable)))
    (bind _asbp_save_usables (Utilities|Casting|CastToBP_SaveUsables _returnvalue_2))
    (LocalVariables|SetSaveGame _asbp_save_usables)
    (else
      (bind _returnvalue_3 (SaveGame|CreateSaveGameObject "/Game/ModernRPG/General/Blueprints/UsableItems/Save/BP_SaveUsables.BP_SaveUsables_C"))
      (LocalVariables|SetSaveGame _returnvalue_3)))
  (Variables|/Game/ModernRPG/General/Blueprints/UsableItems/Save/BP_SaveUsables.BP_SaveUsables_C|SetCurrentUsables (LocalVariables|GetSaveGame) (Variables|Default|GetUsables))
  (SaveGame|SaveGametoSlot (LocalVariables|GetSaveGame) (Variables|Default|GetUsable)))

(fn LoadUsable
  (bind _returnvalue (SaveGame|DoesSaveGameExist (Variables|Default|GetUsable)))
  (if _returnvalue
    (bind _returnvalue_2 (SaveGame|LoadGamefromSlot (Variables|Default|GetUsable)))
    (bind _asbp_save_usables (Utilities|Casting|CastToBP_SaveUsables _returnvalue_2))
    (Variables|Default|SetUsables (Variables|/Game/ModernRPG/General/Blueprints/UsableItems/Save/BP_SaveUsables.BP_SaveUsables_C|GetCurrentUsables _asbp_save_usables))
    (for _array_element (Variables|/Game/ModernRPG/General/Blueprints/UsableItems/Save/BP_SaveUsables.BP_SaveUsables_C|GetCurrentUsables _asbp_save_usables)
      (LocalVariables|SetL_SaveUsableCur _array_element)
      (Utilities|IsValid (.Inventory (Utilities|Struct|BreakS_SaveUsables _array_element))
        (:Is%20Valid
          (Utilities|IsValid (Variables|/Game/ModernRPG/General/Blueprints/ActorComponents/Character/Inventory/AC_Inventory.AC_Inventory_C|GetInventoryWidget (.Inventory (Utilities|Struct|BreakS_SaveUsables (LocalVariables|GetL_SaveUsableCur))))
            (:Is%20Valid
              (Default|InitialzieUsable (Default|GetUsableWidget (Variables|Default|GetMainUI) (Utilities|Select :Index (.Type (Utilities|Struct|BreakS_UsableItem (CallFunction|GetUsableInfo (.Row (Utilities|Struct|BreakS_InvItemDyn (Utilities|Array|Get(acopy) (Variables|/Game/ModernRPG/General/Blueprints/ActorComponents/Character/Inventory/AC_Inventory.AC_Inventory_C|GetInventory (.Inventory (Utilities|Struct|BreakS_SaveUsables _array_element))) (.Index (Utilities|Struct|BreakS_SaveUsables _array_element)))))))) :NewEnumerator1 "NewEnumerator0" :NewEnumerator2 "NewEnumerator0" :NewEnumerator3 "NewEnumerator1" :NewEnumerator15 "NewEnumerator2")) (Utilities|Array|Get(acopy) (Variables|/Game/ModernRPG/General/Blueprints/ActorComponents/Character/Inventory/AC_Inventory.AC_Inventory_C|GetInventory (.Inventory (Utilities|Struct|BreakS_SaveUsables (LocalVariables|GetL_SaveUsableCur)))) (.Index (Utilities|Struct|BreakS_SaveUsables (LocalVariables|GetL_SaveUsableCur)))) (.Index (Utilities|Struct|BreakS_SaveUsables (LocalVariables|GetL_SaveUsableCur))) (Variables|/Game/ModernRPG/General/Blueprints/ActorComponents/Character/Inventory/AC_Inventory.AC_Inventory_C|GetInventoryWidget (.Inventory (Utilities|Struct|BreakS_SaveUsables (LocalVariables|GetL_SaveUsableCur)))) (Default|FindIndexSlot (Variables|/Game/ModernRPG/General/Blueprints/ActorComponents/Character/Inventory/AC_Inventory.AC_Inventory_C|GetInventoryWidget (.Inventory (Utilities|Struct|BreakS_SaveUsables (LocalVariables|GetL_SaveUsableCur)))) (.Index (Utilities|Struct|BreakS_SaveUsables (LocalVariables|GetL_SaveUsableCur)))) "None"))))))))

(fn RemoveUsableSlot
  (params (InputPin :type AC%20Inventory%20Object%20Reference))
  (for (_array_element _array_index) (Variables|Default|GetUsables)
    (if (== (.Inventory (Utilities|Struct|BreakS_SaveUsables _array_element)) InputPin)
      (Utilities|Array|RemoveIndex (Variables|Default|GetUsables) _array_index))))

(fn TranslateUsable
  (params (Index :type E_StatType%20Enum :default "NewEnumerator1"))
  (return (Utilities|Select :Index Index :NewEnumerator1 "NewEnumerator0" :NewEnumerator2 "NewEnumerator0" :NewEnumerator3 "NewEnumerator1" :NewEnumerator15 "NewEnumerator2")))

(fn RemoveUsableType
  (params (InputPin :type E_StatType%20Enum :default "NewEnumerator1"))
  (for (_array_element _array_index) (Variables|Default|GetUsables)
    (if (Utilities|Enum|Equal(Enum) (.Type (Utilities|Struct|BreakS_UsableItem (CallFunction|GetUsableInfo (.Row (Utilities|Struct|BreakS_InvItemDyn (Utilities|Array|Get(acopy) (Variables|/Game/ModernRPG/General/Blueprints/ActorComponents/Character/Inventory/AC_Inventory.AC_Inventory_C|GetInventory (.Inventory (Utilities|Struct|BreakS_SaveUsables _array_element))) (.Index (Utilities|Struct|BreakS_SaveUsables _array_element)))))))) InputPin)
      (Utilities|Array|RemoveIndex (Variables|Default|GetUsables) _array_index)
      (return))))

(fn TranslateSlot
  (params (In :type E_UsableType%20Enum :default "NewEnumerator0"))
  (return (Utilities|Select :Index In :NewEnumerator0 "NewEnumerator1" :NewEnumerator1 "NewEnumerator3" :NewEnumerator2 "NewEnumerator15")))

(fn UpdateIndex
  (params (NewIndex :type Integer) (Type :type E_UsableType%20Enum :default "NewEnumerator0"))
  (for (_array_element _array_index) (Variables|Default|GetUsables)
    (bind _output_get (LocalVariables|SetTempItem _array_element))
    (if (Utilities|Enum|Equal(Enum) (.Type (Utilities|Struct|BreakS_SaveUsables _output_get)) (CallFunction|TranslateSlot Type))
      (Utilities|Struct|SetmembersinS_SaveUsables (LocalVariables|GetTempItem) NewIndex)
      (Utilities|Array|SetArrayElem (Variables|Default|GetUsables) _array_index (LocalVariables|GetTempItem)))))

(fn RemoveItem
  (params (Type :type E_UsableType%20Enum :default "NewEnumerator0"))
  (for (_array_element _array_index) (Variables|Default|GetUsables)
    (bind _output_get (LocalVariables|SetTempItem _array_element))
    (if (Utilities|Enum|Equal(Enum) (.Type (Utilities|Struct|BreakS_SaveUsables _output_get)) (CallFunction|TranslateSlot Type))
      (Utilities|Array|RemoveIndex (Variables|Default|GetUsables) _array_index)
      (return))))

(fn PassEvent
  (params (NotifyName :type Name) (Sound :type Sound%20Base%20Object%20Reference) (Actor :type Actor%20Class%20Reference) (SocketName :type Name))
  (switch name NotifyName
    (:TakeItem
      (bind _returnvalue (Game|SpawnActorfromClass Actor (Transformation|GetActorTransform (Components|GetOwner)) "Undefined" 0 0))
      (bind _output_get (Variables|Default|SetUsedActor _returnvalue))
      (bind _bodymesh (CallFunction|GetCharacterSkeleton (Components|GetOwner)))
      (Transformation|AttachComponentToComponent _output_get _bodymesh SocketName "SnapToTarget" "SnapToTarget" "SnapToTarget" true))
    (:UseItem
      (Audio|PlaySoundatLocation Sound (Transformation|GetActorLocation (Components|GetOwner)) "0, 0, 0" 1.0 1.0 0.0 0 0 0 0))
    (:RemoveItem
      (Actor|DestroyActor (Variables|Default|GetUsedActor)))))