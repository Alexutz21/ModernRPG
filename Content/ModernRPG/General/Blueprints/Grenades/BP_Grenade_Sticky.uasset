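; Sticky grenade Blueprint that stops where it hits and explodes after a delay.
; On a valid hit, it records the hit actor, destroys its projectile movement and turns off collision physics simulation instead of explicitly attaching.
; It then enables box overlap events, waits for the configured explosion delay and calls Explode.
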(event EventBeginPlay
  (|CallParentFunction))

(event Collision|EventHit
  (params (MyComp :type Primitive%20Component%20Object%20Reference) (Other :type Actor%20Object%20Reference) (OtherComp :type Primitive%20Component%20Object%20Reference) (bSelfMoved :type Boolean) (HitLocation :type Vector :default "0, 0, 0") (HitNormal :type Vector :default "0, 0, 0") (NormalImpulse :type Vector :default "0, 0, 0") (Hit :type Hit%20Result%20Structure%20%28by%20ref%29))
  (bind _projectilemovement (Variables|Default|GetProjectileMovement))
  ;[1 1 1] Stick Grenade
  (Variables|Default|SetCurrentHitActor Other)
  (if (CallFunction|CanbeHit)
    (Utilities|IsValid _projectilemovement
      (:Is%20Valid
        (Components|DestroyComponent _projectilemovement)
        (Physics|SetSimulatePhysics (Variables|Default|GetCollision) false)
        (Variables|/Script/Engine.PrimitiveComponent|SetbGenerateOverlapEvents (Variables|Default|GetBox) true)
        (Utilities|FlowControl|Delay (Variables|Default|GetExpDelay))
        (CallFunction|Explode)))))

(fn ConstructionScript
  (|CallParentFunction))