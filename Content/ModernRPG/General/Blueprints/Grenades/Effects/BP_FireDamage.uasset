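; BP_FireDamage is a grenade fire effect that damages characters inside its box while it burns.
; Once activated with an owner as damage causer, a looping timer calls a server event that applies grenade-type point damage to overlapping characters.
; Meanwhile, a timeline shrinks and fades the smoky fire particles, then a second timeline quiets the fire sound before the actor destroys itself.
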(event Custom|ActivateDamage
  (params (Owner :type Actor%20Object%20Reference))
  (Variables|Default|SetDamageCauser Owner)
  (Utilities|Time|SetTimerbyEvent (delegate Custom|Damage) 2.0 true)
  (bind (_direction _alpha1 _alpha2) (Timeline|DestroyFlame PlayFromStart)
    (:Update
      (Effects|Components|ParticleSystem|SetVectorParameter (Variables|Default|GetSmokeyFire) "Size" (Math|Vector|Lerp(Vector) "100.000000,50.000000,1.000000" "0, 0, 0" _alpha1))
      (Effects|Components|ParticleSystem|SetFloatParameter (Variables|Default|GetSmokeyFire) "Opacity" (Math|Float|Lerp 1.0 0.0 _alpha2)))
    (:Finished
      (bind _newtrack_0 (Timeline|Quieter PlayFromStart)
        (:Update
          (Audio|Components|Audio|SetVolumeMultiplier (Variables|Default|GetFireSound) (Math|Float|Lerp (Variables|/Script/Engine.AudioComponent|GetVolumeMultiplier (Variables|Default|GetFireSound)) 0.0 _newtrack_0) :!class /Script/Engine.AudioComponent))
        (:Finished
          (Actor|DestroyActor))))))

(event Custom|Damage
  (CallFunction|Damage-Server))

(event Custom|Damage%20-%20Server
  (bind _returnvalue (Transformation|GetActorLocation))
  (for _array_element (Collision|GetOverlappingActors (Variables|Default|GetBox) "/Script/Engine.Character" :!class /Script/Engine.PrimitiveComponent)
    (Game|Damage|ApplyPointDamage _array_element 5e+01 _returnvalue (Collision|MakeHitResult false false 0.0 0.0 _returnvalue "0, 0, 0" "0,0,1" "0,0,1" 0 0 0 "None" "None" 0 0 0 "0, 0, 0" "0, 0, 0") 0 (Variables|Default|GetDamageCauser) "/Game/ModernRPG/General/Blueprints/DamageTypes/BPDT_Grenade.BPDT_Grenade_C")))

(event EventBeginPlay
  (Audio|Components|Audio|SetSound (Variables|Default|GetFireSound) (Variables|Default|GetSound)))

(fn ConstructionScript)