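; BP_SoundEffect is a grenade effect actor that handles the effect's audio.
; SoundcloudEffect finds controlled Characters within flashbang range and, after a delay, calls PlaySoundOC on their AC_Grenades component at zero volume.
; A separate server-to-all event pair plays the grenade's effect sound at the actor's location, and StopEffect destroys the actor.
; It also defines a view-angle check, unused here, and reports false for both flashbang and grenade type queries.
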(event Custom|SoundcloudEffect
  (bind _outactors (Actor|GetAllActorsOfClass "/Script/Engine.Character"))
  (for _array_element _outactors
    (if (Class|Pawn|IsControlled _array_element)
      (if (<= (Transformation|GetDistanceTo _array_element) (Variables|Default|GetFlashbangEffect_Distance))
        (Utilities|IsValid (Actor|GetComponentbyClass _array_element "/Game/ModernRPG/General/Blueprints/ActorComponents/Character/Grenade/AC_Grenades.AC_Grenades_C")
          (:Is%20Valid
            (Utilities|FlowControl|Delay (Variables|Default|GetFlashDelay))
            (Utilities|IsValid (Actor|GetComponentbyClass _array_element "/Game/ModernRPG/General/Blueprints/ActorComponents/Character/Grenade/AC_Grenades.AC_Grenades_C")
              (:Is%20Valid
                (Default|PlaySound-OC (Actor|GetComponentbyClass _array_element "/Game/ModernRPG/General/Blueprints/ActorComponents/Character/Grenade/AC_Grenades.AC_Grenades_C") (Utilities|Struct|BreakS_Grenades (Variables|Default|GetS_Grenade)) 0.0 self)))))))))

(event Custom|PlaySoundAtLoc%20-%20Server
  (params (S_GrenadeInfoStr :type S%20Grenades%20Structure%20%28by%20ref%29))
  (CallFunction|PlaySoundatLoc-All S_GrenadeInfoStr))

(event Custom|PlaySoundAtLoc%20-%20All
  (params (S_GrenadeInfoStr :type S%20Grenades%20Structure%20%28by%20ref%29))
  (Audio|PlaySoundatLocation (.EffectSound (Utilities|Struct|BreakS_Grenades S_GrenadeInfoStr)) (Transformation|GetActorLocation) "0, 0, 0" 1.0 1.0 0.0 0 0 0 0))

(event EventBeginPlay)

(event EventStopEffect
  (params (New::Flash? :type Boolean))
  (Actor|DestroyActor))

(fn ConstructionScript)

(fn AnglefromFlash
  (params (GrenadeLocation :type Vector) (Character :type Character%20Object%20Reference))
  (bind _camera (Class|BPIAI|GetMainCamera(Message) Character))
  (Utilities|IsValid _camera
    (:Is%20Valid
      (return (or (>= (- (.yaw (Math|Rotator|FindLookatRotation (Transformation|GetWorldLocation _camera) GrenadeLocation)) (.yaw (Transformation|GetWorldRotation _camera))) 9e+01) (<= (- (.yaw (Math|Rotator|FindLookatRotation (Transformation|GetWorldLocation _camera) GrenadeLocation)) (.yaw (Transformation|GetWorldRotation _camera))) -9e+01))))
    (:Is%20Not%20Valid
      (return false))))

(fn IsFlashbangEffect?
  (return false))

(fn IsGrenade
  (return false))