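; BP_SmokeEffect is a grenade smoke effect actor that fades out its particles and sound, then removes itself.
; BeginPlay assigns the configured sound to SmokeSound; the node that would set the particle template is unconnected.
; ActivateSmokes runs two chained timelines: DestroyFlame lerps the particle Alpha parameter to zero, then Timeline_1 lerps volume from its current value toward zero before destroying the actor.
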(event Custom|ActivateSmokes
  (bind _newtrack_0 (Timeline|DestroyFlame Play)
    (:Update
      (Effects|Components|ParticleSystem|SetFloatParameter (Variables|Default|GetParticle) "Alpha" (Math|Float|Lerp 1.0 0.0 _newtrack_0)))
    (:Finished
      (bind _newtrack_0_2 (Timeline|Timeline_1 Play)
        (:Update
          (Audio|Components|Audio|SetVolumeMultiplier (Variables|Default|GetSmokeSound) (Math|Float|Lerp (Variables|/Script/Engine.AudioComponent|GetVolumeMultiplier (Variables|Default|GetSmokeSound)) 0.0 _newtrack_0_2) :!class /Script/Engine.AudioComponent))
        (:Finished
          (Actor|DestroyActor))))))

(event EventBeginPlay
  (Audio|Components|Audio|SetSound (Variables|Default|GetSmokeSound) (Variables|Default|GetSound)))

(fn ConstructionScript)