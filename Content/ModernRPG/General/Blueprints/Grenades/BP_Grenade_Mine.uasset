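; Proximity mine grenade that either sticks where thrown or sits pre-placed in the level, exploding when a living Character overlaps its box.
; On a valid hit, a thrown mine drops its projectile movement, stops physics and arms the box overlap.
; Placed mines skip flight and collision, arm on BeginPlay and take the triggering character as owner.
; Destruction hides the actor and flags it Destroyed.
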(event OnComponentBeginOverlap(Box)
  (params (OverlappedComponent :type Primitive%20Component%20Object%20Reference) (OtherActor :type Actor%20Object%20Reference) (OtherComp :type Primitive%20Component%20Object%20Reference) (OtherBodyIndex :type Integer) (bFromSweep :type Boolean) (SweepResult :type Hit%20Result%20Structure%20%28by%20ref%29))
  ;[1 1 1] Explode On Overlap
  (bind _ascharacter (Utilities|Casting|CastToCharacter OtherActor))
  (Variables|Default|SetCurrentHitActor _ascharacter)
  (if (not (Variables|Default|GetbHidden))
    (if (not (Variables|Setup|GetPlaced))
      _
      (else
        (Actor|SetOwner (Variables|Default|GetCurrentHitActor))))
    (bind _result (Class|BPICharacter|IsAlive?(Message) (Variables|Default|GetCurrentHitActor)))
    (if _result
      (CallFunction|Explode))))

(event EventBeginPlay
  ;[1 1 1] Remove Component if Placed
  (|CallParentFunction)
  (if (Variables|Setup|GetPlaced)
    (Components|DestroyComponent (Variables|Default|GetProjectileMovement))
    (Variables|/Script/Engine.PrimitiveComponent|SetbGenerateOverlapEvents (Variables|Default|GetBox) true)))

(event Collision|EventHit
  (params (MyComp :type Primitive%20Component%20Object%20Reference) (Other :type Actor%20Object%20Reference) (OtherComp :type Primitive%20Component%20Object%20Reference) (bSelfMoved :type Boolean) (HitLocation :type Vector :default "0, 0, 0") (HitNormal :type Vector :default "0, 0, 0") (NormalImpulse :type Vector :default "0, 0, 0") (Hit :type Hit%20Result%20Structure%20%28by%20ref%29))
  (bind _projectilemovement (Variables|Default|GetProjectileMovement))
  ;[1 1 1] Stick Grenade
  (if (not (Variables|Setup|GetPlaced))
    (Variables|Default|SetCurrentHitActor Other)
    (if (CallFunction|CanbeHit)
      (Utilities|IsValid _projectilemovement
        (:Is%20Valid
          (Components|DestroyComponent _projectilemovement))
        (:Is%20Not%20Valid
          _))
      (Physics|SetSimulatePhysics (Variables|Default|GetCollision) false)
      (Variables|/Script/Engine.PrimitiveComponent|SetbGenerateOverlapEvents (Variables|Default|GetBox) true))))

(event EventDestroyGrenade
  (params (InputPin :type AC%20Grenades%20Object%20Reference))
  ;[1 1 1] Destroyed
  (Rendering|SetActorHiddenInGame true)
  (Variables|Default|SetDestroyed true))

(fn ConstructionScript
  (bind _projectilemovement (Variables|Default|GetProjectileMovement))
  (|CallParentFunction)
  (if (Variables|Setup|GetPlaced)
    (Variables|/Script/Engine.ProjectileMovementComponent|SetInitialSpeed _projectilemovement 0.0)
    (Variables|/Script/Engine.ProjectileMovementComponent|SetMaxSpeed _projectilemovement 0.0)
    (Collision|SetCollisionEnabled (Variables|Default|GetCollision) "NoCollision")))