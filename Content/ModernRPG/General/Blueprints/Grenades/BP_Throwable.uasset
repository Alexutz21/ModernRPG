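; Base throwable Blueprint in the grenades folder that applies a configurable mesh to its static mesh component.
; The construction script assigns the Mesh variable to the component.
; BeginPlay assigns it again through an Initialize-Server event that calls Initialize-All, a naming pattern that suggests server-to-all replication.
; No throwing, movement or detonation logic is present here.
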(event Custom|Initialize%20-%20All
  (Components|StaticMesh|SetStaticMesh (Variables|Default|GetStaticMesh) (Variables|Default|GetMesh)))

(event Custom|Initialize%20-%20Server
  (CallFunction|Initialize-All))

(event EventBeginPlay
  (CallFunction|Initialize-Server))

(fn ConstructionScript
  (Components|StaticMesh|SetStaticMesh (Variables|Default|GetStaticMesh) (Variables|Default|GetMesh)))