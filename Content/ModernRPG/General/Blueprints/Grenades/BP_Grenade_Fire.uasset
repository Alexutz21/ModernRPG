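; Fire grenade actor that explodes on a valid hit and plays a fire grenade fall sound.
; On Hit it stores the other actor and checks CanBeHit, then traces vertically on Visibility from above itself to far below.
; It snaps to the traced point, levelled with a yaw derived from the surface normal, before calling Explode.
; The construction script only runs the parent's.
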(event Collision|EventHit
  (params (MyComp :type Primitive%20Component%20Object%20Reference) (Other :type Actor%20Object%20Reference) (OtherComp :type Primitive%20Component%20Object%20Reference) (bSelfMoved :type Boolean) (HitLocation :type Vector :default "0, 0, 0") (HitNormal :type Vector :default "0, 0, 0") (NormalImpulse :type Vector :default "0, 0, 0") (Hit :type Hit%20Result%20Structure%20%28by%20ref%29))
  (bind _returnvalue (Transformation|GetActorLocation))
  (Variables|Default|SetCurrentHitActor Other)
  (if (CallFunction|CanbeHit)
    (bind _outhit (Collision|LineTraceByChannel (- _returnvalue "0, 0,-200.000000") (- _returnvalue "0,0.000000,5000.000000") "TraceTypeQuery1" false 0 "None"))
    (Transformation|SetActorLocationAndRotation (.Location (Collision|BreakHitResult _outhit)) (Math|Rotator|MakeRotator 0.0 0.0 (- (.Yaw (Math|Rotator|BreakRotator (Math|Conversions|RotationFromXVector (.Normal (Collision|BreakHitResult _outhit))))) 1.8e+02)))
    (CallFunction|Explode)
    (Audio|PlaySoundatLocation "/Game/ModernRPG/Shooter/Sounds/Weapon/Grenade/FireGrenade/SC_FireGrenade_Fall.SC_FireGrenade_Fall" (Transformation|GetActorLocation) "0, 0, 0" 1.0 1.0 0.0 0 0 0 0)))

(fn ConstructionScript
  (|CallParentFunction))