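; Grenade projectile actor for casual, flashbang, fire, smoke, sticky, timer and mine types, configured from a DataTable row.
; It explodes after an optional delay or on hitting a valid living target, otherwise playing a throttled bounce sound.
; Explode delegates damage and destruction to the owner's AC_Grenades and triggers per-type effects, with fire spawning damage actors at ground-traced grid points.
; The many vehicle-related interface functions are mostly empty stubs.
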(event OnComponentHit(Collision)
  (params (HitComponent :type Primitive%20Component%20Object%20Reference) (OtherActor :type Actor%20Object%20Reference) (OtherComp :type Primitive%20Component%20Object%20Reference) (NormalImpulse :type Vector :default "0, 0, 0") (Hit :type Hit%20Result%20Structure%20%28by%20ref%29))
  ;[1 1 1] On time ended or the hit event
  (bind _output_get (Variables|Default|SetCurrentHitActor OtherActor))
  (bind _result (Class|BPICharacter|IsAlive?(Message) _output_get))
  (if (and _result (CallFunction|CanbeHit))
    (Utilities|FlowControl|DoOnce false
      (:Completed
        (CallFunction|Explode)))
    (elif (Variables|Default|GetbHitSound)
      (Audio|PlaySoundatLocation (Utilities|Struct|BreakS_Grenades (Variables|Default|GetGrenade)) (Transformation|GetActorLocation) "0, 0, 0" 1.0 1.0 0.0 0 0 0 0)
      (Variables|Default|SetbHitSound false)
      (Utilities|FlowControl|Delay 0.5)
      (Variables|Default|SetbHitSound true))))

(event Custom|Effect-All
  (params (OriginLocal :type Vector))
  ;[1 1 1] Effect
  (CallFunction|Effect OriginLocal))

(event Custom|Explode
  (bind _returnvalue (Components|GetOwner))
  (bind _returnvalue_2 (Actor|GetComponentbyClass _returnvalue "/Game/ModernRPG/General/Blueprints/ActorComponents/Character/Grenade/AC_Grenades.AC_Grenades_C"))
  ;[1 1 1] Destroy Grenade
  (Utilities|IsValid _returnvalue
    (:Is%20Valid
      (Utilities|IsValid _returnvalue_2
        (:Is%20Valid
          (Default|ApplyDamageEffects-ALL _returnvalue_2 (Transformation|GetActorLocation) (Variables|MyProjectile|GetForce) self (Variables|Settings|GetGrenadeType) (Variables|Default|GetGrenade)))
        (:Is%20Not%20Valid
          _)))
    (:Is%20Not%20Valid
      _))
  (bind _output_get (Variables|Default|SetOriginVec (Transformation|GetActorLocation)))
  (CallFunction|Effect-All _output_get)
  (CallFunction|DestroyGrenade _returnvalue_2))

(event Custom|DestroyGrenade
  (params (InputPin :type AC%20Grenades%20Object%20Reference))
  ;[1 1 1] Destroy Grenade
  (if (Variables|Default|GetDestroy?)
    (Utilities|IsValid (Components|GetOwner)
      (:Is%20Valid
        (Utilities|IsValid InputPin
          (:Is%20Valid
            (Default|DestroyGrenadeActoron-Server InputPin self))
          (:Is%20Not%20Valid
            (CallFunction|DestroyGrenade-Server :!label _label))))
      (:Is%20Not%20Valid
        (goto _label)))))

(event Custom|DestroyGrenade%20%20-Server
  ;[1 1 1] Destroy
  (Utilities|FlowControl|Delay 0.2)
  (Class|RadialForceComponent|FireImpulse (Variables|MyProjectile|GetForce))
  (Actor|DestroyActor))

(event EventBeginPlay
  ;[1 1 1] On time ended or the hit event
  (Collision|IgnoreActorwhenMoving (Variables|MyProjectile|GetCollision) (Components|GetOwner) true)
  (CallFunction|Initialize)
  (Variables|Default|SetbHitSound true)
  (Utilities|FlowControl|Delay (Variables|Settings|GetExpDelay))
  (if (Variables|Settings|GetUseExplosionTimer)
    (CallFunction|Explode)))

(fn ConstructionScript)

(fn CanbeHit
  (bind _driver (Class|BPIVehicles|GetDriver(Message) (Variables|Default|GetCurrentHitActor)))
  (Utilities|IsValid _driver
    (:Is%20Valid
      (Utilities|IsValid (Actor|GetComponentbyClass _driver "/Game/ModernRPG/General/Blueprints/ActorComponents/Machinery/AC_VehicleController.AC_VehicleController_C")
        (:Is%20Valid
          (return (Math|Boolean|ANDBoolean (!= (Variables|Default|GetCurrentHitActor) self) (!= (Variables|Default|GetCurrentHitActor) (Components|GetOwner)) (not (.bSuccess (Utilities|Casting|CastToBP_Grenade (Variables|Default|GetCurrentHitActor)))) (!= (Variables|/Game/ModernRPG/General/Blueprints/ActorComponents/Machinery/AC_VehicleController.AC_VehicleController_C|GetVehicle (Actor|GetComponentbyClass _driver "/Game/ModernRPG/General/Blueprints/ActorComponents/Machinery/AC_VehicleController.AC_VehicleController_C")) (Variables|Default|GetCurrentHitActor)))))
        (:Is%20Not%20Valid
          _)))
    (:Is%20Not%20Valid
      _))
  (return (Math|Boolean|ANDBoolean (!= (Variables|Default|GetCurrentHitActor) self) (!= (Variables|Default|GetCurrentHitActor) (Components|GetOwner)) (not (.bSuccess (Utilities|Casting|CastToBP_Grenade (Variables|Default|GetCurrentHitActor)))))))

(fn Effect
  (params (OriginLocal :type Vector))
  (bind _grenade (Variables|Default|GetGrenade))
  (bind (_effectsound _explosionparticle) (Utilities|Struct|BreakS_Grenades _grenade))
  (switch Utilities|FlowControl|Switch|SwitchonE_GrenadeTypes (Variables|Settings|GetGrenadeType)
    (:NewEnumerator0
      (Camera|PlayWorldCameraShake "/Game/ModernRPG/Shooter/CameraShakes/BP_Explode.BP_Explode_C" OriginLocal 0.0 4e+03 1e+01 :!label _label)
      (Utilities|IsValid (Variables|MyProjectile|GetForce)
        (:Is%20Valid
          (Class|RadialForceComponent|FireImpulse (Variables|MyProjectile|GetForce)))
        (:Is%20Not%20Valid
          _))
      (Utilities|IsValid (Utilities|Struct|BreakS_Grenades (Variables|Default|GetGrenade))
        (:Is%20Valid
          (Effects|SpawnEmitteratLocation (Utilities|Struct|BreakS_Grenades (Variables|Default|GetGrenade)) OriginLocal)
          (Audio|PlaySoundatLocation (Utilities|Struct|BreakS_Grenades (Variables|Default|GetGrenade)) OriginLocal "0, 0, 0" 1.0 1.0 0.0 0 0 0 0))
        (:Is%20Not%20Valid
          (Utilities|IsValid (Utilities|Struct|BreakS_Grenades (Variables|Default|GetGrenade))
            (:Is%20Valid
              (Niagara|SpawnSystematLocation (Utilities|Struct|BreakS_Grenades (Variables|Default|GetGrenade)) OriginLocal)
              (Audio|PlaySoundatLocation (Utilities|Struct|BreakS_Grenades (Variables|Default|GetGrenade)) OriginLocal "0, 0, 0" 1.0 1.0 0.0 0 0 0 0))))))
    (:NewEnumerator1
      (Effects|SpawnEmitteratLocation (Utilities|Struct|BreakS_Grenades (Variables|Default|GetGrenade)) OriginLocal)
      (Audio|PlaySoundatLocation (Utilities|Struct|BreakS_Grenades (Variables|Default|GetGrenade)) (Transformation|GetActorLocation) "0, 0, 0" 1.0 1.0 0.0 0 0 0 0)
      (bind _returnvalue (Game|SpawnActorfromClass :Class "/Game/ModernRPG/General/Blueprints/Grenades/Effects/BP_SoundEffect.BP_SoundEffect_C" :SpawnTransform (Math|Conversions|ToTransform(Vector) OriginLocal) :CollisionHandlingOverride "Undefined" :Owner (Components|GetOwner) :Instigator 0))
      (Default|SoundcloudEffect _returnvalue))
    (:NewEnumerator2
      (CallFunction|FireEffect OriginLocal))
    (:NewEnumerator3
      (bind _returnvalue_2 (Game|SpawnActorfromClass "/Game/ModernRPG/General/Blueprints/Grenades/Effects/BP_SmokeEffect.BP_SmokeEffect_C" (Math|Conversions|ToTransform(Vector) OriginLocal) "Undefined" (Components|GetOwner) _effectsound _explosionparticle 0))
      (Default|ActivateSmokes _returnvalue_2)
      (Audio|PlaySoundatLocation (Utilities|Struct|BreakS_Grenades (Variables|Default|GetGrenade)) OriginLocal "0, 0, 0" 1.0 1.0 0.0 0 0 0 0))
    (:NewEnumerator4
      (goto _label))
    (:NewEnumerator5
      (goto _label))
    (:NewEnumerator6
      (goto _label))))

(fn Initialize
  (bind _grenadetablerow (Variables|Settings|GetGrenadeTableRow))
  (bind (_datatable _rowname) (Utilities|Struct|BreakDataTableRowHandle _grenadetablerow))
  (bind _returnvalue (Utilities|GetDataTableRow _datatable _rowname)
    (:then
      (Variables|Default|SetGrenade _returnvalue)
      (return))))

(fn Trace
  (params (Start :type Vector))
  (bind (_x _y _z) (Math|Vector|BreakVector Start))
  (bind (_x_2 _y_2 _z_2) (Math|Vector|BreakVector Start))
  (bind (_outhit _returnvalue) (Collision|LineTraceByChannel (Math|Vector|MakeVector _x_2 _y_2 (- _z_2 -1e+02)) (Math|Vector|MakeVector _x _y (- _z 5e+03)) "TraceTypeQuery5" false 0 "None"))
  (if _returnvalue
    (return (.Location (Collision|BreakHitResult _outhit)))))

(fn FireEffect
  (params (OriginalLocal :type Vector))
  (for _array_element (CallFunction|GetLocations OriginalLocal)
    (bind _returnvalue (Game|SpawnActorfromClass "/Game/ModernRPG/General/Blueprints/Grenades/Effects/BP_FireDamage.BP_FireDamage_C" (Math|Conversions|ToTransform(Vector) _array_element) "Undefined" self (Utilities|Struct|BreakS_Grenades (Variables|Default|GetGrenade)) 0))
    (Default|ActivateDamage _returnvalue (Components|GetOwner)))
  (return))

(fn GetLocations
  (params (InVec :type Vector))
  (bind (_x _y _z) (Math|Vector|BreakVector InVec))
  (bind (_x_2 _y_2 _z_2) (Math|Vector|BreakVector InVec))
  (bind (_x_3 _y_3 _z_3) (Math|Vector|BreakVector InVec))
  (bind (_x_4 _y_4 _z_4) (Math|Vector|BreakVector InVec))
  (bind (_x_5 _y_5 _z_5) (Math|Vector|BreakVector InVec))
  (bind (_x_6 _y_6 _z_6) (Math|Vector|BreakVector InVec))
  (bind (_x_7 _y_7 _z_7) (Math|Vector|BreakVector InVec))
  (bind (_x_8 _y_8 _z_8) (Math|Vector|BreakVector InVec))
  (bind (_x_9 _y_9 _z_9) (Math|Vector|BreakVector InVec))
  (return (Utilities|Array|MakeArray (CallFunction|Trace (Math|Vector|MakeVector (+ _x_4 1e+02) _y_4 _z_4)) (CallFunction|Trace (Math|Vector|MakeVector _x_5 _y_5 _z_5)) (CallFunction|Trace (Math|Vector|MakeVector (+ _x_6 -1e+02) _y_6 _z_6)) (CallFunction|Trace (Math|Vector|MakeVector (+ _x_7 1e+02) (+ _y_7 1e+02) _z_7)) (CallFunction|Trace (Math|Vector|MakeVector _x_8 _y_8 _z_8)) (CallFunction|Trace (Math|Vector|MakeVector (+ _x_9 -1e+02) (+ _y_9 1e+02) _z_9)) (CallFunction|Trace (Math|Vector|MakeVector (+ _x_2 1e+02) (+ _y_2 -1e+02) _z_2)) (CallFunction|Trace (Math|Vector|MakeVector _x_3 _y_3 _z_3)) (CallFunction|Trace (Math|Vector|MakeVector (+ _x -1e+02) (+ _y -1e+02) _z)))))

(fn BulletDamage
  (return 0.0))

(fn GetMinigunShellPlace
  (return 0))

(fn GetTankSettings
  (return ""))

(fn GetActiveCamera
  (return "NewEnumerator0"))

(fn GetAllWeapons
  (return "NewEnumerator0"))

(fn GetArrowBarrel
  (return 0))

(fn GetArrowMinigun
  (return 0))

(fn GetArrowSmoke
  (return 0))

(fn GetAudioAmmunitionExplosion
  (return 0))

(fn GetBarrel
  (return 0))

(fn GetBlackboardRef
  (return 0))

(fn GetBody
  (return 0 0))

(fn GetBodyCamera
  (return 0))

(fn GetBreakThroughSound
  (return 0))

(fn GetCameraAimInside
  (return 0))

(fn GetCameraMinigun
  (return 0))

(fn GetCameraTurret
  (return 0))

(fn GetCountOfMachineGun
  (return 0))

(fn GetCountOfShells
  (return 0))

(fn GetCountOfSmokes
  (return 0))

(fn GetDefaultAim
  (return 0))

(fn GetDemoSkeletalMeshes
  (return 0 0 0 0 0 0))

(fn GetDestroyedTankParticle
  (return 0))

(fn GetDestroyedTankSmokeParticle
  (return 0))

(fn GetDetectionDistance[Fighter]
  (return 0.0))

(fn GetDriverInside
  (return 0))

(fn GetExpInfo
  (return 0.0 0.0))

(fn GetHealth
  (return 0.0 0.0))

(fn GetHitWidget
  (return 0))

(fn GetLastActiveWeapon
  (return "NewEnumerator0"))

(fn GetLastWheels
  (return 0))

(fn GetLeftWheels
  (return 0))

(fn GetMainCamera
  (return 0))

(fn GetMainShotParticle
  (return 0))

(fn GetMainSpringArm
  (return 0))

(fn GetMaxSpeed
  (return 0.0))

(fn GetMinigunAim
  (return 0))

(fn GetMiniGunTurret
  (return 0))

(fn GetPawnType
  (return "NewEnumerator0"))

(fn GetPlaceforAmmunitionExplosionParticle
  (return 0))

(fn GetPlaneSettings
  (return ""))

(fn GetPointtoShot
  (return 0))

(fn GetPredictAim
  (return 0))

(fn GetRicochetSound
  (return 0))

(fn GetRightWheels
  (return 0))

(fn GetSecondShotParticle
  (return 0))

(fn GetShellDamage
  (return 0.0))

(fn GetShotAudio
  (return 0))

(fn GetSpeed
  (return 0.0))

(fn GetSplineL
  (return 0))

(fn GetSplineR
  (return 0))

(fn GetSusp
  (return 0))

(fn GetSuspensions
  (return 0))

(fn GetTarget
  (return 0))

(fn GetTeam
  (return "NewEnumerator2"))

(fn GetTrackL
  (return 0))

(fn GetTrackR
  (return 0))

(fn GetTurret
  (return 0))

(fn GetVehicleHealthInfo
  (return ""))

(fn IamParent
  (return false))

(fn IsAI
  (return false))

(fn IsDestroyed
  (return false))

(fn IsFlashbangEffect?
  (return false))

(fn IsGrenade
  (return true))

(fn IsHeatTrap
  (return false))

(fn IsTank
  (return false))

(fn IsTankActive
  (return false))

(fn IsVehicleTarget
  (return false))

(fn NoImpulse
  (return false))

(fn PlaceforShotSound
  (return 0))

(fn PointtoMove
  (return false))

(fn Sensible
  (return false))

(fn TankStarted
  (return false))

(fn TypeOfShell
  (return "NewEnumerator0"))