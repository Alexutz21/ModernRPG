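; BP_Marker is a world map marker actor that is removed from a player's map data when that character reaches it.
; On BeginPlay it configures its WB_MapArea widget as a marker, passing area info, itself and the owning player.
; Sphere overlap finds the character's AC_WorldMap component, looks up this marker's index and removes it.
; Ownership changes pass from SetOwner-S to SetOwner-ALL, named as a server-to-multicast relay.
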(event OnComponentBeginOverlap(Sphere)
  (params (OverlappedComponent :type Primitive%20Component%20Object%20Reference) (OtherActor :type Actor%20Object%20Reference) (OtherComp :type Primitive%20Component%20Object%20Reference) (OtherBodyIndex :type Integer) (bFromSweep :type Boolean) (SweepResult :type Hit%20Result%20Structure%20%28by%20ref%29))
  (bind _ascharacter (Utilities|Casting|CastToCharacter OtherActor))
  (Utilities|IsValid (Actor|GetComponentbyClass _ascharacter "/Game/ModernRPG/General/Blueprints/MapComponents/WorldMap/AC_WorldMap.AC_WorldMap_C")
    (:Is%20Valid
      (Variables|Default|SetWorldMap (Actor|GetComponentbyClass _ascharacter "/Game/ModernRPG/General/Blueprints/MapComponents/WorldMap/AC_WorldMap.AC_WorldMap_C"))
      (bind _index (Default|GetMarkerIndexbyReference (Variables|Default|GetWorldMap) self))
      (Default|RemoveMarkerIndex (Variables|Default|GetWorldMap) _index))))

(event Custom|SetOwner%20-S
  (params (NewOwner :type Actor%20Object%20Reference))
  ;[1 1 1] Set Owner
  (CallFunction|SetOwner-ALL NewOwner))

(event Custom|SetOwner%20-ALL
  (params (NewOwner :type Actor%20Object%20Reference))
  ;[1 1 1] Set Owner
  (Actor|SetOwner NewOwner))

(event EventBeginPlay
  (bind _aswb_map_area (Utilities|Casting|CastToWB_MapArea (UserInterface|GetUserWidgetObject (Variables|Default|GetWidget))))
  (Variables|Default|SetMapAreaWidget _aswb_map_area)
  (Variables|/Game/ModernRPG/General/GUI/Widgets/WorldMap/WorldPlace/WB_MapArea.WB_MapArea_C|Setmarkered? (Variables|Default|GetMapAreaWidget) true)
  (Variables|/Game/ModernRPG/General/GUI/Widgets/WorldMap/WorldPlace/WB_MapArea.WB_MapArea_C|SetAreaInfo (Variables|Default|GetMapAreaWidget) (Variables|Default|GetAreaInfo))
  (Variables|/Game/ModernRPG/General/GUI/Widgets/WorldMap/WorldPlace/WB_MapArea.WB_MapArea_C|SetActor (Variables|Default|GetMapAreaWidget) self)
  (Default|SetMapAreaOwner (Variables|Default|GetMapAreaWidget) (Variables|Default|GetPlayerOwner)))

(fn ConstructionScript)