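; Blueprint interface for HUD and UI widgets in the ModernRPG project, declaring calls that other objects use to drive them.
; It covers open/close animations, selection, values, kill log, chat, death screen and killer name.
; Combat functions handle aiming, shots, weapon changes, damage and suspicion indicators, plus tank and fighter UI getters, vehicle interaction, radius and item-look events.
; All functions are empty declarations, so behavior lives in the implementing widgets.
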(fn PlayOpenedAnimation
  (return 0))

(fn PlayClosedAnimation
  (return 0))

(fn Select)

(fn Unselect)

(fn SetValue
  (params (Value :type Float%20%28double-precision%29)))

(fn UpdateKillLog
  (params (KillerType :type E_Team%20Enum :default "NewEnumerator2") (KilledType :type E_Team%20Enum :default "NewEnumerator2") (KillerName :type Text) (KilledName :type Text) (Icon :type Texture%202D%20Object%20Reference)))

(fn SetKillLogType
  (params (GameMode :type E_GameType%20Enum :default "NewEnumerator0")))

(fn UpdateChat
  (params (Sender :type Text) (Text :type Text)))

(fn GetMainTankUI
  (return 0))

(fn GetMainFighterUI
  (return 0))

(fn SetTargetF
  (params (Actor :type Actor%20Object%20Reference) (Mode :type E_Target%20Enum :default "NewEnumerator0")))

(fn DeathScreen
  (params (Enabled? :type Boolean)))

(fn GetAimImage
  (return 0))

(fn AimingInside
  (params (Aiming :type Boolean)))

(fn WeaponChanged)

(fn MakeShotUI)

(fn GetTanksWB
  (return 0 0 0))

(fn Aiming
  (params (Aiming :type Boolean)))

(fn Shot
  (params (WeaponType :type E_WeaponType%20Enum :default "NewEnumerator0")))

(fn ChangeWeaponType
  (params (WeaponType :type E_WeaponType%20Enum :default "NewEnumerator0")))

(fn ControlAim
  (params (Show/Hide :type E_Show_Hide%20Enum :default "NewEnumerator0")))

(fn UpdateDamageLocation
  (params (Location :type Vector)))

(fn SuspiciousLocation
  (params (Location :type Vector)))

(fn UpdateSuspiciousValue
  (params (Value :type Float%20%28double-precision%29)))

(fn SetKillerName
  (params (Show :type Boolean) (Name :type Text))
  (return))

(fn InteractwithVehicle
  (params (HideAim :type Boolean)))

(fn SetTankInfo
  (params (S_Tank :type Boolean)))

(fn EnterRadius)

(fn LeaveRadius)

(fn StartLookitem)

(fn StopLookitem)