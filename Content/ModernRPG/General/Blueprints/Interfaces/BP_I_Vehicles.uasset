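; Blueprint interface that vehicles and their parts use to communicate in the game, covering tanks as well as plane and drone features.
; It declares weapon calls for cannon, minigun and smoke launchers, including firing, reloading, shell counts, aiming, sounds and particles.
; Other calls handle movement, driver and passengers, damage and track breaking, hit and kill reports, skins, lights and UI.
; All functions are signatures only, with behavior left to implementers.
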(fn MakeShot)

(fn IsTankValid
  (return false))

(fn CanShot?
  (return false))

(fn SetCanShotValue
  (params (Set :type Boolean)))

(fn GetCannonSettings
  (return ""))

(fn SetCountOfShells
  (params (Value :type Integer) (Weapon :type E_WeaponTypeTank%20Enum :default "NewEnumerator0") (FromSave :type Boolean)))

(fn ActivateShotParticles)

(fn GetCannonSound
  (return 0))

(fn ActivateShotSound)

(fn IsAiming
  (return false))

(fn Reload)

(fn Initialize)

(fn SetTossCache
  (params (Toss :type Vector)))

(fn SetMinigunToss
  (params (Toss :type Vector :default "0, 0, 0")))

(fn GetMinigunSettings
  (return ""))

(fn StopShooting)

(fn AfterShotAction
  (params (Weapon :type E_WeaponTypeTank%20Enum :default "NewEnumerator0")))

(fn MakeMinigunShot
  (params (Scatter :type Vector)))

(fn GetSmokeSettings
  (return ""))

(fn MakeSmokeShot)

(fn ActivateReloadSound)

(fn GetCountOfCannonShells
  (return 0))

(fn SetCurrentActiveSmokeIndex
  (params (Value :type Integer)))

(fn SetSmokesState
  (params (Index :type Integer) (State :type Boolean)))

(fn BreakTracks)

(fn IsComponentAllright
  (return false))

(fn SwitchSkins
  (params (E_Team :type E_Team%20Enum :default "NewEnumerator2") (Dead :type Boolean)))

(fn SetMaxSpeed
  (params (MaxSpeed :type Float%20%28double-precision%29)))

(fn IsItTrack
  (return false))

(fn SetCameraForwardVector
  (params (Camera :type Vector)))

(fn GetParentOwner
  (return 0))

(fn TurretExplosion
  (params (isSimulatingPhysics? :type Boolean)))

(fn VehicleHitted)

(fn GetReloadTime
  (return 0.0))

(fn ToggleLight)

(fn InitializeUI)

(fn TurnOff)

(fn GetDriver
  (return 0))

(fn ControlComponent'sState
  (params (Active :type Boolean)))

(fn OnInteractwithVehicle
  (params (GotOut? :type Boolean)))

(fn GetCountOfMinigunShells
  (return 0))

(fn GetHitDecalClass
  (return 0))

(fn UpdateSpeed
  (params (SpeedParam :type Float%20%28double-precision%29)))

(fn UpdateMoves
  (params (Forward :type Float%20%28double-precision%29) (Backward :type Float%20%28double-precision%29) (Left :type Float%20%28double-precision%29) (Right :type Float%20%28double-precision%29)))

(fn SetRate
  (params (Rate :type Float%20%28double-precision%29)))

(fn SetZ
  (params (Z :type Float%20%28double-precision%29)))

(fn SetSide
  (params (Side :type E_Side%20Enum :default "NewEnumerator0")))

(fn Aim
  (params (Aim :type Boolean)))

(fn AfterShotAction-Child)

(fn GetDriverPlace
  (return 0))

(fn ReporttoTarget
  (params (Causer :type Actor%20Object%20Reference)))

(fn GetHeight
  (return 0.0))

(fn ReportAboutKill
  (params (Victim :type Actor%20Object%20Reference)))

(fn EndOfAfterKillCam)

(fn GetWBTank
  (return 0))

(fn ReportAboutNoPenetration)

(fn ReportAboutHit
  (params (Damage :type Float%20%28double-precision%29)))

(fn Turnon)

(fn UpdatePlaneSettings
  (params (AimSens :type Float%20%28double-precision%29) (Invert :type Boolean)))

(fn CanHit
  (return false))

(fn HitCharacterVelocity
  (return 0.0 0))

(fn GetPassengers
  (return 0))

(fn ContinueLMBEvent)

(fn IsDrone
  (return false))

(fn IsSiucideMode
  (return false))

(fn IsBOMBLOAD
  (return false))

(fn GetForward/SideSpeed
  (return 0.0 0.0 0.0))

(fn ControlExitfromVehicle)

(fn IsShell
  (return false))

(fn IsVehicleActive
  (return false))

(fn GetMinimapArrow
  (return 0))