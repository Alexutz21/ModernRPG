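; BP_I_AI is a Blueprint interface shared by AI and vehicles, mainly tanks with some plane and fighter queries.
; It declares AI hooks for team, targets, behavior and behavior tree, plus calls for driving, weapons, damage and destruction.
; Getters expose vehicle cameras, aim points, track parts, effects, sounds, settings, health, experience and minimap state.
; All functions are empty stubs, so callers can query pawns without casting and implementers supply the logic.
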(fn GetTeam
  (return "NewEnumerator0"))

(fn Sensible
  (return false))

(fn SetTargetIII
  (params (Target :type Actor%20Object%20Reference))
  (return))

(fn GetTarget
  (return 0))

(fn GetSpeed
  (return 0.0))

(fn SetCanShot
  (params (Rocket%20Launched :type Boolean)))

(fn GetBody
  (return 0 0))

(fn GetDetectionDistance[Fighter]
  (return 0.0))

(fn IsHeatTrap
  (return false))

(fn GetHealth
  (return 0.0 0.0))

(fn ShowHealthUI)

(fn GetHitWidget
  (return 0))

(fn SetHUD
  (params (FighterHUD :type WB%20Plane%20Object%20Reference))
  (return))

(fn SetBehavior
  (params (State :type E_StateAI%20Enum :default "NewEnumerator0")))

(fn SetNewTarget
  (params (Target :type Actor%20Object%20Reference) (Stimulus :type AI%20Stimulus%20Structure)))

(fn RemoveTarget)

(fn GetCountOfShells
  (return 0))

(fn GetAllWeapons
  (return "NewEnumerator0"))

(fn GetActiveCamera
  (return "NewEnumerator0"))

(fn GetCountOfMachineGun
  (return 0))

(fn GetCountOfSmokes
  (return 0))

(fn GetPointtoShot
  (return 0))

(fn GetLastActiveWeapon
  (return "NewEnumerator0"))

(fn ApDamage
  (params (Damage :type Float%20%28double-precision%29) (Causer :type Actor%20Object%20Reference) (Component :type Primitive%20Component%20Object%20Reference) (ShouldKill :type Boolean) (TypeOfShell :type E_TypeOfShell%20Enum :default "NewEnumerator0")))

(fn GetDriverInside
  (return 0))

(fn IsTankActive
  (return false))

(fn GetBlackboardRef
  (return 0))

(fn TypeOfShell
  (return "NewEnumerator0"))

(fn SetTeam
  (params (Team :type E_Team%20Enum :default "NewEnumerator2")))

(fn RunBT)

(fn TankShot)

(fn GetTurret
  (return 0))

(fn IsDestroyed
  (return false))

(fn SetCamera
  (params (Camera :type E_Camera%20Enum :default "NewEnumerator0")))

(fn GetBodyCamera
  (return 0))

(fn GetCameraTurret
  (return 0))

(fn GetCameraAimInside
  (return 0))

(fn GetCameraMinigun
  (return 0))

(fn GetMainSpringArm
  (return 0))

(fn GetDefaultAim
  (return 0))

(fn GetPredictAim
  (return 0))

(fn GetMinigunAim
  (return 0))

(fn GetPlaceforAmmunitionExplosionParticle
  (return 0))

(fn GetAudioAmmunitionExplosion
  (return 0))

(fn DestroyVehicle
  (params (Killer :type Actor%20Object%20Reference) (DamageType :type E_DamageType%20Enum :default "NewEnumerator0") (KillDriver :type Boolean) (Saved :type Boolean)))

(fn GetDestroyedTankParticle
  (return 0))

(fn GetDestroyedTankSmokeParticle
  (return 0))

(fn GetDeathStatistics)

(fn BreakTrack
  (params (Side :type E_Side%20Enum :default "NewEnumerator0") (Shell :type Actor%20Object%20Reference)))

(fn GetRicochetSound
  (return 0))

(fn TankStarted
  (return false))

(fn IamParent
  (return false))

(fn BulletDamage
  (return 0.0))

(fn GetLeftWheels
  (return 0))

(fn GetSplineL
  (return 0))

(fn GetRightWheels
  (return 0))

(fn GetSplineR
  (return 0))

(fn GetTrackR
  (return 0))

(fn GetTrackL
  (return 0))

(fn GetBarrel
  (return 0))

(fn SetMoveRight
  (params (Target :type Object%20Object%20Reference)))

(fn GetSuspensions
  (return 0))

(fn SetMoveForward
  (params (Target :type Object%20Object%20Reference)))

(fn ShotMachinegun)

(fn StopShotMachinegun)

(fn IsTank
  (return false))

(fn GetArrowMinigun
  (return 0))

(fn GetTankSettings
  (return ""))

(fn SetLastActiveWeapon
  (params (LastActiveWeapon :type E_WeaponTypeTank%20Enum :default "NewEnumerator0")))

(fn GetArrowSmoke
  (return 0))

(fn ControlHatch
  (params (Open/Close :type E_OpenClose%20Enum :default "NewEnumerator0")))

(fn JammingRecoil)

(fn GetMiniGunTurret
  (return 0))

(fn GetArrowBarrel
  (return 0))

(fn PlaceforShotSound
  (return 0))

(fn GetMainShotParticle
  (return 0))

(fn GetSecondShotParticle
  (return 0))

(fn GetSusp
  (return 0))

(fn GetLastWheels
  (return 0))

(fn GetMinigunShellPlace
  (return 0))

(fn GetBreakThroughSound
  (return 0))

(fn GetShotAudio
  (return 0))

(fn GetMainCamera
  (return 0))

(fn IsVehicleTarget
  (return false))

(fn GetPawnType
  (return "NewEnumerator0"))

(fn GetShellDamage
  (return 0.0))

(fn GetVehicleHealthInfo
  (return ""))

(fn GetPlaneSettings
  (return ""))

(fn NoImpulse
  (return false))

(fn GetMaxSpeed
  (return 0.0))

(fn PointtoMove
  (return false))

(fn ClearEnemy)

(fn GetDemoSkeletalMeshes
  (return 0 0 0 0 0 0))

(fn GetExpInfo
  (return 0.0 0.0))

(fn IsAI
  (return false))

(fn OnPlayerMinimapState
  (return false 0 "" ""))