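; Blueprint interface through which other objects query a player or fighter for combat info and set its target.
; It declares getters for fighter settings, smoke arrows, barrels, miniguns and smoke state, plus flags for AI control and multiplayer.
; SetTarget passes a target actor to the implementer; all functions are empty declarations left to implementing classes.
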(fn GetFighterSettings
  (return ""))

(fn IsAI?
  (return false))

(fn SetTarget
  (params (TargetActor :type Actor%20Object%20Reference)))

(fn GetSmokeArrows
  (return 0))

(fn GetBarrels
  (return 0))

(fn GetMiniguns
  (return 0))

(fn GetSmokesState
  (return 0))

(fn IsMultiplayer
  (return false))