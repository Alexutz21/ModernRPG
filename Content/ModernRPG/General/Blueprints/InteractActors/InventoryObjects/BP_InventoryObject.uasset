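; BP_InventoryObject is an interactable world inventory, such as a chest, that opens its contents beside the player's inventory.
; Interacting while not busy transfers ownership of the object and its tagged bags to the character, then routes through server and owning-client events.
; The client plays a sound, hides the interact prompt and adds a container widget to the player's inventory UI.
; Closing the inventory restores the prompt and clears busy.
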(event Custom|OnInventoryClosed_Event_0
  (bind _currentactor (Variables|Default|GetCurrentActor))
  ;[1 1 1] Create Widget
  (Utilities|IsValid _currentactor
    (:Is%20Valid
      (Default|ToggleInteractWidgetVisibility (Actor|GetComponentbyClass _currentactor "/Game/ModernRPG/General/Blueprints/ActorComponents/InteractActors/AC_Interaction.AC_Interaction_C") true))
    (:Is%20Not%20Valid
      _))
  (CallFunction|ToggleBusy false))

(event Custom|OpenWidget%20-OC
  (params (Target :type Actor%20Object%20Reference))
  ;[1 1 1] Create Widget
  (Variables|Default|SetCurrentActor Target)
  (Audio|PlaySoundatLocation (Variables|Default|GetChestSound) (Transformation|GetActorLocation) "0, 0, 0" 1.0 1.0 0.0 0 0 0 0)
  (Utilities|FlowControl|DoOnce false :!label _label
    (:Completed
      (Utilities|FlowControl|Sequence
        (:then_0
          (Default|ToggleInteractWidgetVisibility (Actor|GetComponentbyClass (Variables|Default|GetCurrentActor) "/Game/ModernRPG/General/Blueprints/ActorComponents/InteractActors/AC_Interaction.AC_Interaction_C") false)
          (Default|OpenInventory (Actor|GetComponentbyClass (Variables|Default|GetCurrentActor) "/Game/ModernRPG/General/Blueprints/ActorComponents/Character/Inventory/AC_Inventory.AC_Inventory_C"))
          (EventDispatchers|AssignOnInventoryClosed (Actor|GetComponentbyClass (Variables|Default|GetCurrentActor) "/Game/ModernRPG/General/Blueprints/ActorComponents/Character/Inventory/AC_Inventory.AC_Inventory_C") (delegate Custom|OnInventoryClosed_Event_0))
          (CallFunction|ToggleBusy true)
          (Utilities|IsValid (Variables|/Game/ModernRPG/General/Blueprints/ActorComponents/Character/Inventory/AC_Inventory.AC_Inventory_C|GetPlayerInventoryWidget (Actor|GetComponentbyClass (Variables|Default|GetCurrentActor) "/Game/ModernRPG/General/Blueprints/ActorComponents/Character/Inventory/AC_Inventory.AC_Inventory_C"))
            (:Is%20Valid
              (bind _returnvalue (UserInterface|CreateWidget (Variables|Default|GetInventoryWidget) (.AsPlayer%20Controller (Utilities|Casting|CastToPlayerController (Pawn|GetController (.AsPawn (Utilities|Casting|CastToPawn (Variables|Default|GetCurrentActor))))))))
              (Utilities|FlowControl|Delay 0.05)
              (Default|AddWidget (Variables|/Game/ModernRPG/General/Blueprints/ActorComponents/Character/Inventory/AC_Inventory.AC_Inventory_C|GetPlayerInventoryWidget (Actor|GetComponentbyClass (Variables|Default|GetCurrentActor) "/Game/ModernRPG/General/Blueprints/ActorComponents/Character/Inventory/AC_Inventory.AC_Inventory_C")) _returnvalue (Variables|Default|GetAC_Inventory)))))
        (:then_1
          (Utilities|FlowControl|Delay 0.1)
          (goto _label Reset))))))

(event Custom|OpenWidget%20-Server
  (params (NewOwner :type Actor%20Object%20Reference))
  ;[1 1 1] Open Widget Replicated
  (CallFunction|OpenWidget-OC NewOwner))

(event Custom|SetOwners
  (params (NewOwner :type Actor%20Object%20Reference))
  ;[1 1 1] Set current owner of the inventroy
  (Actor|SetOwner NewOwner)
  (for _array_element (Variables|/Game/ModernRPG/General/Blueprints/ActorComponents/Character/Inventory/AC_Inventory.AC_Inventory_C|GetInventory (Variables|Default|GetAC_Inventory))
    (if (Utilities|Name|NotEqual(Name) (.BagTag (Utilities|Struct|BreakS_InvSlotHelper (.Helper (Utilities|Struct|BreakS_InvItemDyn _array_element)))) "None")
      (Utilities|IsValid (CallFunction|GetBagbyTag (.BagTag (Utilities|Struct|BreakS_InvSlotHelper (.Helper (Utilities|Struct|BreakS_InvItemDyn _array_element)))))
        (:Is%20Valid
          (Actor|SetOwner (CallFunction|GetBagbyTag (.BagTag (Utilities|Struct|BreakS_InvSlotHelper (.Helper (Utilities|Struct|BreakS_InvItemDyn _array_element))))) NewOwner))))))

(event EventInteract
  (params (Character :type Character%20Object%20Reference))
  ;[1 1 1] On Interacter - Set owner, open widget
  (if (not (Variables|Default|GetBusy))
    (CallFunction|SetOwners Character)
    (|CallParentFunction Character)
    (CallFunction|OpenWidget-Server Character)))

(fn ConstructionScript
  (|CallParentFunction))