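; Anim notify state, shown as "DisableInput", that flags input as disabled on the animating actor for the duration of its window.
; Begin sets DisableInput on the owner's AC_Conditions component and End clears it.
; End also calls EnableInput for a player-controlled Character owner, while the matching DisableInput call in Begin is disconnected, so blocking relies on the flag alone.
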(fn ReceivedNotifyBegin
  (params (MeshComp :type Skeletal%20Mesh%20Component%20Object%20Reference) (Animation :type Anim%20Sequence%20Base%20Object%20Reference) (TotalDuration :type Float%20%28single-precision%29) (EventReference :type Anim%20Notify%20Event%20Reference%20Structure%20%28by%20ref%29))
  (bind _returnvalue (Components|GetOwner MeshComp))
  (bind _returnvalue_2 (Actor|GetComponentbyClass _returnvalue "/Game/ModernRPG/General/Blueprints/ActorComponents/Character/Conditions/AC_Conditions.AC_Conditions_C"))
  ;[1 1 1] Start hits registration
  (Utilities|FlowControl|Sequence
    (:then_0
      (Utilities|IsValid _returnvalue_2
        (:Is%20Valid
          (Variables|/Game/ModernRPG/General/Blueprints/ActorComponents/Character/Conditions/AC_Conditions.AC_Conditions_C|SetDisableInput _returnvalue_2 true))))
    (:then_1
      (bind _ascharacter (Utilities|Casting|CastToCharacter (Components|GetOwner MeshComp)))
      (bind _asplayer_controller (Utilities|Casting|CastToPlayerController (Pawn|GetController _ascharacter))))
    (:then_2
      (return true))))

(fn ReceivedNotifyEnd
  (params (MeshComp :type Skeletal%20Mesh%20Component%20Object%20Reference) (Animation :type Anim%20Sequence%20Base%20Object%20Reference) (EventReference :type Anim%20Notify%20Event%20Reference%20Structure%20%28by%20ref%29))
  (bind _returnvalue (Components|GetOwner MeshComp))
  (bind _returnvalue_2 (Components|GetOwner MeshComp))
  (bind _returnvalue_3 (Actor|GetComponentbyClass _returnvalue_2 "/Game/ModernRPG/General/Blueprints/ActorComponents/Character/Conditions/AC_Conditions.AC_Conditions_C"))
  ;[1 1 1] Start hits registration
  (Utilities|FlowControl|Sequence
    (:then_0
      (Utilities|IsValid _returnvalue_3
        (:Is%20Valid
          (Variables|/Game/ModernRPG/General/Blueprints/ActorComponents/Character/Conditions/AC_Conditions.AC_Conditions_C|SetDisableInput _returnvalue_3 false))))
    (:then_1
      (bind _ascharacter (Utilities|Casting|CastToCharacter _returnvalue))
      (bind _asplayer_controller (Utilities|Casting|CastToPlayerController (Pawn|GetController _ascharacter)))
      (Input|EnableInput _returnvalue _asplayer_controller))
    (:then_2
      (return true))))

(fn GetNotifyName
  (return "DisableInput"))