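; Melee damage component that detects weapon hits while tracing is switched on and broadcasts them with a damage multiplier.
; A fast looping timer stores each mesh socket's position and sphere-traces from the previous position to the current one, covering the swing path.
; Per-component lists of damaged actors, seeded with the owner, become trace ignore lists to prevent repeat hits.
; Parallel surface-hit functions exist but are not called here.
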(event Custom|UpdateSockets
  ;[1 1 1] Set weapon Socketes Every 0.1 sec
  (if (Variables|Default|GetColliding)
    (if (Variables|Default|GetActive)
      (CallFunction|GetHitInformation))
    (CallFunction|SetSocketPosition)
    (Variables|Default|SetActive true)
    (else
      (Utilities|Time|ClearandInvalidateTimerbyHandle (Variables|Default|GetTraceTimer)))))

(event Custom|StartTracing
  ;[1 1 1] Set weapon Socketes Every 0.1 sec
  (bind _returnvalue (Utilities|Time|SetTimerbyEvent (delegate Custom|UpdateSockets) 0.01 true))
  (Variables|Default|SetTraceTimer _returnvalue))

(event Custom|SetSocketPosition
  ;[1 1 1] Set Socket Locations
  (for _array_element (Variables|Default|GetMeshes)
    (CallFunction|GenerateSockets _array_element)))

(event Custom|GetHitInformation
  ;[1 1 1] Weapon Positions Trace
  (for _array_element (Variables|Default|GetMeshes)
    (Variables|Default|SetCurrentComponent (.Component (Utilities|Struct|BreakS_MeleeWeapon _array_element)))
    (Utilities|IsValid (Variables|Default|GetCurrentComponent)
      (:Is%20Valid
        (for _array_element_2 (.Socket (Utilities|Struct|BreakS_MeleeWeapon _array_element))
          (if (not (Utilities|Array|ContainsItem (Variables|Default|GetIgnoredSockets) _array_element_2))
            (bind _outhits (Collision|MultiSphereTraceByChannel (.Value (Utilities|Map|Find (Variables|Default|GetSockets) (Utilities|String|StringToName (Utilities|String|Append (Utilities|String|ToString(Name) _array_element_2) "_" (Utilities|GetDisplayName (Variables|Default|GetCurrentComponent)))))) (Transformation|GetSocketLocation (Variables|Default|GetCurrentComponent) _array_element_2) 1.0 "TraceTypeQuery3" false (CallFunction|GetDamagedActors (Variables|Default|GetCurrentComponent)) "None" true "(R=0.000000,G=0.532451,B=1.000000,A=1.000000)"))
            (CallFunction|OnHit _outhits)))))))

(event EventTick
  (params (DeltaSeconds :type Float%20%28single-precision%29))
  ;[1 1 1] Set weapon Socketes Every 0.1 sec
)

(fn GetActorIndex
  (params (Component :type Primitive%20Component%20Object%20Reference))
  (for (_array_element _array_index) (Variables|Default|GetDamagedActors)
    (if (== (.Component (Utilities|Struct|BreakS_DamagedActors _array_element)) Component)
      (return _array_index)))
  (return -1))

(fn GetDamagedActors
  (params (Component :type Primitive%20Component%20Object%20Reference))
  (bind _index (CallFunction|GetActorIndex Component))
  (if (>= _index 0)
    (return (Utilities|Struct|BreakS_DamagedActors (Utilities|Array|Get(acopy) (Variables|Default|GetDamagedActors) _index)))
    (else
      (bind _returnvalue (Utilities|Array|Add (Variables|Default|GetDamagedActors) (Utilities|Struct|MakeS_DamagedActors Component (Utilities|Array|MakeArray (Components|GetOwner)))))
      (Utilities|Array|Add (LocalVariables|GetFinalActors) (Components|GetOwner))
      (Utilities|Array|AppendArray (LocalVariables|GetFinalActors) (Utilities|Struct|BreakS_DamagedActors (Utilities|Array|Get(acopy) (Variables|Default|GetDamagedActors) _returnvalue)))
      (return (LocalVariables|GetFinalActors)))))

(fn AddDamagedActor
  (params (Component :type Primitive%20Component%20Object%20Reference) (HitActor :type Actor%20Object%20Reference))
  (bind _index (CallFunction|GetActorIndex Component))
  (if (>= _index 0)
    (Utilities|Array|Add (Utilities|Struct|BreakS_DamagedActors (Utilities|Array|Get(acopy) (Variables|Default|GetDamagedActors) _index)) HitActor)))

(fn Traceon
  (Variables|Default|SetColliding true)
  (Utilities|Array|Clear (Variables|Default|GetDamagedActors))
  (Utilities|Array|Clear (Variables|Default|GetSurfaceActors))
  (CallFunction|StartTracing))

(fn TraceOff
  (Variables|Default|SetColliding false)
  (Variables|Default|SetActive false)
  (Variables|Default|SetDamageMultiplier 0.0)
  (Utilities|Time|ClearandInvalidateTimerbyHandle (Variables|Default|GetTraceTimer)))

(fn InitializeCollisions
  (params (Meshes :type Array%20of%20S%20Melee%20Weapon%20Structures))
  (Variables|Default|SetMeshes Meshes)
  (CallFunction|SetSocketPosition))

(fn OnHit
  (params (Array :type Array%20of%20Hit%20Result%20Structures))
  (for _array_element Array
    (Default|CallDamage _array_element (Variables|Default|GetDamageMultiplier))
    (CallFunction|AddDamagedActor (Variables|Default|GetCurrentComponent) (.HitActor (Collision|BreakHitResult _array_element)))))

(fn GenerateSockets
  (params (S_CollisionSockets :type S%20Melee%20Weapon%20Structure%20%28by%20ref%29))
  (bind (_component _socket) (Utilities|Struct|BreakS_MeleeWeapon S_CollisionSockets))
  (Utilities|IsValid _component
    (:Is%20Valid
      (for _array_element _socket
        (Utilities|Map|Add (Variables|Default|GetSockets) (Utilities|String|StringToName (Utilities|String|Append (Utilities|String|ToString(Name) _array_element) "_" (Utilities|GetDisplayName _component))) (Transformation|GetSocketLocation _component _array_element))))))

(fn OnSurfaceHit
  (params (Array :type Array%20of%20Hit%20Result%20Structures))
  (for _array_element Array
    (Default|CallEDHit _array_element)
    (CallFunction|AddSurfaceActor (Variables|Default|GetCurrentComponent) (.HitActor (Collision|BreakHitResult _array_element)))))

(fn AddSurfaceActor
  (params (Component :type Primitive%20Component%20Object%20Reference) (HitActor :type Actor%20Object%20Reference))
  (bind _index (CallFunction|GetSurfaceIndex Component))
  (if (>= _index 0)
    (Utilities|Array|Add (Utilities|Struct|BreakS_DamagedActors (Utilities|Array|Get(acopy) (Variables|Default|GetSurfaceActors) _index)) HitActor)))

(fn GetSurfaceIndex
  (params (Component :type Primitive%20Component%20Object%20Reference))
  (for (_array_element _array_index) (Variables|Default|GetSurfaceActors)
    (if (== (.Component (Utilities|Struct|BreakS_DamagedActors _array_element)) Component)
      (return _array_index)))
  (return -1))

(fn GetSurfaceActors
  (params (Component :type Primitive%20Component%20Object%20Reference))
  (bind _index (CallFunction|GetSurfaceIndex Component))
  (if (>= _index 0)
    (return (Utilities|Struct|BreakS_DamagedActors (Utilities|Array|Get(acopy) (Variables|Default|GetSurfaceActors) _index)))
    (else
      (bind _returnvalue (Utilities|Array|Add (Variables|Default|GetSurfaceActors) (Utilities|Struct|MakeS_DamagedActors Component (Utilities|Array|MakeArray (Components|GetOwner)))))
      (Utilities|Array|Add (LocalVariables|GetFinalActors) (Components|GetOwner))
      (Utilities|Array|AppendArray (LocalVariables|GetFinalActors) (Utilities|Struct|BreakS_DamagedActors (Utilities|Array|Get(acopy) (Variables|Default|GetSurfaceActors) _returnvalue)))
      (return (LocalVariables|GetFinalActors)))))