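; Team player start that tracks whether it is free to spawn at, with no event logic of its own.
; SetBusy flags the start as busy, returns its location and rotation, and schedules Release by timer to clear the flag seconds later.
; HasSomeoneNear sphere-traces for pawns at the start and reports occupied unless the first hit actor's class is in IgnoreList.
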(event EventBeginPlay)

(event EventTick
  (params (DeltaSeconds :type Float%20%28single-precision%29)))

(fn ConstructionScript)

(fn SetBusy
  ;[1 1 1] This start is busy now
  (Variables|Default|SetBusy true)
  (Utilities|Time|SetTimerbyFunctionName 0 "Release" 3.0)
  (return (Transformation|GetActorLocation) (Transformation|GetActorRotation)))

(fn Release
  (Variables|Default|SetBusy false))

(fn HasSomeoneNear
  (bind (_outhit _returnvalue) (Collision|SphereTraceForObjects (Transformation|GetActorLocation) (+ (Transformation|GetActorLocation) 1.0) 3e+01 (Utilities|Array|MakeArray "ObjectTypeQuery3") false 0 "None"))
  (if _returnvalue
    (return (not (Utilities|Array|ContainsItem (Variables|Default|GetIgnoreList) (Utilities|GetClass (.HitActor (Collision|BreakHitResult _outhit))))))
    (else
      (return false))))