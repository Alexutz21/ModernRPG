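; GM_Polygon is the game mode for the Polygon gameplay mode, handling player join, logout and kill-log broadcasting.
; It tracks controllers on post-login and relays kill-log updates to each PC_Gameplay.
; On logout it releases the pawn's reload clip, destroys its current weapon actor and destroys that controller's session.
; The getters for time, gameplay widget, player info and team points are empty stubs.
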(event Custom|LoggedOut
  (params (ExitingController :type Controller%20Object%20Reference))
  (bind _returnvalue (Pawn|GetControlledPawn ExitingController))
  (bind _returnvalue_2 (Actor|GetComponentbyClass _returnvalue "/Game/ModernRPG/General/Blueprints/ActorComponents/InteractActors/AC_EquipmentHandler.AC_EquipmentHandler_C"))
  (bind _returnvalue_3 (Actor|GetComponentbyClass _returnvalue "/Game/ModernRPG/General/Blueprints/ActorComponents/Weapon/AC_Reload.AC_Reload_C"))
  (bind _actor (Default|GetCurrentWeaponActorbyType _returnvalue_2))
  ;[1 1 1] Logout
  (|CallParentFunction ExitingController)
  (Utilities|IsValid _returnvalue
    (:Is%20Valid
      (Utilities|IsValid _returnvalue_3
        (:Is%20Valid
          (Default|ReleaseClip-Server _returnvalue_3))
        (:Is%20Not%20Valid
          _))
      (Utilities|IsValid _actor
        (:Is%20Valid
          (Actor|DestroyActor _actor))))))

(event EventPostLogin
  (params (NewPlayer :type Player%20Controller%20Object%20Reference))
  ;[1 1 1] Track new Player Controllers
  (Class|BPIGameMode|Possessed(Message) NewPlayer)
  (Utilities|Array|Add (Variables|GameInfo|GetAllPlayerControllers) NewPlayer))

(event EventOnLogout
  (params (ExitingController :type Controller%20Object%20Reference))
  ;[1 1 1] Event on Logout | Destroysession for that PC
  (CallFunction|LoggedOut ExitingController)
  (bind _aspc_gameplay (Utilities|Casting|CastToPC_Gameplay ExitingController))
  (|DestroySession (.AsBP%20Game%20Instanceinfo (Utilities|Casting|CastToBP_GameInstanceinfo (Game|GetGameInstance))) _aspc_gameplay))

(event EventUpdateKillLog
  (params (KillerTeam :type E_Team%20Enum :default "NewEnumerator2") (KilledTeam :type E_Team%20Enum :default "NewEnumerator2") (KillerName :type Text) (KilledName :type Text) (Icon :type Texture%202D%20Object%20Reference))
  ;[1 1 1] Update Kill Log
  (for _array_element (Variables|GameInfo|GetAllPlayerControllers)
    (Utilities|IsValid _array_element
      (:Is%20Valid
        (bind _aspc_gameplay (Utilities|Casting|CastToPC_Gameplay _array_element))
        (Default|UpdateKillLogPC _aspc_gameplay KillerTeam KilledTeam KillerName KilledName Icon)))))

(fn ConstructionScript)

(fn GetCurrentTime
  (return 0))

(fn GetGameplayWB
  (return 0))

(fn GetPlayerInformaion
  (return ""))

(fn GetTeamPoints
  (return 0))