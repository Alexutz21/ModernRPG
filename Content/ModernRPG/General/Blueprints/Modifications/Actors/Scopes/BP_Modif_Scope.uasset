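; Weapon scope modification actor that renders a picture-in-picture zoomed view on its lens while aiming.
; Aiming creates a fresh render target for the SceneCapture2D, feeds it into a dynamic lens material and activates capture, while ZoomControl sets the capture FOV.
; Aim release waits out the blend time, rechecks state, then disables capture and restores the glass material.
; A separate authority-switched event routes render target creation through server and all-client events.
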(event Custom|CreateRT%20Event
  (bind _scenecapturecomponent2d (Variables|Default|GetSceneCaptureComponent2D))
  ;[1 1 1] Create a render target
  (Networking|SwitchHasAuthority
    (:Authority
      (CallFunction|CreateRT-All _scenecapturecomponent2d))
    (:Remote
      (CallFunction|CreateRT-Server _scenecapturecomponent2d))))

(event Custom|CreateRT%20-%20Server
  (params (SceneCaptureComponent2D :type Scene%20Capture%20Component%202D%20Object%20Reference))
  ;[1 1 1] Create a render target
  (CallFunction|CreateRT-All SceneCaptureComponent2D))

(event Custom|CreateRT-All
  (params (SceneCaptureComponent2D :type Scene%20Capture%20Component%202D%20Object%20Reference))
  ;[1 1 1] Create a render target
  (CallFunction|CreateRT-Scope SceneCaptureComponent2D))

(event EventAimControl
  (params (Start :type Boolean) (AimBlendTime :type Float%20%28double-precision%29))
  (bind _output_get (Variables|Default|SetState Start))
  (if _output_get
    (CallFunction|CreateRT-Scope (Variables|Default|GetSceneCaptureComponent2D))
    (Rendering|SetVisibility (Variables|Default|GetRT_Aim) true false)
    (Components|Activation|SetActive (Variables|Default|GetSceneCaptureComponent2D) true false)
    (Rendering|SceneCapture|CaptureScene (Variables|Default|GetSceneCaptureComponent2D) :!class /Script/Engine.SceneCaptureComponent2D)
    (Rendering|Material|SetMaterial (Variables|Default|GetRT_Aim) 0 (Variables|Default|GetDynamicMaterial))
    (else
      (Utilities|FlowControl|Delay AimBlendTime)
      (if (not (Variables|Default|GetState))
        (Rendering|SetVisibility (Variables|Default|GetRT_Aim) false false)
        (Components|Activation|SetActive (Variables|Default|GetSceneCaptureComponent2D) false false)
        (Rendering|Material|SetMaterial (Variables|Default|GetRT_Aim) 0 "/Game/ModernRPG/Shooter/Materials/Combat/Weapon/Modifications/MI_Scope4x_Glass.MI_Scope4x_Glass")))))

(event EventZoomControl
  (params (NewParam :type Float%20%28double-precision%29))
  (Variables|/Script/Engine.SceneCaptureComponent2D|SetFOVAngle (Variables|Default|GetSceneCaptureComponent2D) NewParam))

(fn ConstructionScript
  (|CallParentFunction))

(fn CreateRT-Scope
  (params (InputPin :type Scene%20Capture%20Component%202D%20Object%20Reference))
  (Utilities|IsValid InputPin
    (:Is%20Valid
      (bind _returnvalue (Rendering|CreateRenderTarget2D 1300 1300 "RTF_RGBA16f"))
      (bind _output_get (Variables|/Script/Engine.SceneCaptureComponent2D|SetTextureTarget InputPin _returnvalue))
      (Utilities|IsValid (Variables|Default|GetDynamicMaterial)
        (:Is%20Valid
          (Rendering|Material|SetTextureParameterValue (Variables|Default|GetDynamicMaterial) "Render" (Variables|/Script/Engine.SceneCaptureComponent2D|GetTextureTarget InputPin)))
        (:Is%20Not%20Valid
          (bind _returnvalue_2 (Rendering|Material|CreateDynamicMaterialInstance "/Game/ModernRPG/Shooter/Materials/Combat/Aim/Scope/MI_RT_Scope.MI_RT_Scope" "None" "None" :!class /Script/Engine.KismetMaterialLibrary))
          (Variables|Default|SetDynamicMaterial _returnvalue_2)
          (Rendering|Material|SetTextureParameterValue (Variables|Default|GetDynamicMaterial) "Render" _output_get))))))