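; Modification actor that displays a static mesh on a socket of a weapon mesh.
; Initialize stores the socket name, weapon mesh and display mesh, then calls AttachActor.
; AttachActor snaps its StaticMesh component to that socket in location, rotation and scale, then assigns the mesh.
; Only the component is attached to the weapon, and BeginPlay and the construction script are empty.
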(event Custom|Initialize
  (params (Socket :type Name) (Mesh :type Scene%20Component%20Object%20Reference) (InitializeMesh :type Static%20Mesh%20Object%20Reference))
  (Variables|Default|SetSocket Socket)
  (Variables|Default|SetWeaponMesh Mesh)
  (Variables|Default|SetInitializeMesh InitializeMesh)
  (CallFunction|AttachActor))

(event Custom|AttachActor
  (Transformation|AttachComponentToComponent (Variables|Default|GetStaticMesh) (Variables|Default|GetWeaponMesh) (Variables|Default|GetSocket) "SnapToTarget" "SnapToTarget" "SnapToTarget" true)
  (Components|StaticMesh|SetStaticMesh (Variables|Default|GetStaticMesh) (Variables|Default|GetInitializeMesh)))

(event EventBeginPlay)

(fn ConstructionScript)