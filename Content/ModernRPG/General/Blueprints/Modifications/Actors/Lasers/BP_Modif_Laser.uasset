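; Laser weapon attachment that draws a Niagara beam and impact effect where the weapon points.
; Each tick it line-traces from AC_Weapon's laser vectors or the emitter's right vector, chosen by aiming, view, player and movement state, then updates beam end and impact.
; LaserControl toggles tick and visibility and sets laser color and power in MPC_ModernRPG.
; Tick bypasses the unused server path, as replicating per-tick traces is deliberately avoided.
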(event Custom|TraceLaser%20-%20Server
  (params (Hit :type Boolean) (Target :type Vector) (Impact :type Vector))
  ;[1 1 1] We decided not to replicate the laser because event tick + multiplayer is a very bad idea
  (CallFunction|TraceLaser-ALL Hit Target Impact))

(event Custom|TraceLaser%20-ALL
  (params (Hit :type Boolean) (Target :type Vector) (Impact :type Vector))
  ;[1 1 1] We decided not to replicate the laser because event tick + multiplayer is a very bad idea
  (CallFunction|ControlLaserLocation Hit Target Impact))

(event Custom|CalculateEndLocation
  (bind (_block _returnvalue _location) (CallFunction|GetLocationfromWeapon))
  ;[1 1 1] We decided not to replicate the laser because event tick + multiplayer is a very bad idea
  (CallFunction|TraceLaser-Server _block _returnvalue _location))

(event EventTick
  (params (DeltaSeconds :type Float%20%28single-precision%29))
  (bind (_block _returnvalue _location) (CallFunction|GetLocationfromWeapon))
  ;[1 1 1] We decided not to replicate the laser because event tick + multiplayer is a very bad idea
  (CallFunction|TraceLaser-ALL _block _returnvalue _location))

(event EventLaserControl
  (params (Value :type Boolean))
  ;[1 1 1] We decided not to replicate the laser because event tick + multiplayer is a very bad idea
  (Actor|Tick|SetActorTickEnabled Value)
  (Rendering|SetVisibility (Variables|Default|GetNS_LaserImpact) Value false)
  (if Value
    (Rendering|Material|SetVectorParameterValue "/Game/ModernRPG/Shooter/Materials/Combat/Weapon/Modifications/Laser/MPC_ModernRPG.MPC_ModernRPG" "LaserColor" (Variables|Settings|GetLaserColor) :!class /Script/Engine.KismetMaterialLibrary)
    (Rendering|Material|SetScalarParameterValue "/Game/ModernRPG/Shooter/Materials/Combat/Weapon/Modifications/Laser/MPC_ModernRPG.MPC_ModernRPG" "LaserPower" 0.0 :!class /Script/Engine.KismetMaterialLibrary)
    (else
      (Rendering|Material|SetVectorParameterValue "/Game/ModernRPG/Shooter/Materials/Combat/Weapon/Modifications/Laser/MPC_ModernRPG.MPC_ModernRPG" "LaserColor" (Utilities|Struct|MakeLinearColor 0.0 0.0 0.0 1.0) :!class /Script/Engine.KismetMaterialLibrary)
      (Rendering|Material|SetScalarParameterValue "/Game/ModernRPG/Shooter/Materials/Combat/Weapon/Modifications/Laser/MPC_ModernRPG.MPC_ModernRPG" "LaserPower" 1e+01 :!class /Script/Engine.KismetMaterialLibrary))))

(fn ConstructionScript
  (|CallParentFunction))

(fn LaseratCenter
  (if (Default|Aiming? (Actor|GetComponentbyClass (Components|GetOwner) "/Game/ModernRPG/General/Blueprints/ActorComponents/Weapon/AC_Aiming.AC_Aiming_C"))
    (if (Default|IsThirdPerson (Actor|GetComponentbyClass (Components|GetOwner) "/Game/ModernRPG/General/Blueprints/ActorComponents/Weapon/AC_Aiming.AC_Aiming_C"))
      (if (Default|Scopable (Actor|GetComponentbyClass (Components|GetOwner) "/Game/ModernRPG/General/Blueprints/ActorComponents/Weapon/AC_Aiming.AC_Aiming_C"))
        (return true)
        (else
          (return false)))
      (else
        (return true)))
    (else
      (return false))))

(fn GetLocationfromWeapon
  (bind _fromaimcamera (CallFunction|LaseratCenter))
  (bind _returnvalue (Components|GetOwner))
  (bind _returnvalue_2 (Components|GetOwner))
  (bind _returnvalue_3 (Components|GetOwner))
  (bind _returnvalue_4 (Components|GetOwner))
  (bind _ns_laser (Variables|Default|GetNS_Laser))
  (bind _returnvalue_5 (Actor|GetComponentbyClass _returnvalue_2 "/Script/Engine.CharacterMovementComponent"))
  (bind _returnvalue_6 (Actor|GetComponentbyClass _returnvalue_4 "/Game/ModernRPG/General/Blueprints/ActorComponents/Weapon/AC_Aiming.AC_Aiming_C"))
  (bind _returnvalue_7 (Actor|GetComponentbyClass _returnvalue_2 "/Game/ModernRPG/General/Blueprints/ActorComponents/Character/State/AC_PlayerCurrentState.AC_PlayerCurrentState_C"))
  (bind _returnvalue_8 (Actor|GetComponentbyClass _returnvalue "/Game/ModernRPG/General/Blueprints/ActorComponents/Weapon/AC_Weapon.AC_Weapon_C"))
  (bind _returnvalue_9 (Actor|GetComponentbyClass _returnvalue_3 "/Game/ModernRPG/General/Blueprints/ActorComponents/Weapon/AC_Weapon.AC_Weapon_C"))
  (bind _returnvalue_10 (Transformation|GetWorldLocation _ns_laser))
  (bind _returnvalue_11 (select _fromaimcamera "NewEnumerator0" "NewEnumerator1"))
  (bind (_startlocation _endlocation) (Default|LASERGetTraceVectors _returnvalue_8 _returnvalue_11))
  (bind (_startlocation_2 _endlocation_2) (Default|LASERGetTraceVectors _returnvalue_9 "NewEnumerator0"))
  (bind _currentstate (Variables|/Game/ModernRPG/General/Blueprints/ActorComponents/Character/State/AC_PlayerCurrentState.AC_PlayerCurrentState_C|GetCurrentState _returnvalue_7))
  (bind _movementmode (Variables|/Script/Engine.CharacterMovementComponent|GetMovementMode _returnvalue_5))
  (Utilities|IsValid _returnvalue_2
    (:Is%20Valid
      (Utilities|IsValid (Actor|GetComponentbyClass _returnvalue_2 "/Game/ModernRPG/General/Blueprints/ActorComponents/Weapon/AC_Aiming.AC_Aiming_C")
        (:Is%20Valid
          (Utilities|IsValid _returnvalue_7
            (:Is%20Valid
              (if (Math|Boolean|ANDBoolean (and (Utilities|Enum|NotEqual(Enum) _currentstate "NewEnumerator1") (Utilities|Enum|NotEqual(Enum) _currentstate "NewEnumerator2")) (Utilities|Enum|Equal(Enum) (Variables|/Game/ModernRPG/General/Blueprints/ActorComponents/SpeedChange/AC_SpeedChange.AC_SpeedChange_C|GetCurrentWalkState (Actor|GetComponentbyClass _returnvalue_2 "/Game/ModernRPG/General/Blueprints/ActorComponents/SpeedChange/AC_SpeedChange.AC_SpeedChange_C")) "NewEnumerator3") (Math|Boolean|ANDBoolean (Utilities|Enum|NotEqual(Enum) _movementmode "MOVE_Falling") (Utilities|Enum|NotEqual(Enum) _movementmode "MOVE_Swimming") (Utilities|Enum|NotEqual(Enum) _movementmode "MOVE_Flying")))
                (bind (_outhit _returnvalue_12) (Collision|LineTraceByChannel _startlocation _endlocation "TraceTypeQuery1" false (Utilities|Array|MakeArray self (Components|GetOwner)) "None" true "(R=0.069618,G=0.000000,B=1.000000,A=1.000000)" "(R=0.855045,G=1.000000,B=0.000000,A=1.000000)" 0.5))
                (if _returnvalue_12
                  (return _returnvalue_12 (.Location (Collision|BreakHitResult _outhit)) (.Location (Collision|BreakHitResult _outhit)))
                  (else
                    (return _returnvalue_12 (.TraceEnd (Collision|BreakHitResult _outhit)) (.TraceEnd (Collision|BreakHitResult _outhit)))))
                (else
                  (if (and (Default|Aiming? _returnvalue_6) (Default|Scopable _returnvalue_6))
                    _
                    (elif (and (Default|Aiming? (Actor|GetComponentbyClass (Components|GetOwner) "/Game/ModernRPG/General/Blueprints/ActorComponents/Weapon/AC_Aiming.AC_Aiming_C")) (not (Default|IsThirdPerson (Actor|GetComponentbyClass (Components|GetOwner) "/Game/ModernRPG/General/Blueprints/ActorComponents/Weapon/AC_Aiming.AC_Aiming_C"))))
                      _
                      (else
                        (bind (_outhit_2 _returnvalue_13) (Collision|LineTraceByChannel _returnvalue_10 (+ _returnvalue_10 (* (Math|Vector|GetRightVector _ns_laser) 10000)) "TraceTypeQuery1" false (Utilities|Array|MakeArray self (Components|GetOwner)) "None"))
                        (if _returnvalue_13
                          (return true (.Location (Collision|BreakHitResult _outhit_2)) (.Location (Collision|BreakHitResult _outhit_2)))
                          (else
                            (return true (.TraceEnd (Collision|BreakHitResult _outhit_2)) (.TraceEnd (Collision|BreakHitResult _outhit_2))))))))
                  (bind (_outhit_3 _returnvalue_14) (Collision|LineTraceByChannel _startlocation_2 _endlocation_2 "TraceTypeQuery1" false (Utilities|Array|MakeArray self (Components|GetOwner)) "None" true "(R=0.069618,G=0.000000,B=1.000000,A=1.000000)" "(R=0.855045,G=1.000000,B=0.000000,A=1.000000)" 0.5))
                  (if _returnvalue_14
                    (return _returnvalue_14 (.Location (Collision|BreakHitResult _outhit_3)) (.Location (Collision|BreakHitResult _outhit_3)))
                    (else
                      (return _returnvalue_14 (.TraceEnd (Collision|BreakHitResult _outhit_3)) (.TraceEnd (Collision|BreakHitResult _outhit_3))))))))))))))

(fn ControlLaserLocation
  (params (Hit :type Boolean) (Target :type Vector) (Impact :type Vector))
  (Rendering|SetVisibility (Variables|Default|GetNS_LaserImpact) Hit false)
  (Effects|Components|ParticleSystem|SetVectorParameter (Variables|Default|GetNS_Laser) "LaserEnd" Target)
  (if Hit
    (Transformation|SetWorldLocation (Variables|Default|GetNS_LaserImpact) Impact false true)))