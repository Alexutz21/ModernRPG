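; PC_Menu is the player controller for the main menu, creating the WBP_MainMenu widget on BeginPlay.
; After a zero-second delay it checks authority, so only the authority builds the menu, shows the cursor and switches to UI-only input focused on the widget.
; Remote instances just print an error advising Standalone net mode, as replication begins at the Lobby menu.
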(event Custom|CreateMenu
  ;[1 1 1] Create menu widget
  (bind _returnvalue (UserInterface|CreateWidget "/Game/ModernRPG/General/GUI/Widgets/MainMenu/WBP_MainMenu.WBP_MainMenu_C" self))
  (UserInterface|Viewport|AddtoViewport _returnvalue 0)
  (Variables|/Script/Engine.PlayerController|SetbShowMouseCursor self true)
  (Class|Widget|SetUserFocus _returnvalue self)
  (Input|SetInputModeUIOnly self _returnvalue "DoNotLock"))

(event EventBeginPlay
  ;[1 1 1] Create menu widget
  (Utilities|FlowControl|Delay 0.0)
  (Networking|SwitchHasAuthority
    (:Authority
      (CallFunction|CreateMenu))
    (:Remote
      (Development|PrintString "ERROR: Please, don't use menu on clients.  
Replicated part starts from Lobby menu.  
Change your net mode to Play Standalone. " true true "(R=1.000000,G=0.034472,B=0.000000,A=1.000000)" 1e+01))))

(fn ConstructionScript)