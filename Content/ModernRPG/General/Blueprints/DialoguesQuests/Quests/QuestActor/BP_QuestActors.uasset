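; BP_QuestActors is a world quest trigger that advances a quest subtask when a player reaches its sphere, on foot or as a vehicle driver.
; On overlap it takes that character as owner, then checks the subtask type and that their AC_QuestsHandler is exactly one step behind.
; It then calls SetNewQuestSubslotEveryone with the reward for multiplayer progress and hides its icon widget, which MarkArea can show.
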(event OnComponentBeginOverlap(Sphere)
  (params (OverlappedComponent :type Primitive%20Component%20Object%20Reference) (OtherActor :type Actor%20Object%20Reference) (OtherComp :type Primitive%20Component%20Object%20Reference) (OtherBodyIndex :type Integer) (bFromSweep :type Boolean) (SweepResult :type Hit%20Result%20Structure%20%28by%20ref%29))
  (bind _ac_questactor (Variables|Default|GetAC_QuestActor))
  (bind _ac_questactor_2 (Variables|Default|GetAC_QuestActor))
  (bind _ac_questactor_3 (Variables|Default|GetAC_QuestActor))
  (bind _currentquest (Variables|/Game/ModernRPG/General/Blueprints/DialoguesQuests/Quests/AC_QuestActor.AC_QuestActor_C|GetCurrentQuest _ac_questactor))
  (bind _currentquest_2 (Variables|/Game/ModernRPG/General/Blueprints/DialoguesQuests/Quests/AC_QuestActor.AC_QuestActor_C|GetCurrentQuest _ac_questactor_2))
  (bind _currentquest_3 (Variables|/Game/ModernRPG/General/Blueprints/DialoguesQuests/Quests/AC_QuestActor.AC_QuestActor_C|GetCurrentQuest _ac_questactor_3))
  (bind (_quest _marked _discovered _currentsubtask) (Utilities|Struct|BreakS_QuestDynam _currentquest_3))
  (bind (_quest_2 _marked_2 _discovered_2 _currentsubtask_2) (Utilities|Struct|BreakS_QuestDynam _currentquest_2))
  (bind (_quest_3 _marked_3 _discovered_3 _currentsubtask_3) (Utilities|Struct|BreakS_QuestDynam _currentquest))
  (bind _quest_4 (CallFunction|GetQuestInfo _quest_3))
  (bind _returnvalue (- _currentsubtask_3 1))
  (bind _subtasksname (Utilities|Struct|BreakS_QuestsMain _quest_4))
  (bind _output (Utilities|Array|Get(acopy) _subtasksname _returnvalue))
  (bind _type (Utilities|Struct|BreakS_SubtaskComplete _output))
  (bind _returnvalue_2 (Utilities|Enum|Equal(Enum) _type "NewEnumerator2"))
  ;[1 1 1] Multiplayered Overlap
  (bind _ascharacter (Utilities|Casting|CastToCharacter OtherActor)
    (:then
      (Utilities|IsValid (Actor|GetComponentbyClass _ascharacter "/Game/ModernRPG/General/Blueprints/DialoguesQuests/MapComponents/AC_QuestsHandler.AC_QuestsHandler_C")
        (:Is%20Valid
          (Actor|SetOwner _ascharacter)
          (if _returnvalue_2
            (bind (_res _outputpin) (CallFunction|SameQuest (Actor|GetComponentbyClass _ascharacter "/Game/ModernRPG/General/Blueprints/DialoguesQuests/MapComponents/AC_QuestsHandler.AC_QuestsHandler_C")))
            (if (and _res (== _outputpin (- (.CurrentSubTask (Utilities|Struct|BreakS_QuestDynam (Variables|/Game/ModernRPG/General/Blueprints/DialoguesQuests/Quests/AC_QuestActor.AC_QuestActor_C|GetCurrentQuest (Variables|Default|GetAC_QuestActor)))) 1)))
              (Default|SetNewQuestSubslotEveryone (Actor|GetComponentbyClass _ascharacter "/Game/ModernRPG/General/Blueprints/DialoguesQuests/MapComponents/AC_QuestsHandler.AC_QuestsHandler_C") _quest _currentsubtask (Variables|/Game/ModernRPG/General/Blueprints/DialoguesQuests/Quests/AC_QuestActor.AC_QuestActor_C|GetReward (Variables|Default|GetAC_QuestActor)))
              (CallFunction|UnmarkArea))))))
    (:CastFailed
      (bind _driver (Class|BPIVehicles|GetDriver(Message) OtherActor))
      (Utilities|IsValid _driver
        (:Is%20Valid
          (Utilities|IsValid (Actor|GetComponentbyClass _driver "/Game/ModernRPG/General/Blueprints/DialoguesQuests/MapComponents/AC_QuestsHandler.AC_QuestsHandler_C")
            (:Is%20Valid
              (Actor|SetOwner _driver)
              (if _returnvalue_2
                (bind (_res_2 _outputpin_2) (CallFunction|SameQuest (Actor|GetComponentbyClass _driver "/Game/ModernRPG/General/Blueprints/DialoguesQuests/MapComponents/AC_QuestsHandler.AC_QuestsHandler_C")))
                (if (and _res_2 (== _outputpin_2 (- (.CurrentSubTask (Utilities|Struct|BreakS_QuestDynam (Variables|/Game/ModernRPG/General/Blueprints/DialoguesQuests/Quests/AC_QuestActor.AC_QuestActor_C|GetCurrentQuest (Variables|Default|GetAC_QuestActor)))) 1)))
                  (Default|SetNewQuestSubslotEveryone (Actor|GetComponentbyClass _driver "/Game/ModernRPG/General/Blueprints/DialoguesQuests/MapComponents/AC_QuestsHandler.AC_QuestsHandler_C") _quest_2 _currentsubtask_2 (Variables|/Game/ModernRPG/General/Blueprints/DialoguesQuests/Quests/AC_QuestActor.AC_QuestActor_C|GetReward (Variables|Default|GetAC_QuestActor)))
                  (CallFunction|UnmarkArea))))))))))

(event EventBeginPlay
  ;[1 1 1] Multiplayered Overlap
  (Variables|/Game/ModernRPG/General/Blueprints/DialoguesQuests/Quests/AC_QuestActor.AC_QuestActor_C|SetCurrentQuest (Variables|Default|GetAC_QuestActor) (Utilities|Struct|MakeS_QuestDynam (Variables|Default|GetCurrentQuest) false false (Variables|Default|GetQuestSubtask) "(Actor_3_348972AC44C49AF3725683A39EE06BC7=None,Index_5_01C400D3483335F3258472B60A86882B=0)"))
  (bind _aswb_world_actor_widget (Utilities|Casting|CastToWB_WorldActorWidget (UserInterface|GetUserWidgetObject (Variables|Default|GetWidget))))
  (Default|Initialize _aswb_world_actor_widget (Variables|Default|GetItemTexture)))

(event EventMarkArea
  (params (Owner :type Actor%20Object%20Reference))
  ;[1 1 1] Mark
  (Rendering|SetVisibility (Variables|Default|GetWidget) true false))

(event EventUnmarkArea
  ;[1 1 1] Mark
  (Rendering|SetVisibility (Variables|Default|GetWidget) false false))

(fn ConstructionScript)

(fn SameQuest
  (params (Target :type AC%20Quests%20Handler%20Object%20Reference))
  (for _array_element (Variables|/Game/ModernRPG/General/Blueprints/DialoguesQuests/MapComponents/AC_QuestsHandler.AC_QuestsHandler_C|GetQuests Target)
    (if (Utilities|Name|Equal(Name) (.RowName (Utilities|Struct|BreakDataTableRowHandle (.Quest (Utilities|Struct|BreakS_QuestDynam _array_element)))) (.RowName (Utilities|Struct|BreakDataTableRowHandle (.Quest (Utilities|Struct|BreakS_QuestDynam (Variables|/Game/ModernRPG/General/Blueprints/DialoguesQuests/Quests/AC_QuestActor.AC_QuestActor_C|GetCurrentQuest (Variables|Default|GetAC_QuestActor)))))))
      (return true (.CurrentSubTask (Utilities|Struct|BreakS_QuestDynam _array_element)))))
  (return false 0))