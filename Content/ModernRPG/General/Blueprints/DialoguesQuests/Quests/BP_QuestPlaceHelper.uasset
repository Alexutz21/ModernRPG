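; Quest place marker actor that shows a widget at a quest location and hides it when the player is near.
; BeginPlay initializes the widget as WB_WorldActorWidget with a texture, actor and owner.
; SetNewLocation teleports the marker, updates the widget cast as WB_QuestPoint, and hides it if the owner is within the sphere radius.
; Player-controlled pawn overlaps toggle hiding, while separate events set widget visibility.
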(event OnComponentBeginOverlap(Sphere)
  (params (OverlappedComponent :type Primitive%20Component%20Object%20Reference) (OtherActor :type Actor%20Object%20Reference) (OtherComp :type Primitive%20Component%20Object%20Reference) (OtherBodyIndex :type Integer) (bFromSweep :type Boolean) (SweepResult :type Hit%20Result%20Structure%20%28by%20ref%29))
  (bind _aspawn (Utilities|Casting|CastToPawn OtherActor))
  (if (Pawn|IsPlayerControlled _aspawn)
    (Development|SetHiddeninGame (Variables|Default|GetWidget) true false)))

(event OnComponentEndOverlap(Sphere)
  (params (OverlappedComponent :type Primitive%20Component%20Object%20Reference) (OtherActor :type Actor%20Object%20Reference) (OtherComp :type Primitive%20Component%20Object%20Reference) (OtherBodyIndex :type Integer))
  (bind _aspawn (Utilities|Casting|CastToPawn OtherActor))
  (if (Pawn|IsPlayerControlled _aspawn)
    (Development|SetHiddeninGame (Variables|Default|GetWidget) false false)))

(event Custom|ToggleVisibility
  (params (bNewVisibility :type Boolean))
  ;[1 1 1] Toggle Vis
  (Rendering|SetVisibility (Variables|Default|GetWidget) bNewVisibility false))

(event Custom|ToggleVis
  (params (bNewVisibility :type Boolean))
  ;[1 1 1] Toggle Vis
  (Rendering|SetVisibility (Variables|Default|GetWidget) bNewVisibility false))

(event Custom|SetNewLocation
  (params (NewLocation :type Vector))
  ;[1 1 1] New Actor Location
  (Transformation|SetActorLocation NewLocation false true)
  (bind _aswb_quest_point (Utilities|Casting|CastToWB_QuestPoint (UserInterface|GetUserWidgetObject (Variables|Default|GetWidget))))
  (Variables|/Game/ModernRPG/General/GUI/Widgets/DialoguesQuests/Quests/WB_QuestPoint.WB_QuestPoint_C|SetLocation _aswb_quest_point NewLocation)
  (if (<= (Math|Vector|Distance(Vector) (Transformation|GetActorLocation) (Transformation|GetActorLocation (Components|GetOwner))) (Variables|/Script/Engine.SphereComponent|GetSphereRadius (Variables|Default|GetSphere)))
    (Development|SetHiddeninGame (Variables|Default|GetWidget) true false)))

(event EventBeginPlay
  (bind _aswb_world_actor_widget (Utilities|Casting|CastToWB_WorldActorWidget (UserInterface|GetUserWidgetObject (Variables|Default|GetWidget))))
  (Default|Initialize _aswb_world_actor_widget (Variables|Default|GetTexture))
  (Variables|/Game/ModernRPG/General/GUI/Widgets/WorldMap/WB_WorldActorWidget.WB_WorldActorWidget_C|SetActor _aswb_world_actor_widget self)
  (Variables|/Game/ModernRPG/General/GUI/Widgets/WorldMap/WB_WorldActorWidget.WB_WorldActorWidget_C|SetOwner _aswb_world_actor_widget (Components|GetOwner)))

(fn ConstructionScript)