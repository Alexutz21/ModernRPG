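; Lockpicking minigame actor that renders a 3D lock into a widget image through a scene capture, render target and dynamic material.
; Moving slides Device0 within a clamped range; its closeness to NeededLocation limits how far Device1 can rotate in steps.
; Full rotation reports success to the player's AC_LockedActor and destroys the actor; stopping reports failure, and PickBack eases rotation back with a timeline.
; Render target creation branches on authority through server and all-client events.
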(event Custom|MoveEvent
  (params (Value :type Vector%202D%20Structure))
  (bind _device_0 (Variables|Default|GetDevice_0))
  (bind _relativelocation (Variables|/Script/Engine.SceneComponent|GetRelativeLocation _device_0))
  ;[1 1 1] Move Event
  (Transformation|SetRelativeLocation (Variables|Default|GetDevice_0) (Math|Vector|MakeVector (.x _relativelocation) (Math|Float|Clamp(Float) (+ (.y _relativelocation) (/ (.y Value) 5.0)) -8e+01 -4e+01) (.z _relativelocation)) false false))

(event Custom|CreateRT%20Event
  (bind _scenecapturecomponent2d (Variables|Default|GetSceneCaptureComponent2D))
  ;[1 1 1] Create a render target
  (Networking|SwitchHasAuthority
    (:Authority
      (CallFunction|CreateRT-All _scenecapturecomponent2d))
    (:Remote
      (CallFunction|CreateRT-Server _scenecapturecomponent2d))))

(event Custom|CreateRT%20-%20Server
  (params (SceneCaptureComponent2D :type Scene%20Capture%20Component%202D%20Object%20Reference))
  ;[1 1 1] Create a render target
  (CallFunction|CreateRT-All SceneCaptureComponent2D))

(event Custom|TryToRotate
  (bind _device_1 (Variables|Default|GetDevice_1))
  (bind _device_1_2 (Variables|Default|GetDevice_1))
  (bind _relativerotation (Variables|/Script/Engine.SceneComponent|GetRelativeRotation _device_1))
  (bind (_roll _pitch _yaw) (Math|Rotator|BreakRotator _relativerotation))
  (bind _returnvalue (+ _pitch -5.0))
  ;[1 1 1] Try to rotate the lockpick
  (CallFunction|CalculateMaxRotation)
  (Audio|Components|Audio|Stop (Variables|Default|GetLerpBack))
  (if (>= _returnvalue (Variables|Default|GetDynamicStop))
    (Transformation|SetRelativeRotation _device_1_2 (Math|Rotator|MakeRotator _roll _returnvalue _yaw) false false)
    (if (<= (.Pitch (Math|Rotator|BreakRotator (Variables|/Script/Engine.SceneComponent|GetRelativeRotation _device_1_2))) -8e+01)
      (Default|EndUnlock (Actor|GetComponentbyClass (Class|UserWidget|GetOwningPlayerPawn (Variables|Default|GetWidget)) "/Game/ModernRPG/General/Blueprints/LockAndHead/Lock/AC_LockedActor.AC_LockedActor_C") true)
      (Transformation|SetRelativeRotation (Variables|Default|GetDevice_1) (Variables|Default|GetRememberStartRotation) false false)
      (Actor|DestroyActor))))

(event Custom|StopUnlocking
  ;[1 1 1] Stip Unlocking Process
  (Default|EndUnlock (Actor|GetComponentbyClass (Class|UserWidget|GetOwningPlayerPawn (Variables|Default|GetWidget)) "/Game/ModernRPG/General/Blueprints/LockAndHead/Lock/AC_LockedActor.AC_LockedActor_C") false)
  (Transformation|SetRelativeRotation (Variables|Default|GetDevice_1) (Variables|Default|GetRememberStartRotation) false false)
  (Actor|DestroyActor))

(event Custom|PickBack
  (bind _rememberstartrotation (Variables|Default|GetRememberStartRotation))
  (bind (_roll _pitch _yaw) (Math|Rotator|BreakRotator _rememberstartrotation))
  ;[1 1 1] Return Pick back
  (Variables|Default|SetRememberDynamicRotation (Variables|/Script/Engine.SceneComponent|GetRelativeRotation (Variables|Default|GetDevice_1)))
  (bind _alpha (Timeline|LerpBack PlayFromStart)
    (:Update
      (Transformation|SetRelativeRotation (Variables|Default|GetDevice_1) (Math|Rotator|Lerp(Rotator) (Math|Rotator|MakeRotator _roll (.pitch (Variables|Default|GetRememberDynamicRotation)) _yaw) _rememberstartrotation _alpha) false false))))

(event Custom|CalculateMaxRotation
  ;[1 1 1] Max Rotation
  (Variables|Default|SetDynamicStop (CallFunction|CalculateNewDynamicRotation)))

(event Custom|CreateRT-All
  (params (SceneCaptureComponent2D :type Scene%20Capture%20Component%202D%20Object%20Reference))
  ;[1 1 1] Create a render target
  (CallFunction|CreateRT SceneCaptureComponent2D))

(event Custom|Initialize
  (params (Widget :type WB%20Lockpicking%20Object%20Reference) (NeededLocation :type Float%20%28double-precision%29))
  ;[1 1 1] Initialize Blueprint
  (bind _output_get (Variables|Default|SetWidget Widget))
  (Variables|Default|SetNeededLocation NeededLocation)
  (Variables|Default|SetImage (Variables|/Game/ModernRPG/General/GUI/WB_Lockpicking.WB_Lockpicking_C|GetImg_LockRendering _output_get))
  (CallFunction|CreateRTEvent))

(event EventBeginPlay
  ;[1 1 1] Initialize start rotation
  (Variables|Default|SetRememberStartRotation (Variables|/Script/Engine.SceneComponent|GetRelativeRotation (Variables|Default|GetDevice_0))))

(fn ConstructionScript)

(fn CalculateNewDynamicRotation
  (return (* (Math|Float|Absolute(Float) (- 9e+01 (* (Math|Float|Absolute(Float) (- 1.0 (/ (Math|Float|Absolute(Float) (Variables|Default|GetNeededLocation)) (Math|Float|Absolute(Float) (.y (Variables|/Script/Engine.SceneComponent|GetRelativeLocation (Variables|Default|GetDevice_0))))))) 1e+02))) -1.0)))

(fn CreateRT
  (params (SceneCaptureComponent2D%20loc :type Scene%20Capture%20Component%202D%20Object%20Reference))
  (bind _image (Variables|Default|GetImage))
  (bind _brush (Variables|/Script/UMG.Image|GetBrush _image))
  (Utilities|IsValid SceneCaptureComponent2D%20loc
    (:Is%20Valid
      (Components|Activation|Activate SceneCaptureComponent2D%20loc false)
      (bind _returnvalue (Rendering|CreateRenderTarget2D 1920 1920 "RTF_RGBA16f"))
      (Variables|/Script/Engine.SceneCaptureComponent2D|SetTextureTarget SceneCaptureComponent2D%20loc _returnvalue)
      (Utilities|IsValid (Variables|Default|GetDynamicMaterial)
        (:Is%20Valid
          (Rendering|Material|SetTextureParameterValue (Variables|Default|GetDynamicMaterial) "Render" (Variables|/Script/Engine.SceneCaptureComponent2D|GetTextureTarget SceneCaptureComponent2D%20loc)))
        (:Is%20Not%20Valid
          (Utilities|IsValid (Variables|Default|GetImage)
            (:Is%20Valid
              (bind _returnvalue_2 (Rendering|Material|CreateDynamicMaterialInstance "/Game/ModernRPG/Shooter/Materials/M_RenderLock.M_RenderLock" "None" "None" :!class /Script/Engine.KismetMaterialLibrary))
              (bind _output_get (Variables|Default|SetDynamicMaterial _returnvalue_2))
              (Class|Image|SetBrush _image (Utilities|Struct|MakeSlateBrush (.imagesize _brush) (.margin _brush) (.tintcolor _brush) "(CornerRadii=(X=0.000000,Y=0.000000,Z=0.000000,W=1.000000),Color=(SpecifiedColor=(R=0.000000,G=0.000000,B=0.000000,A=0.000000),ColorUseRule=UseColor_Specified),Width=0.000000,RoundingType=HalfHeightRadius,bUseBrushTransparency=False)" _output_get (.drawas _brush) (.tiling _brush) (.mirroring _brush)))
              (Class|Image|SetBrushfromMaterial (Variables|Default|GetImage) (Variables|Default|GetDynamicMaterial))
              (Rendering|Material|SetTextureParameterValue (Variables|Default|GetDynamicMaterial) "Render" (Variables|/Script/Engine.SceneCaptureComponent2D|GetTextureTarget SceneCaptureComponent2D%20loc))
              (return))
            (:Is%20Not%20Valid
              (return))))))))