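; Combat assist component that turns and pulls the owning player toward an enemy.
; StartHelper keeps a valid target or takes one from AC_FocusTarget, otherwise sphere-tracing for the living, visible, non-player pawn nearest the owner's facing angle.
; While enabled, Tick interpolates control yaw toward the target and teleport-steps the owner to within a maximum distance, allowing for target mesh size.
; StopHelper disables Tick without clearing the target.
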(event EventTick
  (params (DeltaSeconds :type Float%20%28single-precision%29))
  ;[1 1 1] Move player to target
  (if (Variables|Default|GetbShouldRotate)
    (CallFunction|RotatePlayer))
  (if (Variables|Default|GetbShouldMove)
    (CallFunction|MovePlayer)))

(fn GetEnemies
  (bind (_outhits _returnvalue) (Collision|MultiSphereTraceForObjects (Transformation|GetActorLocation (Components|GetOwner)) (+ (Transformation|GetActorLocation (Components|GetOwner)) 1) (Variables|Settings|GetEnemiesSphere) (Utilities|Array|MakeArray "ObjectTypeQuery3") false (Utilities|Array|MakeArray (Components|GetOwner)) "None"))
  (if _returnvalue
    (return _outhits)))

(fn StartHelper
  (params (bShouldRotate :type Boolean) (bShouldMove :type Boolean))
  (Variables|Default|SetbShouldRotate bShouldRotate)
  (Variables|Default|SetbShouldMove bShouldMove)
  (if (CallFunction|CanTarget (Variables|Default|GetCurrentTarget))
    (Components|Tick|SetComponentTickEnabled true)
    (else
      (bind _output_get (Variables|Default|SetCurrentTarget (CallFunction|FindTarget)))
      (Components|Tick|SetComponentTickEnabled (Utilities|IsValid _output_get)))))

(fn StopHelper
  (Components|Tick|SetComponentTickEnabled false))

(fn RotatePlayer
  (LocalVariables|SetTargetRotation (Math|Rotator|FindLookatRotation (Transformation|GetActorLocation (Components|GetOwner)) (Transformation|GetActorLocation (Variables|Default|GetCurrentTarget))))
  (bind _aspawn (Utilities|Casting|CastToPawn (Components|GetOwner)))
  (LocalVariables|SetPawnTarget _aspawn)
  (bind _asplayer_controller (Utilities|Casting|CastToPlayerController (Pawn|GetController _aspawn)))
  (LocalVariables|SetPlayerController _asplayer_controller)
  (bind _output_get (LocalVariables|SetNewRotation (Math|Interpolation|RInterpTo (Transformation|GetActorRotation (LocalVariables|GetPawnTarget)) (LocalVariables|GetTargetRotation) (Utilities|Time|GetWorldDeltaSeconds) (Variables|Settings|GetInterpRotation))))
  (Pawn|SetControlRotation (LocalVariables|GetPlayerController) (Math|Rotator|MakeRotator (.roll (Pawn|GetControlRotation (LocalVariables|GetPlayerController) :!class /Script/Engine.Controller)) (.pitch (Pawn|GetControlRotation (LocalVariables|GetPlayerController) :!class /Script/Engine.Controller)) (.Yaw (Math|Rotator|BreakRotator _output_get)))))

(fn MovePlayer
  (bind _currenttarget (Variables|Default|GetCurrentTarget))
  (bind _returnvalue (Actor|GetComponentbyClass _currenttarget "/Script/Engine.SkeletalMeshComponent"))
  (bind _boxextent (Collision|GetComponentBounds _returnvalue))
  (bind (_x _y) (Math|Vector|BreakVector _boxextent))
  (LocalVariables|SetTargetSize (/ (+ _x _y) 2.0))
  (bind _output_get (LocalVariables|SetDistance (- (Transformation|GetDistanceTo (Variables|Default|GetCurrentTarget) (Components|GetOwner)) (LocalVariables|GetTargetSize))))
  (if (> _output_get (Variables|Settings|GetMaxDistanceToTarget))
    (LocalVariables|SetUnitVector (Math|Vector|GetUnitDirection(Vector) (Transformation|GetActorLocation (Components|GetOwner)) (Transformation|GetActorLocation (Variables|Default|GetCurrentTarget))))
    (bind _output_get_2 (LocalVariables|SetNewLocation (+ (Transformation|GetActorLocation (Components|GetOwner)) (* (LocalVariables|GetUnitVector) (- (LocalVariables|GetDistance) (Variables|Settings|GetMaxDistanceToTarget))))))
    (Transformation|SetActorLocation (Components|GetOwner) (Math|Interpolation|VInterpTo (Transformation|GetActorLocation (Components|GetOwner)) _output_get_2 (Utilities|Time|GetWorldDeltaSeconds) (Variables|Settings|GetInterpLocation)) false true)))

(fn CheckVisibility
  (params (Target :type Actor%20Object%20Reference))
  (bind _returnvalue (Collision|LineTraceByChannel (Transformation|GetSocketLocation (Actor|GetComponentbyClass Target "/Script/Engine.SkeletalMeshComponent") "head") (Transformation|GetSocketLocation (Actor|GetComponentbyClass (Components|GetOwner) "/Script/Engine.SkeletalMeshComponent") "head") "TraceTypeQuery2" false (Utilities|Array|MakeArray Target (Components|GetOwner)) "None"))
  (return (not _returnvalue)))

(fn CanTarget
  (params (Target :type Actor%20Object%20Reference))
  (bind _aspawn (Utilities|Casting|CastToPawn Target))
  (bind _result (Class|BPICharacter|IsAlive?(Message) _aspawn))
  (return (Math|Boolean|ANDBoolean _result (not (Pawn|IsPlayerControlled _aspawn)) (CallFunction|CheckVisibility _aspawn) (< (CallFunction|CheckRadius _aspawn) (Variables|Settings|GetMaxRadiusToTarget)))))

(fn CheckRadius
  (params (Target :type Actor%20Object%20Reference))
  (bind _returnvalue (Transformation|GetActorLocation Target))
  (bind _returnvalue_2 (Components|GetOwner))
  (bind _returnvalue_3 (Transformation|GetActorLocation _returnvalue_2))
  (bind _returnvalue_4 (Transformation|GetActorRotation _returnvalue_2))
  (bind _returnvalue_5 (Math|Rotator|FindLookatRotation _returnvalue _returnvalue_3))
  (bind _returnvalue_6 (Math|Rotator|Delta(Rotator) _returnvalue_5 _returnvalue_4))
  (return (Math|Float|Absolute(Float) (* (- 1.8e+02 (Math|Float|Absolute(Float) (.yaw _returnvalue_6))) (Math|Float|Sign(Float) (.yaw _returnvalue_6))))))

(fn FindTarget
  (bind _returnvalue (Components|GetOwner))
  (bind _returnvalue_2 (Actor|GetComponentbyClass _returnvalue "/Game/ModernRPG/General/Blueprints/Combat/AC_FocusTarget.AC_FocusTarget_C"))
  (if (Default|HasTarget _returnvalue_2)
    (bind _aspawn (Utilities|Casting|CastToPawn (Variables|/Game/ModernRPG/General/Blueprints/Combat/AC_FocusTarget.AC_FocusTarget_C|GetCurrentTarget _returnvalue_2)))
    (return _aspawn)
    (else
      (bind _output_get (LocalVariables|SetEnemies (CallFunction|GetEnemies)))
      (LocalVariables|SetMinRadius 1.8e+02)
      (if (Utilities|Array|IsNotEmpty _output_get)
        (for _array_element (LocalVariables|GetEnemies)
          (bind _output_get_2 (LocalVariables|SetTestTarget (.HitActor (Collision|BreakHitResult _array_element))))
          (Utilities|IsValid _output_get_2
            (:Is%20Valid
              (if (CallFunction|CanTarget (LocalVariables|GetTestTarget))
                (if (< (CallFunction|CheckRadius (LocalVariables|GetTestTarget)) (LocalVariables|GetMinRadius))
                  (LocalVariables|SetBestTarget (LocalVariables|GetTestTarget))
                  (LocalVariables|SetMinRadius (CallFunction|CheckRadius (LocalVariables|GetTestTarget))))))))
        (bind _aspawn_2 (Utilities|Casting|CastToPawn (LocalVariables|GetBestTarget)))
        (return _aspawn_2)
        (else
          (return 0))))))

(fn TraceGround
  (params (NewLocation :type Vector))
  (bind (_outhit _returnvalue) (Collision|LineTraceForObjects (+ NewLocation "0,0,100.000000") (+ NewLocation "0,0,-200.000000") (Utilities|Array|MakeArray "ObjectTypeQuery1") false (Utilities|Array|MakeArray (Components|GetOwner)) "None"))
  (return (select _returnvalue (.Location (Collision|BreakHitResult _outhit)) NewLocation)))