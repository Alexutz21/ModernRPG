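; Lock-on targeting component that toggles focus on a BP_I_Focusable actor and turns its owning character and control rotation toward it.
; Targeting picks among living, on-screen, in-range, unobstructed actors by horizontal closeness to screen center.
; Tick interpolates rotation, releasing the lock on death or excess distance; ControllerState adds pitch tracking and blocks look input.
; Movement rotation settings are saved, switched via server-to-multicast RPCs, then restored locally on release.
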(event Custom|SpawnHelper
  ;[1 1 1] Spawn Helper
  (bind _returnvalue (Game|SpawnActorfromClass "/Game/ModernRPG/General/Blueprints/Combat/BP_ArrowHelper.BP_ArrowHelper_C" (Math|Transform|MakeTransform "0, 0, 0" "0, 0, 0" "1.000000,1.000000,1.000000") "Undefined" 0 0))
  (Variables|Default|SetArrowComponent (Variables|/Game/ModernRPG/General/Blueprints/Combat/BP_ArrowHelper.BP_ArrowHelper_C|GetDirection _returnvalue))
  (Transformation|AttachActorToActor _returnvalue (Components|GetOwner) "None" "SnapToTarget" "SnapToTarget" "SnapToTarget" true))

(event Custom|SelectReplicated
  (params (Condition :type Boolean) (Target :type Object%20Object%20Reference))
  ;[1 1 1] Replicate Toggle Aim Point
  (if (Ability|HasAuthority (Components|GetOwner))
    (CallFunction|SelectReplicated-OC Condition Target)
    (else
      (CallFunction|SelectReplicated-Server Condition Target))))

(event Custom|SelectReplicated%20-Server
  (params (Condition :type Boolean) (Target :type Object%20Object%20Reference))
  ;[1 1 1] Replicate Toggle Aim Point
  (CallFunction|SelectReplicated-OC Condition Target))

(event Custom|SelectReplicated%20-OC
  (params (Condition :type Boolean) (Target :type Object%20Object%20Reference))
  (bind _returnvalue (Components|GetOwner))
  ;[1 1 1] Replicate Toggle Aim Point
  (if Condition
    (Class|BPIFocusable|OnSelected(Message) Target _returnvalue)
    (else
      (Class|BPIFocusable|OnDeselected(Message) Target _returnvalue))))

(event Custom|ToggleActive%20-Server
  (params (Selection :type E_RotationType%20Enum :default "NewEnumerator0"))
  ;[1 1 1] Toggle Active
  (CallFunction|ToggleActive-ALL Selection))

(event Custom|ToggleActive%20-ALL
  (params (Selection :type E_RotationType%20Enum :default "NewEnumerator0"))
  (bind _owner (Variables|Default|GetOwner))
  (bind _owner_2 (Variables|Default|GetOwner))
  (bind _charactermovement (Variables|/Script/Engine.Character|GetCharacterMovement _owner_2))
  (bind _charactermovement_2 (Variables|/Script/Engine.Character|GetCharacterMovement _owner))
  ;[1 1 1] Toggle Active
  (switch Utilities|FlowControl|Switch|SwitchonE_RotationType Selection
    (:NewEnumerator0
      (Variables|/Script/Engine.Pawn|SetbUseControllerRotationYaw _owner_2 false)
      (Variables|/Script/Engine.CharacterMovementComponent|SetbUseControllerDesiredRotation _charactermovement true)
      (Variables|/Script/Engine.CharacterMovementComponent|SetbOrientRotationToMovement _charactermovement false))
    (:NewEnumerator1
      (Variables|/Script/Engine.Pawn|SetbUseControllerRotationYaw _owner false)
      (Variables|/Script/Engine.CharacterMovementComponent|SetbUseControllerDesiredRotation _charactermovement_2 (Variables|RememberSettings|GetController))
      (Variables|/Script/Engine.CharacterMovementComponent|SetbOrientRotationToMovement _charactermovement_2 true))))

(event EventBeginPlay
  ;[1 1 1] Initialize Component
  (CallFunction|SpawnHelper)
  (bind _ascharacter (Utilities|Casting|CastToCharacter (Components|GetOwner)))
  (bind _output_get (Variables|Default|SetOwner _ascharacter))
  (bind _asplayer_controller (Utilities|Casting|CastToPlayerController (Pawn|GetController _output_get)))
  (Variables|Default|SetPlayerController _asplayer_controller))

(event EventTick
  (params (DeltaSeconds :type Float%20%28single-precision%29))
  (bind _returnvalue (Components|GetOwner))
  (bind _returnvalue_2 (Components|GetOwner))
  (bind _currenttarget (Variables|Default|GetCurrentTarget))
  (bind _currenttarget_2 (Variables|Default|GetCurrentTarget))
  (bind _controllerstate (Variables|Default|GetControllerState))
  (bind _returnvalue_3 (Transformation|GetActorLocation _returnvalue))
  (bind _returnvalue_4 (Transformation|GetActorLocation _currenttarget))
  (bind _returnvalue_5 (Transformation|GetDistanceTo _returnvalue_2 _currenttarget_2))
  (bind _instigator (Variables|/Script/Engine.Actor|GetInstigator _returnvalue))
  (bind _returnvalue_6 (- _returnvalue_4 "0, 0,50.000000"))
  (bind _returnvalue_7 (Pawn|GetControlRotation _instigator :!class /Script/Engine.Pawn))
  (bind _returnvalue_8 (Pawn|GetController _instigator))
  (bind _returnvalue_9 (Math|Rotator|FindLookatRotation _returnvalue_3 _returnvalue_6))
  ;[1 1 1] Change Controll Rotation if the target is enabled
  (if (CallFunction|HasTarget)
    (bind _result (Class|BPICharacter|IsAlive?(Message) (Variables|Default|GetCurrentTarget)))
    (if (Math|Boolean|ANDBoolean (>= _returnvalue_5 0.0) (<= _returnvalue_5 (Variables|Default|GetDistanceToTarget)) _result)
      (Utilities|IsValid (Variables|Default|GetArrowComponent)
        (:Is%20Valid
          (Utilities|IsValid _returnvalue_8
            (:Is%20Valid
              _)))
        (:Is%20Not%20Valid
          _))
      (Pawn|SetControlRotation _returnvalue_8 (Class|KismetMathLibrary|RInterptoConstant (Pawn|GetControlRotation _instigator :!class /Script/Engine.Pawn) (Math|Rotator|MakeRotator (select _controllerstate (.roll _returnvalue_9) (.roll _returnvalue_7)) (select _controllerstate (.pitch _returnvalue_9) (.pitch _returnvalue_7)) (.yaw _returnvalue_9)) (Utilities|Time|GetWorldDeltaSeconds) 3e+02))
      (else
        (Camera|RemoveLock)))))

(fn FindTarget
  (bind _outactors (Actor|GetAllActorswithInterface "/Game/ModernRPG/General/Blueprints/Combat/AI/BP_I_Focusable.BP_I_Focusable_C"))
  (for _array_element _outactors
    (bind _output_get (LocalVariables|SetL_Target _array_element))
    (if (CallFunction|CanbeTargetedRightNow _output_get)
      (Utilities|Array|Add (LocalVariables|GetL_Targets) (LocalVariables|GetL_Target))))
  (for (_array_element_2 _array_index) (LocalVariables|GetL_Targets)
    (LocalVariables|SetL_Target _array_element_2)
    (if (== _array_index 0)
      (LocalVariables|SetL_Distance (Math|Float|Absolute(Float) (- (.X (Math|Vector2D|BreakVector2D (.ScreenPosition (Class|GameplayStatics|ProjectWorldtoScreen (Variables|Default|GetPlayerController) (Transformation|GetActorLocation (LocalVariables|GetL_Target)) false)))) (/ (.x (Viewport|GetViewportSize)) 2.0))) :!label _label)
      (Variables|Default|SetCurrentTarget (LocalVariables|GetL_Target))
      (Components|Tick|SetComponentTickEnabled true)
      (elif (< (Math|Float|Absolute(Float) (- (.X (Math|Vector2D|BreakVector2D (.ScreenPosition (Class|GameplayStatics|ProjectWorldtoScreen (Variables|Default|GetPlayerController) (Transformation|GetActorLocation (LocalVariables|GetL_Target)) false)))) (/ (.x (Viewport|GetViewportSize)) 2.0))) (LocalVariables|GetL_Distance))
        (goto _label))))
  (Utilities|IsValid (Variables|Default|GetCurrentTarget)
    (:Is%20Valid
      (TargetingEvents|EnableTarget))))

(fn EnableTarget
  (Remember|RememberStats)
  (CallFunction|SelectReplicated true (Variables|Default|GetCurrentTarget))
  (CallFunction|ToggleLockMode "NewEnumerator0")
  (bind _returnvalue (Utilities|Time|SetTimerbyFunctionName 0 "SelectTarget" 0.15 true))
  (Variables|Default|SetTimer _returnvalue)
  (if (and (Variables|Default|GetControllerState) (Utilities|IsValid (Variables|Default|GetOwner)))
    (Input|SetIgnoreLookInput (Pawn|GetController (Variables|Default|GetOwner)) true)))

(fn RemoveLock
  (CallFunction|SelectReplicated false (Variables|Default|GetCurrentTarget))
  (Variables|Default|SetCurrentTarget 0)
  (Components|Tick|SetComponentTickEnabled false)
  (Remember|RestoreStats)
  (Utilities|Time|ClearandInvalidateTimerbyHandle (Variables|Default|GetTimer))
  (if (and (Variables|Default|GetControllerState) (Utilities|IsValid (Variables|Default|GetOwner)))
    (Input|SetIgnoreLookInput (Pawn|GetController (Variables|Default|GetOwner)) false)))

(fn ToggleTargeting
  (if (CallFunction|HasTarget)
    (Camera|RemoveLock)
    (else
      (TargetingEvents|FindTarget))))

(fn RememberStats
  (Utilities|IsValid (Variables|Default|GetOwner)
    (:Is%20Valid
      (Variables|RememberSettings|SetYaw (Variables|/Script/Engine.Pawn|GetbUseControllerRotationYaw (Variables|Default|GetOwner)))
      (Variables|RememberSettings|SetMovement (Variables|/Script/Engine.CharacterMovementComponent|GetbOrientRotationToMovement (Variables|/Script/Engine.Character|GetCharacterMovement (Variables|Default|GetOwner))))
      (Variables|RememberSettings|SetController (Variables|/Script/Engine.CharacterMovementComponent|GetbUseControllerDesiredRotation (Variables|/Script/Engine.Character|GetCharacterMovement (Variables|Default|GetOwner)))))))

(fn ToggleLockMode
  (params (Mode :type E_RotationType%20Enum :default "NewEnumerator0"))
  (if (Ability|HasAuthority (Components|GetOwner))
    (CallFunction|ToggleActive-ALL Mode)
    (else
      (CallFunction|ToggleActive-Server Mode))))

(fn RestoreStats
  (Utilities|IsValid (Variables|Default|GetOwner)
    (:Is%20Valid
      (Variables|/Script/Engine.Pawn|SetbUseControllerRotationYaw (Variables|Default|GetOwner) (Variables|RememberSettings|GetYaw))
      (Variables|/Script/Engine.CharacterMovementComponent|SetbUseControllerDesiredRotation (Variables|/Script/Engine.Character|GetCharacterMovement (Variables|Default|GetOwner)) (Variables|RememberSettings|GetController))
      (Variables|/Script/Engine.CharacterMovementComponent|SetbOrientRotationToMovement (Variables|/Script/Engine.Character|GetCharacterMovement (Variables|Default|GetOwner)) (Variables|RememberSettings|GetMovement)))))

(fn HasTarget
  (return (Utilities|IsValid (Variables|Default|GetCurrentTarget))))

(fn SetTargetActive
  (Camera|RemoveLock)
  (TargetingEvents|FindTarget))

(fn CanbeTargetedRightNow
  (params (Target :type Actor%20Object%20Reference))
  (bind _returnvalue (Transformation|GetActorLocation Target))
  (bind _returnvalue_2 (Viewport|GetViewportSize))
  (bind _playercontroller (Variables|Default|GetPlayerController))
  (bind (_x _y) (Math|Vector2D|BreakVector2D _returnvalue_2))
  (bind (_screenposition _returnvalue_3) (Class|GameplayStatics|ProjectWorldtoScreen _playercontroller _returnvalue false))
  (bind (_x_2 _y_2) (Math|Vector2D|BreakVector2D _screenposition))
  (bind _result (Class|BPICharacter|IsAlive?(Message) Target))
  (if (Math|Boolean|ANDBoolean _result (not (CallFunction|HaveAnythingBetween Target)) (!= (Components|GetOwner) Target))
    (return (Math|Boolean|ANDBoolean (Math|Boolean|ANDBoolean (> _x_2 0.0) (> _y_2 0.0) (<= _x_2 _x) (<= _y_2 _y)) _returnvalue_3 (<= (Transformation|GetDistanceTo (Components|GetOwner) Target) (Variables|Default|GetDistanceToTarget))))
    (else
      (return false))))

(fn HaveAnythingBetween
  (params (Target :type Actor%20Object%20Reference))
  (bind _returnvalue (Components|GetOwner))
  (bind _returnvalue_2 (Collision|LineTraceByChannel (Transformation|GetActorLocation Target) (Transformation|GetActorLocation _returnvalue) "TraceTypeQuery1" false (Utilities|Array|MakeArray Target _returnvalue) "None"))
  (return _returnvalue_2))