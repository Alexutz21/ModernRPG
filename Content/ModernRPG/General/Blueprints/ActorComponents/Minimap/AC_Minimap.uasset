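; AC_Minimap is an actor component that populates the owner's minimap UI with icons for AI actors.
; On Initialize it gets the optimized minimap widget and its overlay through the owner's main widget handler component.
; It queries every other BP_I_AI actor and, for those allowed to be visible, creates a styled, rotation-following icon widget.
; Each icon starts centered and hidden in the overlay and is registered in the minimap's included-actors list.
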(event Custom|Initialize
  (bind (_overlay _wb_minimap_optimized) (CallFunction|GetMinimapOverlay))
  (Variables|Default|SetMinimapOverlay _overlay)
  (Variables|Default|SetWB%20Minimap%20Optimized _wb_minimap_optimized)
  (bind _outactors (Actor|GetAllActorswithInterface "/Game/ModernRPG/General/Blueprints/Interfaces/BP_I_AI.BP_I_AI_C"))
  (for _array_element _outactors
    (if (!= _array_element (Components|GetOwner))
      (bind (_i_can_be_visible _onminimapicon _onminimapiconcolor _size) (Class|BPIAI|OnPlayerMinimapState(Message) _array_element))
      (if _i_can_be_visible
        (bind _returnvalue (UserInterface|CreateWidget "/Game/ModernRPG/General/GUI/Widgets/Buttons/Minimap/WB_ActorOnMinimap.WB_ActorOnMinimap_C" 0 _onminimapicon _array_element true _onminimapiconcolor _size))
        (bind _returnvalue_2 (Class|Overlay|AddChildtoOverlay (Variables|Default|GetMinimapOverlay) _returnvalue))
        (bind _output_get (Variables|/Game/ModernRPG/General/GUI/Widgets/Buttons/Minimap/WB_ActorOnMinimap.WB_ActorOnMinimap_C|SetMyOverlaySlot _returnvalue _returnvalue_2))
        (Layout|GridSlot|SetVerticalAlignment _output_get "VAlign_Center")
        (Layout|GridSlot|SetHorizontalAlignment _output_get "HAlign_Center")
        (Widget|SetVisibility _returnvalue "Hidden")
        (Utilities|Array|AddUnique (Variables|/Game/ModernRPG/General/GUI/Widgets/Buttons/Minimap/WB_Minimap_Optimized.WB_Minimap_Optimized_C|GetIncludedActors (Variables|Default|GetWB%20Minimap%20Optimized)) _returnvalue)))))

(fn GetMinimapOverlay
  (bind _returnvalue (Components|GetOwner))
  (bind _returnvalue_2 (Actor|GetComponentbyClass _returnvalue "/Game/ModernRPG/General/Blueprints/DialoguesQuests/WidgetHandler/AC_MainWidgetHandler.AC_MainWidgetHandler_C"))
  (bind _castedmainui (Variables|/Game/ModernRPG/General/Blueprints/DialoguesQuests/WidgetHandler/AC_MainWidgetHandler.AC_MainWidgetHandler_C|GetCastedMainUI _returnvalue_2))
  (bind _wb_minimap_optimized (Variables|/Game/ModernRPG/General/GUI/Widgets/WB_MainUI.WB_MainUI_C|GetWB_Minimap_Optimized _castedmainui))
  (Utilities|IsValid _castedmainui
    (:Is%20Valid
      (return (Variables|/Game/ModernRPG/General/GUI/Widgets/Buttons/Minimap/WB_Minimap_Optimized.WB_Minimap_Optimized_C|GetOverlay _wb_minimap_optimized) _wb_minimap_optimized))))