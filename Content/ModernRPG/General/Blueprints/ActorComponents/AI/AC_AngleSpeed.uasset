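; Actor component that derives a speed value for its owning Character from the slope it is moving along.
; AngleSpeedPerc only computes when the Character is moving and not falling.
; It feeds the pitch from the previous to the current location into SpeedCurve, then stores the new location.
; A downward trace checks for Landscape, but both branches are empty, so it does not affect the result.
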(event EventBeginPlay
  ;[1 1 1] Set New Owner
  (bind _ascharacter (Utilities|Casting|CastToCharacter (Components|GetOwner)))
  (Variables|Default|SetOwner _ascharacter))

(fn AngleSpeedPerc
  (if (CallFunction|ShouldUpdateSpeed)
    (return (CallFunction|GetNewSpeed(Angle)))))

(fn ShouldUpdateSpeed
  (bind _owner (Variables|Default|GetOwner))
  (return (and (not (AI|Components|NavMovement|IsFalling (Variables|/Script/Engine.Character|GetCharacterMovement _owner))) (!= (Math|Vector|VectorLength (Transformation|GetVelocity _owner)) 0.0))))

(fn GetNewSpeed(Angle)
  (bind _returnvalue (Components|GetOwner))
  (bind _returnvalue_2 (Transformation|GetActorLocation _returnvalue))
  (bind (_x _y _z) (Math|Vector|BreakVector _returnvalue_2))
  (bind _outhit (Collision|LineTraceByChannel _returnvalue_2 (Math|Vector|MakeVector _x _y (- _z 1e+03)) "TraceTypeQuery2" false (Utilities|Array|MakeArray (Components|GetOwner)) "None"))
  (if (== (Utilities|GetClass (.HitActor (Collision|BreakHitResult _outhit))) "/Script/Landscape.Landscape")
    _
    (else
      _))
  (LocalVariables|SetSpeed (Math|Curves|GetFloatValue (Variables|Setup|GetSpeedCurve) (.Pitch (Math|Rotator|BreakRotator (Math|Rotator|FindLookatRotation (Variables|Default|GetPreviousLocation) (Transformation|GetActorLocation (Variables|Default|GetOwner)))))))
  (Variables|Default|SetPreviousLocation (Transformation|GetActorLocation (Variables|Default|GetOwner)))
  (return (LocalVariables|GetSpeed)))