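; AC_FightHandler is an actor component that tracks whether its owner is in a fight by keeping a list of unique enemies.
; The first AddEnemy and the RemoveEnemy that empties the list switch music through the owner's AC_AudioManager, updating the InFightEvent flag only when that component exists.
; InFight reports whether any enemies remain, and a debug print of that state and the count is left disconnected from Tick.
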(event Custom|AddEnemy
  (params (Owner :type Actor%20Object%20Reference))
  (bind _returnvalue (Components|GetOwner))
  (bind _returnvalue_2 (Actor|GetComponentbyClass _returnvalue "/Game/ModernRPG/General/Blueprints/ActorComponents/Audio/AC_AudioManager.AC_AudioManager_C"))
  ;[1 1 1] Changes
  (Utilities|Array|AddUnique (Variables|Default|GetEnemies) Owner)
  (if (not (Variables|Default|GetInFightEvent))
    (Utilities|IsValid _returnvalue_2
      (:Is%20Valid
        (Default|SwitchMusic-Server _returnvalue_2 "NewEnumerator1")
        (Variables|Default|SetInFightEvent true)))))

(event Custom|RemoveEnemy
  (params (Owner :type Actor%20Object%20Reference))
  (bind _returnvalue (Components|GetOwner))
  (bind _returnvalue_2 (Actor|GetComponentbyClass _returnvalue "/Game/ModernRPG/General/Blueprints/ActorComponents/Audio/AC_AudioManager.AC_AudioManager_C"))
  ;[1 1 1] Changes
  (Utilities|Array|RemoveItem (Variables|Default|GetEnemies) Owner)
  (if (not (CallFunction|InFight))
    (Utilities|IsValid _returnvalue_2
      (:Is%20Valid
        (Default|SwitchMusic-Server _returnvalue_2 "NewEnumerator0")
        (Variables|Default|SetInFightEvent false)))))

(event EventTick
  (params (DeltaSeconds :type Float%20%28single-precision%29))
  ;[1 1 1] Connect if you need to debug
)

(fn InFight
  (return (> (Utilities|Array|Length (Variables|Default|GetEnemies)) 0)))

(fn DebuginFight
  (Development|PrintString (Utilities|String|Append (Utilities|String|ToString(Boolean) (CallFunction|InFight)) " " (Utilities|String|ToString(Integer) (Utilities|Array|Length (Variables|Default|GetEnemies)))) true true "(R=0.000000,G=0.660000,B=1.000000,A=1.000000)" 0.0))