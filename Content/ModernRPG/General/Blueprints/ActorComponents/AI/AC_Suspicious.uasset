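; AC_Suspicious is an AI-related actor component that tracks a suspicion value and shows it through a WB_Suspicious widget.
; On BeginPlay, a server event calls an owning-client event that creates the widget and adds it to the viewport.
; SetLocationAndValue accumulates suspicion, passes value and location to the widget until the widget's value reaches one, and returns whether the component's total has reached that threshold.
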(event Custom|CreateSuspWidget%20-Server
  ;[1 1 1] Create Widget on Client
  (CallFunction|CreateSuspWidget-OC))

(event Custom|CreateSuspWidget%20-OC
  ;[1 1 1] Create Widget on Client
  (bind _returnvalue (UserInterface|CreateWidget "/Game/ModernRPG/General/GUI/Widgets/WB_Suspicious.WB_Suspicious_C"))
  (Utilities|IsValid _returnvalue
    (:Is%20Valid
      (UserInterface|Viewport|AddtoViewport _returnvalue 0)
      (Variables|Default|SetSuspWidget _returnvalue))))

(event EventBeginPlay
  ;[1 1 1] Create Widget on Client
  (CallFunction|CreateSuspWidget-Server))

(fn SetLocationandValue
  (params (Value :type Float%20%28double-precision%29) (Location :type Vector))
  (bind _suspwidget (Variables|Default|GetSuspWidget))
  (Variables|Default|SetCurrentValue (+ Value (Variables|Default|GetCurrentValue)))
  (Utilities|IsValid _suspwidget
    (:Is%20Valid
      (if (>= (Variables|/Game/ModernRPG/General/GUI/Widgets/WB_Suspicious.WB_Suspicious_C|GetCurrentValue _suspwidget) 1.0)
        (return (>= (Variables|Default|GetCurrentValue) 1.0))
        (else
          (Class|BPIWidgetsInfo|UpdateSuspiciousValue(Message) (Variables|Default|GetSuspWidget) (Variables|Default|GetCurrentValue))
          (Class|BPIWidgetsInfo|SuspiciousLocation(Message) (Variables|Default|GetSuspWidget) Location)
          (return (>= (Variables|Default|GetCurrentValue) 1.0)))))
    (:Is%20Not%20Valid
      (return (>= (Variables|Default|GetCurrentValue) 1.0)))))