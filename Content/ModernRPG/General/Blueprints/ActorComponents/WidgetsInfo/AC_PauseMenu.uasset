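; Actor component that manages the pause menu widget for its owning pawn.
; On BeginPlay it briefly creates a hidden menu, adds it to the viewport and immediately removes it, so that settings load.
; OpenPauseMenu creates and stores a fresh widget, then gives the player controller a cursor, focus and UI-only input.
; TryRemovePauseMenu calls the stored widget's own RemoveWidget if it is on screen.
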(event Custom|OpenPauseMenu
  ;[1 1 1] Open pause menu, set focuse
  (bind _returnvalue (UserInterface|CreateWidget "/Game/ModernRPG/General/GUI/Widgets/MainMenu/WBP_PauseMenu.WBP_PauseMenu_C"))
  (bind _output_get (Variables|Default|SetPauseMenu _returnvalue))
  (UserInterface|Viewport|AddtoViewport _output_get 0)
  (bind _aspawn (Utilities|Casting|CastToPawn (Components|GetOwner)))
  (bind _asplayer_controller (Utilities|Casting|CastToPlayerController (Pawn|GetController _aspawn)))
  (Variables|/Script/Engine.PlayerController|SetbShowMouseCursor _asplayer_controller true)
  (Class|Widget|SetUserFocus (Variables|Default|GetPauseMenu) _asplayer_controller)
  (Input|SetInputModeUIOnly _asplayer_controller (Variables|Default|GetPauseMenu) "DoNotLock"))

(event Custom|TryRemovePauseMenu
  (bind _pausemenu (Variables|Default|GetPauseMenu))
  ;[1 1 1] Remove Widget
  (Utilities|IsValid _pausemenu
    (:Is%20Valid
      (if (UserInterface|Viewport|IsinViewport _pausemenu)
        (Default|RemoveWidget (Variables|Default|GetPauseMenu))))))

(event EventBeginPlay
  ;[1 1 1] Create pause menu to load settings
  (bind _returnvalue (UserInterface|CreateWidget "/Game/ModernRPG/General/GUI/Widgets/MainMenu/WBP_PauseMenu.WBP_PauseMenu_C"))
  (Utilities|IsValid _returnvalue
    (:Is%20Valid
      (Widget|SetVisibility _returnvalue "Hidden")
      (UserInterface|Viewport|AddtoViewport _returnvalue 0)
      (Widget|RemovefromParent _returnvalue))))