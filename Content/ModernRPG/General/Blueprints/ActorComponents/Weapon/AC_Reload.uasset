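; Character component that runs weapon reloading with networked montages and a physical magazine prop.
; ReloadStart checks state, holster and ammo (bypassed for AI), stops aiming, then plays the montage through server/multicast events, filling ammo on completion.
; Montage notifies, debounced, spawn and destroy BP_PhysicsClip actors to drop the magazine, put one in the hand and attach it to the weapon.
; AC_EquipmentHandler supplies the weapon, animations and modification-aware clip mesh and socket.
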(event Custom|AttachClipWeapon%20-ALL
  (params (InputPin :type BP%20Physics%20Clip%20Object%20Reference))
  ;[1 1 1] Weapon Clip
  ;;[1 1 1] Attach Clip
  (Utilities|IsValid InputPin
    (:Is%20Valid
      (Transformation|AttachComponentToComponent InputPin (Variables|Default|GetSK_Weapon) (CallFunction|GetClipSocket) "SnapToTarget" "SnapToTarget" "KeepRelative" true))))

(event Custom|PassEvent
  (params (Selection :type Name))
  ;[1 1 1] Reload Animation  | Give Ammo on End
  (Utilities|PhysicClipEvents Selection))

(event Custom|InitializeClip%20-Server
  (params (Clip :type BP%20Physics%20Clip%20Object%20Reference))
  ;[1 1 1] Initialization
  (CallFunction|InitializeClip-ALL Clip))

(event Custom|Reload%20-ALL
  (params (MontageToPlay :type Anim%20Montage%20Object%20Reference) (HandClip :type Name) (Sounds :type S%20Weapon%20Sound%20Structure))
  ;[1 1 1] Reload Animation  | Give Ammo on End
  (Variables|Default|SetHandClip HandClip)
  (Variables|Default|SetSounds Sounds)
  (Variables|Default|SetisReloading true)
  (Utilities|MPlayAnyMontage MontageToPlay
    (:OnInterrupted
      (Default|CallReloadEnded)
      (CallFunction|UpdateState "NewEnumerator4"))
    (:onComplteted
      (Default|CallReloadEnded)))
  (Variables|Default|SetisReloading false))

(event Custom|InitializeClip%20-ALL
  (params (Clip :type BP%20Physics%20Clip%20Object%20Reference))
  ;[1 1 1] Initialization
  (Variables|Default|SetClip Clip))

(event Custom|AttachClipWeapon%20-Server
  (params (NewMesh :type Static%20Mesh%20Object%20Reference) (Materials :type Array%20of%20Material%20Instance%20Object%20References) (DefaultMaterial :type Boolean))
  ;[1 1 1] Weapon Clip
  ;;[1 1 1] Attach Clip
  (Utilities|IsValid (Variables|Default|GetClip)
    (:Is%20Valid
      (CallFunction|AttachClipWeapon-ALL (Variables|Default|GetClip))
      (Default|Initialize-ALL (Variables|Default|GetClip) NewMesh false Materials DefaultMaterial))))

(event Custom|Realod%20-Server
  (params (MontageToPlay :type Anim%20Montage%20Object%20Reference) (HandClip :type Name) (Sounds :type S%20Weapon%20Sound%20Structure))
  ;[1 1 1] Store Reloading Information and start Reloading
  (CallFunction|Reload-ALL MontageToPlay HandClip Sounds))

(event Custom|ReloadStart
  ;[1 1 1] Store Reloading Information and start Reloading
  (Utilities|FlowControl|Delay 0.0)
  (if (CallFunction|ReloadAllowed)
    (CallFunction|InitializeWeapon)
    (Default|CallReloadStarted)
    (Default|ForceStopCheck (Actor|GetComponentbyClass (Components|GetOwner) "/Game/ModernRPG/General/Blueprints/ActorComponents/Weapon/AC_Aiming.AC_Aiming_C"))
    (CallFunction|UpdateState "NewEnumerator1")
    (CallFunction|SwitchReloadNetwork)))

(event Custom|SpawnAndConnectClip
  (bind _actor (CallFunction|GetWeaponActor))
  (bind (_mesh _clip_materials) (CallFunction|GetClipMesh))
  ;[1 1 1] Weapon Clip
  ;;[1 1 1] Spawn Clip for the first time
  (Utilities|FlowControl|Delay 1.0)
  (CallFunction|InitializeWeapon)
  (Utilities|IsValid (Variables|Default|GetSK_Weapon)
    (:Is%20Valid
      (bind _returnvalue (Game|SpawnActorfromClass "/Game/ModernRPG/General/Blueprints/Weapon/BP_PhysicsClip.BP_PhysicsClip_C" (Transformation|GetSocketTransform (Variables|Default|GetSK_Weapon) (CallFunction|GetClipSocket) "RTS_World") "AlwaysSpawn" 0 0))
      (Default|InitializeClip-Server _returnvalue _mesh false _clip_materials false)
      (Collision|SetActorEnableCollision _returnvalue false)
      (Utilities|IsValid (Variables|Default|GetClip)
        (:Is%20Valid
          (Actor|DestroyActor (Variables|Default|GetClip)))
        (:Is%20Not%20Valid
          _))
      (CallFunction|InitializeClip _returnvalue)
      (CallFunction|AttachClipWeapon-ALL (Variables|Default|GetClip))
      (Utilities|IsValid _actor
        (:Is%20Valid
          (Default|RemoveClip _actor))))))

(event Custom|ReleaseClip%20-ALL
  (bind _clip (Variables|Default|GetClip))
  ;[1 1 1] Weapon Clip
  ;;[1 1 1] Release Clip
  (Utilities|IsValid _clip
    (:Is%20Valid
      (Actor|DestroyActor _clip))))

(event Custom|ReleaseClip%20-Server
  ;[1 1 1] Weapon Clip
  ;;[1 1 1] Release Clip
  (CallFunction|ReleaseClip-ALL))

(event Custom|AttachClipMesh%20-ALL
  (params (Target :type Actor%20Object%20Reference))
  ;[1 1 1] Weapon Clip
  ;;[1 1 1] Attach Clip
  ;;;[1 1 1] Comment
  (Utilities|IsValid Target
    (:Is%20Valid
      (Transformation|AttachComponentToComponent Target (Variables|Default|GetSK_Mesh) (Variables|Default|GetHandClip) "SnapToTarget" "SnapToTarget" "KeepWorld" true))))

(event EventBeginPlay
  ;[1 1 1] Initialization
  (bind _ascharacter (Utilities|Casting|CastToCharacter (Components|GetOwner)))
  (bind (_defaultbodymesh _headmesh) (Class|BPIAI|GetDemoSkeletalMeshes(Message) _ascharacter))
  (Variables|Default|SetSK_Mesh _defaultbodymesh)
  (Variables|Default|SetSK_Head%20Mesh _headmesh)
  (Utilities|FlowControl|Delay 0.0)
  (CallFunction|InitializeWeapon))

(fn InitializeWeapon
  (bind _actor (CallFunction|GetWeaponActor))
  (bind (_ammotype _reload) (CallFunction|GetAnimations))
  (Utilities|IsValid _actor
    (:Is%20Valid
      (bind _asskeletal_mesh_component (Utilities|Casting|CastToSkeletalMeshComponent (Default|GetUsedSceneComponent _actor)))
      (Variables|Default|SetSK_Weapon _asskeletal_mesh_component)
      (Variables|Default|SetAmmoType _ammotype)
      (Variables|Default|SetAM_Reload _reload))
    (:Is%20Not%20Valid
      (Default|UpdateWeaponInformation (Actor|GetComponentbyClass (Components|GetOwner) "/Game/ModernRPG/General/Blueprints/ActorComponents/InteractActors/AC_EquipmentHandler.AC_EquipmentHandler_C") true))))

(fn GetWeaponActor
  (return (Default|GetCurrentWeaponActorbyType (Actor|GetComponentbyClass (Components|GetOwner) "/Game/ModernRPG/General/Blueprints/ActorComponents/InteractActors/AC_EquipmentHandler.AC_EquipmentHandler_C"))))

(fn GetAnimations
  (bind _returnvalue (Components|GetOwner))
  (bind _returnvalue_2 (Actor|GetComponentbyClass _returnvalue "/Game/ModernRPG/General/Blueprints/ActorComponents/InteractActors/AC_EquipmentHandler.AC_EquipmentHandler_C"))
  (bind _array_element (Default|GetCurrentWeapon _returnvalue_2))
  (bind _row (Utilities|Struct|BreakS_InvItemDyn _array_element))
  (bind _weapon (CallFunction|GetWeaponInfo _row))
  (bind (_weapon_characteristics _action_animations _action_animations_ai_optional) (Utilities|Struct|BreakS_Weapon _weapon))
  (bind _value (Class|BPIAI|IsAI(Message) (Components|GetOwner)))
  (return (Utilities|Struct|BreakS_WeaponCharacteristics _weapon_characteristics) (Utilities|Struct|BreakS_ActionAnimations (select _value _action_animations_ai_optional _action_animations))))

(fn GetWeaponInfo
  (return (CallFunction|GetWeaponInfo (.Row (Utilities|Struct|BreakS_InvItemDyn (.Array%20Element (Default|GetCurrentWeapon (Actor|GetComponentbyClass (Components|GetOwner) "/Game/ModernRPG/General/Blueprints/ActorComponents/InteractActors/AC_EquipmentHandler.AC_EquipmentHandler_C"))))))))

(fn GetClipMesh
  (bind _returnvalue (Components|GetOwner))
  (bind _returnvalue_2 (Actor|GetComponentbyClass _returnvalue "/Game/ModernRPG/General/Blueprints/ActorComponents/InteractActors/AC_EquipmentHandler.AC_EquipmentHandler_C"))
  (bind _modification (Default|GetCurrentModificationCharacteristics _returnvalue_2 "NewEnumerator2"))
  (bind _mesh (Utilities|Struct|BreakS_ModificationInform _modification))
  (bind _clip_materials (CallFunction|GetCurrentWeaponSkinbyStructure (.Row (Utilities|Struct|BreakS_InvItemDyn (.Array%20Element (Default|GetCurrentWeapon (Actor|GetComponentbyClass (Components|GetOwner) "/Game/ModernRPG/General/Blueprints/ActorComponents/InteractActors/AC_EquipmentHandler.AC_EquipmentHandler_C")))))))
  (if (.Has (Default|GetCurrentModificationCharacteristics (Actor|GetComponentbyClass (Components|GetOwner) "/Game/ModernRPG/General/Blueprints/ActorComponents/InteractActors/AC_EquipmentHandler.AC_EquipmentHandler_C") "NewEnumerator2"))
    (for _array_element (Variables|/Script/Engine.StaticMesh|GetStaticMaterials _mesh)
      (bind _asmaterial_instance (Utilities|Casting|CastToMaterialInstance (.MaterialInterface (Utilities|Struct|BreakStaticMaterial _array_element))))
      (Utilities|Array|Add (LocalVariables|GetmatLocal) _asmaterial_instance))
    (return _mesh (LocalVariables|GetmatLocal))
    (else
      (return (.Clip (Utilities|Struct|BreakS_Appearance (Utilities|Struct|BreakS_Weapon (CallFunction|GetWeaponInfo)))) _clip_materials))))

(fn GetClipSocket
  (bind _returnvalue (Components|GetOwner))
  (bind _returnvalue_2 (Actor|GetComponentbyClass _returnvalue "/Game/ModernRPG/General/Blueprints/ActorComponents/InteractActors/AC_EquipmentHandler.AC_EquipmentHandler_C"))
  (bind (_has _modification) (Default|GetCurrentModificationCharacteristics _returnvalue_2 "NewEnumerator2"))
  (if _has
    (return (Utilities|Struct|BreakS_ModificationInform _modification))
    (else
      (return (Variables|Setup|GetClipSocket)))))

(fn ABPNotify
  (Utilities|IsValid (Variables|Default|GetAM_Reload)
    (:Is%20Valid
      (bind _defaultbodymesh (Class|BPIAI|GetDemoSkeletalMeshes(Message) (Components|GetOwner)))
      (Class|BPIABP|Reload(Message) (Components|SkeletalMesh|GetAnimInstance _defaultbodymesh) (Variables|/Script/Engine.AnimSequenceBase|GetSequenceLength (Variables|Default|GetAM_Reload))))))

(fn ReloadAllowed
  (bind _returnvalue (Components|GetOwner))
  (bind _returnvalue_2 (Components|GetOwner))
  (bind _returnvalue_3 (Actor|GetComponentbyClass _returnvalue "/Game/ModernRPG/General/Blueprints/ActorComponents/Character/State/AC_PlayerCurrentState.AC_PlayerCurrentState_C"))
  (bind _returnvalue_4 (Actor|GetComponentbyClass _returnvalue_2 "/Game/ModernRPG/General/Blueprints/ActorComponents/InteractActors/AC_EquipmentHandler.AC_EquipmentHandler_C"))
  (bind _currentstate (Variables|/Game/ModernRPG/General/Blueprints/ActorComponents/Character/State/AC_PlayerCurrentState.AC_PlayerCurrentState_C|GetCurrentState _returnvalue_3))
  (return (or (and (and (or (not (Math|Boolean|ORBoolean (Utilities|Enum|Equal(Enum) _currentstate "NewEnumerator1") (Utilities|Enum|Equal(Enum) _currentstate "NewEnumerator2") (Utilities|Enum|Equal(Enum) _currentstate "NewEnumerator0") (Variables|/Game/ModernRPG/General/Blueprints/ActorComponents/Weapon/AC_HolsterWeapon.AC_HolsterWeapon_C|GetHolstered (Actor|GetComponentbyClass (Components|GetOwner) "/Game/ModernRPG/General/Blueprints/ActorComponents/Weapon/AC_HolsterWeapon.AC_HolsterWeapon_C")))) (Variables|Setup|GetIsAI)) (> (Default|GetAllAmmo (Actor|GetComponentbyClass (Components|GetOwner) "/Game/ModernRPG/General/Blueprints/ActorComponents/Character/Inventory/AC_Inventory.AC_Inventory_C")) 0)) (< (Utilities|Struct|BreakS_InvItemDyn (.Array%20Element (Default|GetCurrentWeapon _returnvalue_4))) (Default|GetCurWeaponMaxAmmo _returnvalue_4))) (Variables|Setup|GetIsAI))))

(fn UpdateState
  (params (State :type E_WeaponState%20Enum :default "NewEnumerator4"))
  (Default|UpdateState (Actor|GetComponentbyClass (Components|GetOwner) "/Game/ModernRPG/General/Blueprints/ActorComponents/Character/State/AC_PlayerCurrentState.AC_PlayerCurrentState_C") State))

(fn GetSoundsandHandclip
  (bind _weapon (CallFunction|GetWeaponInfo))
  (bind (_sockets _sounds) (Utilities|Struct|BreakS_Weapon _weapon))
  (return (Utilities|Struct|BreakS_WeaponSockets _sockets) _sounds))

(fn SwitchReloadNetwork
  (bind (_socket_handclip _sounds) (CallFunction|GetSoundsandHandclip))
  (bind (_socket_handclip_2 _sounds_2) (CallFunction|GetSoundsandHandclip))
  (Networking|SwitchHasAuthority
    (:Authority
      (CallFunction|Reload-ALL (.Reload (CallFunction|GetAnimations)) _socket_handclip_2 _sounds_2))
    (:Remote
      (CallFunction|Realod-Server (.Reload (CallFunction|GetAnimations)) _socket_handclip _sounds))))

(fn InitializeClip
  (params (Clip :type BP%20Physics%20Clip%20Object%20Reference))
  (if (Ability|HasAuthority (Components|GetOwner))
    (CallFunction|InitializeClip-ALL Clip)
    (else
      (CallFunction|InitializeClip-Server Clip))))