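; Character component for aim-pitch spine rotation, replicated through throttled server-to-multicast calls.
; BoneRotation derives clamped spine pitch from control rotation, and UpdateCapsule widens the replicated capsule radius as pitch grows, except while swimming.
; The main logic, including building-mode easing, is disconnected: UpdateWiggle calls an empty SpineRotator.
; CanRotate always returns true, leaving its state, view and aiming checks unused.
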(event Custom|BoneRotationReplicate
  (bind _spinerotation (Variables|Default|GetSpineRotation))
  ;[1 1 1] Bone Rotation Replication
  (Utilities|FlowControl|Gate false
    (:Exit
      (if (Ability|HasAuthority (Components|GetOwner))
        (CallFunction|BoneRotation-ALL _spinerotation)
        (else
          (CallFunction|BoneRotation-Server _spinerotation)))
      (CallFunction|CloseBoneRotation)
      (Utilities|FlowControl|Delay 0.075)
      (CallFunction|OpenBoneRotation))))

(event Custom|ReturnFromBuildingMode
  ;[1 1 1] Spine Rotation
  (Variables|Default|SetSpineRotation (Math|Interpolation|RInterpTo (Variables|Default|GetSpineRotation) (CallFunction|BoneRotation) (Utilities|Time|GetWorldDeltaSeconds) 1e+01))
  (if (< (Math|Float|Absolute(Float) (- (.pitch (Variables|Default|GetSpineRotation)) (.pitch (CallFunction|BoneRotation)))) 1.0)
    (Default|SetReturnfromBMode-Server (Actor|GetComponentbyClass (Components|GetOwner) "/Game/ModernRPG/General/Blueprints/Building/AC_Building.AC_Building_C") false)))

(event Custom|ReplicatePlayerVariable%20-%20ALL
  (params (Player :type Boolean))
  ;[1 1 1] Is Player Replicate
  (Variables|Default|SetPlayer Player))

(event Custom|ReplicateCapsuleSize%20-ALL
  (params (Radius :type Float%20%28double-precision%29) (Target :type Capsule%20Component%20Object%20Reference))
  ;[1 1 1] ReplicateCapsule
  (Components|Capsule|SetCapsuleRadius Target Radius true))

(event Custom|CheckFirstDisabled
  ;[1 1 1] Disabled at first
  (if (Variables|Default|GetFirstlyDisabled)
    (Variables|Default|SetFirstlyDisabled false)
    (if (Ability|HasAuthority (Components|GetOwner))
      (CallFunction|BoneRotation-ALL "0, 0, 0")
      (else
        (CallFunction|BoneRotation-Server "0, 0, 0")))))

(event Custom|BoneRotation%20-Server
  (params (Rotation :type Rotator))
  ;[1 1 1] Bone Rotation Replication
  (CallFunction|BoneRotation-ALL Rotation))

(event Custom|OpenBoneRotation
  (bind _spinerotation (Variables|Default|GetSpineRotation))
  ;[1 1 1] Bone Rotation Replication
  (Utilities|FlowControl|Gate false) ; enters at Open
)

(event Custom|ReplicateCapsuleSize%20-Server
  (params (Radius :type Float%20%28double-precision%29) (Target :type Capsule%20Component%20Object%20Reference))
  ;[1 1 1] ReplicateCapsule
  (CallFunction|ReplicateCapsuleSize-ALL Radius Target))

(event Custom|ReplicateCapsuleSize
  (params (Radius :type Float%20%28double-precision%29) (Target :type Capsule%20Component%20Object%20Reference))
  ;[1 1 1] ReplicateCapsule
  (if (not (AI|Components|NavMovement|IsSwimming (Variables|/Script/Engine.Character|GetCharacterMovement (Variables|Default|GetCharacter)) :!class /Script/Engine.NavMovementComponent))
    (if (Ability|HasAuthority (Components|GetOwner))
      (CallFunction|ReplicateCapsuleSize-ALL Radius Target)
      (else
        (CallFunction|ReplicateCapsuleSize-Server Radius Target)))))

(event Custom|BoneRotation%20-ALL
  (params (Rotation :type Rotator))
  ;[1 1 1] Bone Rotation Replication
  (Variables|Default|SetSpineRotation Rotation))

(event Custom|CloseBoneRotation
  (bind _spinerotation (Variables|Default|GetSpineRotation))
  ;[1 1 1] Bone Rotation Replication
  (Utilities|FlowControl|Gate false) ; enters at Close
)

(event Custom|SpineRotator
  ;[1 1 1] Spine Rotation
)

(event Custom|UpdateWiggle
  ;[1 1 1] Update Wiggle
  (CallFunction|SpineRotator))

(event EventBeginPlay
  ;[1 1 1] Initialize Component
  (bind _ascharacter (Utilities|Casting|CastToCharacter (Components|GetOwner)))
  (bind _output_get (Variables|Default|SetCharacter _ascharacter))
  (Utilities|FlowControl|Delay 2.0)
  (Variables|Default|SetCapsule (Variables|/Script/Engine.Character|GetCapsuleComponent _output_get))
  (Variables|Default|SetDefaultCapsuleSize (Variables|/Script/Engine.CapsuleComponent|GetCapsuleRadius (Variables|/Script/Engine.Character|GetCapsuleComponent _output_get)))
  (CallFunction|ReplicatePlayerVariable-ALL (Pawn|IsPlayerControlled (Variables|Default|GetCharacter))))

(fn BoneRotation
  (bind _character (Variables|Default|GetCharacter))
  (bind _returnvalue (Pawn|GetControlRotation _character :!class /Script/Engine.Pawn))
  (bind _pitch (Math|Rotator|BreakRotator _returnvalue))
  (Utilities|IsValid (Variables|Default|GetCharacter)
    (:Is%20Valid
      (return (Math|Rotator|MakeRotator 0.0 (Math|Float|Clamp(Float) (Math|Float|SelectFloat (- 3.6e+02 _pitch) (* _pitch -1.0) (> _pitch 1.8e+02)) -9e+01 9e+01) 0.0)))))

(fn UpdateCapsule
  (bind _capsule (Variables|Default|GetCapsule))
  (Utilities|IsValid _capsule
    (:Is%20Valid
      (CallFunction|ReplicateCapsuleSize (select (CallFunction|CanRotate) (Math|Float|MapRangeClamped (Math|Float|Absolute(Float) (.Pitch (Math|Rotator|BreakRotator (Variables|Default|GetSpineRotation)))) 0.0 9e+01 (Variables|Default|GetDefaultCapsuleSize) 1e+02) (Variables|Default|GetDefaultCapsuleSize)) _capsule))))

(fn CanRotate
  (return true))