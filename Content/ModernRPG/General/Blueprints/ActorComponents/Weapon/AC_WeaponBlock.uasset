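; Actor component that detects when the character's weapon is blocked by nearby geometry in first person or while aiming.
; A looping timer sphere-traces from the head socket along the camera forward and interpolates a distance-mapped block amount, ignoring actors with the character interface.
; Any trace hit also cancels active aiming; otherwise the block eases back to zero.
; Other systems set trace length, read block state, or test whether aiming is unobstructed.
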(event EventBeginPlay
  ;[1 1 1] Initialize Camera
  (Variables|Default|SetCameraFirstPerson (Utilities|Array|Get(acopy) (Actor|GetComponentsbyTag (Components|GetOwner) "/Script/Engine.CameraComponent" "Main")))
  (bind _ascharacter (Utilities|Casting|CastToCharacter (Components|GetOwner)))
  (Variables|Default|SetCharacter _ascharacter)
  (Utilities|Time|SetTimerbyFunctionName 0 "CalculateBlockVariables" (Variables|Default|GetTImer) true))

(fn LineTrace
  (bind _bodymesh (CallFunction|GetCharacterSkeleton (Variables|Default|GetCharacter)))
  (return (Transformation|GetSocketLocation _bodymesh (Variables|Setup|GetHeadSocket)) (+ (Transformation|GetSocketLocation _bodymesh (Variables|Setup|GetHeadSocket)) (* (Math|Vector|GetForwardVector (Variables|Default|GetCameraFirstPerson)) (Variables|Setup|GetCurDistToBlock)))))

(fn ModifyBlockDistance
  (params (Value :type Float%20%28double-precision%29))
  (return (Math|Interpolation|FInterpTo (Variables|Default|GetBlockedDistance) (Math|Float|MapRangeClamped Value 0.0 (+ (Variables|Setup|GetCurDistToBlock) 65.0) 1.5 -0.5) (Variables|Default|GetTImer) 8.0)))

(fn CalculateBlockVariables
  (bind (_start _end) (CallFunction|LineTrace))
  (bind _returnvalue (Components|GetOwner))
  (bind _returnvalue_2 (Actor|GetComponentbyClass _returnvalue "/Game/ModernRPG/General/Blueprints/ActorComponents/Weapon/AC_Aiming.AC_Aiming_C"))
  (if (CallFunction|FPP)
    ;[1 1 1] Check Validity
    (Utilities|IsValid (Variables|Default|GetCameraFirstPerson)
      (:Is%20Valid
        (bind (_outhits _returnvalue_3) (Collision|MultiSphereTraceByChannel _start _end 35.0 "TraceTypeQuery2" false (Utilities|Array|MakeArray (Components|GetOwner)) "None"))
        (LocalVariables|SetL_Hits _outhits)
        (if _returnvalue_3
          (if (Variables|/Game/ModernRPG/General/Blueprints/ActorComponents/Weapon/AC_Aiming.AC_Aiming_C|GetAiming _returnvalue_2)
            (Default|StopAiming-Server _returnvalue_2))
          ;[1 1 1] Block Hit And Distance
          (for _array_element (LocalVariables|GetL_Hits)
            (if (not (Utilities|DoesObjectImplementInterface (.HitActor (Collision|BreakHitResult _array_element)) "/Game/ModernRPG/General/Blueprints/Interfaces/BP_I_Character.BP_I_Character_C"))
              (Variables|Default|SetBlockedDistance (CallFunction|ModifyBlockDistance (.Distance (Collision|BreakHitResult _array_element))))
              (Variables|Default|SetBlockedWeapon true)))
          (else
            ;[1 1 1] Unblock
            (CallFunction|Unblock))))
      (:Is%20Not%20Valid
        (CallFunction|Unblock :!label _label)))
    (else
      (goto _label))))

(fn Unblock
  (Variables|Default|SetBlockedDistance (Math|Interpolation|FInterpTo (Variables|Default|GetBlockedDistance) 0.0 (Variables|Default|GetTImer) 8.0))
  (Variables|Default|SetBlockedWeapon false))

(fn GetBlockInformation
  (return (Variables|Default|GetBlockedDistance) (Variables|Default|GetBlockedWeapon)))

(fn InitializeBlockDistance
  (params (DistToBlock :type Float%20%28double-precision%29))
  (Variables|Setup|SetCurDistToBlock DistToBlock))

(fn FPP
  (return (or (not (Variables|/Game/ModernRPG/General/Blueprints/ActorComponents/ViewSwitch/AC_ViewSwitch.AC_ViewSwitch_C|GetInThirdPerson (Actor|GetComponentbyClass (Components|GetOwner) "/Game/ModernRPG/General/Blueprints/ActorComponents/ViewSwitch/AC_ViewSwitch.AC_ViewSwitch_C"))) (Variables|/Game/ModernRPG/General/Blueprints/ActorComponents/Weapon/AC_Aiming.AC_Aiming_C|GetAiming (Actor|GetComponentbyClass (Components|GetOwner) "/Game/ModernRPG/General/Blueprints/ActorComponents/Weapon/AC_Aiming.AC_Aiming_C")))))

(fn CalculateBlockVariableswithAimTesting
  (params (Aim? :type Boolean))
  (bind (_start _end) (CallFunction|LineTrace))
  (if Aim?
    ;[1 1 1] Check Validity
    (Utilities|IsValid (Variables|Default|GetCameraFirstPerson)
      (:Is%20Valid
        (bind (_outhits _returnvalue) (Collision|MultiSphereTraceByChannel _start _end 35.0 "TraceTypeQuery2" false (Utilities|Array|MakeArray (Components|GetOwner)) "None"))
        (LocalVariables|SetL_Hits _outhits)
        (if _returnvalue
          ;[1 1 1] Block Hit And Distance
          (for _array_element (LocalVariables|GetL_Hits)
            (if (not (Utilities|DoesObjectImplementInterface (.HitActor (Collision|BreakHitResult _array_element)) "/Game/ModernRPG/General/Blueprints/Interfaces/BP_I_Character.BP_I_Character_C"))
              (return false)))
          (else
            (return true)))))))