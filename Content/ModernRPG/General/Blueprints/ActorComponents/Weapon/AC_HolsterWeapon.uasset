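; Actor component that handles drawing, holstering and switching a character's weapons, including cycling and equipping by subtype.
; Draw and holster montages come from the current weapon's data row (with an AI variant), and their notifies trigger attach/remove through DoOnce gates.
; Player state, montage and aiming checks gate actions, which replicate via Server/ALL event pairs.
; It drives AC_EquipmentHandler and updates the anim blueprint, with weapon UI and fire mode reset on holster.
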(event Custom|SwitchEvent%20-ALL
  (params (Item :type S%20Inv%20Item%20Dyn%20Structure) (Index :type Integer))
  ;[1 1 1] Switch Event
  (CallFunction|SwitchEvent Item Index))

(event Custom|SwitchEvent%20-Server
  (params (Item :type S%20Inv%20Item%20Dyn%20Structure) (Index :type Integer))
  ;[1 1 1] Switch Event
  (CallFunction|SwitchEvent-ALL Item Index))

(event Custom|EquipWeaponType
  (params (Subtype :type E_WeaponType%20Enum :default "NewEnumerator0"))
  (bind _returnvalue (Components|GetOwner))
  (bind _returnvalue_2 (Actor|GetComponentbyClass _returnvalue "/Game/ModernRPG/General/Blueprints/ActorComponents/InteractActors/AC_EquipmentHandler.AC_EquipmentHandler_C"))
  (bind (_array_element _array_index _has) (Default|GetWeaponItembySubtype _returnvalue_2 Subtype))
  ;[1 1 1] Circle Weapon
  (if (CallFunction|CanEquip)
    (if (Variables|Settings|GetHolstered)
      (CallFunction|HolsterSwitch-Server Subtype)
      (Utilities|FlowControl|Delay 0.05)
      (CallFunction|HolsterWeapon false false false false)
      (elif (Utilities|Enum|NotEqual(Enum) Subtype (Variables|/Game/ModernRPG/General/Blueprints/ActorComponents/InteractActors/AC_EquipmentHandler.AC_EquipmentHandler_C|GetCurrentWeaponSubtype _returnvalue_2))
        (if _has
          (CallFunction|SwitchEvent-Server _array_element _array_index))))))

(event Custom|Initialize%20-Server
  (params (Index :type Boolean))
  ;[1 1 1] Initialize New Weapon
  (CallFunction|Initialize-ALL Index))

(event Custom|HolsterSwitch%20-ALL
  (params (CurrentWeaponSubtype :type E_WeaponType%20Enum :default "NewEnumerator0"))
  (bind _returnvalue (Components|GetOwner))
  (bind _returnvalue_2 (Actor|GetComponentbyClass _returnvalue "/Game/ModernRPG/General/Blueprints/ActorComponents/InteractActors/AC_EquipmentHandler.AC_EquipmentHandler_C"))
  ;[1 1 1] Holster Switch Replicated
  (Variables|/Game/ModernRPG/General/Blueprints/ActorComponents/InteractActors/AC_EquipmentHandler.AC_EquipmentHandler_C|SetCurrentWeaponSubtype _returnvalue_2 CurrentWeaponSubtype)
  (Default|InitializeNewItems _returnvalue_2))

(event Custom|Redraw%20-ALL
  ;[1 1 1] Redraw weapon
  (Utilities|FlowControl|Delay 0.1)
  (CallFunction|UpdateInformation false)
  (Default|UpdateState (Actor|GetComponentbyClass (Components|GetOwner) "/Game/ModernRPG/General/Blueprints/ActorComponents/Character/State/AC_PlayerCurrentState.AC_PlayerCurrentState_C") "NewEnumerator2")
  (Default|CallRemoveWeapon)
  (CallFunction|DrawHolster true false))

(event Custom|CircleWeapon
  (params (Up :type Boolean))
  (bind _returnvalue (Components|GetOwner))
  (bind _returnvalue_2 (Actor|GetComponentbyClass _returnvalue "/Game/ModernRPG/General/Blueprints/ActorComponents/InteractActors/AC_EquipmentHandler.AC_EquipmentHandler_C"))
  (bind _type (Default|GetPreviousSubtype _returnvalue_2))
  (bind _type_2 (Default|GetNextSubtype _returnvalue_2))
  (bind _returnvalue_3 (select Up _type_2 _type))
  (bind (_array_element _array_index _has) (Default|GetWeaponItembySubtype _returnvalue_2 _returnvalue_3))
  ;[1 1 1] Circle Weapon
  (if (CallFunction|HaveAnyEquipment?)
    (if (Variables|Settings|GetHolstered)
      (CallFunction|HolsterWeapon true false false false)
      (elif _has
        (CallFunction|SwitchEvent-Server _array_element _array_index)))))

(event Custom|Redraw%20-Server
  (params (Type :type E_WeaponType%20Enum :default "NewEnumerator7") (NewItem :type S%20Inv%20Item%20Dyn%20Structure) (NewWeapon :type Boolean))
  ;[1 1 1] Redraw weapon
  (Variables|Engine|SetDrawType Type)
  (Variables|Engine|SetNewItem (select NewWeapon NewItem (.Array%20Element (Default|GetWeaponItembySubtype (Actor|GetComponentbyClass (Components|GetOwner) "/Game/ModernRPG/General/Blueprints/ActorComponents/InteractActors/AC_EquipmentHandler.AC_EquipmentHandler_C") (Variables|Engine|GetDrawType)))))
  (CallFunction|Redraw-ALL))

(event Custom|HolsterSwitch%20-Server
  (params (CurrentWeaponSubtype :type E_WeaponType%20Enum :default "NewEnumerator0"))
  ;[1 1 1] Holster Switch Replicated
  (CallFunction|HolsterSwitch-ALL CurrentWeaponSubtype))

(event Custom|HolsterWeapon
  (params (Circle :type Boolean) (ForceHolster :type Boolean) (Take? :type Boolean) (SuperForce :type Boolean))
  (bind _returnvalue (CallFunction|GetEquipmentComponent))
  (bind (_result _weapontype) (Default|GetFirstWeaponType _returnvalue))
  ;[1 1 1] Holster Weapon
  (if (CallFunction|CanHolster? SuperForce)
    (if (Variables|Settings|GetHolstered)
      (Default|UpdateWeaponInformation (CallFunction|GetEquipmentComponent) false :!label _label)
      (if (.Has (Default|GetCurrentWeapon (CallFunction|GetEquipmentComponent)))
        (CallFunction|InitializeWeaponMontages true :!label _label_2)
        (Utilities|FlowControl|Delay 0.1)
        (Variables|Engine|SetFirstDraw false)
        (Networking|SwitchHasAuthority
          (:Authority
            (CallFunction|HolsterWeapon-ALL Circle ForceHolster Take?))
          (:Remote
            (CallFunction|HolsterWeapon-Server Circle ForceHolster Take?)))
        (elif _result
          (Variables|/Game/ModernRPG/General/Blueprints/ActorComponents/InteractActors/AC_EquipmentHandler.AC_EquipmentHandler_C|SetCurrentWeaponSubtype (CallFunction|GetEquipmentComponent) _weapontype)))
      (else
        (goto _label_2)))
    (elif ForceHolster
      (goto _label))))

(event Custom|Initialize%20-ALL
  (params (Index :type Boolean))
  ;[1 1 1] Initialize New Weapon
  (CallFunction|Initialize Index))

(event Custom|DrawHolster
  (params (Redraw :type Boolean) (Force :type Boolean))
  (bind _returnvalue (CallFunction|GetEquipmentComponent))
  (bind _returnvalue_2 (CallFunction|GetEquipmentComponent))
  (bind _a_draw (Variables|Animations|GetA_Draw))
  ;[1 1 1] Draw
  (CallFunction|Initialize Redraw)
  (if Force
    (Default|CallTakeWeapon)
    (else
      (Default|UpdateState (Actor|GetComponentbyClass (Components|GetOwner) "/Game/ModernRPG/General/Blueprints/ActorComponents/Character/State/AC_PlayerCurrentState.AC_PlayerCurrentState_C") "NewEnumerator2")
      (Utilities|IsValid _a_draw
        (:Is%20Valid
          (CallFunction|MESSAGETOABPEquip (* (Variables|/Script/Engine.AnimSequenceBase|GetSequenceLength _a_draw) 10.5))
          (bind _notifyname (Animation|Montage|PlayMontage (Variables|Default|GetSK_Mesh) (Variables|Animations|GetA_Draw))
            (:then
              (Utilities|IsValid (Variables|Animations|GetA_Draw) :!label _label
                (:Is%20Valid
                  (CallFunction|MESSAGETOABPEquip (* (Variables|/Script/Engine.AnimSequenceBase|GetSequenceLength (Variables|Animations|GetA_Draw)) 0.5)))
                (:Is%20Not%20Valid
                  (Utilities|FlowControl|Delay 0.05)
                  (CallFunction|DrawNotify)
                  (Default|UpdateState (Actor|GetComponentbyClass (Components|GetOwner) "/Game/ModernRPG/General/Blueprints/ActorComponents/Character/State/AC_PlayerCurrentState.AC_PlayerCurrentState_C") "NewEnumerator4"))))
            (:OnCompleted
              (Default|UpdateState (Actor|GetComponentbyClass (Components|GetOwner) "/Game/ModernRPG/General/Blueprints/ActorComponents/Character/State/AC_PlayerCurrentState.AC_PlayerCurrentState_C") "NewEnumerator4" :!label _label_2)
              (Default|UpdateWeaponItemABP _returnvalue (Variables|/Game/ModernRPG/General/Blueprints/ActorComponents/InteractActors/AC_EquipmentHandler.AC_EquipmentHandler_C|GetCurrentWeaponSlot _returnvalue)))
            (:OnBlendOut
              (goto _label_2))
            (:OnInterrupted
              (goto _label_2))
            (:OnNotifyBegin
              (if (Utilities|Name|Equal(Name) _notifyname (Variables|NotifyNames|GetDrawNotifyName))
                (Utilities|FlowControl|DoOnce false :!label _label_3
                  (:Completed
                    (Default|CallTakeWeapon)
                    (Default|UpdateWeaponItemABP _returnvalue_2 (Variables|/Game/ModernRPG/General/Blueprints/ActorComponents/InteractActors/AC_EquipmentHandler.AC_EquipmentHandler_C|GetCurrentWeaponSlot _returnvalue_2))
                    (Utilities|FlowControl|Delay 0.2)
                    (goto _label_3 Reset)))))))
        (:Is%20Not%20Valid
          (goto _label))))))

(event Custom|DrawNotify
  ;[1 1 1] Draw
  (if (Utilities|Name|Equal(Name) (stale Custom|DrawHolster%20-ALL _notifyname) (Variables|NotifyNames|GetDrawNotifyName))
    (Utilities|FlowControl|DoOnce false :!label _label
      (:Completed
        (Default|CallTakeWeapon)
        (Utilities|FlowControl|Delay 0.2)
        (goto _label Reset)))))

(event Custom|HolsterWeaponDelay
  ;[1 1 1] Holster Weapon Delay
  (Utilities|FlowControl|Delay 0.0)
  (CallFunction|HolsterWeapon false false false false))

(event Custom|Initialize
  (params (Index :type Boolean))
  (bind _returnvalue (Components|GetOwner))
  (bind _newitem (Variables|Engine|GetNewItem))
  (bind _returnvalue_2 (Actor|GetComponentbyClass _returnvalue "/Game/ModernRPG/General/Blueprints/ActorComponents/InteractActors/AC_EquipmentHandler.AC_EquipmentHandler_C"))
  (bind (_has _array_element) (Default|GetCurrentWeapon _returnvalue_2))
  (bind _returnvalue_3 (select Index _newitem _array_element))
  (bind _row (Utilities|Struct|BreakS_InvItemDyn _returnvalue_3))
  (bind _weapon (CallFunction|GetWeaponInfo _row))
  (bind (_action_animations _action_animations_ai_optional) (Utilities|Struct|BreakS_Weapon _weapon))
  ;[1 1 1] Initialize New Weapon
  (Utilities|IsValid _returnvalue_2
    (:Is%20Valid
      (if _has
        (bind _value (Class|BPIAI|IsAI(Message) (Components|GetOwner)))
        (Utilities|IsValid (.WEAPON_AM_Draw (Utilities|Struct|BreakS_ActionAnimations (select _value _action_animations_ai_optional _action_animations)))
          (:Is%20Valid
            (Variables|Animations|SetA_Draw (.WEAPON_AM_Draw (Utilities|Struct|BreakS_ActionAnimations (select _value _action_animations_ai_optional _action_animations))))
            (Variables|Animations|SetA_Holster (.WEAPON_AM_Holster (Utilities|Struct|BreakS_ActionAnimations (select _value _action_animations_ai_optional _action_animations))))
            (CallFunction|SetAnimations-Server (Variables|Animations|GetA_Draw) (Variables|Animations|GetA_Holster))))))))

(event Custom|SetAnimations%20-Server
  (params (DrawWeapon :type Anim%20Montage%20Object%20Reference) (A_Holster :type Anim%20Montage%20Object%20Reference))
  ;[1 1 1] Set Animations
  (CallFunction|SetAnimations-ALL DrawWeapon A_Holster))

(event Custom|SetAnimations%20-ALL
  (params (DrawWeapon :type Anim%20Montage%20Object%20Reference) (A_Holster :type Anim%20Montage%20Object%20Reference))
  ;[1 1 1] Set Animations
  (Variables|Animations|SetA_Draw DrawWeapon)
  (Variables|Animations|SetA_Holster A_Holster))

(event Custom|ForceDraw
  ;[1 1 1] Draw
  (Utilities|FlowControl|DoOnce false :!label _label
    (:Completed
      (Default|CallTakeWeapon)
      (Utilities|FlowControl|Delay 0.2)
      (goto _label Reset))))

(event Custom|ToggleUnarmed
  ;[1 1 1] Toggle Unarmed State
  (Default|ToggleUnarmed (Actor|GetComponentbyClass (Components|GetOwner) "/Game/ModernRPG/General/Blueprints/Combat/AC_CombatEvents.AC_CombatEvents_C"))
  (Variables|/Game/ModernRPG/General/Blueprints/ActorComponents/Weapon/AC_Weapon.AC_Weapon_C|SetCurrentFireMode (Actor|GetComponentbyClass (Components|GetOwner) "/Game/ModernRPG/General/Blueprints/ActorComponents/Weapon/AC_Weapon.AC_Weapon_C") "NewEnumerator5"))

(event Custom|HolsterNotify
  ;[1 1 1] Holster Weapon
  (Utilities|FlowControl|DoOnce false :!label _label
    (:Completed
      (Default|CallRemoveWeapon)
      (Utilities|SetUnarmedABP)
      (Utilities|FlowControl|Delay 0.2)
      (goto _label Reset))))

(event Custom|UpdateInformation
  (params (Redraw :type Boolean))
  ;[1 1 1] Mesh
  (bind _ascharacter (Utilities|Casting|CastToCharacter (Components|GetOwner)))
  (bind (_defaultbodymesh _headmesh) (Class|BPIAI|GetDemoSkeletalMeshes(Message) _ascharacter))
  (Variables|Default|SetSK_Mesh _defaultbodymesh)
  (Variables|Default|SetSK_Head%20Mesh _headmesh)
  (Utilities|FlowControl|Delay 0.0) ; Let Weapon Spawn
  (bind _asskeletal_mesh_component (Utilities|Casting|CastToSkeletalMeshComponent (CallFunction|GetOwnerSceneComponent)))
  (Variables|Default|SetWeaponMesh _asskeletal_mesh_component)
  ;[1 1 1] Montage
  (CallFunction|InitializeWeaponMontages Redraw))

(event Custom|HolsterWeapon%20-ALL
  (params (Circle :type Boolean) (ForceHolster :type Boolean) (Take :type Boolean))
  (bind _returnvalue (Components|GetOwner))
  (bind _returnvalue_2 (Actor|GetComponentbyClass _returnvalue "/Game/ModernRPG/General/Blueprints/ActorComponents/Weapon/AC_Weapon.AC_Weapon_C"))
  (bind _array_element_actor (Default|GetCurrentWeapon _returnvalue_2))
  ;[1 1 1] Holster Weapon
  (if ForceHolster
    (if Take
      (Utilities|SetUnarmedABP :!label _label)
      (Utilities|IsValid _array_element_actor :!label _label_2
        (:Is%20Valid
          (Default|ControlLaserVisibility _array_element_actor false))
        (:Is%20Not%20Valid
          _))
      (Variables|Settings|SetHolstered true)
      (if ForceHolster
        (Default|CallRemoveWeapon)
        (CallFunction|SetWeaponUI "NewEnumerator7" :!label _label_3)
        (CallFunction|InitializeUnarmedSockets)
        (Variables|/Game/ModernRPG/General/Blueprints/ActorComponents/Weapon/AC_Weapon.AC_Weapon_C|SetCurrentFireMode (Actor|GetComponentbyClass (Components|GetOwner) "/Game/ModernRPG/General/Blueprints/ActorComponents/Weapon/AC_Weapon.AC_Weapon_C") "NewEnumerator5")
        (elif Circle
          (Default|UpdateState (Actor|GetComponentbyClass (Components|GetOwner) "/Game/ModernRPG/General/Blueprints/ActorComponents/Character/State/AC_PlayerCurrentState.AC_PlayerCurrentState_C") "NewEnumerator4" :!label _label_4)
          (goto _label_3)
          (else
            (bind _notifyname (Animation|Montage|PlayMontage (Variables|Default|GetSK_Mesh) (Variables|Animations|GetA_Holster))
              (:then
                (Utilities|IsValid (Variables|Animations|GetA_Holster)
                  (:Is%20Valid
                    (goto _label_4))
                  (:Is%20Not%20Valid
                    (Utilities|FlowControl|Delay 0.05)
                    (CallFunction|HolsterNotify)
                    (goto _label_4))))
              (:OnCompleted
                (goto _label_4))
              (:OnBlendOut
                (goto _label_4))
              (:OnInterrupted
                (Default|CallRemoveWeapon)
                (Utilities|SetUnarmedABP)
                (goto _label_4))
              (:OnNotifyBegin
                (if (Utilities|Name|Equal(Name) _notifyname (Variables|NotifyNames|GetHolsterNotifyName))
                  (Utilities|FlowControl|DoOnce false :!label _label_5
                    (:Completed
                      (Default|CallRemoveWeapon)
                      (Utilities|SetUnarmedABP)
                      (Utilities|FlowControl|Delay 0.2)
                      (goto _label_5 Reset)))))))))
      (else
        (CallFunction|DrawHolster false ForceHolster :!label _label_6)
        (Variables|Settings|SetHolstered false)))
    (elif (not (Variables|Settings|GetHolstered))
      (if ForceHolster
        (goto _label)
        (else
          (Default|UpdateState (Actor|GetComponentbyClass (Components|GetOwner) "/Game/ModernRPG/General/Blueprints/ActorComponents/Character/State/AC_PlayerCurrentState.AC_PlayerCurrentState_C") "NewEnumerator2")
          (goto _label_2)))
      (else
        (goto _label_6)))))

(event Custom|HolsterWeapon%20-Server
  (params (Circle :type Boolean) (ForceHolster :type Boolean) (Take :type Boolean))
  ;[1 1 1] Holster Weapon
  (CallFunction|HolsterWeapon-ALL Circle ForceHolster Take))

(event Custom|DrawHolster%20-ALL
  (params (Redraw :type Boolean) (Force :type Boolean))
  (bind _returnvalue (CallFunction|GetEquipmentComponent))
  (bind _returnvalue_2 (CallFunction|GetEquipmentComponent))
  (bind _a_draw (Variables|Animations|GetA_Draw))
  ;[1 1 1] Draw
  (CallFunction|Initialize Redraw)
  (if Force
    (Default|CallTakeWeapon)
    (Variables|Settings|SetHolstered false)
    (else
      (Default|UpdateState (Actor|GetComponentbyClass (Components|GetOwner) "/Game/ModernRPG/General/Blueprints/ActorComponents/Character/State/AC_PlayerCurrentState.AC_PlayerCurrentState_C") "NewEnumerator2")
      (Utilities|IsValid _a_draw
        (:Is%20Valid
          (CallFunction|MESSAGETOABPEquip (* (Variables|/Script/Engine.AnimSequenceBase|GetSequenceLength _a_draw) 0.5))
          (bind _notifyname (Animation|Montage|PlayMontage (Variables|Default|GetSK_Mesh) (Variables|Animations|GetA_Draw))
            (:then
              (Utilities|IsValid (Variables|Animations|GetA_Draw) :!label _label
                (:Is%20Not%20Valid
                  (Utilities|FlowControl|Delay 0.05)
                  (CallFunction|DrawNotify)
                  (Default|UpdateState (Actor|GetComponentbyClass (Components|GetOwner) "/Game/ModernRPG/General/Blueprints/ActorComponents/Character/State/AC_PlayerCurrentState.AC_PlayerCurrentState_C") "NewEnumerator4")
                  (Default|UpdateWeaponItemABP _returnvalue (Variables|/Game/ModernRPG/General/Blueprints/ActorComponents/InteractActors/AC_EquipmentHandler.AC_EquipmentHandler_C|GetCurrentWeaponSlot _returnvalue)))))
            (:OnCompleted
              (Default|UpdateState (Actor|GetComponentbyClass (Components|GetOwner) "/Game/ModernRPG/General/Blueprints/ActorComponents/Character/State/AC_PlayerCurrentState.AC_PlayerCurrentState_C") "NewEnumerator4" :!label _label_2)
              (Default|UpdateWeaponItemABP _returnvalue_2 (Variables|/Game/ModernRPG/General/Blueprints/ActorComponents/InteractActors/AC_EquipmentHandler.AC_EquipmentHandler_C|GetCurrentWeaponSlot _returnvalue_2)))
            (:OnBlendOut
              (goto _label_2))
            (:OnInterrupted
              (goto _label_2))
            (:OnNotifyBegin
              (if (Utilities|Name|Equal(Name) _notifyname (Variables|NotifyNames|GetDrawNotifyName))
                (Utilities|FlowControl|DoOnce false :!label _label_3
                  (:Completed
                    (Default|CallTakeWeapon)
                    (Utilities|FlowControl|Delay 0.2)
                    (goto _label_3 Reset)))))))
        (:Is%20Not%20Valid
          (goto _label))))))

(event Custom|DrawHolster%20-Server
  (params (Redraw :type Boolean) (Force :type Boolean))
  ;[1 1 1] Draw
  (CallFunction|DrawHolster-ALL Redraw Force))

(event Custom|TakeWeaponType
  (params (Subtype :type E_WeaponType%20Enum :default "NewEnumerator0"))
  (bind _returnvalue (Components|GetOwner))
  (bind _returnvalue_2 (Actor|GetComponentbyClass _returnvalue "/Game/ModernRPG/General/Blueprints/ActorComponents/InteractActors/AC_EquipmentHandler.AC_EquipmentHandler_C"))
  (bind (_array_element _array_index _has) (Default|GetWeaponItembySubtype _returnvalue_2 Subtype))
  ;[1 1 1] Take Any Weapon
  (if _has
    (CallFunction|SwitchEvent-Server _array_element _array_index)))

(event EventBeginPlay
  ;[1 1 1] Initialize
  (Variables|Default|SetPlayerState (Actor|GetComponentbyClass (Components|GetOwner) "/Game/ModernRPG/General/Blueprints/ActorComponents/Character/State/AC_PlayerCurrentState.AC_PlayerCurrentState_C"))
  (Utilities|FlowControl|Delay 2.0)
  (CallFunction|UpdateInformation false)
  (CallFunction|Initialize false))

(event EventSetMainUIRef
  (params (UI :type User%20Widget%20Object%20Reference))
  ;[1 1 1] Initialize
  (Variables|Engine|SetMainUI UI))

(fn GetOwnerSceneComponent
  (bind _returnvalue (Components|GetOwner))
  (bind _returnvalue_2 (Actor|GetComponentbyClass _returnvalue "/Game/ModernRPG/General/Blueprints/ActorComponents/InteractActors/AC_EquipmentHandler.AC_EquipmentHandler_C"))
  (bind _actor (Default|GetCurrentWeaponActorbyType _returnvalue_2))
  (bind _mesh (Default|GetUsedSceneComponent _actor))
  (Utilities|IsValid _returnvalue_2
    (:Is%20Valid
      (Utilities|IsValid _actor
        (:Is%20Valid
          (Utilities|IsValid _mesh
            (:Is%20Valid
              (return _mesh))))))))

(fn InitializeWeaponMontages
  (params (Redraw :type Boolean))
  (CallFunction|Initialize-Server Redraw))

(fn SwitchEvent
  (params (Item :type S%20Inv%20Item%20Dyn%20Structure) (Index :type Integer))
  (if (Math|Boolean|ANDBoolean (not (Variables|Settings|GetHolstered)) (Utilities|Enum|NotEqual(Enum) (Variables|/Game/ModernRPG/General/Blueprints/ActorComponents/Character/State/AC_PlayerCurrentState.AC_PlayerCurrentState_C|GetCurrentState (Actor|GetComponentbyClass (Components|GetOwner) "/Game/ModernRPG/General/Blueprints/ActorComponents/Character/State/AC_PlayerCurrentState.AC_PlayerCurrentState_C")) "NewEnumerator2") (not (Default|Aiming? (Actor|GetComponentbyClass (Components|GetOwner) "/Game/ModernRPG/General/Blueprints/ActorComponents/Weapon/AC_Aiming.AC_Aiming_C"))))
    (Default|SwitchTypes (Actor|GetComponentbyClass (Components|GetOwner) "/Game/ModernRPG/General/Blueprints/ActorComponents/InteractActors/AC_EquipmentHandler.AC_EquipmentHandler_C") Item Index false false false)))

(fn GetCurrentWeapon
  (return (CallFunction|GetWeaponInfo (.Row (Utilities|Struct|BreakS_InvItemDyn (Variables|/Game/ModernRPG/General/Blueprints/ActorComponents/InteractActors/AC_EquipmentHandler.AC_EquipmentHandler_C|GetNewItem (Actor|GetComponentbyClass (Components|GetOwner) "/Game/ModernRPG/General/Blueprints/ActorComponents/InteractActors/AC_EquipmentHandler.AC_EquipmentHandler_C")))))))

(fn HaveAnyEquipment?
  (return (> (Utilities|Array|Length (Variables|/Game/ModernRPG/General/Blueprints/ActorComponents/InteractActors/AC_EquipmentHandler.AC_EquipmentHandler_C|GetINV_Equipment (Actor|GetComponentbyClass (Components|GetOwner) "/Game/ModernRPG/General/Blueprints/ActorComponents/InteractActors/AC_EquipmentHandler.AC_EquipmentHandler_C"))) 1)))

(fn SetWeaponUI
  (params (WeaponType :type E_WeaponType%20Enum :default "NewEnumerator0"))
  (Class|BPIWidgetsInfo|ChangeWeaponType(Message) (Variables|/Game/ModernRPG/General/Blueprints/DialoguesQuests/WidgetHandler/AC_MainWidgetHandler.AC_MainWidgetHandler_C|GetCastedMainUI (Actor|GetComponentbyClass (Components|GetOwner) "/Game/ModernRPG/General/Blueprints/DialoguesQuests/WidgetHandler/AC_MainWidgetHandler.AC_MainWidgetHandler_C")) WeaponType))

(fn CanHolster?
  (params (Force :type Boolean))
  (bind _returnvalue (Components|GetOwner))
  (bind _defaultbodymesh (Class|BPIAI|GetDemoSkeletalMeshes(Message) _returnvalue))
  (return (and (Utilities|Enum|Equal(Enum) (Variables|/Game/ModernRPG/General/Blueprints/ActorComponents/Character/State/AC_PlayerCurrentState.AC_PlayerCurrentState_C|GetCurrentState (Actor|GetComponentbyClass _returnvalue "/Game/ModernRPG/General/Blueprints/ActorComponents/Character/State/AC_PlayerCurrentState.AC_PlayerCurrentState_C")) "NewEnumerator4") (or (not (Class|AnimInstance|IsAnyMontagePlaying (Components|SkeletalMesh|GetAnimInstance _defaultbodymesh))) Force))))

(fn GetEquipmentComponent
  (return (Actor|GetComponentbyClass (Components|GetOwner) "/Game/ModernRPG/General/Blueprints/ActorComponents/InteractActors/AC_EquipmentHandler.AC_EquipmentHandler_C")))

(fn SetUnarmedABP
  (bind _ascharacter (Utilities|Casting|CastToCharacter (Components|GetOwner)))
  (bind _defaultbodymesh (Class|BPIAI|GetDemoSkeletalMeshes(Message) _ascharacter))
  (Class|BPIOptimization|SetUnarmed(Message) (Components|SkeletalMesh|GetAnimInstance _defaultbodymesh) (Variables|Settings|GetHolstered)))

(fn InitializeUnarmedSockets
  (Default|SetUnarmedState (Actor|GetComponentbyClass (Components|GetOwner) "/Game/ModernRPG/General/Blueprints/Combat/AC_CombatEvents.AC_CombatEvents_C")))

(fn CanEquip
  (bind _defaultbodymesh (Class|BPIAI|GetDemoSkeletalMeshes(Message) (.AsCharacter (Utilities|Casting|CastToCharacter (Components|GetOwner)))))
  (return (not (Class|AnimInstance|IsAnyMontagePlaying (Components|SkeletalMesh|GetAnimInstance _defaultbodymesh)))))

(fn MESSAGETOABPEquip
  (params (SequenceLength :type Float%20%28double-precision%29))
  (Class|BPIABP|Equip(Message) (Components|SkeletalMesh|GetAnimInstance (Variables|/Script/Engine.Character|GetMesh (.AsCharacter (Utilities|Casting|CastToCharacter (Components|GetOwner))))) SequenceLength))