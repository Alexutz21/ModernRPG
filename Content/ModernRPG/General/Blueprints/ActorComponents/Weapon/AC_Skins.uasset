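; Actor component that applies the current character skin to its owner's modular body meshes.
; Shortly after BeginPlay it applies any non-default skin, routing through a Server event when remote and an ALL event to reach every machine.
; The loop pairs head, body, torso, legs and feet components with the skin's entries, setting each skeletal mesh, materials and a shared AnimBP.
; InitializeNewSkin is an empty stub.
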(event Custom|ApplySkinsToAllMeshComponents
  ;[1 1 1] Initialize Mesh Information
  (Networking|SwitchHasAuthority
    (:Authority
      (CallFunction|ApplySkinstoAllMeshComponents-ALL))
    (:Remote
      (CallFunction|ApplySkinstoAllMeshComponents-Server))))

(event Custom|ApplySkinsToAllMeshComponents%20-%20ALL
  ;[1 1 1] Initialize Mesh Information
  (CallFunction|ApplySkinstoAllMeshComponents-Loop))

(event Custom|ApplySkinsToAllMeshComponents%20-%20Server
  ;[1 1 1] Initialize Mesh Information
  (CallFunction|ApplySkinstoAllMeshComponents-ALL))

(event EventBeginPlay
  ;[1 1 1] Initialize Skins
  (bind _ascharacter (Utilities|Casting|CastToCharacter (Components|GetOwner)))
  (Variables|Default|SetPlayer _ascharacter)
  (Utilities|FlowControl|Delay 0.1)
  (bind _default (CallFunction|GetCurrentSkin))
  (if (not _default)
    (CallFunction|ApplySkinstoAllMeshComponents)))

(fn InitializeNewSkin)

(fn ApplyNewBodyPartNewMaterials
  (params (CurrentBodyPart%28instance%29 :type Skeletal%20Mesh%20Component%20Object%20Reference) (NewBodyPart :type Skeletal%20Mesh%20Object%20Reference) (NewMaterials :type Array%20of%20Material%20Instance%20Object%20References) (NewAnimClass :type Object%20Class%20Reference))
  (Class|SkinnedMeshComponent|SetSkeletalMesh CurrentBodyPart%28instance%29 NewBodyPart true)
  (Class|SkeletalMeshComponent|SetAnimClass CurrentBodyPart%28instance%29 NewAnimClass)
  (for (_array_element _array_index) NewMaterials
    (Rendering|Material|SetMaterial CurrentBodyPart%28instance%29 _array_index _array_element))
  (return))

(fn ApplySkinstoAllMeshComponents-Loop
  (bind (_head _body _torso _legs _feet _animbp) (CallFunction|GetCurrentSkin))
  (LocalVariables|SettempArray (Utilities|Array|MakeArray _head _body _torso _legs _feet))
  (LocalVariables|SettempAnimBP _animbp)
  (bind (_headmesh _bodymesh _torsomesh _legsmesh _feetmesh) (CallFunction|GetCharacterSkeleton (Variables|Default|GetPlayer)))
  (for (_array_element _array_index) (Utilities|Array|MakeArray _headmesh _bodymesh _torsomesh _legsmesh _feetmesh)
    (Utilities|IsValid _array_element
      (:Is%20Valid
        (CallFunction|ApplyNewBodyPartNewMaterials _array_element (.SkeletalMesh (Utilities|Struct|BreakS_CharacterSkin_Separated (Utilities|Array|Get(acopy) (LocalVariables|GettempArray) _array_index))) (.Materials (Utilities|Struct|BreakS_CharacterSkin_Separated (Utilities|Array|Get(acopy) (LocalVariables|GettempArray) _array_index))) (LocalVariables|GettempAnimBP)))))
  (return))