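; Actor component that lets a character hold breath while aiming, slowing the body mesh's animation during the hold.
; Starting requires the aiming component to report aiming; a timer ends the hold if not stopped earlier, then a delay gates the next one.
; Tick eases the mesh's global animation rate between min and max, switching itself off once the target is reached.
; Start and end each play a 2D sound.
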(event Custom|StartHoldBreath
  ;[1 1 1] Start and Stop breathing
  (if (Default|Aiming? (Actor|GetComponentbyClass (Components|GetOwner) "/Game/ModernRPG/General/Blueprints/ActorComponents/Weapon/AC_Aiming.AC_Aiming_C"))
    (if (Variables|Default|GetCanHoldBreath)
      (Variables|Default|SetCanHoldBreath false)
      (Audio|PlaySound2D (Variables|Sounds|GetHoldBreathStartSound) 1.0 1.0 0.0 0 0)
      (Variables|Default|SetHoldingBreath true)
      (bind _returnvalue (Utilities|Time|SetTimerbyEvent (delegate Custom|StopHoldBreath) (Variables|Setup|GetBreathTime)))
      (Variables|Default|SetBreathTimer _returnvalue)
      (Variables|Default|SetAnimate? true)
      (Components|Tick|SetComponentTickEnabled true))))

(event Custom|StopHoldBreath
  ;[1 1 1] Start and Stop breathing
  (if (Variables|Default|GetHoldingBreath)
    (Audio|PlaySound2D (Variables|Sounds|GetHoldBreathEndSound) 1.0 1.0 0.0 0 0)
    (Variables|Default|SetHoldingBreath false)
    (Utilities|Time|PauseTimerbyHandle (Variables|Default|GetBreathTimer))
    (Variables|Default|SetAnimate? true)
    (Components|Tick|SetComponentTickEnabled true)
    (Utilities|FlowControl|Delay (Variables|Setup|GetHoldBreathDelay))
    (Variables|Default|SetCanHoldBreath true)))

(event EventTick
  (params (DeltaSeconds :type Float%20%28single-precision%29))
  (bind _playermesh (Variables|Default|GetPlayerMesh))
  ;[1 1 1] Interpolation of the AnimationPlayRate
  (if (Variables|Default|GetAnimate?)
    (bind _output_get (Variables|/Script/Engine.SkeletalMeshComponent|SetGlobalAnimRateScale _playermesh (Math|Interpolation|FInterpTo (Variables|/Script/Engine.SkeletalMeshComponent|GetGlobalAnimRateScale _playermesh) (select (Variables|Default|GetHoldingBreath) (Variables|AnimationRate|GetMinPlayRate) (Variables|AnimationRate|GetMaxPlayRate)) (Utilities|Time|GetWorldDeltaSeconds) 13.0)))
    (if (select (Variables|Default|GetHoldingBreath) (<= _output_get (Variables|AnimationRate|GetMinPlayRate)) (>= _output_get (Variables|AnimationRate|GetMaxPlayRate)))
      (Variables|Default|SetAnimate? false)
      (Components|Tick|SetComponentTickEnabled false))))

(event EventBeginPlay
  ;[1 1 1] Initialize Player Mesh
  (bind _ascharacter (Utilities|Casting|CastToCharacter (Components|GetOwner)))
  (bind _defaultbodymesh (Class|BPIAI|GetDemoSkeletalMeshes(Message) _ascharacter))
  (Variables|Default|SetPlayerMesh _defaultbodymesh))