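; Actor component that manages 2D background music, starting it on BeginPlay and switching tracks by music type when audio is enabled.
; Tracks come from a level BP_AudioHelper actor if present, otherwise randomly from matching data table rows.
; Two audio components alternate as current and free, crossfading with delayed fade-in on type changes.
; Server events forward to owning-client events, except helper-based setup, which creates sounds directly.
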(event Custom|SwitchMusic%20-Server
  (params (Type :type E_AudioType%20Enum :default "NewEnumerator0"))
  ;[1 1 1] Switch Music
  (if (Variables|Settings|GetAudioEnabled)
    (CallFunction|SwitchMusic-OC Type)))

(event Custom|CreateMusic%20-Server
  ;[1 1 1] Initialize Sounds
  (CallFunction|CreateMusic-OC))

(event Custom|CreateMusic%20-OC
  ;[1 1 1] Initialize Sounds
  (bind _returnvalue (Audio|CreateSound2D (CallFunction|GetSoundbyType "NewEnumerator0") 1.0 1.0 0.0 0 false false))
  (Variables|Default|SetSound_1 _returnvalue)
  (bind _returnvalue_2 (Audio|CreateSound2D (CallFunction|GetSoundbyType "NewEnumerator1") 1.0 1.0 0.0 0 false false))
  (Variables|Default|SetSound_2 _returnvalue_2)
  (Utilities|IsValid (Variables|Default|GetSound_1)
    (:Is%20Valid
      (Audio|Components|Audio|Play (Variables|Default|GetSound_1) 0.0))))

(event Custom|SwitchMusic%20-OC
  (params (Type :type E_AudioType%20Enum :default "NewEnumerator0"))
  ;[1 1 1] Switch Music
  (if (Utilities|Enum|NotEqual(Enum) Type (Variables|Default|GetCurrentType))
    (Variables|Default|SetCurrentType Type)
    (Audio|Components|Audio|FadeOut (CallFunction|GetCurrentSound) 2.0 0.0 "SCurve" :!class /Script/Engine.AudioComponent)
    (Utilities|FlowControl|Sequence
      (:then_0
        (Utilities|FlowControl|Delay 1.0)
        (Utilities|IsValid (Variables|Default|GetHelperActor)
          (:Is%20Valid
            (Variables|Default|SetCurSound (Default|GetSoundbyType (Variables|Default|GetHelperActor) (Variables|Default|GetCurrentType))))
          (:Is%20Not%20Valid
            (Variables|Default|SetCurSound (CallFunction|GetSoundbyType (Variables|Default|GetCurrentType)))))
        (Utilities|IsValid (Variables|Default|GetCurSound)
          (:Is%20Valid
            (Audio|Components|Audio|SetSound (CallFunction|GetFreeSound) (Variables|Default|GetCurSound))
            (Audio|Components|Audio|FadeIn (CallFunction|GetFreeSound) 3.0 1.0 0.0 "SCurve" :!class /Script/Engine.AudioComponent))
          (:Is%20Not%20Valid
            _))
        (Variables|Default|SetCurrentSoundFirst (not (Variables|Default|GetCurrentSoundFirst))))
      (:then_1
        (Utilities|FlowControl|Delay 0.5)
        (Audio|Components|Audio|Stop (CallFunction|GetFreeSound))))))

(event Custom|CreateMusicHelper%20-Server
  ;[1 1 1] Create Sounds Classes
  (bind _returnvalue (Audio|CreateSound2D (Default|GetSoundbyType (Variables|Default|GetHelperActor) "NewEnumerator0") 1.0 1.0 0.0 0 false false))
  (Variables|Default|SetSound_1 _returnvalue)
  (bind _returnvalue_2 (Audio|CreateSound2D (Default|GetSoundbyType (Variables|Default|GetHelperActor) "NewEnumerator0") 1.0 1.0 0.0 0 false false))
  (Variables|Default|SetSound_2 _returnvalue_2)
  (Utilities|IsValid (Variables|Default|GetSound_1)
    (:Is%20Valid
      (Audio|Components|Audio|Play (Variables|Default|GetSound_1) 0.0))))

(event EventBeginPlay
  ;[1 1 1] Initialzie Music Actors
  (if (Variables|Settings|GetAudioEnabled)
    (bind _returnvalue (Actor|GetActorOfClass "/Game/ModernRPG/General/Blueprints/Audio/BP_AudioHelper.BP_AudioHelper_C"))
    (Utilities|IsValid _returnvalue
      (:Is%20Valid
        (Variables|Default|SetHelperActor _returnvalue)
        (Variables|Default|SetHelperValid true))
      (:Is%20Not%20Valid
        _))
    (if (Variables|Default|GetHelperValid)
      (CallFunction|CreateMusicHelper-Server)
      (else
        (CallFunction|CreateMusic-Server)))))

(fn GetSoundbyType
  (params (Type :type E_AudioType%20Enum :default "NewEnumerator0"))
  (bind _outrownames (DataTable|GetDataTableRowNames (Variables|Settings|GetAudioDataTable)))
  (for _array_element _outrownames
    (bind _returnvalue (Utilities|GetDataTableRow (Variables|Settings|GetAudioDataTable) _array_element)
      (:then
        (if (Utilities|Enum|Equal(Enum) (.Type (Utilities|Struct|BreakS_AudioTypes _returnvalue)) Type)
          (return (Utilities|Array|Get(acopy) (.Sounds (Utilities|Struct|BreakS_AudioTypes _returnvalue)) (Math|Random|RandomIntegerinRange 0 (- (Utilities|Array|Length (.Sounds (Utilities|Struct|BreakS_AudioTypes _returnvalue))) 1)))))))))

(fn GetCurrentSound
  (return (select (Variables|Default|GetCurrentSoundFirst) (Variables|Default|GetSound_1) (Variables|Default|GetSound_2))))

(fn GetFreeSound
  (return (select (Variables|Default|GetCurrentSoundFirst) (Variables|Default|GetSound_2) (Variables|Default|GetSound_1))))