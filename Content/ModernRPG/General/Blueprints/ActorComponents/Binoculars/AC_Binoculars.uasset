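; Actor component that switches its owner's binoculars camera between a night-vision look and the default look.
; InteractWithBinoculars toggles the binocular state, swapping the main camera's post-process settings, which it fetches from the owner through an interface message.
; A half-second lock after each toggle blocks rapid repeat switching.
; DisableNightMode forces the default post-process and the Off state directly, bypassing the lock.
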(event Custom|DisableNightMode-%20OC
  ;[1 1 1] Control night/default camera mode
  (bind _camera (Class|BPIAI|GetMainCamera(Message) (Components|GetOwner)))
  (Variables|/Script/Engine.CameraComponent|SetPostProcessSettings _camera (Variables|Default|GetDefault%20Post%20Process))
  (Variables|Default|SetE_BinType "NewEnumerator3"))

(event Custom|InteractWithBinoculars%20-%20OC
  ;[1 1 1] Control night/default camera mode
  (if (not (Variables|Default|GetLocked))
    (switch Utilities|FlowControl|Switch|SwitchonE_BinType (Variables|Default|GetE_BinType)
      (:NewEnumerator1
        (bind _camera (Class|BPIAI|GetMainCamera(Message) (Components|GetOwner)))
        (Variables|/Script/Engine.CameraComponent|SetPostProcessSettings _camera (Variables|Default|GetDefault%20Post%20Process))
        (Variables|Default|SetE_BinType "NewEnumerator3"))
      (:NewEnumerator3
        (bind _camera_2 (Class|BPIAI|GetMainCamera(Message) (Components|GetOwner)))
        (Variables|/Script/Engine.CameraComponent|SetPostProcessSettings _camera_2 (Variables|Default|GetNight%20Post%20Process))
        (Variables|Default|SetE_BinType "NewEnumerator1")))
    (Variables|Default|SetLocked true)
    (Utilities|FlowControl|Delay 0.5)
    (Variables|Default|SetLocked false)))