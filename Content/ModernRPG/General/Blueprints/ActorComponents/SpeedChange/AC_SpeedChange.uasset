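; Character actor component that switches replicated walk states such as sprint, setting movement speed and camera arm length for each.
; States read a data table, with speed scaled by the skill tree modifier, and notify the animation blueprint.
; Tick interpolates players outside vehicles toward idle or state targets and replicates speed, while AI disables tick and applies speed instantly.
; Sprint binds a characteristic's spend event, and depletion resets the walk state.
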(event Custom|ChangeWalkSpeed%20-Server
  (params (InputPin :type E_WalkState%20Enum :default "NewEnumerator3"))
  ;[1 1 1] Multiplayered Speed Change
  (CallFunction|ChangeWalkSpeed-ALL InputPin))

(event Custom|ChangeWalkSpeed
  (params (InputPin :type E_WalkState%20Enum :default "NewEnumerator3"))
  (bind _returnvalue (Components|GetOwner))
  (bind _component (CallFunction|GetCharacteristicbyType _returnvalue "NewEnumerator2"))
  ;[1 1 1] Replicated Walk Speed Change
  (if (Utilities|Enum|NotEqual(Enum) InputPin (Variables|Default|GetCurrentWalkState))
    (Variables|Default|SetCurrentWalkState InputPin)
    (if (Ability|HasAuthority (Components|GetOwner))
      (CallFunction|ChangeWalkSpeed-ALL (Variables|Default|GetCurrentWalkState))
      (else
        (CallFunction|ChangeWalkSpeed-Server (Variables|Default|GetCurrentWalkState))))
    (Utilities|IsValid _component
      (:Is%20Valid
        (CallFunction|ChangeWalkSpeed-OC (Utilities|Enum|Equal(Enum) (Variables|Default|GetCurrentWalkState) "NewEnumerator1") _component)))))

(event Custom|BelowZero_Event_0
  (params (SpentDamage :type Float%20%28double-precision%29))
  ;[1 1 1] Set start speed
  (Class|BPIInput|ResetSprint(Message) (Components|GetOwner))
  (CallFunction|ChangeWalkSpeed "NewEnumerator0"))

(event Custom|ChangeWalkSpeed%20-ALL
  (params (InputPin :type E_WalkState%20Enum :default "NewEnumerator3"))
  ;[1 1 1] Multiplayered Speed Change
  (CallFunction|ChangeWalkState InputPin)
  (Default|CallCurrentWalkStateCHANGED)
  (CallFunction|MESSAGETOABPWalkState)
  (if (Variables|Default|GetOwnerAI)
    (Variables|Default|SetLastWalkSpeed (Variables|Default|GetTargetSpeed))
    (Variables|/Script/Engine.CharacterMovementComponent|SetMaxWalkSpeed (Variables|Default|GetCharacterMovement) (Variables|Default|GetLastWalkSpeed))))

(event Custom|ChangeWalkSpeed%20-OC
  (params (Condition :type Boolean) (InputPin :type AC%20Characteristics%20Object%20Reference))
  ;[1 1 1] Multiplayered Speed Change
  (Utilities|IsValid InputPin
    (:Is%20Valid
      (if Condition
        (Default|BindSpentEvent InputPin)
        (else
          (Default|StopSpentEvent InputPin))))))

(event Custom|ReplicateSpeed%20-ALL
  (params (LastWalkSpeed :type Float%20%28double-precision%29))
  ;[1 1 1] Replicate Speed
  (Variables|Default|SetLastWalkSpeed LastWalkSpeed))

(event Custom|ReplicateSpeed
  (bind _lastwalkspeed (Variables|Default|GetLastWalkSpeed))
  ;[1 1 1] Replicate Speed
  (if (Ability|HasAuthority (Components|GetOwner))
    (CallFunction|ReplicateSpeed-ALL _lastwalkspeed)
    (else
      (CallFunction|ReplicateSpeed-Server _lastwalkspeed))))

(event Custom|ReplicateSpeed%20-Server
  (params (LastWalkSpeed :type Float%20%28double-precision%29))
  ;[1 1 1] Replicate Speed
  (CallFunction|ReplicateSpeed-ALL LastWalkSpeed))

(event EventBeginPlay
  (bind _returnvalue (Components|GetOwner))
  (bind _component (CallFunction|GetCharacteristicbyType _returnvalue "NewEnumerator2"))
  ;[1 1 1] Set start speed
  (Utilities|FlowControl|Sequence
    (:then_0
      (CallFunction|SetIdleValues)
      (CallFunction|RememberSpringArm)
      (Variables|Default|SetLastWalkSpeed (Variables|/Script/Engine.CharacterMovementComponent|GetMaxWalkSpeed (Actor|GetComponentbyClass (Components|GetOwner) "/Script/Engine.CharacterMovementComponent")))
      (Variables|Default|SetCharacterMovement (Actor|GetComponentbyClass (Components|GetOwner) "/Script/Engine.CharacterMovementComponent"))
      (Utilities|IsValid _component
        (:Is%20Valid
          (EventDispatchers|AssignBelowZero _component (delegate Custom|BelowZero_Event_0))
          (bind _output_get (Variables|Default|SetMinimap (Actor|GetComponentbyClass (Components|GetOwner) "/Game/ModernRPG/General/Blueprints/ActorComponents/Minimap/AC_Minimap.AC_Minimap_C")))
          (Utilities|IsValid _output_get
            (:Is%20Valid
              (Variables|Default|SetHasMimimap true))
            (:Is%20Not%20Valid
              (Variables|Default|SetHasMimimap false))))))
    (:then_1
      (bind _ascharacter (Utilities|Casting|CastToCharacter (Components|GetOwner)))
      (if (not (Pawn|IsPlayerControlled _ascharacter))
        (Components|Tick|SetComponentTickEnabled false)
        (Variables|Default|SetOwnerAI true)))))

(event EventTick
  (params (DeltaSeconds :type Float%20%28single-precision%29))
  ;[1 1 1] Change Speed
  (if (not (CallFunction|InVehicle))
    (if (not (CallFunction|GenerationFinished))
      (if (Variables|Default|GetCanChange)
        (if (Variables|Default|GetHasMimimap)
          _
          (else
            _))
        (Utilities|IsValid (Variables|Default|GetSpringArm)
          (:Is%20Valid
            (Variables|/Script/Engine.SpringArmComponent|SetTargetArmLength (Variables|Default|GetSpringArm) (select (Variables|/Game/ModernRPG/General/Blueprints/ActorComponents/ViewSwitch/AC_ViewSwitch.AC_ViewSwitch_C|GetInThirdPerson (Actor|GetComponentbyClass (Components|GetOwner) "/Game/ModernRPG/General/Blueprints/ActorComponents/ViewSwitch/AC_ViewSwitch.AC_ViewSwitch_C")) (Math|Interpolation|FInterpTo (Variables|/Script/Engine.SpringArmComponent|GetTargetArmLength (Variables|Default|GetSpringArm)) (CallFunction|GetSpringArm) (Utilities|Time|GetWorldDeltaSeconds) (Variables|Default|GetArmInterpSpeed)) 0.0)))
          (:Is%20Not%20Valid
            _))
        (Variables|Default|SetLastWalkSpeed (Math|Interpolation|FInterpTo (Variables|Default|GetLastWalkSpeed) (CallFunction|GetSpeed) (Utilities|Time|GetWorldDeltaSeconds) (Variables|Default|GetArmInterpSpeed)))
        (Variables|/Script/Engine.CharacterMovementComponent|SetMaxWalkSpeed (Variables|Default|GetCharacterMovement) (Variables|Default|GetLastWalkSpeed))
        (CallFunction|ReplicateSpeed))
      (else
        (Variables|/Script/Engine.CharacterMovementComponent|SetMaxWalkSpeed (Variables|Default|GetCharacterMovement) (Variables|Default|GetLastWalkSpeed))))))

(fn GetAngleSpeed
  (bind _returnvalue (Components|GetOwner))
  (bind _returnvalue_2 (Actor|GetComponentbyClass _returnvalue "/Game/ModernRPG/General/Blueprints/ActorComponents/AI/AC_AngleSpeed.AC_AngleSpeed_C"))
  (bind _newspeed (Default|AngleSpeedPerc _returnvalue_2))
  (bind _returnvalue_3 (+ 0.0 _newspeed))
  (Utilities|IsValid _returnvalue_2
    (:Is%20Valid
      (return (Math|Float|Clamp(Float) (select (< _returnvalue_3 0.0) (+ (/ (Math|Float|Absolute(Float) _returnvalue_3) 1e+02) 1.0) (- 1.0 (/ _returnvalue_3 1e+02))) 0.15 3.0)))
    (:Is%20Not%20Valid
      (return 1.0))))

(fn ChangeWalkState
  (params (InputPin :type E_WalkState%20Enum :default "NewEnumerator3"))
  (bind (_newspeed _newspringarm _minimap) (CallFunction|GetTypeSpeed InputPin))
  (Variables|Default|SetCurrentWalkState InputPin)
  (Variables|Default|SetTargetSpeed (* (CallFunction|GetSkillModification) _newspeed))
  (Variables|Default|SetTargetMinimap _minimap)
  (Variables|Default|SetTargetSpringArm _newspringarm))

(fn GetTypeSpeed
  (params (InputPin :type E_WalkState%20Enum :default "NewEnumerator3"))
  (bind _outrownames (DataTable|GetDataTableRowNames (Variables|Setup|GetSpeed%20Data%20Table)))
  (for _array_element _outrownames
    (bind _returnvalue (Utilities|GetDataTableRow (Variables|Setup|GetSpeed%20Data%20Table) _array_element)
      (:then
        (if (Utilities|Enum|Equal(Enum) (.Type (Utilities|Struct|BreakS_WalkStateStr _returnvalue)) InputPin)
          (return (.Speed (Utilities|Struct|BreakS_WalkStateStr _returnvalue)) (.CamSpringArm (Utilities|Struct|BreakS_WalkStateStr _returnvalue)) (.Minimap (Utilities|Struct|BreakS_WalkStateStr _returnvalue))))))))

(fn Sprint?
  (return (Utilities|Enum|Equal(Enum) (Variables|Default|GetCurrentWalkState) "NewEnumerator1")))

(fn GetCurrentTypeSpeed
  (LocalVariables|SetCheckedWalkSPeed (select (<= (Math|Vector|VectorLength (Transformation|GetVelocity (Components|GetOwner))) 0.0) "NewEnumerator3" (Variables|Default|GetCurrentWalkState)))
  (bind _outrownames (DataTable|GetDataTableRowNames (Variables|Setup|GetSpeed%20Data%20Table)))
  (for _array_element _outrownames
    (bind _returnvalue (Utilities|GetDataTableRow (Variables|Setup|GetSpeed%20Data%20Table) _array_element)
      (:then
        (if (Utilities|Enum|Equal(Enum) (.Type (Utilities|Struct|BreakS_WalkStateStr _returnvalue)) (LocalVariables|GetCheckedWalkSPeed))
          (return (.Speed (Utilities|Struct|BreakS_WalkStateStr _returnvalue)) (.CamSpringArm (Utilities|Struct|BreakS_WalkStateStr _returnvalue)) (.Minimap (Utilities|Struct|BreakS_WalkStateStr _returnvalue))))))))

(fn GetSkillModification
  (bind _returnvalue (Components|GetOwner))
  (bind _returnvalue_2 (Actor|GetComponentbyClass _returnvalue "/Game/ModernRPG/ModernSkillTree/ActorComponent/AC_SkillTree.AC_SkillTree_C"))
  (Utilities|IsValid _returnvalue_2
    (:Is%20Valid
      (return (+ 1.0 (/ (Variables|/Game/ModernRPG/ModernSkillTree/ActorComponent/AC_SkillTree.AC_SkillTree_C|GetSpeed_Modifier _returnvalue_2) 1e+02))))
    (:Is%20Not%20Valid
      (return 1.0))))

(fn RememberSpringArm
  (bind _returnvalue (Components|GetOwner))
  (bind _returnvalue_2 (Actor|GetComponentsbyTag _returnvalue "/Script/Engine.SpringArmComponent" "Main"))
  (if (Utilities|Array|IsValidIndex _returnvalue_2)
    (Variables|Default|SetSpringArm (Utilities|Array|Get(acopy) _returnvalue_2))))

(fn GenerationFinished
  (return (Math|Float|NearlyEqual(Float) (Variables|Default|GetLastWalkSpeed) (CallFunction|GetSpeed) 1.0)))

(fn InVehicle
  (bind _returnvalue (Components|GetOwner))
  (bind _returnvalue_2 (Actor|GetComponentbyClass _returnvalue "/Game/ModernRPG/General/Blueprints/ActorComponents/Machinery/AC_VehicleController.AC_VehicleController_C"))
  (Utilities|IsValid _returnvalue_2
    (:Is%20Valid
      (Utilities|IsValid (Variables|/Game/ModernRPG/General/Blueprints/ActorComponents/Machinery/AC_VehicleController.AC_VehicleController_C|GetVehicle _returnvalue_2)
        (:Is%20Valid
          (return true))
        (:Is%20Not%20Valid
          _)))
    (:Is%20Not%20Valid
      _))
  (return false))

(fn SetIdleValues
  (bind (_newspeed _newspringarm _minimap) (CallFunction|GetTypeSpeed "NewEnumerator0"))
  (bind (_newspeed_2 _newspringarm_2 _minimap_2) (CallFunction|GetTypeSpeed "NewEnumerator3"))
  (Variables|Default|SetIdleSpeed _newspeed_2)
  (Variables|Default|SetTargetSpeed (* (CallFunction|GetSkillModification) _newspeed))
  (Variables|Default|SetIdleMinimap _minimap_2)
  (Variables|Default|SetTargetMinimap _minimap)
  (Variables|Default|SetIdleSpringArm _newspringarm_2)
  (Variables|Default|SetTargetSpringArm _newspringarm))

(fn Idle?
  (return (<= (Math|Vector|VectorLength (Transformation|GetVelocity (Components|GetOwner))) 0.0)))

(fn GetMinimap
  (return (select (CallFunction|Idle?) (Variables|Default|GetIdleMinimap) (Variables|Default|GetTargetMinimap))))

(fn GetSpeed
  (return (select (CallFunction|Idle?) (Variables|Default|GetIdleSpeed) (Variables|Default|GetTargetSpeed))))

(fn GetSpringArm
  (return (select (CallFunction|Idle?) (Variables|Default|GetIdleSpringArm) (Variables|Default|GetTargetSpringArm))))

(fn SetCanChange
  (params (CanChange :type Boolean))
  (Variables|Default|SetCanChange CanChange))

(fn MESSAGETOABPWalkState
  (bind _defaultbodymesh (Class|BPIAI|GetDemoSkeletalMeshes(Message) (Components|GetOwner)))
  (Class|BPIABP|OnWalkStateChanged(Message) (Components|SkeletalMesh|GetAnimInstance _defaultbodymesh) (Variables|Default|GetCurrentWalkState)))