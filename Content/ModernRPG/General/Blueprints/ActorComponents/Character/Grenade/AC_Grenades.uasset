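; Character actor component that manages grenade selection, throwing and detonation effects in multiplayer.
; Throws consume inventory items and replicate a weapon-specific montage through server-to-all events, with anim notifies spawning the projectile and clearing the hand mesh.
; Detonations report AI noise and apply radial damage, or for flashbangs use a camera dot-product test to trigger owner-only screen effects.
; Selection updates a chooser widget and HUD icon, and can persist through SaveGame.
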(event Custom|Apply%20Damage%20Effects%20%20-Server
  (params (Location :type Vector) (RadialForce :type Radial%20Force%20Component%20Object%20Reference) (DamageCauser :type Actor%20Object%20Reference) (GrenadeType :type E_GrenadeTypes%20Enum :default "NewEnumerator0") (GrenadeInfo :type S%20Grenades%20Structure))
  ;[1 1 1] Manupulate Grenade Effects
  (CallFunction|ApplyDamageEffects-ALL Location RadialForce DamageCauser GrenadeType GrenadeInfo))

(event Custom|ThrowGrenade%20-Server
  (params (MontageToPlay :type Anim%20Montage%20Object%20Reference))
  ;[1 1 1] Replicated Throw
  (CallFunction|ThrowGrenadeALL MontageToPlay))

(event Custom|CreateChooseGrenadeWidget%20-OC
  ;[1 1 1] Create Grenade Widget
  (UserInterface|Viewport|AddtoViewport (Variables|Default|GetGrenadeWidget) 0)
  (Variables|Default|SetInWidget true))

(event Custom|RemoveGrenadeType%20-%20Server
  (params (Type :type E_GrenadeTypes%20Enum :default "NewEnumerator0"))
  ;[1 1 1] Remove Grenade Type
  (CallFunction|RemoveGrenadeType-ALL Type))

(event Custom|SelectNextGrenade
  (params (Up :type Boolean))
  ;[1 1 1] Remove Grenade Type
  (Default|SelectNextGrenade (Variables|Default|GetGrenadeWidget) Up))

(event Custom|ConnectGrenade%20-Server
  ;[1 1 1] Connect mesh
  (Utilities|FlowControl|DoOnce false
    (:Completed
      (bind _returnvalue (Game|SpawnActorfromClass "/Game/ModernRPG/General/Blueprints/Grenades/BP_Throwable.BP_Throwable_C" (Math|Transform|MakeTransform (Transformation|GetSocketLocation (Variables|Default|GetSK_Mesh) (Variables|Default|GetGrenadeSocket)) (Pawn|GetControlRotation (Variables|Default|GetCharacter) :!class /Script/Engine.Pawn)) "AlwaysSpawn" (Components|GetOwner) (Variables|Default|GetCurrentMesh) 0))
      (bind _output_get (Variables|Default|SetMeshActor _returnvalue))
      (CallFunction|ConnectGrenade-ALL _output_get (Variables|Default|GetSK_Mesh) (Variables|Default|GetGrenadeSocket))
      (Utilities|FlowControl|Delay 0.2)
      (CallFunction|ResetDO))))

(event Custom|RemoveGrenadeType
  (params (Type :type E_GrenadeTypes%20Enum :default "NewEnumerator0"))
  ;[1 1 1] Remove Grenade Type
  (Utilities|HasAutority
    (:Has
      (CallFunction|RemoveGrenadeType-ALL Type))
    (:No
      (CallFunction|RemoveGrenadeType-Server Type))))

(event Custom|SpawnGrenade%20-Server
  ;[1 1 1] Spawn Grenade
  (Utilities|FlowControl|DoOnce false :!label _label
    (:Completed
      (Game|SpawnActorfromClass :Class (Variables|Default|GetCurGrenade) :SpawnTransform (CallFunction|GetGrenadeTransform) :CollisionHandlingOverride "AdjustIfPossibleButAlwaysSpawn" :Owner (Components|GetOwner) :Velocity (CallFunction|GetVelocity) :Instigator 0)
      (Utilities|FlowControl|Delay 0.3)
      (goto _label Reset))))

(event Custom|CreateChooseGrenadeWidget%20-Server
  ;[1 1 1] Create Grenade Widget
  (CallFunction|CreateChooseGrenadeWidget-OC))

(event Custom|CloseGrenadesWidget
  ;[1 1 1] Create Grenade Widget
  (Widget|RemovefromParent (Variables|Default|GetGrenadeWidget))
  (Variables|Default|SetInWidget false))

(event Custom|SetGrenadeType
  (params (Type :type E_GrenadeTypes%20Enum :default "NewEnumerator0"))
  ;[1 1 1] Set Grenade Type Replicated
  (Utilities|HasAutority
    (:Has
      (CallFunction|SetGrenadeType-ALL Type))
    (:No
      (CallFunction|SetGrenadeType-Server Type))))

(event Custom|PlaySound%20-%20OC
  (params (Sound :type Sound%20Base%20Object%20Reference) (VolumeMultiplier :type Float%20%28double-precision%29) (Instigator :type Actor%20Object%20Reference))
  ;[1 1 1] Play Sound
  (CallFunction|SpawnNewEffectSound Sound VolumeMultiplier Instigator)
  (Utilities|FlowControl|Delay (Variables|/Script/Engine.SoundBase|GetDuration (Variables|/Script/Engine.AudioComponent|GetSound (Variables|Default|GetPlayingFlashlightSound))))
  (Variables|Default|SetInFlashbang 0)
  (Variables|Default|SetPlayingFlashlightSound 0))

(event Custom|ResetDO
  ;[1 1 1] Connect mesh
  (Utilities|FlowControl|DoOnce false) ; enters at Reset
)

(event Custom|SetGrenadeType%20-Server
  (params (Type :type E_GrenadeTypes%20Enum :default "NewEnumerator0"))
  ;[1 1 1] Set Grenade Type Replicated
  (CallFunction|SetGrenadeType-ALL Type))

(event Custom|SetGrenadeType%20-ALL
  (params (Type :type E_GrenadeTypes%20Enum :default "NewEnumerator0"))
  (bind _grenadewidget (Variables|Default|GetGrenadeWidget))
  ;[1 1 1] Set Grenade Type Replicated
  (bind _output_get (Variables|GrenadeTypes|SetCurrentGrenadeType Type))
  (Utilities|Array|AddUnique (Variables|GrenadeTypes|GetGrenadeTypesCharacterHas) _output_get)
  (Utilities|IsValid _grenadewidget
    (:Is%20Valid
      (Default|SetSelectedbyType _grenadewidget _output_get)
      (CallFunction|UpdateGrenadeType))))

(event Custom|ThrowGrenade%20ALL
  (params (MontageToPlay :type Anim%20Montage%20Object%20Reference))
  ;[1 1 1] Throw Grenade if you can
  (CallFunction|PlayAnimation MontageToPlay))

(event Custom|InitializeVariables%20-ALL
  (params (GrenadeThrowMontage :type Anim%20Montage%20Object%20Reference) (GrenadeSocket :type Name) (CurGrenade :type BP%20Grenade%20Class%20Reference) (LastThrowedGrenade :type S%20Grenades%20Structure) (CurrentMesh :type Static%20Mesh%20Object%20Reference) (GrenadeArrayIndex :type Integer) (Condition :type Boolean))
  ;[1 1 1] Throw Grenade if you can
  (Variables|Default|SetGrenadeThrowMontage GrenadeThrowMontage)
  (Variables|Default|SetGrenadeSocket GrenadeSocket)
  (Variables|Default|SetCurGrenade CurGrenade)
  (Variables|Default|SetHasGrenade Condition)
  (Variables|Default|SetLast%20Throwed%20Grenade LastThrowedGrenade)
  (Variables|Default|SetCurrentMesh CurrentMesh)
  (Variables|Default|SetGrenadeArrayIndex GrenadeArrayIndex))

(event Custom|InitializeVariables%20-Server
  (params (GrenadeThrowMontage :type Anim%20Montage%20Object%20Reference) (GrenadeSocket :type Name) (CurGrenade :type BP%20Grenade%20Class%20Reference) (LastThrowedGrenade :type S%20Grenades%20Structure) (CurrentMesh :type Static%20Mesh%20Object%20Reference) (GrenadeArrayIndex :type Integer) (Condition :type Boolean))
  ;[1 1 1] Throw Grenade if you can
  (CallFunction|InitializeVariables-ALL GrenadeThrowMontage GrenadeSocket CurGrenade LastThrowedGrenade CurrentMesh GrenadeArrayIndex Condition))

(event Custom|InitializeVariables
  (bind _returnvalue (Components|GetOwner))
  (bind (_grenade _grenadesocket) (CallFunction|GetWeaponInfo))
  (bind _currentgrenadetype (Variables|GrenadeTypes|GetCurrentGrenadeType))
  (bind _returnvalue_2 (Actor|GetComponentbyClass _returnvalue "/Game/ModernRPG/General/Blueprints/ActorComponents/Character/Inventory/AC_Inventory.AC_Inventory_C"))
  (bind (_res _actor _overviewmesh _array_index _icon _grenadeinfo) (Default|GetGrenade _returnvalue_2 _currentgrenadetype))
  ;[1 1 1] Throw Grenade if you can
  (CallFunction|InitializeVariables-Server _grenade _grenadesocket _actor _grenadeinfo _overviewmesh _array_index _res))

(event Custom|PlayAnimation
  (params (MontageToPlay :type Anim%20Montage%20Object%20Reference))
  (bind _equipment (Variables|Default|GetEquipment))
  (bind _actor (Default|GetCurrentWeaponActorbyType _equipment))
  ;[1 1 1] Play Throw Grenade Animation
  (Variables|Default|SetThrowing true)
  (Default|UpdateState (Actor|GetComponentbyClass (Components|GetOwner) "/Game/ModernRPG/General/Blueprints/ActorComponents/Character/State/AC_PlayerCurrentState.AC_PlayerCurrentState_C") "NewEnumerator3")
  (bind _notifyname (Utilities|PlayAnyMontage MontageToPlay)
    (:then
      (Utilities|IsValid (Variables|Default|GetGrenadeThrowMontage)
        (:Is%20Not%20Valid
          (Utilities|IsValid _actor
            (:Is%20Valid
              (Default|AttachActor _actor))
            (:Is%20Not%20Valid
              _))
          (Default|UpdateState (Actor|GetComponentbyClass (Components|GetOwner) "/Game/ModernRPG/General/Blueprints/ActorComponents/Character/State/AC_PlayerCurrentState.AC_PlayerCurrentState_C") "NewEnumerator4"))))
    (:On%20Completed
      (Default|UpdateState (Actor|GetComponentbyClass (Components|GetOwner) "/Game/ModernRPG/General/Blueprints/ActorComponents/Character/State/AC_PlayerCurrentState.AC_PlayerCurrentState_C") "NewEnumerator4"))
    (:On%20Notify%20Begin
      (CallFunction|OnNotifyBegin _notifyname))
    (:On%20Notify%20End
      (CallFunction|OnNotifyEnd _notifyname))))

(event Custom|FlashEvent
  ;[1 1 1] Flash Event
  (if (Ability|HasAuthority (Components|GetOwner))
    (CallFunction|FlashEvent-OC)
    (else
      (CallFunction|FlashEvent-Server))))

(event Custom|FlashEvent%20-Server
  ;[1 1 1] Flash Event
  (CallFunction|FlashEvent-OC))

(event Custom|DestroyGrenadeActorOn%20-Server
  (params (Target :type Actor%20Object%20Reference))
  ;[1 1 1] Remove Replicated
  (Utilities|IsValid Target
    (:Is%20Valid
      (Actor|DestroyActor Target))))

(event Custom|DestroyConnectedMesh%20-%20Server
  ;[1 1 1] Remove Grenade
  (CallFunction|DestroyConnectedMesh-ALL))

(event Custom|DestroyConnectedMesh%20-%20ALL
  ;[1 1 1] Remove Grenade
  (CallFunction|DestroyConnectedMesh))

(event Custom|FlashEvent%20-OC
  ;[1 1 1] Flash Event
  (bind _returnvalue (UserInterface|CreateWidget "/Game/ModernRPG/General/Blueprints/ActorComponents/Character/Grenade/WB_FlashlightEffect.WB_FlashlightEffect_C"))
  (UserInterface|Viewport|AddtoViewport _returnvalue 0))

(event Custom|TryToRotateTowards
  (params (MontageToPlay :type Anim%20Montage%20Object%20Reference))
  ;[1 1 1] Replicated Throw
  (if (Variables|/Game/ModernRPG/General/Blueprints/ActorComponents/ViewSwitch/AC_ViewSwitch.AC_ViewSwitch_C|GetInThirdPerson (Actor|GetComponentbyClass (Components|GetOwner) "/Game/ModernRPG/General/Blueprints/ActorComponents/ViewSwitch/AC_ViewSwitch.AC_ViewSwitch_C"))
    (bind _aspawn (Utilities|Casting|CastToPawn (Components|GetOwner)))
    (Variables|/Script/Engine.Pawn|SetbUseControllerRotationYaw _aspawn true)
    (Utilities|FlowControl|Delay (Variables|/Script/Engine.AnimSequenceBase|GetSequenceLength MontageToPlay))))

(event Custom|Apply%20Damage%20Effects
  (params (Location :type Vector) (DamageCauser :type Actor%20Object%20Reference) (RadialForce :type Radial%20Force%20Component%20Object%20Reference) (GrenadeType :type E_GrenadeTypes%20Enum :default "NewEnumerator0") (Grenade :type S%20Grenades%20Structure))
  ;[1 1 1] Remove Grenade
  (Utilities|HasAutority
    (:Has
      (CallFunction|ApplyDamageEffects-ALL Location RadialForce DamageCauser GrenadeType Grenade))
    (:No
      (CallFunction|ApplyDamageEffects-Server Location RadialForce DamageCauser GrenadeType Grenade))))

(event Custom|Apply%20Damage%20Effects%20-%20ALL
  (params (Location :type Vector) (RadialForce :type Radial%20Force%20Component%20Object%20Reference) (DamageCauser :type Actor%20Object%20Reference) (GrenadeType :type E_GrenadeTypes%20Enum :default "NewEnumerator0") (GrenadeInfo :type S%20Grenades%20Structure))
  ;[1 1 1] Manupulate Grenade Effects
  (CallFunction|ApplyDamageEffectsFunctionality Location RadialForce DamageCauser GrenadeType GrenadeInfo))

(event Custom|RemoveGrenadeType%20-%20ALL
  (params (Type :type E_GrenadeTypes%20Enum :default "NewEnumerator0"))
  (bind _grenadetypescharacterhas (Variables|GrenadeTypes|GetGrenadeTypesCharacterHas))
  ;[1 1 1] Remove Grenade Type
  (Utilities|Array|RemoveItem _grenadetypescharacterhas Type)
  (if (Utilities|Array|IsValidIndex _grenadetypescharacterhas)
    (Variables|GrenadeTypes|SetCurrentGrenadeType (Utilities|Array|Get(acopy) _grenadetypescharacterhas))))

(event Custom|ConnectGrenade%20-ALL
  (params (Target :type Actor%20Object%20Reference) (Parent :type Scene%20Component%20Object%20Reference) (SocketName :type Name))
  ;[1 1 1] Connect Grenade Replicated
  (Utilities|IsValid Target
    (:Is%20Valid
      (Transformation|AttachComponentToComponent Target Parent SocketName "SnapToTarget" "SnapToTarget" "SnapToTarget" true))))

(event Custom|ThrowGrenade
  (bind _grenadethrowmontage (Variables|Default|GetGrenadeThrowMontage))
  ;[1 1 1] Replicated Throw
  (if (CallFunction|CanThrow?)
    (CallFunction|InitializeVariables)
    (Utilities|FlowControl|Delay 0.06)
    (if (Variables|Default|GetHasGrenade)
      (bind _removed_all (Default|RemoveItem (Actor|GetComponentbyClass (Components|GetOwner) "/Game/ModernRPG/General/Blueprints/ActorComponents/Character/Inventory/AC_Inventory.AC_Inventory_C") (Variables|Default|GetGrenadeArrayIndex) 1))
      (if _removed_all
        (CallFunction|RemoveGrenadeType (Variables|GrenadeTypes|GetCurrentGrenadeType)))
      (Utilities|HasAutority
        (:Has
          (CallFunction|ThrowGrenadeALL _grenadethrowmontage))
        (:No
          (CallFunction|ThrowGrenade-Server _grenadethrowmontage))))))

(event EventBeginPlay
  ;[1 1 1] Initialize
  (CallFunction|InitializeRefandMesh)
  (Variables|Default|SetEquipment (Actor|GetComponentbyClass (Components|GetOwner) "/Game/ModernRPG/General/Blueprints/ActorComponents/InteractActors/AC_EquipmentHandler.AC_EquipmentHandler_C"))
  (bind _returnvalue (UserInterface|CreateWidget "/Game/ModernRPG/General/GUI/Widgets/Grenades/WB_ChooseGrenade.WB_ChooseGrenade_C"))
  (Variables|Default|SetGrenadeWidget _returnvalue)
  (CallFunction|LoadGrenades)
  (Utilities|IsValid (Variables|Default|GetGrenadeWidget)
    (:Is%20Valid
      (Default|SetSelectedbyType (Variables|Default|GetGrenadeWidget) (Variables|GrenadeTypes|GetCurrentGrenadeType)))
    (:Is%20Not%20Valid
      _))
  (CallFunction|InitializeVariables))

(fn InitializeRefandMesh
  (bind _ascharacter (Utilities|Casting|CastToCharacter (Components|GetOwner)))
  (bind _output_get (Variables|Default|SetCharacter _ascharacter))
  (bind (_defaultbodymesh _headmesh) (Class|BPIAI|GetDemoSkeletalMeshes(Message) _output_get))
  (Variables|Default|SetSK_Mesh _defaultbodymesh)
  (Variables|Default|SetSK_Head _headmesh))

(fn ApplyDamageEffectsFunctionality
  (params (Origin :type Vector%20%28by%20ref%29) (RadialForce :type Radial%20Force%20Component%20Object%20Reference) (Grenade :type Actor%20Object%20Reference) (GrenadeType :type E_GrenadeTypes%20Enum :default "NewEnumerator0") (GrenadeInfo :type S%20Grenades%20Structure))
  (bind _returnvalue (Components|GetOwner))
  (bind _returnvalue_2 (Components|GetOwner))
  (switch Utilities|FlowControl|Switch|SwitchonE_GrenadeTypes GrenadeType
    (:NewEnumerator0
      (Game|Damage|ApplyRadialDamage 2e+03 (+ Origin "0, 0,50.000000") 5e+02 "/Game/ModernRPG/General/Blueprints/DamageTypes/BPDT_Grenade.BPDT_Grenade_C" 0 Grenade (Pawn|GetController (.AsPawn (Utilities|Casting|CastToPawn (Components|GetOwner)))) true "ECC_Pawn" :!label _label)
      (Class|AISenseHearing|ReportNoiseEvent (Transformation|GetActorLocation _returnvalue) 1.0 _returnvalue 6e+03 "Noise"))
    (:NewEnumerator1
      (Class|AISenseHearing|ReportNoiseEvent (Transformation|GetActorLocation _returnvalue_2) 1.0 _returnvalue_2 3e+03 "Noise")
      (bind _asbp_grenade (Utilities|Casting|CastToBP_Grenade Grenade))
      (for _array_element (Collision|GetOverlappingActors (Variables|/Game/ModernRPG/General/Blueprints/Grenades/BP_Grenade.BP_Grenade_C|GetSphere _asbp_grenade) (Variables|Default|GetPlayerClass) :!class /Script/Engine.PrimitiveComponent)
        (bind _camera (Class|BPIAI|GetMainCamera(Message) _array_element))
        (if (Math|Float|InRange(Float) (Math|Vector|DotProduct (Math|Vector|Normalize (- (Transformation|GetActorLocation Grenade) (Transformation|GetWorldLocation _camera))) (Math|Vector|GetForwardVector (Transformation|GetWorldRotation _camera))) 0.7 1.0)
          (CallFunction|FlashEvent (Actor|GetComponentbyClass _array_element "AC_Grenades_C")))))
    (:NewEnumerator4
      (goto _label))
    (:NewEnumerator5
      (goto _label))
    (:NewEnumerator6
      (goto _label))))

(fn CanAddGrenades?
  (return (>= (Variables|Default|GetCurrentAmount) (Variables|Default|GetMaxAmount))))

(fn ChooseGrenadeIndex)

(fn GetWeaponInfo
  (bind _returnvalue (Components|GetOwner))
  (bind _returnvalue_2 (Actor|GetComponentbyClass _returnvalue "/Game/ModernRPG/General/Blueprints/ActorComponents/InteractActors/AC_EquipmentHandler.AC_EquipmentHandler_C"))
  (bind _array_element (Default|GetCurrentWeapon _returnvalue_2))
  (bind _row (Utilities|Struct|BreakS_InvItemDyn _array_element))
  (bind _weapon (CallFunction|GetWeaponInfo _row))
  (bind (_sockets _action_animations) (Utilities|Struct|BreakS_Weapon _weapon))
  (if (Variables|/Game/ModernRPG/General/Blueprints/ActorComponents/Weapon/AC_HolsterWeapon.AC_HolsterWeapon_C|GetHolstered (Actor|GetComponentbyClass (Components|GetOwner) "/Game/ModernRPG/General/Blueprints/ActorComponents/Weapon/AC_HolsterWeapon.AC_HolsterWeapon_C"))
    (bind _returnvalue_3 (Utilities|GetDataTableRow "/Game/ModernRPG/General/Blueprints/DataTables/DT_Weapon.DT_Weapon" "Unarmed")
      (:then
        (return (.GRENADE_Toss (Utilities|Struct|BreakS_ActionAnimations (Utilities|Struct|BreakS_Weapon _returnvalue_3))) "GRENADE")))
    (else
      (return (.GRENADE_Toss (Utilities|Struct|BreakS_ActionAnimations _action_animations)) (Utilities|Struct|BreakS_WeaponSockets _sockets)))))

(fn CanThrow?
  (bind _returnvalue (Components|GetOwner))
  (bind _returnvalue_2 (Components|GetOwner))
  (bind _returnvalue_3 (Actor|GetComponentbyClass _returnvalue_2 "/Game/ModernRPG/General/Blueprints/ActorComponents/Character/State/AC_PlayerCurrentState.AC_PlayerCurrentState_C"))
  (bind _returnvalue_4 (Actor|GetComponentbyClass _returnvalue "/Game/ModernRPG/General/Blueprints/ActorComponents/Character/State/AC_PlayerCurrentState.AC_PlayerCurrentState_C"))
  (bind _currentstate (Variables|/Game/ModernRPG/General/Blueprints/ActorComponents/Character/State/AC_PlayerCurrentState.AC_PlayerCurrentState_C|GetCurrentState _returnvalue_4))
  (bind _currentstate_2 (Variables|/Game/ModernRPG/General/Blueprints/ActorComponents/Character/State/AC_PlayerCurrentState.AC_PlayerCurrentState_C|GetCurrentState _returnvalue_3))
  (Utilities|IsValid (Variables|/Game/ModernRPG/General/Blueprints/ActorComponents/InteractActors/AC_EquipmentHandler.AC_EquipmentHandler_C|GetCurrentWeaponActor (Actor|GetComponentbyClass (Components|GetOwner) "/Game/ModernRPG/General/Blueprints/ActorComponents/InteractActors/AC_EquipmentHandler.AC_EquipmentHandler_C"))
    (:Is%20Valid
      (return (not (Math|Boolean|ORBoolean (Utilities|Enum|Equal(Enum) _currentstate "NewEnumerator2") (Utilities|Enum|Equal(Enum) _currentstate "NewEnumerator3") (.BlockedWeapon (Default|GetBlockInformation (Actor|GetComponentbyClass (Components|GetOwner) "/Game/ModernRPG/General/Blueprints/ActorComponents/Weapon/AC_WeaponBlock.AC_WeaponBlock_C")))))))
    (:Is%20Not%20Valid
      (return (not (Math|Boolean|ORBoolean (Utilities|Enum|Equal(Enum) _currentstate_2 "NewEnumerator2") (Utilities|Enum|Equal(Enum) _currentstate_2 "NewEnumerator3") (.BlockedWeapon (Default|GetBlockInformation (Actor|GetComponentbyClass (Components|GetOwner) "/Game/ModernRPG/General/Blueprints/ActorComponents/Weapon/AC_WeaponBlock.AC_WeaponBlock_C")))))))))

(fn SpawnNewEffectSound
  (params (Sound[loc] :type Sound%20Base%20Object%20Reference) (VolumeMultiplier :type Float%20%28double-precision%29) (EffectInstigator[loc] :type Actor%20Object%20Reference))
  (Utilities|IsValid (Variables|Default|GetEffectInstigator)
    (:Is%20Valid
      (if (not (== (Variables|Default|GetEffectInstigator) EffectInstigator[loc]))
        (bind _return (Class|BPIGrenade|IsFlashbangEffect?(Message) EffectInstigator[loc]))
        (Class|BPIGrenade|StopEffect(Message) (Variables|Default|GetEffectInstigator) _return)
        (Utilities|IsValid (Variables|Default|GetPlayingFlashlightSound)
          (:Is%20Valid
            (Audio|Components|Audio|SetVolumeMultiplier (Variables|Default|GetPlayingFlashlightSound) 0.0 :!class /Script/Engine.AudioComponent))
          (:Is%20Not%20Valid
            _))
        (Variables|Default|SetEffectInstigator EffectInstigator[loc])
        (bind _returnvalue (Audio|SpawnSound2D Sound[loc] 1.0 1.0 0.0 0))
        (Variables|Default|SetPlayingFlashlightSound _returnvalue)))
    (:Is%20Not%20Valid
      (bind _returnvalue_2 (Audio|SpawnSound2D Sound[loc] 1.0 1.0 0.0 0))
      (Variables|Default|SetPlayingFlashlightSound _returnvalue_2)
      (Variables|Default|SetEffectInstigator EffectInstigator[loc]))))

(fn OnNotifyBegin
  (params (Selection :type Name))
  (switch name Selection
    (:Throw
      (CallFunction|SpawnGrenade-Server)
      (Audio|PlaySoundatLocation (Utilities|Struct|BreakS_Grenades (Variables|Default|GetLast%20Throwed%20Grenade)) (Transformation|GetActorLocation (Components|GetOwner)) "0, 0, 0" 1.0 1.0 0.0 0 0 0 0))
    (:Draw
      (Audio|PlaySoundatLocation (Utilities|Struct|BreakS_Grenades (Variables|Default|GetLast%20Throwed%20Grenade)) (Transformation|GetActorLocation (Components|GetOwner)) "0, 0, 0" 1.0 1.0 0.0 0 0 0 0))))

(fn OnNotifyEnd
  (params (Selection :type Name))
  (bind _equipment (Variables|Default|GetEquipment))
  (bind _actor (Default|GetCurrentWeaponActorbyType _equipment))
  (switch name Selection
    (:Grenade
      (CallFunction|DestroyConnectedMesh))
    (:Weapon
      (Utilities|IsValid _actor
        (:Is%20Valid
          (Default|AttachActor _actor))
        (:Is%20Not%20Valid
          _))
      (Default|UpdateState (Actor|GetComponentbyClass (Components|GetOwner) "/Game/ModernRPG/General/Blueprints/ActorComponents/Character/State/AC_PlayerCurrentState.AC_PlayerCurrentState_C") "NewEnumerator4")
      (Variables|Default|SetThrowing false))))

(fn OnRepGrenadeArrayIndex)

(fn GetVelocity
  (return (* (Math|Vector|GetForwardVector (Pawn|GetControlRotation (.AsCharacter (Utilities|Casting|CastToCharacter (Components|GetOwner))) :!class /Script/Engine.Pawn)) 5e+03)))

(fn DestroyConnectedMesh
  (Utilities|IsValid (Variables|Default|GetMeshActor)
    (:Is%20Valid
      (Actor|DestroyActor (Variables|Default|GetMeshActor)))))

(fn SaveGrenades
  (bind _returnvalue (SaveGame|DoesSaveGameExist (Variables|Default|GetGrenadeSlot)))
  (if _returnvalue
    (bind _returnvalue_2 (SaveGame|LoadGamefromSlot (Variables|Default|GetGrenadeSlot)))
    (bind _asbp_save_grenade (Utilities|Casting|CastToBP_SaveGrenade _returnvalue_2))
    (LocalVariables|SetL_SaveGame _asbp_save_grenade)
    (else
      (bind _returnvalue_3 (SaveGame|CreateSaveGameObject "/Game/ModernRPG/General/Blueprints/ActorComponents/Character/Grenade/BP_SaveGrenade.BP_SaveGrenade_C"))
      (LocalVariables|SetL_SaveGame _returnvalue_3)))
  (Variables|/Game/ModernRPG/General/Blueprints/ActorComponents/Character/Grenade/BP_SaveGrenade.BP_SaveGrenade_C|SetsGrenade (LocalVariables|GetL_SaveGame) (Utilities|Struct|MakeS_SaveGrenades (Variables|GrenadeTypes|GetCurrentGrenadeType) (Variables|GrenadeTypes|GetGrenadeTypesCharacterHas)))
  (SaveGame|SaveGametoSlot (LocalVariables|GetL_SaveGame) (Variables|Default|GetGrenadeSlot)))

(fn LoadGrenades
  (bind _returnvalue (SaveGame|DoesSaveGameExist (Variables|Default|GetGrenadeSlot)))
  (if _returnvalue
    (bind _returnvalue_2 (SaveGame|LoadGamefromSlot (Variables|Default|GetGrenadeSlot)))
    (bind _asbp_save_grenade (Utilities|Casting|CastToBP_SaveGrenade _returnvalue_2))
    (bind _output_get (LocalVariables|SetL_SaveGame _asbp_save_grenade))
    (Variables|GrenadeTypes|SetCurrentGrenadeType (.grenadetype (Variables|/Game/ModernRPG/General/Blueprints/ActorComponents/Character/Grenade/BP_SaveGrenade.BP_SaveGrenade_C|GetsGrenade _output_get)))
    (Variables|GrenadeTypes|SetGrenadeTypesCharacterHas (.playertypes (Variables|/Game/ModernRPG/General/Blueprints/ActorComponents/Character/Grenade/BP_SaveGrenade.BP_SaveGrenade_C|GetsGrenade _output_get)))))

(fn GetGrenadeTransform
  (bind _springarmbody (Class|BPIAI|GetMainSpringArm(Message) (Variables|Default|GetCharacter)))
  (return (Math|Transform|MakeTransform (+ (* (Math|Vector|GetRightVector _springarmbody) 50) (Transformation|GetWorldLocation _springarmbody)) (Pawn|GetControlRotation (Variables|Default|GetCharacter) :!class /Script/Engine.Pawn))))

(fn GetMainUI
  (return (Variables|/Game/ModernRPG/General/Blueprints/DialoguesQuests/WidgetHandler/AC_MainWidgetHandler.AC_MainWidgetHandler_C|GetCastedMainUI (Actor|GetComponentbyClass (Components|GetOwner) "/Game/ModernRPG/General/Blueprints/DialoguesQuests/WidgetHandler/AC_MainWidgetHandler.AC_MainWidgetHandler_C"))))

(fn UpdateGrenadeType
  (Default|UpdateGrenadeType (CallFunction|GetMainUI) (Class|WidgetBlueprintLibrary|MakeBrushfromTexture (.Icon (Default|GetGrenade (Actor|GetComponentbyClass (Components|GetOwner) "/Game/ModernRPG/General/Blueprints/ActorComponents/Character/Inventory/AC_Inventory.AC_Inventory_C") (Variables|GrenadeTypes|GetCurrentGrenadeType))) 20 20)))