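; Actor component that lets its owner select world actors by holding aim on them, with an on-screen progress widget.
; While selecting, a looping timer line-traces from the "Main" camera, remembering actors implementing BP_I_Selectable that are not already selected.
; Sustained aim fills the timer until SelectMessage fires; looking away drains or resets it.
; The binoculars check that would suppress selection is an unwired stub.
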(event Custom|StartSelecting
  ;[1 1 1] Animation
  (if (not (CallFunction|InBinoculars?))
    (Variables|Default|SetTimer 0.0)
    (CallFunction|UpdateWidget)
    (Default|Fade (Variables|Default|GetSelectedWidget) true)
    (bind _returnvalue (Utilities|Time|SetTimerbyEvent (delegate Custom|TryToSelect) 0.1 true))
    (Variables|Default|SetSelectTimer _returnvalue)))

(event Custom|TryToSelect
  (bind _camera (Variables|Default|GetCamera))
  (bind _returnvalue (Transformation|GetWorldLocation _camera))
  ;[1 1 1] Animation
  (if (CallFunction|InBinoculars?)
    (Default|Fade (Variables|Default|GetSelectedWidget) false)
    (CallFunction|StopSelecting)
    (else
      (CallFunction|UpdateWidget)
      (bind (_outhit _returnvalue_2) (Collision|LineTraceByChannel _returnvalue (+ _returnvalue (* (Math|Vector|GetForwardVector _camera) (Variables|Settings|GetMaxDistance))) "TraceTypeQuery1" false (Utilities|Array|MakeArray (Components|GetOwner)) "None"))
      (if _returnvalue_2
        (bind _output_get (Variables|Default|SetCurrentActor (.HitActor (Collision|BreakHitResult _outhit))))
        (Utilities|IsValid _output_get
          (:Is%20Valid
            (Utilities|IsValid (Variables|Default|GetRememberedActor)
              (:Is%20Valid
                (if (== (Variables|Default|GetRememberedActor) (Variables|Default|GetCurrentActor))
                  (CallFunction|ChangeTimer 0.1)
                  (if (>= (Variables|Default|GetTimer) (Variables|Settings|GetSelectTime))
                    (Class|BPISelectable|Select(Message) (Variables|Default|GetRememberedActor))
                    (Variables|Default|SetRememberedActor 0)
                    (CallFunction|StartSelecting))
                  (else
                    (CallFunction|ChangeTimer -1e+01)
                    (Variables|Default|SetRememberedActor 0))))
              (:Is%20Not%20Valid
                (if (Utilities|DoesObjectImplementInterface (Variables|Default|GetCurrentActor) "/Game/ModernRPG/General/Blueprints/Interfaces/BP_I_Selectable.BP_I_Selectable_C")
                  (bind _busy (Class|BPISelectable|SelectState(Message) (Variables|Default|GetCurrentActor)))
                  (if (not _busy)
                    (Variables|Default|SetRememberedActor (Variables|Default|GetCurrentActor)))
                  (else
                    (CallFunction|ChangeTimer -0.1))))))
          (:Is%20Not%20Valid
            (CallFunction|ChangeTimer -0.1 :!label _label)))
        (else
          (goto _label))))))

(event Custom|StopSelecting
  ;[1 1 1] On Selected / Begin play
  (if (CallFunction|InBinoculars?)
    _
    (else
      (Default|Fade (Variables|Default|GetSelectedWidget) false)))
  (Variables|Default|SetRememberedActor 0)
  (Utilities|Time|PauseTimerbyHandle (Variables|Default|GetSelectTimer)))

(event Custom|UpdateWidget
  ;[1 1 1] Timer and Widget
  (Default|SetValue (Variables|Default|GetSelectedWidget) (/ (Variables|Default|GetTimer) (Variables|Settings|GetSelectTime))))

(event Custom|ChangeTimer
  (params (Value :type Float%20%28double-precision%29))
  ;[1 1 1] Timer and Widget
  (Variables|Default|SetTimer (Math|Float|Clamp(Float) (+ (Variables|Default|GetTimer) Value) 0.0 (Variables|Settings|GetSelectTime)))
  (CallFunction|UpdateWidget))

(event Custom|CreateSelectedWidget%20-Server
  ;[1 1 1] Create Widget
  (CallFunction|CreateSelectedWidget-OC))

(event Custom|CreateSelectedWidget%20-OC
  ;[1 1 1] Create Widget
  (bind _returnvalue (UserInterface|CreateWidget "/Game/ModernRPG/General/GUI/Widgets/WB_SelectedAim.WB_SelectedAim_C"))
  (bind _output_get (Variables|Default|SetSelectedWidget _returnvalue))
  (Utilities|IsValid _output_get
    (:Is%20Valid
      (UserInterface|Viewport|AddtoViewport _output_get 0))))

(event EventBeginPlay
  (CallFunction|CreateSelectedWidget-Server)
  (Variables|Default|SetCamera (Utilities|Array|Get(acopy) (Actor|GetComponentsbyTag (Components|GetOwner) "/Script/Engine.CameraComponent" "Main"))))

(fn InBinoculars?)