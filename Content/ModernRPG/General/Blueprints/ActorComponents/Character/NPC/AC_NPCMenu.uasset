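; Character component that tracks the NPC the player is interacting with, apparently to support NPC menus.
; On BeginPlay it caches the owning character's PlayerController.
; SetNPC stores the NPC and copies the owner's PlayerInventoryWidget reference into the NPC's AC_Inventory.
; GetNPC returns the stored NPC with its inventory's Seller flag, or Seller false when the NPC or its inventory is invalid.
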(event EventBeginPlay
  ;[1 1 1] Initialize Component
  (bind _ascharacter (Utilities|Casting|CastToCharacter (Components|GetOwner)))
  (bind _asplayer_controller (Utilities|Casting|CastToPlayerController (Pawn|GetController _ascharacter)))
  (Variables|Default|SetPlayerController _asplayer_controller))

(fn GetNPC
  (bind _npc (Variables|Default|GetNPC))
  (bind _returnvalue (Actor|GetComponentbyClass _npc "/Game/ModernRPG/General/Blueprints/ActorComponents/Character/Inventory/AC_Inventory.AC_Inventory_C"))
  (Utilities|IsValid _npc
    (:Is%20Valid
      (Utilities|IsValid _returnvalue
        (:Is%20Valid
          (return (Variables|Default|GetNPC) (Variables|/Game/ModernRPG/General/Blueprints/ActorComponents/Character/Inventory/AC_Inventory.AC_Inventory_C|GetSeller _returnvalue)))
        (:Is%20Not%20Valid
          _)))
    (:Is%20Not%20Valid
      _))
  (return 0 false))

(fn SetNPC
  (params (NPC :type Actor%20Object%20Reference))
  (bind _output_get (Variables|Default|SetNPC NPC))
  (Utilities|IsValid _output_get
    (:Is%20Valid
      (Utilities|IsValid (Actor|GetComponentbyClass _output_get "/Game/ModernRPG/General/Blueprints/ActorComponents/Character/Inventory/AC_Inventory.AC_Inventory_C")
        (:Is%20Valid
          (Variables|/Game/ModernRPG/General/Blueprints/ActorComponents/Character/Inventory/AC_Inventory.AC_Inventory_C|SetPlayerInventoryWidget (Actor|GetComponentbyClass _output_get "/Game/ModernRPG/General/Blueprints/ActorComponents/Character/Inventory/AC_Inventory.AC_Inventory_C") (Variables|/Game/ModernRPG/General/Blueprints/ActorComponents/Character/Inventory/AC_Inventory.AC_Inventory_C|GetPlayerInventoryWidget (Actor|GetComponentbyClass (Components|GetOwner) "/Game/ModernRPG/General/Blueprints/ActorComponents/Character/Inventory/AC_Inventory.AC_Inventory_C"))))))))