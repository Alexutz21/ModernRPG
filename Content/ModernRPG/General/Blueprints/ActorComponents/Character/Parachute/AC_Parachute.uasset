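; Character component that runs skydiving and parachuting, from freefall through canopy opening or cancel to landing.
; Looping server timers trace ground distance to start skydiving, spawn an attached backpack, tune gravity and speed, and land, pausing the trace when not falling or flying.
; Multicasts sync state and parachute rotation.
; OnRep functions update the anim instance and camera view, and input feeds steering to the anim instance.
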(event Custom|ControlPO%20-All
  (params (ParachuteOpenned :type Boolean))
  (bind _returnvalue (Components|GetOwner))
  (bind _ascharacter (Utilities|Casting|CastToCharacter _returnvalue))
  (bind _charactermovement (Variables|/Script/Engine.Character|GetCharacterMovement _ascharacter))
  ;[1 1 1] ControlParachute
  (bind _output_get (Variables|Default|SetParachuteOpenned ParachuteOpenned))
  (if _output_get
    (if (CallFunction|NotEqualtoCustomMode "MOVE_Falling") :!label _label
      (Pawn|Components|CharacterMovement|SetMovementMode _charactermovement "MOVE_Falling" 0))
    (elif (Variables|Default|GetIsSkydiving)
      (goto _label)
      (elif (CallFunction|NotEqualtoCustomMode "MOVE_Walking")
        (Pawn|Components|CharacterMovement|SetMovementMode _charactermovement "MOVE_Walking" 0)))))

(event Custom|CustomEvent_0
  (params (Character :type Character%20Object%20Reference) (PrevMovementMode :type EMovementMode%20Enum :default "MOVE_None") (PreviousCustomMode :type Byte))
  ;[1 1 1] Initializing
  (Variables|Default|SetPrevMovementMode PrevMovementMode))

(event Custom|ControlParachute%20-%20Server
  ;[1 1 1] ControlParachute
  (bind (_isskydiving _parachuteopenned _cancontinue) (CallFunction|ControlParachute))
  (if _cancontinue
    (CallFunction|ControlIsSkydiving-All _isskydiving)
    (CallFunction|ControlPO-All _parachuteopenned)))

(event Custom|ControlIsSkydiving%20-All
  (params (IsSkydiving :type Boolean))
  (bind _returnvalue (Components|GetOwner))
  (bind _ascharacter (Utilities|Casting|CastToCharacter _returnvalue))
  (bind _charactermovement (Variables|/Script/Engine.Character|GetCharacterMovement _ascharacter))
  ;[1 1 1] ControlParachute
  (bind _output_get (Variables|Default|SetIsSkydiving IsSkydiving))
  (if _output_get
    (if (CallFunction|NotEqualtoCustomMode "MOVE_Falling") :!label _label
      (Pawn|Components|CharacterMovement|SetMovementMode _charactermovement "MOVE_Falling" 0))
    (elif (Variables|Default|GetParachuteOpenned)
      (goto _label)
      (elif (CallFunction|NotEqualtoCustomMode "MOVE_Walking")
        (Pawn|Components|CharacterMovement|SetMovementMode _charactermovement "MOVE_Walking" 0)))))

(event Custom|Initialize
  ;[1 1 1] Initializing
  (bind _ascharacter (Utilities|Casting|CastToCharacter (Components|GetOwner)))
  (Variables|Default|SetCharacterMovement (Variables|/Script/Engine.Character|GetCharacterMovement _ascharacter))
  (bind _bodyskeletal (Class|BPIAI|GetBody(Message) _ascharacter))
  (Variables|Default|SetMesh _bodyskeletal)
  (|CG_CheckDistanceToGround))

(event Custom|Spawn%20Backpack%20-%20Server
  ;[1 1 1] Spawn Backpack
  (CallFunction|SpawnBackpack))

(event Custom|SetParachuteRotation%20-%20Server
  (bind _backpack (Variables|Default|GetBackpack))
  (bind _sk_parachute (Variables|/Game/ModernRPG/General/Blueprints/Parachute/BP_Backpack.BP_Backpack_C|GetSK_Parachute _backpack))
  ;[1 1 1] Event tick. Disable rotation of a parachute skeletal mesh while character rotates.
  (Utilities|IsValid _sk_parachute
    (:Is%20Valid
      (CallFunction|SetParachuteRotation-All _sk_parachute (CallFunction|GetOwnerWRotation)))))

(event Custom|SetParachuteRotation%20-%20All
  (params (Target :type Scene%20Component%20Object%20Reference) (NewRotation :type Rotator))
  ;[1 1 1] Event tick. Disable rotation of a parachute skeletal mesh while character rotates.
  (Utilities|IsValid Target
    (:Is%20Valid
      (Transformation|SetWorldRotation Target NewRotation false true))))

(event EventBeginPlay
  ;[1 1 1] Initializing
  (Utilities|SwitchHasAuthority
    (:Authority
      (bind _asbp_demo_character (Utilities|Casting|CastToBP_DemoCharacter (Components|GetOwner)))
      (Character|BindEventtoMovementModeChangedDelegate _asbp_demo_character (delegate Custom|CustomEvent_0))
      (CallFunction|Initialize)
      (|CG_CheckPossibleOfOpenParachute))))

(fn ControlParachute
  (bind _backpack (Variables|Default|GetBackpack))
  (Utilities|SwitchHasAuthority
    (:Authority
      (if (Variables|Default|GetParachuteOpenned)
        ;[1 1 1] Freefall
        (if (Variables|Default|GetCancelParachute)
          (Utilities|IsValid _backpack
            (:Is%20Valid
              (Default|ParachuteControl-Server _backpack false)
              (return true false true))))
        (elif (Variables|Default|GetIsSkydiving)
          ;[1 1 1] Open parachute
          (if (>= (Variables|Default|GetCurrentDistance) (Variables|Settings|GetLowestDistance))
            (Default|ParachuteControl-Server (Variables|Default|GetBackpack) true)
            (return false true true)
            (else
              (return false true false))))))))

(fn SpawnBackpack
  (Utilities|IsValid (Variables|Default|GetBackpack)
    (:Is%20Not%20Valid
      (bind _bodymesh (CallFunction|GetCharacterSkeleton (Components|GetOwner)))
      (Utilities|IsValid _bodymesh
        (:Is%20Valid
          ;[1 1 1] Spawn Backpack
          (bind _returnvalue (Game|SpawnActorfromClass "/Game/ModernRPG/General/Blueprints/Parachute/BP_Backpack.BP_Backpack_C" (Transformation|GetSocketTransform _bodymesh "SPINE_01_Parachute" "RTS_World") "Undefined" 0 0))
          (Variables|Default|SetBackpack _returnvalue)
          ;[1 1 1] Attach to Backpack Slot
          (Transformation|AttachComponentToComponent _returnvalue _bodymesh "SPINE_01_Parachute" "SnapToTarget" "SnapToTarget" "KeepRelative" true))))))

(fn CheckDistancetoGround
  (bind _returnvalue (Components|GetOwner))
  ;[1 1 1] Distance between character and ground
  (bind _bodymesh (CallFunction|GetCharacterSkeleton (Components|GetOwner)))
  (Utilities|IsValid _returnvalue
    (:Is%20Valid
      (bind _outhit (Collision|LineTraceByChannel (.location (Transformation|GetSocketTransform _bodymesh "Point" "RTS_World")) (+ (.location (Transformation|GetSocketTransform _bodymesh "Point" "RTS_World")) (* (Math|Vector|GetUpVector (Variables|/Script/Engine.Character|GetCapsuleComponent (.AsCharacter (Utilities|Casting|CastToCharacter (Components|GetOwner))))) "0, 0,-100000000.000000")) "TraceTypeQuery1" false (Utilities|Array|MakeArray _returnvalue) "None" true "(R=0.035046,G=0.000000,B=1.000000,A=1.000000)"))
      (return (Math|Vector|Distance(Vector) (.Location (Collision|BreakHitResult _outhit)) (.TraceStart (Collision|BreakHitResult _outhit)))))))

(fn ParachuteLand
  (Utilities|IsValid (Variables|Default|GetBackpack)
    (:Is%20Valid
      (Actor|DestroyActor (Variables|Default|GetBackpack)))))

(fn SetFallSpeedWithoutParachute
  (if (not (== (CallFunction|GetGravityScale) 1.0))
    (Variables|/Script/Engine.CharacterMovementComponent|SetGravityScale (Variables|/Script/Engine.Character|GetCharacterMovement (.AsCharacter (Utilities|Casting|CastToCharacter (Components|GetOwner)))) 1.0)))

(fn OnRepParachuteOpenned
  (bind _returnvalue (Components|GetOwner))
  (bind _returnvalue_2 (Actor|GetComponentbyClass _returnvalue "/Game/ModernRPG/General/Blueprints/ActorComponents/ViewSwitch/AC_ViewSwitch.AC_ViewSwitch_C"))
  (bind _defaultbodymesh (Class|BPIAI|GetDemoSkeletalMeshes(Message) (Components|GetOwner)))
  (Class|BPIABP|SetParachuteOpenned(Message) (Components|SkeletalMesh|GetAnimInstance _defaultbodymesh) (Variables|Default|GetParachuteOpenned))
  (if (Variables|Default|GetParachuteOpenned)
    (Default|ForceView _returnvalue_2 4.5e+02)
    (else
      (Default|ParachuteTP _returnvalue_2))))

(fn OnRepIsSkydiving
  (bind _defaultbodymesh (Class|BPIAI|GetDemoSkeletalMeshes(Message) (Components|GetOwner)))
  (Class|BPIABP|SetIsSkydiving(Message) (Components|SkeletalMesh|GetAnimInstance _defaultbodymesh) (Variables|Default|GetIsSkydiving)))

(fn GetOwnerWRotation
  (return (Transformation|GetWorldRotation (Variables|/Script/Engine.Character|GetCapsuleComponent (.AsCharacter (Utilities|Casting|CastToCharacter (Components|GetOwner)))))))

(fn Input
  (params (Direction :type Float%20%28double-precision%29) (Axis :type Float%20%28double-precision%29))
  (if (or (Variables|Default|GetParachuteOpenned) (Variables|Default|GetIsSkydiving))
    (Class|BPIABP|ParachuteDirection(Message) (CallFunction|GetAnimInstace) Direction)
    (Class|BPIABP|ParachuteAxis(Message) (CallFunction|GetAnimInstace) Axis)))

(fn GetAnimInstace
  (bind _defaultbodymesh (Class|BPIAI|GetDemoSkeletalMeshes(Message) (Components|GetOwner)))
  (return (Components|SkeletalMesh|GetAnimInstance _defaultbodymesh)))

(fn GetOwnerInfo
  (bind _returnvalue (Components|GetOwner))
  (bind _ascharacter (Utilities|Casting|CastToCharacter _returnvalue))
  (return _ascharacter (Variables|/Script/Engine.Character|GetCharacterMovement _ascharacter)))

(fn GetGravityScale
  (return (Variables|/Script/Engine.CharacterMovementComponent|GetGravityScale (Variables|/Script/Engine.Character|GetCharacterMovement (.AsCharacter (Utilities|Casting|CastToCharacter (Components|GetOwner)))))))

(fn NotEqualtoCustomMode
  (params (MovementMode :type EMovementMode%20Enum :default "MOVE_None"))
  (return (Utilities|Enum|NotEqual(Enum) (Variables|/Script/Engine.CharacterMovementComponent|GetMovementMode (Variables|/Script/Engine.Character|GetCharacterMovement (.AsCharacter (Utilities|Casting|CastToCharacter (Components|GetOwner))))) MovementMode)))

(event Custom|CheckDistanceToGround%20-%20Server
  (bind _returnvalue (Components|GetOwner))
  (bind _returnvalue_2 (Actor|GetComponentbyClass _returnvalue "/Game/ModernRPG/General/Blueprints/ClimbSystem/AC_ClimbComponent.AC_ClimbComponent_C"))
  ;[1 1 1] Control distance to ground and check can character use a parachute
  (Utilities|NotonLadder
    (:Not
      (if (Utilities|Enum|NotEqual(Enum) (Variables|/Script/Engine.CharacterMovementComponent|GetMovementMode (Variables|Default|GetCharacterMovement)) "MOVE_Swimming")
        (bind _result (Class|BPICharacter|IsAlive?(Message) (Components|GetOwner)))
        (if _result
          (if (Default|NotinVehicle (Actor|GetComponentbyClass (Components|GetOwner) "/Game/ModernRPG/General/Blueprints/ActorComponents/Character/Conditions/AC_Conditions.AC_Conditions_C"))
            (if (AI|Components|NavMovement|IsMovingonGround (Variables|/Script/Engine.Character|GetCharacterMovement (.AsCharacter (Utilities|Casting|CastToCharacter (Components|GetOwner)))))
              (Utilities|FlowControl|Sequence
                (:then_0
                  (Utilities|FlowControl|DoOnce false :!label _label
                    (:Completed
                      (CallFunction|ControlIsSkydiving-All false))))
                (:then_1
                  (CallFunction|ResetSpawnBackpack)))
              (else
                (Utilities|FlowControl|Sequence
                  (:then_0
                    (goto _label Reset))
                  (:then_1
                    (if (Variables|Default|GetParachuteOpenned)
                      (if (== (CallFunction|GetGravityScale) (Variables|Settings|GetParachute_Gravity))
                        _
                        (else
                          (Variables|/Script/Engine.CharacterMovementComponent|SetGravityScale (Variables|/Script/Engine.Character|GetCharacterMovement (.AsCharacter (Utilities|Casting|CastToCharacter (Components|GetOwner)))) (Variables|Settings|GetParachute_Gravity))
                          (Variables|/Script/Engine.CharacterMovementComponent|SetMaxWalkSpeed (Variables|/Script/Engine.Character|GetCharacterMovement (.AsCharacter (Utilities|Casting|CastToCharacter (Components|GetOwner)))) (Variables|Settings|GetHorizontalSpeedWithParaсhute))))
                      (if (<= (CallFunction|CheckDistancetoGround) (Variables|Default|GetCheckDistanceToGroundForLanding))
                        (Utilities|FlowControl|DoOnce false :!label _label_2
                          (:Completed
                            (CallFunction|OnLanded))))
                      (elif (> (CallFunction|CheckDistancetoGround) (Variables|Settings|GetLowestDistance))
                        (Variables|Default|SetCurrentDistance (CallFunction|CheckDistancetoGround))
                        (CallFunction|ControlIsSkydiving-All true)
                        (Utilities|FlowControl|Sequence
                          (:then_0
                            (Utilities|FlowControl|DoOnce false
                              (:Completed
                                (CallFunction|SpawnBackpack-Server)
                                (Variables|/Script/Engine.CharacterMovementComponent|SetMaxWalkSpeed (Variables|/Script/Engine.Character|GetCharacterMovement (.AsCharacter (Utilities|Casting|CastToCharacter (Components|GetOwner)))) (Variables|Settings|GetHorizontalSpeedWithoutParaсhute))
                                (goto _label_2 Reset))))
                          (:then_1
                            (CallFunction|SetFallSpeedWithoutParachute)
                            (goto _label_2 Reset)))
                        (else
                          (Utilities|IsValid _returnvalue_2
                            (:Is%20Valid
                              (if (not (Variables|/Game/ModernRPG/General/Blueprints/ClimbSystem/AC_ClimbComponent.AC_ClimbComponent_C|GetParkour _returnvalue_2))
                                (if (Utilities|Enum|NotEqual(Enum) (Variables|Default|GetPrevMovementMode) "MOVE_Swimming")
                                  (Utilities|FlowControl|Sequence
                                    (:then_0
                                      (if (CallFunction|NotEqualtoCustomMode "MOVE_Falling")
                                        (Pawn|Components|CharacterMovement|SetMovementMode (Variables|/Script/Engine.Character|GetCharacterMovement (.AsCharacter (Utilities|Casting|CastToCharacter (Components|GetOwner)))) "MOVE_Falling" 0)))
                                    (:then_1
                                      (CallFunction|SetFallSpeedWithoutParachute))))))))))))))))))))

(event Custom|onLanded
  ;[1 1 1] Control distance to ground and check can character use a parachute
  (CallFunction|ControlIsSkydiving-All false)
  (CallFunction|ControlPO-All false)
  (CallFunction|ParachuteLand))

(event Custom|ResetSpawnBackpack
  ;[1 1 1] Control distance to ground and check can character use a parachute
  (Utilities|FlowControl|DoOnce false) ; enters at Reset
)

(event Custom|Check
  (bind _returnvalue (Components|GetOwner))
  (bind _ascharacter (Utilities|Casting|CastToCharacter _returnvalue))
  (bind _charactermovement (Variables|/Script/Engine.Character|GetCharacterMovement _ascharacter))
  (bind _movementmode (Variables|/Script/Engine.CharacterMovementComponent|GetMovementMode _charactermovement))
  (Utilities|NotonLadder
    (:Not
      (if (Utilities|Enum|NotEqual(Enum) (Variables|/Script/Engine.CharacterMovementComponent|GetMovementMode (Variables|Default|GetCharacterMovement)) "MOVE_Swimming")
        (Utilities|FlowControl|Sequence
          (:then_0
            (if (or (Utilities|Enum|Equal(Enum) _movementmode "MOVE_Falling") (Utilities|Enum|Equal(Enum) _movementmode "MOVE_Flying"))
              (if (Class|KismetSystemLibrary|IsTimerPausedHandle (Variables|Default|GetTimer))
                (Utilities|Time|UnpauseTimerbyHandle (Variables|Default|GetTimer))
                (CallFunction|ResetControl))
              (elif (Class|KismetSystemLibrary|IsTimerPausedHandle (Variables|Default|GetTimer))
                (Utilities|FlowControl|DoOnce false
                  (:Completed
                    (CallFunction|ControlIsSkydiving-All false)
                    (CallFunction|ControlPO-All false)))
                (else
                  (Utilities|Time|PauseTimerbyHandle (Variables|Default|GetTimer))
                  (CallFunction|ResetSpawnBackpack)
                  (CallFunction|ResetControl)
                  (Utilities|IsValid (Variables|Default|GetBackpack)
                    (:Is%20Valid
                      (CallFunction|ParachuteLand)))))))
          (:then_1
            (Utilities|IsValid (Variables|Default|GetBackpack)
              (:Is%20Valid
                (CallFunction|SetParachuteRotation-Server)))))))))

(event Custom|ResetControl
  (Utilities|FlowControl|DoOnce false) ; enters at Reset
)