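; Actor component in the character parachute system that measures how far an airborne character is above the ground.
; On Tick, while the owner is not moving on the ground, the server updates GroundDistance.
; The value comes from a long downward Visibility line trace from the body mesh's root socket, ignoring the owner, taking the distance between trace start and hit location.
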(event EventBeginPlay)

(event EventTick
  (params (DeltaSeconds :type Float%20%28single-precision%29))
  ;[1 1 1] Distance between character and ground
  (if (not (AI|Components|NavMovement|IsMovingonGround (Variables|/Script/Engine.Character|GetCharacterMovement (.AsCharacter (Utilities|Casting|CastToCharacter (Components|GetOwner))))))
    (Networking|SwitchHasAuthority
      (:Authority
        (bind _returnvalue (CallFunction|Calculate))
        (Variables|Default|SetGroundDistance _returnvalue)))))

(fn Calculate
  (bind _returnvalue (Components|GetOwner))
  (bind _bodymesh (CallFunction|GetCharacterSkeleton (.AsCharacter (Utilities|Casting|CastToCharacter (Components|GetOwner)))))
  (Utilities|IsValid _returnvalue
    (:Is%20Valid
      (bind _outhit (Collision|LineTraceByChannel (.location (Transformation|GetSocketTransform _bodymesh "root" "RTS_World")) (+ (.location (Transformation|GetSocketTransform _bodymesh "root" "RTS_World")) (* (Math|Vector|GetUpVector (Variables|/Script/Engine.Character|GetCapsuleComponent (.AsCharacter (Utilities|Casting|CastToCharacter (Components|GetOwner))))) "0, 0,-100000.000000")) "TraceTypeQuery1" false (Utilities|Array|MakeArray _returnvalue) "None" true "(R=0.035046,G=0.000000,B=1.000000,A=1.000000)"))
      (return (Math|Float|Max(Float) (Math|Vector|Distance(Vector) (.Location (Collision|BreakHitResult _outhit)) (.TraceStart (Collision|BreakHitResult _outhit))) 0.0)))))