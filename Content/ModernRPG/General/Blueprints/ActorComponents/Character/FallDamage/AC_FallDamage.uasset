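; AC_FallDamage is an actor component that calculates fall damage and the matching landing sound for its owner.
; GetCurrentDamage traces down from the owner and maps vertical velocity through a curve to damage, zeroed for exempt actor classes or missing physical materials.
; GetFallSound matches the surface type against a data table, falling back to a default step sound.
; The component only returns damage, sound and a play-sound flag, applying none itself.
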(fn GetCurrentDamage
  (bind _returnvalue (Components|GetOwner))
  (bind _returnvalue_2 (Components|GetOwner))
  (bind _curve (Variables|Settings|GetCurve))
  (bind _returnvalue_3 (Transformation|GetVelocity _returnvalue_2))
  (bind _returnvalue_4 (Transformation|GetActorLocation _returnvalue))
  (bind _z (Math|Vector|BreakVector _returnvalue_3))
  (bind _returnvalue_5 (Math|Curves|GetFloatValue _curve _z))
  (bind _outhit (Collision|LineTraceByChannel _returnvalue_4 (- _returnvalue_4 "0, 0,500.000000") "TraceTypeQuery1" false 0 "None"))
  (Utilities|IsValid (.PhysMat (Collision|BreakHitResult _outhit))
    (:Is%20Valid
      (return (select (Utilities|Array|ContainsItem (Variables|Settings|GetNoFallDamageClasses) (Utilities|GetClass (.HitActor (Collision|BreakHitResult _outhit)))) 0.0 (Math|Float|MapRangeClamped _returnvalue_5 0.0 1.0 0.0 1e+02)) (CallFunction|GetFallSound (Variables|/Script/PhysicsCore.PhysicalMaterial|GetSurfaceType (.PhysMat (Collision|BreakHitResult _outhit)))) (> _returnvalue_5 0.1)))
    (:Is%20Not%20Valid
      (return 0.0 0 false))))

(fn GetFallSound
  (params (Type :type EPhysicalSurface%20Enum :default "SurfaceType_Default"))
  (bind _outrownames (DataTable|GetDataTableRowNames (Variables|Settings|GetFallTable)))
  (for _array_element _outrownames
    (bind _returnvalue (Utilities|GetDataTableRow (Variables|Settings|GetFallTable) _array_element)
      (:then
        (if (Utilities|Enum|Equal(Enum) (.Type (Utilities|Struct|BreakS_FallSound _returnvalue)) Type)
          (return (.Sound (Utilities|Struct|BreakS_FallSound _returnvalue)))))))
  (return "/Game/ModernRPG/Shooter/Sounds/Drop/SC_CasualDropStep.SC_CasualDropStep"))