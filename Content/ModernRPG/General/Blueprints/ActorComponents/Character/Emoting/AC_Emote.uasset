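; AC_Emote is a character actor component that plays an emote montage on a supplied skeletal mesh.
; A Server event forwards to an ALL event, which plays the montage and sends its length to the anim instance through an emotions message.
; It then binds to character movement updates, stopping the montage and unbinding all movement-update handlers once the character has velocity or crouches.
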(event Custom|CheckForMovement
  (params (DeltaSeconds :type Float%20%28single-precision%29) (OldLocation :type Vector) (OldVelocity :type Vector))
  (if (or (> (Math|Vector|VectorLength OldVelocity) 0.0) (AI|Components|NavMovement|IsCrouching (Variables|/Script/Engine.Character|GetCharacterMovement (Variables|Default|GetAs%20Character))))
    (EventDispatchers|UnbindallEventsfromOnCharacterMovementUpdated (Variables|Default|GetAs%20Character))
    (Animation|StopAnimMontage (Variables|Default|GetAs%20Character) (Variables|Default|GetEmoteMontage))))

(event Custom|Emote%20-%20ALL
  (params (InSkeletalMeshComponent :type Skeletal%20Mesh%20Component%20Object%20Reference))
  (Animation|Montage|PlayMontage InSkeletalMeshComponent (Variables|Default|GetEmoteMontage)
    (:then
      (Class|BPIABP|SetEmotions(Message) (Components|SkeletalMesh|GetAnimInstance InSkeletalMeshComponent) (Variables|/Script/Engine.AnimSequenceBase|GetSequenceLength (Variables|Default|GetEmoteMontage)))
      (Character|BindEventtoOnCharacterMovementUpdated (Variables|Default|GetAs%20Character) (EventDispatchers|CreateEvent :!event Custom|CheckForMovement)))))

(event Custom|Emote%20-%20Server
  (params (InSkeletalMeshComponent :type Skeletal%20Mesh%20Component%20Object%20Reference))
  (CallFunction|Emote-ALL InSkeletalMeshComponent))

(event EventBeginPlay
  (bind _ascharacter (Utilities|Casting|CastToCharacter (Components|GetOwner)))
  (Variables|Default|SetAs%20Character _ascharacter))