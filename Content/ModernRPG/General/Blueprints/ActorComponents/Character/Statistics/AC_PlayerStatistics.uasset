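; Actor component that tracks and persists general and per-weapon-type statistics for a player-controlled pawn.
; On BeginPlay it loads both arrays from a BP_SaveStatistics slot, or seeds them from data tables and saves.
; Add functions accumulate values by row name, with weapon stats also keyed by the weapon type from AC_EquipmentHandler.
; Changes trigger a flag-guarded delayed save, batching frequent updates into one write.
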(event Custom|SaveStatisticsDelay
  ;[1 1 1] Save Statistics With Delay
  (if (not (Variables|Default|GetInSaveDelay))
    (Variables|Default|SetInSaveDelay true)
    (Utilities|FlowControl|Delay (Variables|Default|GetSaveDelay))
    (CallFunction|SaveStatistics)
    (Variables|Default|SetInSaveDelay false)))

(event EventTick
  (params (DeltaSeconds :type Float%20%28single-precision%29))
  ;[1 1 1] Connect if you want to Debug Statistics
)

(event EventBeginPlay
  ;[1 1 1] Load Statistics
  (CallFunction|LoadStatistics))

(fn LoadStatistics
  (bind _returnvalue (SaveGame|DoesSaveGameExist (Variables|Default|GetStatSlot)))
  (if _returnvalue
    (bind _returnvalue_2 (SaveGame|LoadGamefromSlot (Variables|Default|GetStatSlot)))
    (bind _asbp_save_statistics (Utilities|Casting|CastToBP_SaveStatistics _returnvalue_2))
    (Variables|Default|SetStatistics (Variables|/Game/ModernRPG/General/Blueprints/Player/BP_SaveStatistics.BP_SaveStatistics_C|GetsStatistics _asbp_save_statistics))
    (Variables|Default|SetWeaponStatistics (Variables|/Game/ModernRPG/General/Blueprints/Player/BP_SaveStatistics.BP_SaveStatistics_C|GetsWeaponStatistics _asbp_save_statistics))
    (else
      (bind _returnvalue_3 (SaveGame|CreateSaveGameObject "/Game/ModernRPG/General/Blueprints/Player/BP_SaveStatistics.BP_SaveStatistics_C"))
      (LocalVariables|SetL_SaveGame _returnvalue_3)
      (bind _outrownames (DataTable|GetDataTableRowNames "/Game/ModernRPG/General/Blueprints/DataTables/DT_StatisticsTypes.DT_StatisticsTypes"))
      (for _array_element _outrownames
        (Utilities|Array|Add (Variables|Default|GetStatistics) (Utilities|Struct|MakeS_StatisticDynamic (Utilities|Struct|MakeDataTableRowHandle "/Game/ModernRPG/General/Blueprints/DataTables/DT_StatisticsTypes.DT_StatisticsTypes" _array_element) 0.0)))
      (bind _outrownames_2 (DataTable|GetDataTableRowNames "/Game/ModernRPG/General/Blueprints/DataTables/DT_WeaponStatistics.DT_WeaponStatistics"))
      (for _array_element_2 _outrownames_2
        (bind _returnvalue_4 (Utilities|GetDataTableRow (.datatable (Utilities|Struct|MakeDataTableRowHandle "/Game/ModernRPG/General/Blueprints/DataTables/DT_WeaponStatistics.DT_WeaponStatistics" _array_element_2)) (.rowname (Utilities|Struct|MakeDataTableRowHandle "/Game/ModernRPG/General/Blueprints/DataTables/DT_WeaponStatistics.DT_WeaponStatistics" _array_element_2)))
          (:then
            (if (Utilities|Enum|Equal(Enum) (.Type (Utilities|Struct|BreakS_WeaponStatisticsF _returnvalue_4)) "NewEnumerator7")
              (for _index (range 0 (- (|GetNumEnumEntries) 1))
                (Utilities|Array|Add (Variables|Default|GetWeaponStatistics) (Utilities|Struct|MakeS_WeaponStatisticsDynamic (Utilities|Struct|MakeDataTableRowHandle (.datatable (Utilities|Struct|MakeDataTableRowHandle "/Game/ModernRPG/General/Blueprints/DataTables/DT_WeaponStatistics.DT_WeaponStatistics" _array_element_2)) (.rowname (Utilities|Struct|MakeDataTableRowHandle "/Game/ModernRPG/General/Blueprints/DataTables/DT_WeaponStatistics.DT_WeaponStatistics" _array_element_2))) (Utilities|Enum|ByteToEnumE_WeaponType (Math|Conversions|ToByte(Integer) _index)) 0.0)))
              (else
                (Utilities|Array|Add (Variables|Default|GetWeaponStatistics) (Utilities|Struct|MakeS_WeaponStatisticsDynamic (Utilities|Struct|MakeDataTableRowHandle (.datatable (Utilities|Struct|MakeDataTableRowHandle "/Game/ModernRPG/General/Blueprints/DataTables/DT_WeaponStatistics.DT_WeaponStatistics" _array_element_2)) (.rowname (Utilities|Struct|MakeDataTableRowHandle "/Game/ModernRPG/General/Blueprints/DataTables/DT_WeaponStatistics.DT_WeaponStatistics" _array_element_2))) (.Type (Utilities|Struct|BreakS_WeaponStatisticsF _returnvalue_4)) 0.0)))))))
      (Variables|/Game/ModernRPG/General/Blueprints/Player/BP_SaveStatistics.BP_SaveStatistics_C|SetsStatistics (LocalVariables|GetL_SaveGame) (Variables|Default|GetStatistics))
      (Variables|/Game/ModernRPG/General/Blueprints/Player/BP_SaveStatistics.BP_SaveStatistics_C|SetsWeaponStatistics (LocalVariables|GetL_SaveGame) (Variables|Default|GetWeaponStatistics))
      (SaveGame|SaveGametoSlot (LocalVariables|GetL_SaveGame) (Variables|Default|GetStatSlot)))))

(fn SaveStatistics
  (bind _returnvalue (SaveGame|DoesSaveGameExist (Variables|Default|GetStatSlot)))
  (if _returnvalue
    (bind _returnvalue_2 (SaveGame|LoadGamefromSlot (Variables|Default|GetStatSlot)))
    (bind _asbp_save_statistics (Utilities|Casting|CastToBP_SaveStatistics _returnvalue_2))
    (LocalVariables|SetL_GameSave _asbp_save_statistics)
    (else
      (bind _returnvalue_3 (SaveGame|CreateSaveGameObject "/Game/ModernRPG/General/Blueprints/Player/BP_SaveStatistics.BP_SaveStatistics_C"))
      (LocalVariables|SetL_GameSave _returnvalue_3)))
  (Variables|/Game/ModernRPG/General/Blueprints/Player/BP_SaveStatistics.BP_SaveStatistics_C|SetsStatistics (LocalVariables|GetL_GameSave) (Variables|Default|GetStatistics))
  (Variables|/Game/ModernRPG/General/Blueprints/Player/BP_SaveStatistics.BP_SaveStatistics_C|SetsWeaponStatistics (LocalVariables|GetL_GameSave) (Variables|Default|GetWeaponStatistics))
  (SaveGame|SaveGametoSlot (LocalVariables|GetL_GameSave) (Variables|Default|GetStatSlot)))

(fn AddStatistics
  (params (Item :type Data%20Table%20Row%20Handle%20Structure) (Value :type Float%20%28double-precision%29))
  (bind (_result _index) (CallFunction|HasStatistic Item))
  (bind _returnvalue (Components|GetOwner))
  (bind _statistics (Variables|Default|GetStatistics))
  (bind (_aspawn _bsuccess) (Utilities|Casting|CastToPawn _returnvalue))
  (bind _output (Utilities|Array|Get(acopy) _statistics _index))
  (bind (_statistic _value) (Utilities|Struct|BreakS_StatisticDynamic _output))
  (if _bsuccess
    (if (Pawn|IsPlayerControlled _aspawn)
      (if _result
        (Utilities|Array|SetArrayElem (Variables|Default|GetStatistics) _index (Utilities|Struct|MakeS_StatisticDynamic _statistic (+ _value Value)))
        (else
          (Utilities|Array|Add (Variables|Default|GetStatistics) (Utilities|Struct|MakeS_StatisticDynamic Item Value))))
      (CallFunction|SaveStatisticsDelay))))

(fn HasStatistic
  (params (InputPin :type Data%20Table%20Row%20Handle%20Structure))
  (for (_array_element _array_index) (Variables|Default|GetStatistics)
    (if (Utilities|Name|Equal(Name) (.RowName (Utilities|Struct|BreakDataTableRowHandle (.Statistic (Utilities|Struct|BreakS_StatisticDynamic _array_element)))) (.RowName (Utilities|Struct|BreakDataTableRowHandle InputPin)))
      (return true _array_index)))
  (return false 0))

(fn GetStatisticValue
  (params (InputPin :type Data%20Table%20Row%20Handle%20Structure))
  (bind (_result _index) (CallFunction|HasStatistic InputPin))
  (if _result
    (return (Utilities|Array|Get(acopy) (Variables|Default|GetStatistics) _index))))

(fn DebugStatistics
  (for _array_element (Variables|Default|GetStatistics)
    (if (!= (.Value (Utilities|Struct|BreakS_StatisticDynamic _array_element)) 0.0)
      (Development|PrintString (Utilities|String|Append (Utilities|String|ToString(Name) (.RowName (Utilities|Struct|BreakDataTableRowHandle (.Statistic (Utilities|Struct|BreakS_StatisticDynamic _array_element))))) " " (Utilities|String|ToString(Float) (.Value (Utilities|Struct|BreakS_StatisticDynamic _array_element)))) true true "(R=0.000000,G=0.660000,B=1.000000,A=1.000000)" 0.0))))

(fn AddWeaponStatistics
  (params (Statistic :type Data%20Table%20Row%20Handle%20Structure) (Value :type Float%20%28double-precision%29))
  (bind _returnvalue (Components|GetOwner))
  (bind (_result _index) (Weapon|HasWeaponStatistic Statistic))
  (bind _weaponstatistics (Variables|Default|GetWeaponStatistics))
  (bind (_aspawn _bsuccess) (Utilities|Casting|CastToPawn _returnvalue))
  (bind _output (Utilities|Array|Get(acopy) _weaponstatistics _index))
  (bind (_item _weapontype _value) (Utilities|Struct|BreakS_WeaponStatisticsDynamic _output))
  (if _bsuccess
    (if (Pawn|IsPlayerControlled _aspawn)
      (if _result
        (Utilities|Array|SetArrayElem (Variables|Default|GetWeaponStatistics) _index (Utilities|Struct|MakeS_WeaponStatisticsDynamic _item _weapontype (+ _value Value)))
        (else
          (Utilities|Array|Add (Variables|Default|GetWeaponStatistics) (Utilities|Struct|MakeS_WeaponStatisticsDynamic Statistic (CallFunction|GetOwnerWeaponType) Value))))
      (CallFunction|SaveStatisticsDelay))))

(fn GetWeaponStatistics
  (params (Item :type Data%20Table%20Row%20Handle%20Structure))
  (bind (_result _index) (Weapon|HasWeaponStatistic Item))
  (if _result
    (return (Utilities|Array|Get(acopy) (Variables|Default|GetWeaponStatistics) _index))))

(fn GetOwnerWeaponType
  (bind _returnvalue (Components|GetOwner))
  (bind _returnvalue_2 (Actor|GetComponentbyClass _returnvalue "/Game/ModernRPG/General/Blueprints/ActorComponents/InteractActors/AC_EquipmentHandler.AC_EquipmentHandler_C"))
  (bind (_has _array_element) (Default|GetCurrentWeapon _returnvalue_2))
  (Utilities|IsValid _returnvalue_2
    (:Is%20Valid
      (if _has
        (return (Utilities|Struct|BreakS_WeaponCharacteristics (.WEAPON_CHARACTERISTICS (Utilities|Struct|BreakS_Weapon (CallFunction|GetWeaponInfo (.Row (Utilities|Struct|BreakS_InvItemDyn _array_element)))))))
        (else
          (return "NewEnumerator0"))))))

(fn HasWeaponStatistic
  (params (InputPin :type Data%20Table%20Row%20Handle%20Structure))
  (for (_array_element _array_index) (Variables|Default|GetWeaponStatistics)
    (if (and (Utilities|Name|Equal(Name) (.RowName (Utilities|Struct|BreakDataTableRowHandle (.Item (Utilities|Struct|BreakS_WeaponStatisticsDynamic _array_element)))) (.RowName (Utilities|Struct|BreakDataTableRowHandle InputPin))) (Utilities|Enum|Equal(Enum) (.WeaponType (Utilities|Struct|BreakS_WeaponStatisticsDynamic _array_element)) (CallFunction|GetOwnerWeaponType)))
      (return true _array_index)))
  (return false 0))

(fn DebugStatisticsWeapon
  (for _array_element (Variables|Default|GetWeaponStatistics)
    (if (!= (.Value (Utilities|Struct|BreakS_WeaponStatisticsDynamic _array_element)) 0.0)
      (Development|PrintString (Utilities|String|Append (Utilities|String|ToString(Name) (.RowName (Utilities|Struct|BreakDataTableRowHandle (.Item (Utilities|Struct|BreakS_WeaponStatisticsDynamic _array_element))))) " " (Utilities|String|ToString(Float) (.Value (Utilities|Struct|BreakS_WeaponStatisticsDynamic _array_element))) " " (Utilities|String|EnumtoString (.WeaponType (Utilities|Struct|BreakS_WeaponStatisticsDynamic _array_element)))) true true "(R=0.000000,G=0.660000,B=1.000000,A=1.000000)" 0.0))))