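; Actor component that handles character death and respawn, replicated through server and multicast events.
; Death records kill statistics, clears gameplay states, disables input and turns the death cam toward the killer.
; The body ragdolls, first playing a hit-direction or explosion montage if airborne or swimming.
; Optional respawn fades the screen, then either reloads the level in solo or restores the character at a random PlayerStart.
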(event Custom|MESSAGE_TO_ABP_Dead%20-%20Server
  (CallFunction|MESSAGETOABPDead-ALL))

(event Custom|Release
  (bind _returnvalue (Components|GetOwner))
  (bind _returnvalue_2 (Components|GetOwner))
  (bind _returnvalue_3 (Components|GetOwner))
  (bind _returnvalue_4 (Components|GetOwner))
  (bind _returnvalue_5 (Components|GetOwner))
  (bind _returnvalue_6 (Components|GetOwner))
  (bind _returnvalue_7 (Components|GetOwner))
  (bind _returnvalue_8 (Components|GetOwner))
  (bind _returnvalue_9 (Components|GetOwner))
  (bind _returnvalue_10 (Components|GetOwner))
  (bind _returnvalue_11 (Actor|GetComponentbyClass _returnvalue_2 "/Game/ModernRPG/General/Blueprints/LockAndHead/Lock/AC_LockedActor.AC_LockedActor_C"))
  (bind _returnvalue_12 (Actor|GetComponentbyClass _returnvalue_9 "/Game/ModernRPG/General/Blueprints/ActorComponents/SpeedChange/AC_SpeedChange.AC_SpeedChange_C"))
  (bind _returnvalue_13 (Actor|GetComponentbyClass _returnvalue "/Game/ModernRPG/General/Blueprints/DialoguesQuests/Dialogue/AC_DialogueSystem.AC_DialogueSystem_C"))
  (bind _returnvalue_14 (Actor|GetComponentbyClass _returnvalue_4 "/Game/ModernRPG/General/Blueprints/ActorComponents/Weapon/AC_Aiming.AC_Aiming_C"))
  (bind _returnvalue_15 (Actor|GetComponentbyClass _returnvalue_10 "/Game/ModernRPG/General/Blueprints/ActorComponents/Character/Inventory/AC_Inventory.AC_Inventory_C"))
  (bind _returnvalue_16 (Actor|GetComponentbyClass _returnvalue_5 "/Game/ModernRPG/General/Blueprints/ActorComponents/Weapon/AC_Weapon.AC_Weapon_C"))
  (bind _returnvalue_17 (Actor|GetComponentbyClass _returnvalue_6 "/Game/ModernRPG/General/Blueprints/ActorComponents/Water/AC_Swimming.AC_Swimming_C"))
  (bind _returnvalue_18 (Actor|GetComponentbyClass _returnvalue_8 "/Game/ModernRPG/General/Blueprints/ActorComponents/WidgetsInfo/AC_PauseMenu.AC_PauseMenu_C"))
  (bind _returnvalue_19 (Actor|GetComponentbyClass _returnvalue_3 "/Game/ModernRPG/General/Blueprints/ActorComponents/InteractActors/AC_Interaction.AC_Interaction_C"))
  (bind _npc (Variables|/Game/ModernRPG/General/Blueprints/DialoguesQuests/Dialogue/AC_DialogueSystem.AC_DialogueSystem_C|GetNPC _returnvalue_13))
  ;[1 1 1] Release
  (Utilities|IsValid _returnvalue_14
    (:Is%20Valid
      (Default|StopAiming-Server _returnvalue_14))
    (:Is%20Not%20Valid
      _))
  (Utilities|IsValid _returnvalue_16
    (:Is%20Valid
      (Default|ShootingReleased _returnvalue_16))
    (:Is%20Not%20Valid
      _))
  (bind _ascharacter (Utilities|Casting|CastToCharacter _returnvalue_7)
    (:then
      (bind _defaultbodymesh (Class|BPIAI|GetDemoSkeletalMeshes(Message) _returnvalue_7))
      (Character|UnCrouch _ascharacter)
      (Class|BPICharacter|ControlCrouch(Message) (Components|GetOwner) false)
      (Class|BPIOptimization|SetCrouching(Message) (Components|SkeletalMesh|GetAnimInstance _defaultbodymesh) false)
      (Character|StopJumping _ascharacter))
    (:CastFailed
      _))
  (Utilities|IsValid _returnvalue_12
    (:Is%20Valid
      (Default|ChangeWalkSpeed _returnvalue_12 "NewEnumerator1"))
    (:Is%20Not%20Valid
      _))
  (Utilities|IsValid _returnvalue_15
    (:Is%20Valid
      (Default|CloseInventory _returnvalue_15))
    (:Is%20Not%20Valid
      _))
  (Utilities|IsValid _returnvalue_18
    (:Is%20Valid
      (Default|TryRemovePauseMenu _returnvalue_18))
    (:Is%20Not%20Valid
      _))
  (Utilities|IsValid _returnvalue_11
    (:Is%20Valid
      (Default|EndUnlock _returnvalue_11 false))
    (:Is%20Not%20Valid
      _))
  (Utilities|IsValid _returnvalue_19
    (:Is%20Valid
      (Default|HideInteractWidget-Server _returnvalue_19))
    (:Is%20Not%20Valid
      _))
  (Utilities|IsValid _returnvalue_17
    (:Is%20Valid
      (Default|HideWidgetReplicated _returnvalue_17))
    (:Is%20Not%20Valid
      _))
  (Utilities|IsValid _npc
    (:Is%20Valid
      (Default|DialogueFinished _npc))))

(event Custom|FadeScreen%20-Server
  ;[1 1 1] Fade Screen Event
  (CallFunction|FadeScreen-OC))

(event Custom|ForceSetDead
  ;[1 1 1] Force Set Dead
  (if (Ability|HasAuthority (Components|GetOwner))
    (CallFunction|ForceSetDead-ALL)
    (else
      (CallFunction|ForceSetDead-Server))))

(event Custom|ForceSetDead%20-ALL
  ;[1 1 1] Force Set Dead
  (Variables|State|SetDead true)
  (Components|Tick|SetComponentTickEnabled true)
  (Input|DisableInput (Variables|Engine|GetCharacter) (Variables|Engine|GetPlayerController)))

(event Custom|ForceSetDead%20-Server
  ;[1 1 1] Force Set Dead
  (CallFunction|ForceSetDead-ALL))

(event Custom|ResetSpawn
  ;[1 1 1] Replicate New Spawn Location
  (bind (_returnvalue _rotation) (CallFunction|GetSpawnLocation))
  (CallFunction|ResetSpawn-ALL _returnvalue _rotation))

(event Custom|ResetSpawn-ALL
  (params (NewLocation :type Vector) (NewRotation :type Rotator))
  ;[1 1 1] Replicate New Spawn Location
  (Transformation|SetActorLocationAndRotation (Variables|Engine|GetCharacter) NewLocation NewRotation false true))

(event Custom|CharResp%20-%20Server
  (CallFunction|CharResp-ALL))

(event Custom|CharResp%20-%20ALL
  (CallFunction|CharacterRespawn-NR))

(event Custom|MESSAGE_TO_ABP_Dead%20-%20ALL
  (bind _defaultbodymesh (Class|BPIAI|GetDemoSkeletalMeshes(Message) (Variables|Engine|GetCharacter)))
  (Class|BPIABP|SetIsDead(Message) (Components|SkeletalMesh|GetAnimInstance _defaultbodymesh) false))

(event Custom|CharResp%20-%20Replicate
  (Networking|SwitchHasAuthority
    (:Authority
      (CallFunction|CharResp-ALL))
    (:Remote
      (CallFunction|CharResp-Server))))

(event Custom|SetCollision%20-ALL
  (bind _character (Variables|Engine|GetCharacter))
  (bind _capsulecomponent (Variables|/Script/Engine.Character|GetCapsuleComponent _character))
  ;[1 1 1] Replicate Collision
  (bind _defaultbodymesh (Class|BPIAI|GetDemoSkeletalMeshes(Message) (Variables|Engine|GetCharacter)))
  (Transformation|AttachComponentToComponent _defaultbodymesh (Variables|/Script/Engine.Character|GetCapsuleComponent (Variables|Engine|GetCharacter)) "None" "SnapToTarget" "SnapToTarget" "KeepRelative" true)
  (Collision|SetCollisionEnabled _capsulecomponent "QueryAndPhysics")
  (Collision|SetCollisionResponsetoChannel _capsulecomponent "ECC_GameTraceChannel4" "ECR_Block"))

(event Custom|WriteDeathStatistics
  (bind _returnvalue (Components|GetOwner))
  (bind _killsstat (Variables|Statistics|GetKillsStat))
  (bind _deathstatistics (Variables|Statistics|GetDeathStatistics))
  (bind _returnvalue_2 (Actor|GetComponentbyClass _returnvalue "/Game/ModernRPG/General/Blueprints/ActorComponents/Character/Statistics/AC_PlayerStatistics.AC_PlayerStatistics_C"))
  (bind _output (Default|GetStatisticValue _returnvalue_2 _killsstat))
  (bind _output_2 (Default|GetStatisticValue _returnvalue_2 _deathstatistics))
  ;[1 1 1] Death Statistics
  (bind _aspawn (Utilities|Casting|CastToPawn (Components|GetOwner)))
  (if (Pawn|IsPlayerControlled _aspawn)
    (Utilities|IsValid _returnvalue_2
      (:Is%20Valid
        (Default|AddStatistics _returnvalue_2 (Variables|Statistics|GetDeathStatistics) 1.0)
        (Default|AddStatistics _returnvalue_2 (Variables|Statistics|GetK/DStatistics) (select (== (.value _output_2) 0.0) (.value _output) (/ (.value _output) (.value _output_2))))))))

(event Custom|CharacterRespawn%20-NR
  (bind _character (Variables|Engine|GetCharacter))
  (bind _returnvalue (Actor|GetComponentbyClass _character "/Game/ModernRPG/General/Blueprints/ActorComponents/ViewSwitch/AC_ViewSwitch.AC_ViewSwitch_C"))
  (Utilities|FlowControl|Sequence
    (:then_0
      ;[1 1 1] Respawn
      (bind _defaultbodymesh (Class|BPIAI|GetDemoSkeletalMeshes(Message) (Variables|Engine|GetCharacter)))
      (Physics|SetSimulatePhysics _defaultbodymesh false)
      (Transformation|DetachFromActor (Components|GetOwner) "KeepWorld" "KeepWorld" "KeepWorld")
      (Variables|State|SetDead false)
      (bind _defaultbodymesh_2 (Class|BPIAI|GetDemoSkeletalMeshes(Message) (Variables|Engine|GetCharacter)))
      (Class|PrimitiveComponent|SetMassOverrideinKg _defaultbodymesh_2 "None" 5e+03 false)
      (bind _camera (Class|BPIDeath|SwitchDeathCam(Message) (Components|GetOwner) true))
      (Transformation|SetRelativeRotation _camera "0, 0, 0" false false)
      (CallFunction|ResetControlRotation)
      (if (> (Variables|Settings|GetAdditionalDelay) 0.0)
        (Utilities|FlowControl|Delay (Variables|Settings|GetAdditionalDelay)))
      (CallFunction|SetCollision-Server)
      (bind _defaultbodymesh_3 (Class|BPIAI|GetDemoSkeletalMeshes(Message) (Variables|Engine|GetCharacter)))
      (Transformation|SetRelativeLocationAndRotation _defaultbodymesh_3 "0.000000,0.000000,-90.000000" "0,-90.000000, 0" false true)
      (Transformation|SetActorLocationAndRotation (Variables|Engine|GetCharacter) "0, 0, 0")
      (CallFunction|ResetSpawn)
      (Input|EnableInput (Variables|Engine|GetCharacter) (Variables|Engine|GetPlayerController))
      (Utilities|FlowControl|Delay 0.5)
      (Components|Tick|SetComponentTickEnabled false)
      (CallFunction|ResetControlRotation)
      (Default|CallRespawned)
      (CallFunction|MESSAGETOABPDead-Server))
    (:then_1
      (if (not (Variables|/Game/ModernRPG/General/Blueprints/ActorComponents/ViewSwitch/AC_ViewSwitch.AC_ViewSwitch_C|GetInThirdPerson _returnvalue))
        (Default|SwitchView _returnvalue)))))

(event Custom|SetCollision%20-Server
  ;[1 1 1] Replicate Collision
  (CallFunction|SetCollision-ALL))

(event Custom|FadeScreen%20-OC
  ;[1 1 1] Fade Screen Event
  (bind _returnvalue (UserInterface|CreateWidget "/Game/ModernRPG/General/GUI/Widgets/Tags/WB_FadeDark.WB_FadeDark_C"))
  (Variables|Engine|SetFadeScreen _returnvalue)
  (Utilities|IsValid (Variables|Engine|GetFadeScreen)
    (:Is%20Valid
      (UserInterface|Viewport|AddtoViewport (Variables|Engine|GetFadeScreen) 0))))

(event EventTick
  (params (DeltaSeconds :type Float%20%28single-precision%29))
  (bind _returnvalue (Components|GetOwner))
  (bind _instigator (Variables|/Script/Engine.Actor|GetInstigator _returnvalue))
  (bind _returnvalue_2 (Pawn|GetController _instigator))
  ;[1 1 1] Focus Camera
  (if (Variables|State|GetDead)
    (Utilities|IsValid (Variables|Default|GetDeathCam)
      (:Is%20Valid
        (Utilities|IsValid (Variables|Engine|GetKiller)
          (:Is%20Valid
            (Utilities|IsValid _returnvalue_2
              (:Is%20Valid
                (Pawn|SetControlRotation _returnvalue_2 (Class|KismetMathLibrary|RInterptoConstant (Pawn|GetControlRotation _instigator :!class /Script/Engine.Pawn) (Math|Rotator|FindLookatRotation (Transformation|GetActorLocation (Components|GetOwner)) (Transformation|GetActorLocation (Variables|Engine|GetKiller))) (Utilities|Time|GetWorldDeltaSeconds) 3e+02))))))))))

(event EventBeginPlay
  ;[1 1 1] Initialize
  (CallFunction|InitializeComponent)
  (Utilities|FlowControl|DoOnce false
    (:Completed
      (Utilities|FlowControl|Delay 0.2)
      (CallFunction|FillHitDegrees))))

(fn GetSpawnLocation
  (bind _outactors (Actor|GetAllActorsOfClass "/Script/Engine.PlayerStart"))
  (return (Transformation|GetActorLocation (Utilities|Array|Get(acopy) _outactors (Math|Random|RandomIntegerinRange 0 (- (Utilities|Array|Length _outactors) 1)))) (Transformation|GetActorRotation (Utilities|Array|Get(acopy) _outactors (Math|Random|RandomIntegerinRange 0 (- (Utilities|Array|Length _outactors) 1))))))

(fn ReleaseClip
  (bind _returnvalue (Components|GetOwner))
  (bind _returnvalue_2 (Actor|GetComponentbyClass _returnvalue "/Game/ModernRPG/General/Blueprints/ActorComponents/Weapon/AC_Reload.AC_Reload_C"))
  (Utilities|IsValid _returnvalue_2
    (:Is%20Valid
      (Default|ReleaseClip-Server _returnvalue_2))))

(fn WriteKillLog
  (params (Killer :type Actor%20Object%20Reference))
  (bind _returnvalue (Components|GetOwner))
  (bind _returnvalue_2 (Actor|GetComponentbyClass Killer "/Game/ModernRPG/General/Blueprints/ActorComponents/Weapon/AC_Aiming.AC_Aiming_C"))
  (bind _returnvalue_3 (Transformation|GetActorLocation Killer))
  (bind _returnvalue_4 (Transformation|GetActorLocation _returnvalue))
  (bind _returnvalue_5 (Math|Vector|Distance(Vector) _returnvalue_4 _returnvalue_3))
  (Utilities|IsValid Killer
    (:Is%20Valid
      (bind _name (Class|BPICharacter|GetName(Message) Killer))
      (Class|BPIWidgetsInfo|SetKillerName(Message) (Variables|/Game/ModernRPG/General/Blueprints/ActorComponents/Characteristics/AC_Characteristics.AC_Characteristics_C|GetDamage (CallFunction|GetCharacteristicbyType (Components|GetOwner) "NewEnumerator1")) true _name)
      (bind _output_get (LocalVariables|SetL_PlayerStatistics (Actor|GetComponentbyClass Killer "/Game/ModernRPG/General/Blueprints/ActorComponents/Character/Statistics/AC_PlayerStatistics.AC_PlayerStatistics_C")))
      (Utilities|IsValid _output_get
        (:Is%20Valid
          (Default|AddStatistics (LocalVariables|GetL_PlayerStatistics) (Variables|Statistics|GetKillsStat) 1.0)
          (Default|AddStatistics (LocalVariables|GetL_PlayerStatistics) (Variables|Statistics|GetK/DStatistics) (CallFunction|GetKDStat (LocalVariables|GetL_PlayerStatistics)))
          (Default|AddStatistics (LocalVariables|GetL_PlayerStatistics) (Variables|Statistics|GetScoresStatistics) 1e+01)
          (Default|AddWeaponStatistics (LocalVariables|GetL_PlayerStatistics) (Variables|Statistics|GetWeaponKillStatistics) 1.0)
          (if (<= (.Value (Utilities|Struct|BreakS_WeaponStatisticsDynamic (Default|GetWeaponStatistics (LocalVariables|GetL_PlayerStatistics) (Variables|Statistics|GetWeaponDistanceKillStat)))) _returnvalue_5)
            (Default|AddWeaponStatistics (LocalVariables|GetL_PlayerStatistics) (Variables|Statistics|GetWeaponDistanceKillStat) _returnvalue_5))
          (Utilities|IsValid _returnvalue_2
            (:Is%20Valid
              (if (Variables|/Game/ModernRPG/General/Blueprints/ActorComponents/Weapon/AC_Aiming.AC_Aiming_C|GetAiming _returnvalue_2)
                (Default|AddWeaponStatistics (LocalVariables|GetL_PlayerStatistics) (Variables|Statistics|GetWeaponKillScopeStat) 1.0)))))))))

(fn GetKDStat
  (params (Actor :type AC%20Player%20Statistics%20Object%20Reference))
  (bind _killsstat (Variables|Statistics|GetKillsStat))
  (bind _deathstatistics (Variables|Statistics|GetDeathStatistics))
  (bind _output (Default|GetStatisticValue Actor _killsstat))
  (bind _output_2 (Default|GetStatisticValue Actor _deathstatistics))
  (return (select (== (.value _output_2) 0.0) (.value _output) (/ (.value _output) (.value _output_2)))))

(fn CalculateHitDirection
  (params (HitNormal :type Vector) (DT :type Damage%20Type%20Object%20Reference))
  (if (not (.bSuccess (Utilities|Casting|CastToBPDT_Grenade DT)))
    (LocalVariables|SetDot%20Product%20-%20Forward%20Hit (Math|Vector|DotProduct (Transformation|GetActorForwardVector (Components|GetOwner)) HitNormal))
    (bind _output_get (LocalVariables|SetDot%20Product%20-%20Right%20Hit (Math|Vector|DotProduct (Transformation|GetActorRightVector (Components|GetOwner)) HitNormal)))
    ;[1 1 1] Use result of dot products to select appropriate animation
    (if (Math|Float|InRange(Float) _output_get -0.5 0.5)
      (LocalVariables|SetHit%20Montage%20Pick (select (> (LocalVariables|GetDot%20Product%20-%20Forward%20Hit) 0.0) (.Animation (CallFunction|GetDirection "NewEnumerator0")) (.Animation (CallFunction|GetDirection "NewEnumerator1"))))
      (else
        (LocalVariables|SetHit%20Montage%20Pick (select (> (LocalVariables|GetDot%20Product%20-%20Right%20Hit) 0.0) (.Animation (CallFunction|GetDirection "NewEnumerator3")) (.Animation (CallFunction|GetDirection "NewEnumerator2"))))))
    (return (LocalVariables|GetHit%20Montage%20Pick))
    (else
      (return "/Game/ModernRPG/NewAnimBP/Locomotion/Actions/Death/AM_ExplosionDeath.AM_ExplosionDeath"))))

(fn FillHitDegrees
  (bind _outrownames (DataTable|GetDataTableRowNames (Variables|Settings|GetHitsDT)))
  (for _array_element _outrownames
    (bind _returnvalue (Utilities|GetDataTableRow (Variables|Settings|GetHitsDT) _array_element)
      (:then
        (Utilities|Array|Add (Variables|Engine|GetHitDegrees) _returnvalue))))
  (return))

(fn GetDirection
  (params (InDirection :type E_HitDirection%20Enum :default "NewEnumerator0"))
  (for _array_element (Variables|Engine|GetHitDegrees)
    (if (Utilities|Enum|Equal(Enum) (.Direction (Utilities|Struct|BreakS_HitDegrees _array_element)) InDirection)
      (return (.Direction (Utilities|Struct|BreakS_HitDegrees _array_element)) (Utilities|Array|Get(acopy) (.Animation (Utilities|Struct|BreakS_HitDegrees _array_element)) (Math|Random|RandomIntegerinRange 0 (- (Utilities|Array|Length (.Animation (Utilities|Struct|BreakS_HitDegrees _array_element))) 1)))))))

(fn InitializeComponent
  (bind _ascharacter (Utilities|Casting|CastToCharacter (Components|GetOwner)))
  (bind _output_get (Variables|Engine|SetCharacter _ascharacter))
  (bind _asplayer_controller (Utilities|Casting|CastToPlayerController (Pawn|GetController _output_get)))
  (Variables|Engine|SetPlayerController _asplayer_controller))

(fn ResetControlRotation
  (bind _returnvalue (CallFunction|ResetCharacterRotationfromSaveFile))
  (bind _aspawn (Utilities|Casting|CastToPawn (Components|GetOwner)))
  (Utilities|IsValid (Pawn|GetController _aspawn)
    (:Is%20Valid
      (Pawn|SetControlRotation (Pawn|GetController _aspawn) (Math|Rotator|MakeRotator 0.0 0.0 (.yaw _returnvalue)))
      (Transformation|SetActorRotation _aspawn (Math|Rotator|MakeRotator 0.0 0.0 (.yaw _returnvalue))))))

(fn GetKillerName
  (bind _aspawn (Utilities|Casting|CastToPawn (Variables|Engine|GetKiller)))
  (return (PlayerState|GetPlayerName (Variables|/Script/Engine.Controller|GetPlayerState (Pawn|GetController _aspawn)))))

(fn IsinVehicle
  (bind _returnvalue (Components|GetOwner))
  (bind _asbp_demo_character (Utilities|Casting|CastToBP_DemoCharacter _returnvalue))
  (return _asbp_demo_character (Utilities|IsValid (Variables|/Game/ModernRPG/General/Blueprints/ActorComponents/Machinery/AC_VehicleController.AC_VehicleController_C|GetVehicle (Actor|GetComponentbyClass _asbp_demo_character "/Game/ModernRPG/General/Blueprints/ActorComponents/Machinery/AC_VehicleController.AC_VehicleController_C")))))

(fn AuthorityDeathEvents
  (params (Respawn? :type Boolean) (RespawnDelay :type Float%20%28double-precision%29) (inVehicle :type Boolean) (HitNormal :type Vector))
  (if inVehicle
    _
    (else
      (LocalVariables|SetDeathAnimation (CallFunction|CalculateHitDirection HitNormal (Variables|Engine|GetLast%20Damage%20Type)))))
  (Networking|SwitchHasAuthority
    (:Authority
      (CallFunction|CharacterDeath-ALL Respawn? RespawnDelay inVehicle (LocalVariables|GetDeathAnimation)))
    (:Remote
      (CallFunction|CharacterDeath-Server Respawn? RespawnDelay inVehicle (LocalVariables|GetDeathAnimation)))))

(fn ResetAllStates
  (bind _returnvalue (Components|GetOwner))
  (bind _returnvalue_2 (Components|GetOwner))
  (bind _character (Variables|Engine|GetCharacter))
  (bind _returnvalue_3 (Actor|GetComponentbyClass _returnvalue "/Game/ModernRPG/General/Blueprints/ActorComponents/Character/Parachute/AC_Parachute.AC_Parachute_C"))
  (bind _returnvalue_4 (Actor|GetComponentbyClass _returnvalue_2 "/Game/ModernRPG/General/Blueprints/Ladder/AC_LadderSystem.AC_LadderSystem_C"))
  (Utilities|FlowControl|Sequence
    (:then_0
      (Variables|/Game/ModernRPG/General/Blueprints/ActorComponents/Character/Parachute/AC_Parachute.AC_Parachute_C|SetParachuteOpenned _returnvalue_3 false)
      (Variables|/Game/ModernRPG/General/Blueprints/ActorComponents/Character/Parachute/AC_Parachute.AC_Parachute_C|SetIsSkydiving _returnvalue_3 false)
      (Variables|/Game/ModernRPG/General/Blueprints/ActorComponents/Weapon/AC_Aiming.AC_Aiming_C|SetAiming (Actor|GetComponentbyClass (Components|GetOwner) "/Game/ModernRPG/General/Blueprints/ActorComponents/Weapon/AC_Aiming.AC_Aiming_C") false)
      (Variables|/Game/ModernRPG/General/Blueprints/ActorComponents/Weapon/AC_Weapon.AC_Weapon_C|SetShooting (Actor|GetComponentbyClass (Components|GetOwner) "/Game/ModernRPG/General/Blueprints/ActorComponents/Weapon/AC_Weapon.AC_Weapon_C") false)
      (Variables|/Game/ModernRPG/General/Blueprints/Ladder/AC_LadderSystem.AC_LadderSystem_C|SetOnLadder _returnvalue_4 false)
      (Variables|/Game/ModernRPG/General/Blueprints/Ladder/AC_LadderSystem.AC_LadderSystem_C|SetInLadderArea _returnvalue_4 false)
      (Variables|/Game/ModernRPG/General/Blueprints/Ladder/AC_LadderSystem.AC_LadderSystem_C|SetCurrentState _returnvalue_4 "NewEnumerator0")
      (Variables|/Game/ModernRPG/General/Blueprints/Ladder/AC_LadderSystem.AC_LadderSystem_C|SetinTransition _returnvalue_4 false)
      (Variables|/Game/ModernRPG/General/Blueprints/ClimbSystem/AC_ClimbComponent.AC_ClimbComponent_C|SetParkour (Actor|GetComponentbyClass (Components|GetOwner) "/Game/ModernRPG/General/Blueprints/ClimbSystem/AC_ClimbComponent.AC_ClimbComponent_C") false))
    (:then_1
      (bind _defaultbodymesh (Class|BPIAI|GetDemoSkeletalMeshes(Message) _character))
      (bind _output_get (LocalVariables|SetAI (Components|SkeletalMesh|GetAnimInstance _defaultbodymesh)))
      (Class|BPIABP|SetParachuteOpenned(Message) _output_get false)
      (Class|BPIABP|SetIsSkydiving(Message) (LocalVariables|GetAI) false)
      (Class|BPIABP|SetIsAim(Message) (LocalVariables|GetAI) false)
      (Class|BPIABP|Shot(Message) (LocalVariables|GetAI) false)
      (Class|BPIABP|SetinTransitionLadder(Message) (LocalVariables|GetAI) false)
      (Class|BPIABP|SetonLadder(Message) (LocalVariables|GetAI) false)
      (Class|BPIABP|SetonLadderState(Message) (LocalVariables|GetAI) "NewEnumerator0")
      (Class|BPIABP|SetMovingonGround(Message) (LocalVariables|GetAI) true))
    (:then_2
      (Pawn|Components|CharacterMovement|SetMovementMode (Variables|/Script/Engine.Character|GetCharacterMovement _character) "MOVE_Walking" 0))
    (:then_3
      (Default|CallStopClimbingLadder (Actor|GetComponentbyClass (Components|GetOwner) "/Game/ModernRPG/General/Blueprints/Ladder/AC_LadderSystem.AC_LadderSystem_C")))))

(fn ResetCharacterRotationfromSaveFile
  (bind _outactors (Actor|GetAllActorsOfClass "/Script/Engine.PlayerStart"))
  (return (Transformation|GetActorRotation (Utilities|Array|Get(acopy) _outactors (Math|Random|RandomIntegerinRange 0 (- (Utilities|Array|Length _outactors) 1))))))

(event Custom|CharacterDeath
  (params (Respawn? :type Boolean) (RespawnDelay :type Float%20%28double-precision%29) (Killer :type Actor%20Object%20Reference) (inVehicle :type Boolean) (LastDamageType :type Damage%20Type%20Object%20Reference) (HitNormal :type Vector))
  ;[1 1 1] Character Death
  (Variables|Engine|SetKiller Killer)
  (Variables|Engine|SetLast%20Damage%20Type LastDamageType)
  (Utilities|FlowControl|DoOnce false
    (:Completed
      (Utilities|FlowControl|Sequence
        (:then_0
          (if (not inVehicle)
            (bind _camera (Class|BPIDeath|SwitchDeathCam(Message) (Variables|Engine|GetCharacter) false))
            (Variables|Default|SetDeathCam _camera))
          (CallFunction|WriteKillLog Killer)
          (CallFunction|ReleaseClip)
          (CallFunction|WriteDeathStatistics)
          (CallFunction|AuthorityDeathEvents Respawn? RespawnDelay inVehicle HitNormal))
        (:then_1
          (Utilities|FlowControl|Delay 3.0)
          (CallFunction|Reset))))))

(event Custom|StartWidgetWithDelay
  (params (Duration :type Float%20%28double-precision%29))
  ;[1 1 1] Death Event
  (Utilities|FlowControl|Delay Duration)
  (CallFunction|FadeScreen-Server))

(event Custom|Reset
  ;[1 1 1] Character Death
  (Utilities|FlowControl|DoOnce false) ; enters at Reset
)

(event Custom|CharacterDeath%20-ALL
  (params (Respawn? :type Boolean) (RespawnDelay :type Float%20%28double-precision%29) (inVehicle :type Boolean) (DeathAnimations :type Anim%20Montage%20Object%20Reference))
  (bind _character (Variables|Engine|GetCharacter))
  (bind _charactermovement (Variables|/Script/Engine.Character|GetCharacterMovement _character))
  (bind _movementmode (Variables|/Script/Engine.CharacterMovementComponent|GetMovementMode _charactermovement))
  ;[1 1 1] Death Event
  (Variables|State|SetDead true)
  (Variables|Engine|SetDeath%20Animations DeathAnimations)
  (Components|Tick|SetComponentTickEnabled true)
  (bind _defaultbodymesh (Class|BPIAI|GetDemoSkeletalMeshes(Message) (Variables|Engine|GetCharacter)))
  (Class|BPIABP|SetIsDead(Message) (Components|SkeletalMesh|GetAnimInstance _defaultbodymesh) true)
  (CallFunction|ResetAllStates)
  (Input|DisableInput (Variables|Engine|GetCharacter) (Variables|Engine|GetPlayerController))
  (if inVehicle
    (Rendering|SetActorHiddenInGame (Variables|Engine|GetCharacter) true)
    (if Respawn? :!label _label
      (CallFunction|StartWidgetwithDelay (- RespawnDelay 2.0))
      (Utilities|FlowControl|Delay RespawnDelay)
      (if (Variables|Settings|GetRestartGameAfterDeath)
        (bind _soloplay_ (CallFunction|IsSolo?))
        (if _soloplay_
          (bind _returnvalue (Game|GetCurrentLevelName true))
          (Game|OpenLevel(byName) (Utilities|String|StringToName _returnvalue))
          (else
            (CallFunction|ToggleAttachedActorsVisibility (Components|GetOwner) false :!label _label_2)
            (CallFunction|CharacterRespawn-NR)))
        (else
          (goto _label_2))))
    (else
      (Utilities|FlowControl|Sequence
        (:then_0
          (CallFunction|Release)
          (goto _label))
        (:then_1
          (if (not inVehicle)
            (if (Math|Boolean|ORBoolean (Utilities|Enum|Equal(Enum) _movementmode "MOVE_Flying") (Utilities|Enum|Equal(Enum) _movementmode "MOVE_Falling") (Utilities|Enum|Equal(Enum) _movementmode "MOVE_Swimming"))
              (bind _defaultbodymesh_2 (Class|BPIAI|GetDemoSkeletalMeshes(Message) (Variables|Engine|GetCharacter)))
              (Animation|Montage|PlayMontage _defaultbodymesh_2 (Variables|Engine|GetDeath%20Animations)
                (:then
                  (Utilities|FlowControl|Delay (* (Variables|/Script/Engine.AnimSequenceBase|GetSequenceLength (Variables|Engine|GetDeath%20Animations)) 0.9))
                  (bind _defaultbodymesh_3 (Class|BPIAI|GetDemoSkeletalMeshes(Message) (Variables|Engine|GetCharacter)))
                  (Animation|Montage|MontageStop (Components|SkeletalMesh|GetAnimInstance _defaultbodymesh_3) 0.05 (Variables|Engine|GetDeath%20Animations)))))
            (bind _defaultbodymesh_4 (Class|BPIAI|GetDemoSkeletalMeshes(Message) (Variables|Engine|GetCharacter)))
            (Physics|SetSimulatePhysics _defaultbodymesh_4 true)))))))

(event Custom|CharacterDeath%20-Server
  (params (Respawn? :type Boolean) (RespawnDelay :type Float%20%28double-precision%29) (inVehicle :type Boolean) (DeathAnimations :type Anim%20Montage%20Object%20Reference))
  ;[1 1 1] Death Event
  (CallFunction|CharacterDeath-ALL Respawn? RespawnDelay inVehicle DeathAnimations))