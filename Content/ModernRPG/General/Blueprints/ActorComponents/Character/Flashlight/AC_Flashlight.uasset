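; Actor component that gives a character a networked flashlight, spawned once on BeginPlay through a server event.
; The spawned actor attaches to a socket on the owner's body mesh.
; Toggle, turn-off and visibility requests go through Server events that relay to All events, keeping clients in step.
; The component tracks on/off state and forwards activation and third-person view changes to the flashlight actor as messages.
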(event Custom|SpawnFlashlight%20-Server
  ;[1 1 1] Spawn and attach
  (Utilities|FlowControl|DoOnce false
    (:Completed
      (bind _returnvalue (Game|SpawnActorfromClass (Variables|Default|GetFlashlight) (Math|Transform|MakeTransform "0, 0, 0" "0, 0, 0" "1.000000,1.000000,1.000000") "Undefined" (Components|GetOwner) 0))
      (Variables|Default|SetFlashlightActor _returnvalue)
      (CallFunction|AttachtoSocket-ALL))))

(event Custom|ActivateFlashlight
  ;[1 1 1] Toggle
  (Class|BPIFlashlight|ActivateFlashlight(Message) (Variables|Default|GetFlashlightActor))
  (Variables|Default|SetState true))

(event Custom|ToggleView
  (params (ThirdPerson :type Boolean))
  ;[1 1 1] Toggle View Mode
  (Class|BPIFlashlight|ToggleView(Message) (Variables|Default|GetFlashlightActor) ThirdPerson))

(event Custom|DeactivateFlashlight
  ;[1 1 1] Toggle
  (Class|BPIFlashlight|DeactivateFlashlight(Message) (Variables|Default|GetFlashlightActor))
  (Variables|Default|SetState false))

(event Custom|ToggleFlashlight%20-ALL
  ;[1 1 1] Flashlight
  (if (Variables|Default|GetState)
    (CallFunction|DeactivateFlashlight)
    (else
      (CallFunction|ActivateFlashlight))))

(event Custom|ToggleFlashlight%20-Server
  ;[1 1 1] Flashlight
  (CallFunction|ToggleFlashlight-ALL))

(event Custom|AttachToSocket%20-ALL
  (bind _flashlightactor (Variables|Default|GetFlashlightActor))
  ;[1 1 1] Spawn and attach
  (bind _bodymesh (CallFunction|GetCharacterSkeleton (Components|GetOwner)))
  (Utilities|IsValid _flashlightactor
    (:Is%20Valid
      (Transformation|AttachComponentToComponent _flashlightactor _bodymesh (Variables|Default|GetSocket) "KeepRelative" "KeepRelative" "KeepRelative" true))))

(event Custom|TurnOff%20-%20Server
  ;[1 1 1] Turn off
  (CallFunction|TurnOff-All))

(event Custom|TurnOff%20-%20All
  ;[1 1 1] Turn off
  (CallFunction|DeactivateFlashlight)
  (Variables|Default|SetState false))

(event Custom|VisibilityFlashlight%20-%20Server
  (params (bNewHidden :type Boolean))
  ;[1 1 1] Toggle Flashlight
  (CallFunction|VisibilityFlashlight-All bNewHidden))

(event Custom|VisibilityFlashlight%20-%20All
  (params (bNewHidden :type Boolean))
  ;[1 1 1] Toggle Flashlight
  (Utilities|IsValid (Variables|Default|GetFlashlightActor)
    (:Is%20Valid
      (Rendering|SetActorHiddenInGame (Variables|Default|GetFlashlightActor) bNewHidden))))

(event EventBeginPlay
  ;[1 1 1] Spawn Flashlight
  (CallFunction|SpawnFlashlight-Server))