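; AC_Conditions is a character component that centralizes checks for whether actions such as sprinting, jumping, holstering, aiming-related focus, leaning and view changes are allowed.
; Small state checks for vehicle, building, parachute and aiming combine into the action-level queries.
; Each query looks up sibling components on the owner or reads character movement state on demand, with no event logic.
; An Invert helper also flips input values based on InvertAxis.
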(event EventBeginPlay)

(fn Invert
  (params (InputPin :type Float%20%28double-precision%29))
  (return (* InputPin (select (Variables|Default|GetInvertAxis) -1.0 1.0))))

(fn NotinVehicle
  (return (not (Utilities|IsValid (Variables|/Game/ModernRPG/General/Blueprints/ActorComponents/Machinery/AC_VehicleController.AC_VehicleController_C|GetVehicle (Actor|GetComponentbyClass (Components|GetOwner) "/Game/ModernRPG/General/Blueprints/ActorComponents/Machinery/AC_VehicleController.AC_VehicleController_C"))))))

(fn CanPlayAnimations
  (params (IgnoreFall :type Boolean))
  (bind _returnvalue (Components|GetOwner))
  (bind _ascharacter (Utilities|Casting|CastToCharacter _returnvalue))
  (return (not (Math|Boolean|ORBoolean (select IgnoreFall false (AI|Components|NavMovement|IsFalling (Variables|/Script/Engine.Character|GetCharacterMovement _ascharacter))) (AI|Components|NavMovement|IsSwimming (Variables|/Script/Engine.Character|GetCharacterMovement _ascharacter) :!class /Script/Engine.NavMovementComponent) (Variables|/Game/ModernRPG/General/Blueprints/Ladder/AC_LadderSystem.AC_LadderSystem_C|GetOnLadder (Actor|GetComponentbyClass _returnvalue "/Game/ModernRPG/General/Blueprints/Ladder/AC_LadderSystem.AC_LadderSystem_C")) (Variables|/Game/ModernRPG/General/Blueprints/ClimbSystem/AC_ClimbComponent.AC_ClimbComponent_C|GetHanging (Actor|GetComponentbyClass _returnvalue "/Game/ModernRPG/General/Blueprints/ClimbSystem/AC_ClimbComponent.AC_ClimbComponent_C"))))))

(fn CanHolster
  (return (Math|Boolean|ANDBoolean (CallFunction|NotinBuildingMode) (CallFunction|NotinVehicle) (CallFunction|NotParachute&Skydiving))))

(fn NotinBuildingMode
  (return (not (Variables|/Game/ModernRPG/General/Blueprints/Building/AC_Building.AC_Building_C|GetBuildingMode (Actor|GetComponentbyClass (Components|GetOwner) "/Game/ModernRPG/General/Blueprints/Building/AC_Building.AC_Building_C")))))

(fn NotParachute&Skydiving
  (bind _returnvalue (Components|GetOwner))
  (bind _returnvalue_2 (Actor|GetComponentbyClass _returnvalue "/Game/ModernRPG/General/Blueprints/ActorComponents/Character/Parachute/AC_Parachute.AC_Parachute_C"))
  (Utilities|IsValid _returnvalue
    (:Is%20Valid
      (Utilities|IsValid _returnvalue_2
        (:Is%20Valid
          (return (and (not (Variables|/Game/ModernRPG/General/Blueprints/ActorComponents/Character/Parachute/AC_Parachute.AC_Parachute_C|GetIsSkydiving _returnvalue_2)) (not (Variables|/Game/ModernRPG/General/Blueprints/ActorComponents/Character/Parachute/AC_Parachute.AC_Parachute_C|GetParachuteOpenned _returnvalue_2)))))))))

(fn CanHoldBreath
  (return (and (CallFunction|NotinBuildingMode) (CallFunction|NotinVehicle))))

(fn NotAiming
  (return (not (Variables|/Game/ModernRPG/General/Blueprints/ActorComponents/Weapon/AC_Aiming.AC_Aiming_C|GetAiming (Actor|GetComponentbyClass (Components|GetOwner) "/Game/ModernRPG/General/Blueprints/ActorComponents/Weapon/AC_Aiming.AC_Aiming_C")))))

(fn CanSprint
  (return (Math|Boolean|ANDBoolean (CallFunction|NotParachute&Skydiving) (CallFunction|NotinVehicle) (CallFunction|NotinProcessAiming))))

(fn CanChangeView
  (return (and (CallFunction|NotParachute&Skydiving) (CallFunction|NotAiming))))

(fn NotinProcessAiming
  (return (Variables|/Game/ModernRPG/General/Blueprints/ActorComponents/Weapon/AC_Aiming.AC_Aiming_C|GetAimProcessEnded (Actor|GetComponentbyClass (Components|GetOwner) "/Game/ModernRPG/General/Blueprints/ActorComponents/Weapon/AC_Aiming.AC_Aiming_C"))))

(fn CanSelect
  (bind _ascharacter (Utilities|Casting|CastToCharacter (Components|GetOwner)))
  (return (Math|Boolean|ANDBoolean (Utilities|Enum|NotEqual(Enum) (Variables|/Script/Engine.CharacterMovementComponent|GetMovementMode (Variables|/Script/Engine.Character|GetCharacterMovement _ascharacter)) "MOVE_Swimming") (Utilities|Enum|NotEqual(Enum) (Variables|/Script/Engine.CharacterMovementComponent|GetMovementMode (Variables|/Script/Engine.Character|GetCharacterMovement _ascharacter)) "MOVE_Flying") (Utilities|Enum|NotEqual(Enum) (Variables|/Script/Engine.CharacterMovementComponent|GetMovementMode (Variables|/Script/Engine.Character|GetCharacterMovement _ascharacter)) "MOVE_Falling"))))

(fn CanJump
  (bind _returnvalue (Components|GetOwner))
  (bind _isaiming (Class|BPIVehicles|IsAiming(Message) (Components|GetOwner)))
  (if _isaiming
    (return false)
    (elif (not (Variables|/Game/ModernRPG/General/Blueprints/Ladder/AC_LadderSystem.AC_LadderSystem_C|GetOnLadder (Actor|GetComponentbyClass _returnvalue "/Game/ModernRPG/General/Blueprints/Ladder/AC_LadderSystem.AC_LadderSystem_C")))
      (if (AI|Components|NavMovement|IsSwimming (Actor|GetComponentbyClass _returnvalue "/Script/Engine.CharacterMovementComponent") :!class /Script/Engine.NavMovementComponent)
        (return false)
        (elif (Variables|AC_Conditions_C|GetDisableInput (Actor|GetComponentbyClass _returnvalue "AC_Conditions_C"))
          (return false)
          (else
            (return true))))
      (else
        (return false)))))

(fn CanFocus
  (return (Math|Boolean|ANDBoolean (CallFunction|NotinVehicle) (Default|InWeaponMode (Actor|GetComponentbyClass (Components|GetOwner) "/Game/ModernRPG/General/Blueprints/Combat/AC_CombatEvents.AC_CombatEvents_C")) (Utilities|Enum|Equal(Enum) (Variables|/Game/ModernRPG/General/Blueprints/Ladder/AC_LadderSystem.AC_LadderSystem_C|GetCurrentState (Actor|GetComponentbyClass (Components|GetOwner) "/Game/ModernRPG/General/Blueprints/Ladder/AC_LadderSystem.AC_LadderSystem_C")) "NewEnumerator0"))))

(fn CanLean
  (bind _returnvalue (Components|GetOwner))
  (bind _ascharacter (Utilities|Casting|CastToCharacter _returnvalue))
  (bind _returnvalue_2 (Pawn|GetMovementComponent _ascharacter))
  (return (not (Math|Boolean|ORBoolean (AI|Components|NavMovement|IsFalling _returnvalue_2) (Class|NavMovementComponent|IsFlying _returnvalue_2) (AI|Components|NavMovement|IsSwimming _returnvalue_2 :!class /Script/Engine.NavMovementComponent)))))

(fn CanChangeSpringArmLocation
  (return (Variables|/Game/ModernRPG/General/Blueprints/ActorComponents/ViewSwitch/AC_ViewSwitch.AC_ViewSwitch_C|GetInThirdPerson (Actor|GetComponentbyClass (Components|GetOwner) "/Game/ModernRPG/General/Blueprints/ActorComponents/ViewSwitch/AC_ViewSwitch.AC_ViewSwitch_C"))))

(fn CanJumpCombat
  (bind _returnvalue (Components|GetOwner))
  (return (and (Utilities|Enum|Equal(Enum) (Variables|/Game/ModernRPG/General/Blueprints/ActorComponents/Character/State/AC_PlayerCurrentState.AC_PlayerCurrentState_C|GetCurrentState (Actor|GetComponentbyClass _returnvalue "/Game/ModernRPG/General/Blueprints/ActorComponents/Character/State/AC_PlayerCurrentState.AC_PlayerCurrentState_C")) "NewEnumerator4") (Variables|/Game/ModernRPG/General/Blueprints/Combat/AC_CombatEvents.AC_CombatEvents_C|GetCanAttack (Actor|GetComponentbyClass _returnvalue "/Game/ModernRPG/General/Blueprints/Combat/AC_CombatEvents.AC_CombatEvents_C")))))