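; AC_VehicleDeath is a vehicle actor component that records the vehicle's destruction in the kill log and statistics.
; VehicleDestroyed runs WriteKillLog once, sending both sides' names and teams plus a damage-type icon to GM_Gameplay, with special handling for crashes.
; It then adds a death to the owner's AC_PlayerStatistics and a kill and score to a valid killer's.
; A server event awards the killer's team a point through the game mode.
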(event Custom|TeamPoints%20-Server
  (params (Target :type Object%20Object%20Reference))
  ;[1 1 1] Replicate Team Poitns
  (bind _team (Class|BPIAI|GetTeam(Message) Target))
  (Class|BPIGameMode|AddTeamPoints(Message) (Game|GetGameMode) _team 1))

(event Custom|WriteKillLog
  (params (Killer :type Actor%20Object%20Reference) (Crached :type Boolean) (DamageType :type E_DamageType%20Enum :default "NewEnumerator0"))
  ;[1 1 1] Update Kill Log
  (Variables|Default|SetKiller Killer)
  (Variables|Default|SetCrached Crached)
  (Variables|Default|SetDamageType DamageType)
  (Utilities|FlowControl|DoOnce false
    (:Completed
      (Utilities|FlowControl|Sequence
        (:then_0
          (if (not (Variables|Default|GetCrached))
            (bind _owner (Class|BPIVehicles|GetParentOwner(Message) (Variables|Default|GetKiller)))
            (bind _team (Class|BPIAI|GetTeam(Message) _owner))
            (Variables|Default|SetKillerTeam _team)
            (bind _name (Class|BPICharacter|GetName(Message) _owner))
            (Variables|Default|SetKillerName _name))
          (bind _team_2 (Class|BPIAI|GetTeam(Message) (Components|GetOwner)))
          (Variables|Default|SetOwnerTeam _team_2)
          (bind _name_2 (Class|BPICharacter|GetName(Message) (Components|GetOwner)))
          (Variables|Default|SetOwnerName _name_2)
          (if (== (Variables|Default|GetDamageType) (Utilities|Enum|LiteralenumE_DamageType "NewEnumerator9"))
            (bind _asgm_gameplay (Utilities|Casting|CastToGM_Gameplay (Game|GetGameMode)))
            (bind _returnvalue (CallFunction|ChangeIcon))
            (Class|BPIGameMode|UpdateKillLog(Message) _asgm_gameplay "NewEnumerator2" (Variables|Default|GetOwnerTeam) "Crashed " (Variables|Default|GetOwnerName) _returnvalue)
            (else
              (bind _asgm_gameplay_2 (Utilities|Casting|CastToGM_Gameplay (Game|GetGameMode)))
              (bind _returnvalue_2 (CallFunction|ChangeIcon))
              (Class|BPIGameMode|UpdateKillLog(Message) _asgm_gameplay_2 (select (Variables|Default|GetCrached) "NewEnumerator2" (Variables|Default|GetKillerTeam)) (Variables|Default|GetOwnerTeam) (select (Variables|Default|GetCrached) "" (Variables|Default|GetKillerName)) (Variables|Default|GetOwnerName) _returnvalue_2))))
        (:then_1
          (CallFunction|WriteDeathStatistics))))))

(event Custom|VehicleDestroyed
  (params (Killer :type Actor%20Object%20Reference) (NotSave? :type Boolean) (Crached :type Boolean) (DamageType :type E_DamageType%20Enum :default "NewEnumerator0"))
  ;[1 1 1] Update Kill Log
  ;;[1 1 1] Tank Destruction
  (CallFunction|WriteKillLog Killer Crached DamageType))

(event Custom|WriteDeathStatistics
  (bind _killer (Variables|Default|GetKiller))
  (bind _returnvalue (Actor|GetComponentbyClass _killer "/Game/ModernRPG/General/Blueprints/ActorComponents/Character/Statistics/AC_PlayerStatistics.AC_PlayerStatistics_C"))
  ;[1 1 1] Kill Statistics
  (Default|AddStatistics (Actor|GetComponentbyClass (Components|GetOwner) "/Game/ModernRPG/General/Blueprints/ActorComponents/Character/Statistics/AC_PlayerStatistics.AC_PlayerStatistics_C") (Variables|Settings|GetDeathStatistics) 1.0)
  (Utilities|IsValid (Variables|Default|GetKiller)
    (:Is%20Valid
      (Utilities|IsValid _returnvalue
        (:Is%20Valid
          (Default|AddStatistics _returnvalue (Variables|Settings|GetKillStatistics) 1.0)
          (Default|AddStatistics _returnvalue (Variables|Settings|GetScoreStatistics) 1e+01)
          (CallFunction|TeamPoints-Server (Variables|Default|GetKiller)))))))

(fn ChangeIcon
  (switch Utilities|FlowControl|Switch|SwitchonE_DamageType (Variables|Default|GetDamageType)
    (:NewEnumerator2
      (return "/Game/ModernRPG/General/GUI/Textures/Tasks/T_Grenade.T_Grenade"))
    (:NewEnumerator3
      (return "/Game/ModernRPG/General/GUI/Textures/WeaponIcons/T_Machinegun.T_Machinegun"))
    (:NewEnumerator4
      (return "/Game/ModernRPG/General/GUI/Textures/WeaponIcons/T_Rocket.T_Rocket"))
    (:NewEnumerator5
      (return "/Game/ModernRPG/General/GUI/Textures/WeaponIcons/T_Shell.T_Shell"))
    (:NewEnumerator7
      (return "/Game/ModernRPG/General/GUI/Textures/WeaponIcons/T_Rocket.T_Rocket"))
    (:NewEnumerator9
      (return "/Game/ModernRPG/General/GUI/Textures/WeaponIcons/T_Shell.T_Shell"))))