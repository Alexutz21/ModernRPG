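; Vehicle health component that tracks and replicates a vehicle's Health.
; A server event subtracts damage, clamps the result between zero and MaxHealth, then passes it to an ALL event that sets Health for everyone.
; The many vehicle, weapon and seat query functions are empty stubs returning defaults, and nothing here handles destruction at zero health.
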(event Custom|SetHealth%20-%20ALL
  (params (Health :type Float%20%28double-precision%29))
  ;[1 1 1] Replicate Veh Health
  (Variables|Stats|SetHealth Health))

(event Custom|HealthDecrease%20-%20Server
  (params (Value :type Float%20%28double-precision%29))
  ;[1 1 1] Replicate Veh Health
  (CallFunction|SetHealth-ALL (Math|Float|Clamp(Float) (- (Variables|Stats|GetHealth) Value) 0.0 (Variables|Default|GetmaxHealth))))

(fn CanHit
  (return false))

(fn CanShot?
  (return false))

(fn GetCannonSettings
  (return ""))

(fn GetCannonSound
  (return 0))

(fn GetCountOfCannonShells
  (return 0))

(fn GetCountOfMinigunSHells
  (return 0))

(fn GetDriver
  (return 0))

(fn GetDriverPlace
  (return 0))

(fn GetForward/SideSpeed
  (return 0.0 0.0 0.0))

(fn GetHeight
  (return 0.0))

(fn GetHitDecalClass
  (return 0))

(fn GetMinigunSettings
  (return ""))

(fn GetMinimapArrow
  (return 0))

(fn GetParentOwner
  (return 0))

(fn GetPassengers
  (return 0))

(fn GetReloadTime
  (return 0.0))

(fn GetSmokeSettings
  (return ""))

(fn GetWBTank
  (return 0))

(fn HitCharacterVelocity
  (return 0.0 0))

(fn IsAiming
  (return false))

(fn IsBOMBLOAD
  (return false))

(fn IsComponentAllright
  (return false))

(fn IsDrone
  (return false))

(fn IsItTrack
  (return false))

(fn IsShell
  (return false))

(fn IsSiucideMode
  (return false))

(fn IsTankValid
  (return false))

(fn IsVehicleActive
  (return false))