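; Actor component that records its owner's death in a Modern RPG match, updating the kill log, death statistics and team points.
; WriteKillLog runs once via DoOnce, sending killer and victim names, teams and an icon to GM_Gameplay.
; It then increments death statistics on the owner's AC_PlayerStatistics and calls a server event that adds a point to the owner's (victim's) team, leaving the passed killer uncredited.
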(event Custom|TeamPoints%20-Server
  ;[1 1 1] Replicate Team Poitns
  (bind _team (Class|BPIAI|GetTeam(Message) (Components|GetOwner)))
  (Class|BPIGameMode|AddTeamPoints(Message) (Game|GetGameMode) _team 1))

(event Custom|WriteKillLog
  (params (Actor :type Actor%20Object%20Reference) (Icon :type Texture%202D%20Object%20Reference))
  ;[1 1 1] Update Kill Log
  (Utilities|IsValid Actor
    (:Is%20Valid
      (Utilities|FlowControl|DoOnce false
        (:Completed
          (Utilities|FlowControl|Sequence
            (:then_0
              (bind _team (Class|BPIAI|GetTeam(Message) Actor))
              (bind _name (Class|BPICharacter|GetName(Message) Actor))
              (bind _team_2 (Class|BPIAI|GetTeam(Message) (Components|GetOwner)))
              (bind _name_2 (Class|BPICharacter|GetName(Message) (Components|GetOwner)))
              (bind _asgm_gameplay (Utilities|Casting|CastToGM_Gameplay (Game|GetGameMode)))
              (Class|BPIGameMode|UpdateKillLog(Message) _asgm_gameplay _team _team_2 _name _name_2 Icon))
            (:then_1
              (CallFunction|WriteDeathStatistics Actor))))))))

(event Custom|WriteDeathStatistics
  (params (Target :type Actor%20Object%20Reference))
  ;[1 1 1] Kill Statistics
  (Default|AddStatistics (Actor|GetComponentbyClass (Components|GetOwner) "/Game/ModernRPG/General/Blueprints/ActorComponents/Character/Statistics/AC_PlayerStatistics.AC_PlayerStatistics_C") (Variables|Default|GetDeathStatistics) 1.0)
  (CallFunction|TeamPoints-Server))