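; Machinery camera component that handles zoom for its owner's body and aiming views.
; On BeginPlay it gets cameras, the main spring arm and aim references from the owner through interface messages.
; ZoomIn and ZoomOut step the passed camera's FOV between 1x and 8x when aiming, otherwise the clamped spring arm length.
; Tick is enabled on zoom to interpolate toward the target, switching off once the FOV is nearly reached.
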(event Custom|Zoom%20Out
  (bind _springarmbody (Variables|Default|GetSpringArmBody))
  (bind _targetarmlength (Variables|/Script/Engine.SpringArmComponent|GetTargetArmLength _springarmbody))
  ;[1 1 1] Changing camera's mode and camera number
  ;;[1 1 1] Zoom
  (Utilities|IsValid _springarmbody
    (:Is%20Valid
      (Variables|Camera|SetCurrentSpringArm _targetarmlength)
      (Variables|Camera|SetTargetSpringArm (Math|Float|Clamp(Float) (+ _targetarmlength 2e+02) (Variables|Camera|GetMinBodySpringArm) (Variables|Camera|GetMaxBodySpringArm)))
      (Components|Tick|SetComponentTickEnabled true)
      (Variables|Default|SetNeedToInterp true))))

(event Custom|Zoom%20In
  (bind _springarmbody (Variables|Default|GetSpringArmBody))
  (bind _targetarmlength (Variables|/Script/Engine.SpringArmComponent|GetTargetArmLength _springarmbody))
  ;[1 1 1] Changing camera's mode and camera number
  ;;[1 1 1] Zoom
  (Utilities|IsValid _springarmbody
    (:Is%20Valid
      (Variables|Camera|SetCurrentSpringArm _targetarmlength)
      (Variables|Camera|SetTargetSpringArm (Math|Float|Clamp(Float) (- _targetarmlength 2e+02) (Variables|Camera|GetMinBodySpringArm) (Variables|Camera|GetMaxBodySpringArm)))
      (Components|Tick|SetComponentTickEnabled true)
      (Variables|Default|SetNeedToInterp true))))

(event EventBeginPlay
  ;[1 1 1] IniIalize Component
  (CallFunction|Initialize))

(event EventTick
  (params (DeltaSeconds :type Float%20%28single-precision%29))
  ;[1 1 1] Changing camera's mode and camera number
  (if (Variables|Default|GetNeedToInterp)
    (Utilities|IsValid (Variables|Default|GetCamera)
      (:Is%20Valid
        (if (Math|Float|NearlyEqual(Float) (Variables|/Script/Engine.CameraComponent|GetFieldOfView (Variables|Default|GetCamera)) (Variables|Default|GetTargetFOV) 0.5)
          (Variables|Default|SetCamera 0)
          (Variables|Default|SetNeedToInterp false)
          (Components|Tick|SetComponentTickEnabled false)
          (else
            (Camera|SetFieldOfView (Variables|Default|GetCamera) (Math|Interpolation|FInterpTo (Variables|/Script/Engine.CameraComponent|GetFieldOfView (Variables|Default|GetCamera)) (Variables|Default|GetTargetFOV) (Utilities|Time|GetWorldDeltaSeconds) 1e+01)))))
      (:Is%20Not%20Valid
        (Variables|/Script/Engine.SpringArmComponent|SetTargetArmLength (Variables|Default|GetSpringArmBody) (Math|Interpolation|FInterpTo (Variables|/Script/Engine.SpringArmComponent|GetTargetArmLength (Variables|Default|GetSpringArmBody)) (Variables|Camera|GetTargetSpringArm) (Utilities|Time|GetWorldDeltaSeconds) 5.0))
        (if (== (Variables|Camera|GetTargetSpringArm) (Variables|Camera|GetCurrentSpringArm))
          (Variables|Default|SetNeedToInterp false)
          (Components|Tick|SetComponentTickEnabled false))))))

(fn GetController
  (return (Pawn|GetController (.AsPawn (Utilities|Casting|CastToPawn (Components|GetOwner))))))

(fn Zoomin
  (params (bIsAiming :type Boolean) (Camera :type Camera%20Component%20Object%20Reference))
  (Components|Tick|SetComponentTickEnabled true)
  (if bIsAiming
    (Variables|Default|SetCamera Camera)
    (switch Utilities|FlowControl|Switch|SwitchonE_ZoomTank (Variables|Camera|GetE_Zoom)
      (:NewEnumerator0
        (Variables|Default|SetcurrentFOV (Variables|/Script/Engine.CameraComponent|GetFieldOfView Camera))
        (Variables|Default|SetTargetFOV 45.0)
        (Variables|Camera|SetE_Zoom "NewEnumerator1")
        (Variables|Default|SetNeedToInterp true))
      (:NewEnumerator1
        (Variables|Default|SetcurrentFOV (Variables|/Script/Engine.CameraComponent|GetFieldOfView Camera))
        (Variables|Default|SetTargetFOV 22.5)
        (Variables|Camera|SetE_Zoom "NewEnumerator2")
        (Variables|Default|SetNeedToInterp true))
      (:NewEnumerator2
        (Variables|Default|SetcurrentFOV (Variables|/Script/Engine.CameraComponent|GetFieldOfView Camera))
        (Variables|Default|SetTargetFOV 11.0)
        (Variables|Camera|SetE_Zoom "NewEnumerator3")
        (Variables|Default|SetNeedToInterp true)))
    (else
      (CallFunction|Zoomin))))

(fn ZoomOut
  (params (bIsAiming :type Boolean) (Camera :type Camera%20Component%20Object%20Reference))
  (Components|Tick|SetComponentTickEnabled true)
  (if bIsAiming
    (Variables|Default|SetCamera Camera)
    (switch Utilities|FlowControl|Switch|SwitchonE_ZoomTank (Variables|Camera|GetE_Zoom)
      (:NewEnumerator1
        (Variables|Default|SetcurrentFOV (Variables|/Script/Engine.CameraComponent|GetFieldOfView Camera))
        (Variables|Default|SetTargetFOV 9e+01)
        (Variables|Camera|SetE_Zoom "NewEnumerator0")
        (Variables|Default|SetNeedToInterp true))
      (:NewEnumerator2
        (Variables|Default|SetcurrentFOV (Variables|/Script/Engine.CameraComponent|GetFieldOfView Camera))
        (Variables|Default|SetTargetFOV 45.0)
        (Variables|Camera|SetE_Zoom "NewEnumerator1")
        (Variables|Default|SetNeedToInterp true))
      (:NewEnumerator3
        (Variables|Default|SetcurrentFOV (Variables|/Script/Engine.CameraComponent|GetFieldOfView Camera))
        (Variables|Default|SetTargetFOV 22.5)
        (Variables|Camera|SetE_Zoom "NewEnumerator2")
        (Variables|Default|SetNeedToInterp true)))
    (else
      (CallFunction|ZoomOut))))

(fn Initialize
  (bind _returnvalue (Components|GetOwner))
  (bind _camera (Class|BPIAI|GetBodyCamera(Message) _returnvalue))
  (Variables|Default|SetCameraBody _camera)
  (bind _camera_2 (Class|BPIAI|GetCameraAimInside(Message) _returnvalue))
  (Variables|Default|SetCameraAimInside _camera_2)
  (bind _camera_3 (Class|BPIAI|GetCameraMinigun(Message) _returnvalue))
  (Variables|Default|SetCameraMinigun _camera_3)
  (bind _camera_4 (Class|BPIAI|GetCameraTurret(Message) _returnvalue))
  (Variables|Default|SetCameraTurret _camera_4)
  (bind _springarmbody (Class|BPIAI|GetMainSpringArm(Message) _returnvalue))
  (Variables|Default|SetSpringArmBody _springarmbody)
  (bind _defaultaim (Class|BPIAI|GetDefaultAim(Message) _returnvalue))
  (Variables|Default|SetDefaultAim _defaultaim)
  (bind _minigunaim (Class|BPIAI|GetMinigunAim(Message) _returnvalue))
  (Variables|Default|SetMinigunAim _minigunaim)
  (bind _predictaim (Class|BPIAI|GetPredictAim(Message) _returnvalue))
  (Variables|Default|SetPredictAim _predictaim))