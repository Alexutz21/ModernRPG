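; Vehicle actor component that picks a clear spot for exiting the vehicle.
; On BeginPlay it orders the owner's "PlaceForExit" billboard components by the index in their second tag.
; Each spot is line-traced vertically for a surface, then from the vehicle, ignoring the driver, to check for obstructions.
; FindCorrectPlaceToExit returns the first passing spot in index order, falling back to the one tagged "1".
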(event EventBeginPlay
  (bind _returnvalue (Components|GetOwner))
  (bind _returnvalue_2 (Actor|GetComponentsbyTag _returnvalue "/Script/Engine.BillboardComponent" "PlaceForExit"))
  ;[1 1 1] Initialize Component
  (Utilities|Array|Clear (Variables|Default|GetPlacesForExit))
  (for _index (range 0 (- (Utilities|Array|Length _returnvalue_2) 1))
    (Utilities|Array|Add (Variables|Default|GetPlacesForExit) 0))
  (for _array_element _returnvalue_2
    (Utilities|Array|SetArrayElem (Variables|Default|GetPlacesForExit) (Math|Conversions|ToInteger(Byte) (Utilities|String|ToString(Name) (Utilities|Array|Get(acopy) (Variables|/Script/Engine.ActorComponent|GetComponentTags _array_element) 1))) _array_element)))

(fn FindCorrectPlacetoExit
  (LocalVariables|SetBillboard 0)
  (Utilities|Array|Clear (LocalVariables|GetStates))
  (if (Utilities|Array|IsValidIndex (Variables|Default|GetPlacesForExit))
    (bind _array_element (Utilities|Array|ForEachLoopwithBreak (Variables|Default|GetPlacesForExit))
      (:LoopBody
        (Utilities|IsValid (CallFunction|Trace _array_element)
          (:Is%20Valid
            (Utilities|Array|Add (LocalVariables|GetStates) true))
          (:Is%20Not%20Valid
            (Utilities|Array|Add (LocalVariables|GetStates) false))))
      (:Completed
        (bind (_array_element_2 _array_index) (Utilities|Array|ForEachLoopwithBreak (LocalVariables|GetStates) :!label _label)
          (:LoopBody
            (if _array_element_2
              (LocalVariables|SetBillboard (Utilities|Array|Get(acopy) (Variables|Default|GetPlacesForExit) _array_index))
              (goto _label Break)))
          (:Completed
            (Utilities|IsValid (LocalVariables|GetBillboard)
              (:Is%20Valid
                (return (LocalVariables|GetBillboard)))
              (:Is%20Not%20Valid
                (for _array_element_3 (Variables|Default|GetPlacesForExit)
                  (if (Utilities|Name|Equal(Name) (Utilities|Array|Get(acopy) (Variables|/Script/Engine.ActorComponent|GetComponentTags _array_element_3) 1) "1")
                    (LocalVariables|SetBillboard _array_element_3)))
                (return (LocalVariables|GetBillboard))))))))))

(fn Trace
  (params ([0] :type Billboard%20Component%20Object%20Reference))
  (bind _returnvalue (Transformation|GetWorldLocation [0]))
  (bind (_x _y _z) (Math|Vector|BreakVector _returnvalue))
  (bind (_outhit _returnvalue_2) (Collision|LineTraceByChannel (Math|Vector|MakeVector _x _y (+ _z 1.5e+02)) (Math|Vector|MakeVector _x _y (- _z 5e+02)) "TraceTypeQuery1" false (Utilities|Array|MakeArray (Components|GetOwner)) "None" true "(R=1.000000,G=0.000000,B=0.000000,A=1.000000)" "(R=0.000000,G=1.000000,B=0.000000,A=1.000000)" 312.0))
  (if _returnvalue_2
    (if (and (!= (Utilities|GetClass (.HitActor (Collision|BreakHitResult _outhit))) "/Script/Engine.Pawn") (!= (Utilities|GetClass (.HitActor (Collision|BreakHitResult _outhit))) "/Script/Engine.Actor"))
      (bind _driver (Class|BPIVehicles|GetDriver(Message) (Components|GetOwner)))
      (bind _outhit_2 (Collision|LineTraceByChannel (Transformation|GetActorLocation (Components|GetOwner)) (Transformation|GetWorldLocation [0]) "TraceTypeQuery1" false (Utilities|Array|MakeArray _driver) "None" true "(R=1.000000,G=0.925721,B=0.000000,A=1.000000)" "(R=0.000000,G=1.000000,B=0.000000,A=1.000000)" 5132.0))
      (if (== (Math|Vector|Distance(Vector) (Transformation|GetWorldLocation [0]) (.TraceStart (Collision|BreakHitResult _outhit_2))) (Math|Vector|Distance(Vector) (.TraceStart (Collision|BreakHitResult _outhit_2)) (select (Math|Vector|Equal(Vector) (.Location (Collision|BreakHitResult _outhit_2)) "0, 0, 0" 0.0001) (.TraceEnd (Collision|BreakHitResult _outhit_2)) (.Location (Collision|BreakHitResult _outhit_2)))))
        (return [0]))
      (else
        (return 0)))
    (else
      (return 0))))