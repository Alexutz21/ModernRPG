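; AC_VehicleController is an actor component that tracks the vehicle its owner occupies, along with passenger index and an in-transition flag.
; SetVehicle and RemoveVehicle store or clear the vehicle reference and fire OnVehicleEnter and OnVehicleLeave notifications.
; Events named for all-client or from-server calls handle vehicle removal, seat index and transition updates, while InTransition exposes the flag.
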(event Custom|SetPasIndex%20-%20All
  (params (PassengerIndex :type Integer))
  (Variables|Default|SetPassengerIndex PassengerIndex))

(event Custom|SetInTransition%20%28FromServer%29
  (params (inTransition :type Boolean))
  (Variables|Default|SetinTransition inTransition))

(event Custom|RemoveVehicle%20-%20ALL
  (CallFunction|RemoveVehicle))

(fn SetVehicle
  (params (Vehicle :type Actor%20Object%20Reference))
  (bind _output_get (Variables|Default|SetVehicle Vehicle))
  (Default|CallOnVehicleEnter _output_get))

(fn RemoveVehicle
  (Variables|Default|SetVehicle 0)
  (Default|CallOnVehicleLeave))

(fn InTransition?
  (return (Variables|Default|GetinTransition)))