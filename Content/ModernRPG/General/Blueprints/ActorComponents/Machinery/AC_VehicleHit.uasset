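; Actor component that resolves weapon hits on a vehicle: damage, destruction, ammunition explosions and non-penetrations.
; NewHit and AmmunitionExplosion resolve the killer by damage type and filter duplicates, generally counting each shell once via the Shells array.
; Valid hits reduce AC_VehicleHealth and may destroy the vehicle; surviving hits and non-penetrations report to the attacker's vehicle.
; CanShootTarget returns only alive and player-controlled status; its team comparison is disconnected.
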(event Custom|PlaySound%20-%20OC
  (params (Sound :type Sound%20Base%20Object%20Reference) (Location :type Vector))
  ;[1 1 1] Play sound of the Hit
  (Audio|PlaySoundatLocation Sound Location "0, 0, 0" 1.0 1.0 0.0 "/Game/ModernRPG/General/Sounds/Attenuations/SA_ImpactShotEffect.SA_ImpactShotEffect" 0 0 0))

(fn OneShell=OneHit
  (params (ItemToFind :type Actor%20Object%20Reference%20%28by%20ref%29))
  (if (Utilities|Array|ContainsItem (Variables|Shells|GetShells) ItemToFind)
    (return false)
    (else
      (Utilities|Array|AddUnique (Variables|Shells|GetShells) ItemToFind)
      (return true))))

(fn CanShootTarget
  (params (Owner :type Object%20Object%20Reference))
  ;[1 1 1] Check if a target is not from my team and is it a character pawn
  (Utilities|IsValid Owner
    (:Is%20Valid
      (LocalVariables|SetCacheLocal Owner)
      (Utilities|IsValid (.AsPawn (Utilities|Casting|CastToPawn (LocalVariables|GetCacheLocal)))
        (:Is%20Valid
          (if (Pawn|IsPlayerControlled (.AsPawn (Utilities|Casting|CastToPawn (LocalVariables|GetCacheLocal))))
            (bind _result (Class|BPICharacter|IsAlive?(Message) (LocalVariables|GetCacheLocal)))
            (bind _owner (Class|BPIVehicles|GetParentOwner(Message) (Components|GetOwner)))
            (bind _team (Class|BPIAI|GetTeam(Message) _owner))
            (bind _team_2 (Class|BPIAI|GetTeam(Message) (LocalVariables|GetCacheLocal)))
            (return _result true)
            (else
              (bind _result_2 (Class|BPICharacter|IsAlive?(Message) (LocalVariables|GetCacheLocal)))
              (bind _owner_2 (Class|BPIVehicles|GetParentOwner(Message) (Components|GetOwner)))
              (bind _team_3 (Class|BPIAI|GetTeam(Message) _owner_2))
              (bind _team_4 (Class|BPIAI|GetTeam(Message) (LocalVariables|GetCacheLocal)))
              (return _result_2 false))))))))

(fn Initialize
  (bind _returnvalue (Components|GetOwner))
  (bind _staticmesh (Class|BPIAI|GetTurret(Message) _returnvalue))
  (Variables|Default|SetTank_Turret _staticmesh)
  (bind _audioammunitionexplosion (Class|BPIAI|GetAudioAmmunitionExplosion(Message) _returnvalue))
  (Variables|Default|SetAudioAmmunitionExplosion _audioammunitionexplosion)
  (bind _placeforammunitionexplosionparticle (Class|BPIAI|GetPlaceforAmmunitionExplosionParticle(Message) _returnvalue))
  (Variables|Default|SetPlaceForAmmunitionExplosionParticle _placeforammunitionexplosionparticle)
  (bind _s_tanksettings (Class|BPIAI|GetTankSettings(Message) _returnvalue))
  (Variables|Settings|SetS_TankSettings _s_tanksettings)
  (bind _isdestroyed (Class|BPIAI|IsDestroyed(Message) _returnvalue))
  (Variables|Alive|SetbDestroyed _isdestroyed))

(fn DestroyVehicleTrace
  (params (DamageType :type E_DamageType%20Enum :default "NewEnumerator0") (Killer :type Actor%20Object%20Reference) (KillDriver :type Boolean))
  (bind _returnvalue (Components|GetOwner))
  (bind _returnvalue_2 (Actor|GetComponentbyClass _returnvalue "/Game/ModernRPG/General/Blueprints/ActorComponents/Machinery/AC_VehicleHealth.AC_VehicleHealth_C"))
  (Utilities|IsValid _returnvalue
    (:Is%20Valid
      (Utilities|IsValid _returnvalue_2
        (:Is%20Valid
          (Default|HealthDecrease-Server _returnvalue_2 (Variables|/Game/ModernRPG/General/Blueprints/ActorComponents/Machinery/AC_VehicleHealth.AC_VehicleHealth_C|GetMaxHealth _returnvalue_2))
          (Class|BPIAI|DestroyVehicle(Message) (Components|GetOwner) Killer DamageType KillDriver false))))))

(fn NewHit
  (params (Damage :type Float%20%28double-precision%29) (DamageType :type E_DamageType%20Enum :default "NewEnumerator0") (Killer/Shell :type Actor%20Object%20Reference))
  (bind _return (CallFunction|GetKiller Killer/Shell DamageType))
  (bind _returnvalue (Actor|GetComponentbyClass _return "/Game/ModernRPG/General/Blueprints/ActorComponents/Machinery/AC_VehicleController.AC_VehicleController_C"))
  (bind _vehicle (Variables|/Game/ModernRPG/General/Blueprints/ActorComponents/Machinery/AC_VehicleController.AC_VehicleController_C|GetVehicle _returnvalue))
  (bind _continue (CallFunction|CheckDuplicatingHit Killer/Shell (CallFunction|GetKiller Killer/Shell DamageType) DamageType))
  (if _continue
    (Default|HealthDecrease-Server (Actor|GetComponentbyClass (Components|GetOwner) "/Game/ModernRPG/General/Blueprints/ActorComponents/Machinery/AC_VehicleHealth.AC_VehicleHealth_C") Damage)
    (if (== (Variables|/Game/ModernRPG/General/Blueprints/ActorComponents/Machinery/AC_VehicleHealth.AC_VehicleHealth_C|GetHealth (Actor|GetComponentbyClass (Components|GetOwner) "/Game/ModernRPG/General/Blueprints/ActorComponents/Machinery/AC_VehicleHealth.AC_VehicleHealth_C")) 0.0)
      (CallFunction|DestroyVehicleTrace DamageType (CallFunction|GetKiller Killer/Shell DamageType) true)
      (else
        (Class|BPIWidgets|ShowHealthWidget(Message) (Components|GetOwner))
        (Utilities|IsValid _return
          (:Is%20Valid
            (Utilities|IsValid _returnvalue
              (:Is%20Valid
                (Utilities|IsValid _vehicle
                  (:Is%20Valid
                    (Class|BPIVehicles|ReportAboutHit(Message) _vehicle Damage)))))))))))

(fn CheckDuplicatingHit
  (params (Killer/Shell :type Actor%20Object%20Reference) (Killer :type Actor%20Object%20Reference) (DT :type E_DamageType%20Enum :default "NewEnumerator0"))
  (bind _isai_ (Class|BPIPlayerInfo|IsAI?(Message) Killer))
  (if _isai_
    (bind _e_pawntype (Class|BPIAI|GetPawnType(Message) Killer))
    (switch Utilities|FlowControl|Switch|SwitchonE_PawnType _e_pawntype
      (:NewEnumerator0
        _)
      (:NewEnumerator1
        (bind _returnvalue (Class|BPIVehicles|IsShell(Message) Killer/Shell :!label _label))
        (if _returnvalue
          (return (Pure|OneShell=OneHit Killer/Shell))
          (else
            (return true))))
      (:NewEnumerator2
        (switch Utilities|FlowControl|Switch|SwitchonE_DamageType DT
          (:NewEnumerator3
            (return true))
          (:NewEnumerator4
            (return (Pure|OneShell=OneHit Killer/Shell)))))
      (:NewEnumerator4
        (goto _label))
      (:NewEnumerator5
        (return (Pure|OneShell=OneHit Killer/Shell)))
      (:NewEnumerator6
        _))
    (return true)
    (else
      (bind _e_pawntype_2 (Class|BPIAI|GetPawnType(Message) Killer))
      (switch Utilities|FlowControl|Switch|SwitchonE_PawnType _e_pawntype_2
        (:NewEnumerator0
          _)
        (:NewEnumerator1
          (bind _returnvalue_2 (Class|BPIVehicles|IsShell(Message) Killer/Shell :!label _label_2))
          (if _returnvalue_2
            (return (Pure|OneShell=OneHit Killer/Shell))
            (else
              _)))
        (:NewEnumerator2
          (goto _label_2))
        (:NewEnumerator4
          (goto _label_2))
        (:NewEnumerator5
          (goto _label_2))
        (:NewEnumerator6
          _))
      (return true))))

(fn GetKiller
  (params (Target :type Actor%20Object%20Reference) (Selection :type E_DamageType%20Enum :default "NewEnumerator0"))
  (Utilities|IsValid Target
    (:Is%20Valid
      (switch Utilities|FlowControl|Switch|SwitchonE_DamageType Selection
        (:NewEnumerator0
          _)
        (:NewEnumerator1
          (bind _owner (Class|BPIVehicles|GetParentOwner(Message) Target :!label _label))
          (return _owner))
        (:NewEnumerator2
          (return (Components|GetOwner Target)))
        (:NewEnumerator3
          _)
        (:NewEnumerator4
          (goto _label))
        (:NewEnumerator5
          _)
        (:NewEnumerator7
          _)
        (:NewEnumerator10
          _))
      (return Target))
    (:Is%20Not%20Valid
      (return 0))))

(fn AmmunitionExplosion
  (params (DamageType :type E_DamageType%20Enum :default "NewEnumerator0") (Killer/Shell :type Actor%20Object%20Reference) (PenetrationZone :type Actor%20Object%20Reference))
  (bind _returnvalue (Components|GetOwner))
  (bind _returnvalue_2 (Actor|GetComponentbyClass _returnvalue "/Game/ModernRPG/General/Blueprints/ActorComponents/Machinery/AC_VehicleHealth.AC_VehicleHealth_C"))
  (bind _continue (CallFunction|CheckDuplicatingHit Killer/Shell (CallFunction|GetKiller Killer/Shell DamageType) DamageType))
  (if _continue
    (Utilities|IsValid _returnvalue_2
      (:Is%20Valid
        (Default|HealthDecrease-Server _returnvalue_2 9999999.0))
      (:Is%20Not%20Valid
        _))
    (Class|BPIVehicles|TurretExplosion(Message) (Components|GetOwner) false)
    (CallFunction|DestroyVehicleTrace DamageType (CallFunction|GetKiller Killer/Shell DamageType) true)))

(fn NoPenetration
  (params (DamageType :type E_DamageType%20Enum :default "NewEnumerator0") (Killer/Shell :type Actor%20Object%20Reference))
  (bind _return (CallFunction|GetKiller Killer/Shell DamageType))
  (bind _returnvalue (Actor|GetComponentbyClass _return "/Game/ModernRPG/General/Blueprints/ActorComponents/Machinery/AC_VehicleController.AC_VehicleController_C"))
  (bind _vehicle (Variables|/Game/ModernRPG/General/Blueprints/ActorComponents/Machinery/AC_VehicleController.AC_VehicleController_C|GetVehicle _returnvalue))
  (Utilities|IsValid Killer/Shell
    (:Is%20Valid
      (Utilities|IsValid _returnvalue
        (:Is%20Valid
          (Utilities|IsValid _vehicle
            (:Is%20Valid
              (Class|BPIVehicles|ReportAboutNoPenetration(Message) _vehicle))))))))