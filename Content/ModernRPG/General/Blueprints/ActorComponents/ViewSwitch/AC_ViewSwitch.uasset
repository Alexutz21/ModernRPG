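; Character component that switches the player camera between first and third person, with forced-view events and restores for parachute and vehicle exit.
; SwitchView starts a camera fade and a gated Tick that lerps spring arm length and socket offset, then disables ticking.
; Third-person arm length follows movement state, combat and vehicle use.
; Switches replicate the view flag via server and all-client events, and update walk speed, depth of field, aim camera and hat visibility.
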(event Custom|SwitchView
  ;[1 1 1] Manipulate Camera
  (if (not (Variables|Default|GetZoomingProcess))
    (if (not (Variables|Setup|GetInThirdPerson))
      (Variables|Default|SetZoomingProcess true)
      (CallFunction|StartCameraAnimation)
      (CallFunction|ReplicateViewSettings true)
      (Variables|Setup|SetInThirdPerson true)
      (CallFunction|UpdateCurrentWalkSpeed)
      (else
        (Variables|Default|SetZoomingProcess true)
        (CallFunction|StartCameraAnimation)
        (CallFunction|ReplicateViewSettings false)
        (Variables|Setup|SetInThirdPerson false)
        (CallFunction|UpdateCurrentWalkSpeed)))
    (Default|CallOnViewSwitched (Variables|Setup|GetInThirdPerson))
    (CallFunction|ToggleCamera)
    (CallFunction|ToggleHat (not (Variables|Setup|GetInThirdPerson)))))

(event Custom|StartCameraAnimation
  (bind _cameramanager (Variables|Default|GetCameraManager))
  ;[1 1 1] Animation
  (Utilities|IsValid _cameramanager
    (:Is%20Valid
      (CameraFades|StartCameraFade :self _cameramanager :FromAlpha 1.0 :Duration 0.2))
    (:Is%20Not%20Valid
      _))
  (Variables|Default|SetAlpha (select (Variables|Setup|GetInThirdPerson) 0.0 1.0))
  (Components|Tick|SetComponentTickEnabled true)
  (Utilities|FlowControl|Gate true) ; enters at Open
)

(event Custom|ResetViewAfterVehicle%20-%20OC
  ;[1 1 1] Manipulate Camera
  (CallFunction|ControlMeshandCamera (Variables|Setup|GetInThirdPerson) (Components|GetOwner))
  (if (Variables|Setup|GetInThirdPerson)
    (Variables|/Script/Engine.SpringArmComponent|SetTargetArmLength (Variables|Default|GetSpringArm) (CallFunction|FinalTargetArm))
    (Variables|Setup|SetInThirdPerson true)
    (else
      (Variables|/Script/Engine.SpringArmComponent|SetTargetArmLength (Variables|Default|GetSpringArm) 0.0)
      (Variables|Setup|SetInThirdPerson false)
      (CallFunction|ToggleHat true))))

(event Custom|EndCameraAnimation
  ;[1 1 1] Animation
  (Components|Tick|SetComponentTickEnabled false)
  (Utilities|FlowControl|Gate true) ; enters at Close
)

(event Custom|ForceFP
  ;[1 1 1] Manipulate Camera
  (Variables|Setup|SetInThirdPerson true)
  (Variables|/Script/Engine.SpringArmComponent|SetTargetArmLength (Variables|Default|GetSpringArm) 0.0)
  (Variables|Setup|SetInThirdPerson false)
  (Default|CallOnViewSwitched (Variables|Setup|GetInThirdPerson))
  (CallFunction|ToggleCamera))

(event Custom|ReplicateViewSettings%20-ALL
  (params (TPP :type Boolean))
  ;[1 1 1] Manipulate Camera
  (Variables|Setup|SetInThirdPerson TPP))

(event Custom|ReplicateViewSettings
  (params (TPP :type Boolean))
  ;[1 1 1] Manipulate Camera
  (Networking|SwitchHasAuthority
    (:Authority
      (CallFunction|ReplicateViewSettings-ALL TPP))
    (:Remote
      (CallFunction|ReplicateViewSettings-Server TPP))))

(event Custom|ParachuteTP
  ;[1 1 1] Manipulate Camera
  (if (Variables|Setup|GetInThirdPerson)
    (Utilities|IsValid (Variables|Default|GetSpringArm)
      (:Is%20Valid
        (Variables|Setup|SetInThirdPerson false)
        (Variables|/Script/Engine.SpringArmComponent|SetTargetArmLength (Variables|Default|GetSpringArm) (CallFunction|FinalTargetArm))
        (Variables|Setup|SetInThirdPerson true)
        (CallFunction|ToggleHat (not (Variables|Setup|GetInThirdPerson)))
        (Default|CallOnViewSwitched (Variables|Setup|GetInThirdPerson))
        (CallFunction|ToggleCamera)))))

(event Custom|ReplicateViewSettings%20-Server
  (params (TPP :type Boolean))
  ;[1 1 1] Manipulate Camera
  (CallFunction|ReplicateViewSettings-ALL TPP))

(event Custom|ForceView
  (params (Target%20Arm%20Length :type Float%20%28double-precision%29))
  ;[1 1 1] Manipulate Camera
  (Utilities|IsValid (Variables|Default|GetSpringArm)
    (:Is%20Valid
      (Variables|Setup|SetInThirdPerson false)
      (Variables|/Script/Engine.SpringArmComponent|SetTargetArmLength (Variables|Default|GetSpringArm) Target%20Arm%20Length)
      (Variables|Setup|SetInThirdPerson true)
      (Default|CallOnViewSwitched (Variables|Setup|GetInThirdPerson))
      (CallFunction|ToggleCamera))))

(event Custom|ForceTP%20-%20Character
  ;[1 1 1] Manipulate Camera
  (Utilities|IsValid (Variables|Default|GetSpringArm)
    (:Is%20Valid
      (Variables|Setup|SetInThirdPerson false)
      (Variables|/Script/Engine.SpringArmComponent|SetTargetArmLength (Variables|Default|GetSpringArm) (CallFunction|FinalTargetArm))
      (Variables|Setup|SetInThirdPerson true)
      (CallFunction|ToggleHat (not (Variables|Setup|GetInThirdPerson)))
      (Default|CallOnViewSwitched (Variables|Setup|GetInThirdPerson))
      (CallFunction|ToggleCamera))))

(event EventBeginPlay
  ;[1 1 1] Initialzie Character
  (Variables|Default|SetSpringArm (Utilities|Array|Get(acopy) (Actor|GetComponentsbyTag (Components|GetOwner) "/Script/Engine.SpringArmComponent" "Main")))
  (bind _ascharacter (Utilities|Casting|CastToCharacter (Components|GetOwner)))
  (bind _asplayer_controller (Utilities|Casting|CastToPlayerController (Pawn|GetController _ascharacter)))
  (Variables|Default|SetCameraManager (Variables|/Script/Engine.PlayerController|GetPlayerCameraManager _asplayer_controller))
  (Variables|Default|SetLastSocketOffset (Variables|/Script/Engine.SpringArmComponent|GetSocketOffset (Variables|Default|GetSpringArm))))

(event EventTick
  (params (DeltaSeconds :type Float%20%28single-precision%29))
  ;[1 1 1] Animation
  (Utilities|FlowControl|Gate true
    (:Exit
      (Variables|Default|SetAlpha (Math|Float|Clamp(Float) (+ (Variables|Default|GetAlpha) (* (Variables|Setup|GetAlphaSpeed) (select (Variables|Setup|GetInThirdPerson) -1.0 1.0)))))
      (bind _output_get (Variables|/Script/Engine.SpringArmComponent|SetSocketOffset (Variables|Default|GetSpringArm) (Math|Vector|Lerp(Vector) (Default|GetCurrentSocketLocation (Actor|GetComponentbyClass (Components|GetOwner) "/Game/ModernRPG/General/Blueprints/ActorComponents/ViewSwitch/AC_ShoulderSwitch.AC_ShoulderSwitch_C")) (Variables|Setup|GetFPPCameraLocation) (Variables|Default|GetAlpha))))
      (Variables|Default|SetLastSocketOffset _output_get)
      (Variables|/Script/Engine.SpringArmComponent|SetTargetArmLength (Variables|Default|GetSpringArm) (Math|Float|Lerp (select (Utilities|IsValid (Variables|/Game/ModernRPG/General/Blueprints/ActorComponents/Machinery/AC_VehicleController.AC_VehicleController_C|GetVehicle (Actor|GetComponentbyClass (Components|GetOwner) "/Game/ModernRPG/General/Blueprints/ActorComponents/Machinery/AC_VehicleController.AC_VehicleController_C"))) 5.5e+02 (CallFunction|FinalTargetArm)) (Variables|Setup|GetFPPArmLength) (Variables|Default|GetAlpha)))
      (if (select (Variables|Setup|GetInThirdPerson) (<= (Variables|Default|GetAlpha) 0.0) (>= (Variables|Default|GetAlpha) 1.0))
        (CallFunction|EndCameraAnimation)
        (Variables|Default|SetZoomingProcess false)))))

(fn UpdateCurrentWalkSpeed
  (bind _returnvalue (Components|GetOwner))
  (bind _returnvalue_2 (Actor|GetComponentbyClass _returnvalue "/Game/ModernRPG/General/Blueprints/ActorComponents/SpeedChange/AC_SpeedChange.AC_SpeedChange_C"))
  (Default|ChangeWalkSpeed _returnvalue_2 (Variables|/Game/ModernRPG/General/Blueprints/ActorComponents/SpeedChange/AC_SpeedChange.AC_SpeedChange_C|GetCurrentWalkState _returnvalue_2)))

(fn ToggleCamera
  (bind _returnvalue (Components|GetOwner))
  (bind _returnvalue_2 (Actor|GetComponentbyClass _returnvalue "/Game/ModernRPG/General/Blueprints/ActorComponents/Weapon/AC_Weapon.AC_Weapon_C"))
  (bind _array_element_actor (Default|GetCurrentWeapon _returnvalue_2))
  (CallFunction|SetFPPDOF)
  (Utilities|IsValid _array_element_actor
    (:Is%20Valid
      (Variables|/Game/ModernRPG/General/Blueprints/ActorComponents/Weapon/AC_Aiming.AC_Aiming_C|SetCamera (Actor|GetComponentbyClass (Components|GetOwner) "/Game/ModernRPG/General/Blueprints/ActorComponents/Weapon/AC_Aiming.AC_Aiming_C") (select (Variables|AC_ViewSwitch_C|GetInThirdPerson (Actor|GetComponentbyClass (Components|GetOwner) "AC_ViewSwitch_C")) (Utilities|Array|Get(acopy) (Actor|GetComponentsbyTag (Components|GetOwner) "/Script/Engine.CameraComponent" "Main")) (Variables|/Game/ModernRPG/General/Blueprints/Weapon/ConnectedMesh/BP_ConnectedMeshComponent.BP_ConnectedMeshComponent_C|GetAimCamera _array_element_actor))))))

(fn SetFPPDOF
  (bind _returnvalue (Components|GetOwner))
  (bind _returnvalue_2 (Actor|GetComponentbyClass _returnvalue "/Game/ModernRPG/General/Blueprints/Weapon/AC_DOF.AC_DOF_C"))
  (if (Variables|AC_ViewSwitch_C|GetInThirdPerson (Actor|GetComponentbyClass (Components|GetOwner) "AC_ViewSwitch_C"))
    (Default|SetTPPDOF _returnvalue_2)
    (else
      (Default|SetFPPDOF _returnvalue_2))))

(fn ToggleHat
  (params (Hide :type Boolean))
  (Default|ToggleHat (Actor|GetComponentbyClass (Components|GetOwner) "/Game/ModernRPG/General/Blueprints/ActorComponents/Weapon/AC_ArmorEquipment.AC_ArmorEquipment_C") Hide))

(fn FinalTargetArm
  (return (+ (.NewSpringArm (Default|GetCurrentTypeSpeed (Actor|GetComponentbyClass (Components|GetOwner) "/Game/ModernRPG/General/Blueprints/ActorComponents/SpeedChange/AC_SpeedChange.AC_SpeedChange_C"))) (select (and (Variables|/Game/ModernRPG/General/Blueprints/Combat/AC_CombatEvents.AC_CombatEvents_C|GetInCombat (Actor|GetComponentbyClass (Components|GetOwner) "/Game/ModernRPG/General/Blueprints/Combat/AC_CombatEvents.AC_CombatEvents_C")) (Variables|Setup|GetInThirdPerson)) (Variables|Default|GetCloseCombatArm) 0.0))))