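; AC_ShoulderSwitch is an actor component that smoothly swaps the owner's camera between left and right shoulder offsets.
; ToggleShoulder flips the side and enables tick through a gate, interpolating the "Main"-tagged spring arm's socket offset until it reaches the target, then disabling tick.
; The target comes from sibling AC_ViewSwitch and AC_Aiming components, choosing normal or aiming shoulder offsets in third person, or the first-person camera location otherwise.
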(event Custom|ToggleShoulder
  ;[1 1 1] Toggle State
  (Variables|Default|SetOnLeft (not (Variables|Default|GetOnLeft)))
  (CallFunction|StartShoulderAnimation))

(event Custom|StartShoulderAnimation
  ;[1 1 1] Switch Animation
  (Variables|Default|SetAnimationStarted true)
  (Components|Tick|SetComponentTickEnabled true)
  (Utilities|FlowControl|Gate true) ; enters at Open
)

(event Custom|StopShoulderAnimation
  ;[1 1 1] Switch Animation
  (Variables|Default|SetAnimationStarted false)
  (Components|Tick|SetComponentTickEnabled false)
  (Utilities|FlowControl|Gate true) ; enters at Close
)

(event EventBeginPlay
  ;[1 1 1] Initialize Component
  (Variables|Default|SetPlayersSpringArm (Utilities|Array|Get(acopy) (Actor|GetComponentsbyTag (Components|GetOwner) "/Script/Engine.SpringArmComponent" "Main"))))

(event EventTick
  (params (DeltaSeconds :type Float%20%28single-precision%29))
  ;[1 1 1] Switch Animation
  (Utilities|FlowControl|Gate true
    (:Exit
      (bind _output_get (Variables|/Script/Engine.SpringArmComponent|SetSocketOffset (Variables|Default|GetPlayersSpringArm) (Math|Interpolation|VInterpTo (Variables|/Script/Engine.SpringArmComponent|GetSocketOffset (Variables|Default|GetPlayersSpringArm)) (CallFunction|CurVector) (Utilities|Time|GetWorldDeltaSeconds) 14.0)))
      (if (Math|Vector|Equal(Vector) _output_get (CallFunction|CurVector) 0.0001)
        (CallFunction|StopShoulderAnimation)))))

(fn CurVector
  (bind _returnvalue (Components|GetOwner))
  (bind _returnvalue_2 (Actor|GetComponentbyClass _returnvalue "/Game/ModernRPG/General/Blueprints/ActorComponents/ViewSwitch/AC_ViewSwitch.AC_ViewSwitch_C"))
  (return (select (Variables|/Game/ModernRPG/General/Blueprints/ActorComponents/ViewSwitch/AC_ViewSwitch.AC_ViewSwitch_C|GetInThirdPerson _returnvalue_2) (select (Default|Aiming? (Actor|GetComponentbyClass (Components|GetOwner) "/Game/ModernRPG/General/Blueprints/ActorComponents/Weapon/AC_Aiming.AC_Aiming_C")) (CallFunction|GetAimingShoulder) (CallFunction|GetShoulder)) (Variables|/Game/ModernRPG/General/Blueprints/ActorComponents/ViewSwitch/AC_ViewSwitch.AC_ViewSwitch_C|GetFPPCameraLocation _returnvalue_2))))

(fn GetState
  (return (Variables|Default|GetOnLeft)))

(fn GetCurrentSocketLocation
  (return (select (Variables|Default|GetOnLeft) (Variables|Setup|GetLeftShoulder) (Variables|Setup|GetRightShoulder))))

(fn GetOppositeLocation
  (return (select (not (Variables|Default|GetOnLeft)) (Variables|Setup|GetLeftShoulder) (Variables|Setup|GetRightShoulder))))

(fn GetAimingShoulder
  (return (Math|Vector|SelectVector (Variables|Setup|GetLeftShoulderAiming) (Variables|Setup|GetRightShoulderAiming) (Variables|Default|GetOnLeft))))

(fn GetShoulder
  (return (Math|Vector|SelectVector (Variables|Setup|GetLeftShoulder) (Variables|Setup|GetRightShoulder) (Variables|Default|GetOnLeft))))