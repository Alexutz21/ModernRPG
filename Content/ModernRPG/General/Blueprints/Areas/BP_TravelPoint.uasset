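; BP_TravelPoint is a fast-travel waypoint actor with a resizable trigger sphere and a teleportation point widget that reflects its discovered state.
; Eagle events show or hide the widget, handing it the map component and location on show.
; Character overlap sets ownership and relays through server to owning-client events, but the latter is empty.
; Discovery logic for map registration, marker removal and new-area popup is disconnected, so never runs.
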(event OnComponentBeginOverlap(Sphere)
  (params (OverlappedComponent :type Primitive%20Component%20Object%20Reference) (OtherActor :type Actor%20Object%20Reference) (OtherComp :type Primitive%20Component%20Object%20Reference) (OtherBodyIndex :type Integer) (bFromSweep :type Boolean) (SweepResult :type Hit%20Result%20Structure%20%28by%20ref%29))
  ;[1 1 1] Start Overlap Event
  (bind _ascharacter (Utilities|Casting|CastToCharacter OtherActor))
  (Actor|SetOwner _ascharacter)
  (CallFunction|Overlap-Server OtherActor))

(event Custom|Overlap%20-OC
  (params (InputPin :type Actor%20Object%20Reference))
  ;[1 1 1] Overlap with multiplayer support
)

(event Custom|Overlap%20-Server
  (params (InputPin :type Actor%20Object%20Reference))
  ;[1 1 1] Overlap with multiplayer support
  (CallFunction|Overlap-OC InputPin))

(event Custom|EagleEvent
  (bind _aswb_teleportation_point (CallFunction|GetTeleportationPoint))
  ;[1 1 1] Eagle Events
  (Variables|Default|SetinEagleEvent true)
  (Variables|/Game/ModernRPG/General/GUI/Widgets/WorldMap/WB_TeleportationPoint.WB_TeleportationPoint_C|SetMapRef _aswb_teleportation_point (Variables|Default|GetMapComp))
  (Variables|/Game/ModernRPG/General/GUI/Widgets/WorldMap/WB_TeleportationPoint.WB_TeleportationPoint_C|SetLocation _aswb_teleportation_point (Transformation|GetActorLocation))
  (Rendering|SetVisibility (Variables|Default|GetAreaWidget) true false))

(event Custom|EagleReversedEvent
  ;[1 1 1] Eagle Events
  (Variables|Default|SetinEagleEvent false)
  (Rendering|SetVisibility (Variables|Default|GetAreaWidget) false false))

(event EventBeginPlay
  ;[1 1 1] Set Discovered by default
  (Rendering|SetVisibility (Variables|Default|GetAreaWidget) false false)
  (Variables|/Game/ModernRPG/General/GUI/Widgets/WorldMap/WB_TeleportationPoint.WB_TeleportationPoint_C|SetDiscovered (CallFunction|GetTeleportationPoint) (.Discovered? (Utilities|Struct|BreakS_AreaStatState (Variables|Default|GetAreaInfo)))))

(fn ConstructionScript
  (|CallParentFunction)
  (Components|Sphere|SetSphereRadius (Variables|Default|GetSphere) (Variables|Default|GetSphereRadius) true))

(fn GetTeleportationPoint
  (bind _aswb_teleportation_point (Utilities|Casting|CastToWB_TeleportationPoint (UserInterface|GetUserWidgetObject (Variables|Default|GetAreaWidget))))
  (return _aswb_teleportation_point))

(fn RemoveMarker
  (bind _aswb_teleportation_point (CallFunction|GetTeleportationPoint))
  (Utilities|IsValid _aswb_teleportation_point
    (:Is%20Valid
      (if (Variables|/Game/ModernRPG/General/GUI/Widgets/WorldMap/WB_TeleportationPoint.WB_TeleportationPoint_C|GetPlayerMarked _aswb_teleportation_point)
        (Default|ToggleMarkerState (Variables|Default|GetWB_Teleportation))))))

(fn GetChracterCompass
  (params (Target :type Actor%20Object%20Reference)))