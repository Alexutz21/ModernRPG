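; BP_Area is a world area actor that becomes discovered when a character with a world map component enters its sphere zone.
; The overlap makes that character the owner, then routes discovery through authority-checked custom events.
; Discovery removes any map marker, shows a new-area popup with name and points, and updates the area's map widget and world map entry.
; The construction script sizes the sphere and rebuilds the done-task list from the area's tasks.
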(event OnComponentBeginOverlap(CasualZone)
  (params (OverlappedComponent :type Primitive%20Component%20Object%20Reference) (OtherActor :type Actor%20Object%20Reference) (OtherComp :type Primitive%20Component%20Object%20Reference) (OtherBodyIndex :type Integer) (bFromSweep :type Boolean) (SweepResult :type Hit%20Result%20Structure%20%28by%20ref%29))
  ;[1 1 1] Overlap Events
  ;;[1 1 1] On Casual zone overlap
  (bind _ascharacter (Utilities|Casting|CastToCharacter OtherActor))
  (Utilities|IsValid _ascharacter
    (:Is%20Valid
      (Utilities|IsValid (Actor|GetComponentbyClass _ascharacter "/Game/ModernRPG/General/Blueprints/MapComponents/WorldMap/AC_WorldMap.AC_WorldMap_C")
        (:Is%20Valid
          (bind _output_get (Variables|Default|SetOverlapedChaarcter _ascharacter))
          (CallFunction|SetOwner-S _output_get)
          (Variables|Default|SetWorldMap (Actor|GetComponentbyClass _ascharacter "/Game/ModernRPG/General/Blueprints/MapComponents/WorldMap/AC_WorldMap.AC_WorldMap_C"))
          (CallFunction|SetAreaDiscovered))))))

(event Custom|UpateArea
  ;[1 1 1] Overlap Events
  ;;[1 1 1] Update The Area
  (Utilities|Struct|SetmembersinS_AreaStatState (Variables|/Game/ModernRPG/General/GUI/Widgets/WorldMap/WorldPlace/WB_MapArea.WB_MapArea_C|GetAreaInfo (Variables|Default|GetWB_Area))))

(event Custom|SetAreaDiscovered
  (bind _returnvalue (Components|GetOwner))
  ;[1 1 1] Set Area Discovered
  (Utilities|IsValid _returnvalue
    (:Is%20Valid
      (if (Ability|HasAuthority _returnvalue)
        (CallFunction|SetAreaDiscovered-OC)
        (else
          (CallFunction|SetAreaDiscovered-Server))))))

(event Custom|SetOwner%20-S
  (params (NewOwner :type Actor%20Object%20Reference))
  ;[1 1 1] Set Owner
  (CallFunction|SetOwner-ALL NewOwner))

(event Custom|SetOwner%20-ALL
  (params (NewOwner :type Actor%20Object%20Reference))
  ;[1 1 1] Set Owner
  (Actor|SetOwner NewOwner))

(event Custom|SetAreaDiscovered%20-Server
  ;[1 1 1] Set Area Discovered
  (CallFunction|SetAreaDiscovered-OC))

(event Custom|SetAreaDiscovered%20-OC
  (bind _self self)
  (bind _worldmap (Variables|Default|GetWorldMap))
  (bind _areainfo (Variables|Default|GetAreaInfo))
  (bind _area (Utilities|Struct|BreakS_AreaStatState _areainfo))
  (bind _value (Default|GetAreaMapbyActor _worldmap _self))
  (bind _out_row (CallFunction|GetAreaMapInfo _area))
  (bind (_name _hiddenicon _observericon _descoverpoints) (Utilities|Struct|BreakS_AreaInfoStat _out_row))
  ;[1 1 1] Set Area Discovered
  (Utilities|IsAlreadyDescovered
    (:else
      (CallFunction|RemoveMarker)
      (Utilities|Struct|SetmembersinS_AreaStatState (Variables|Default|GetAreaInfo) true)
      (bind _returnvalue (UserInterface|CreateWidget "/Game/ModernRPG/General/GUI/Widgets/AnnounceScreen/WB_NewArea.WB_NewArea_C" 0 _name _descoverpoints))
      (Utilities|IsValid _returnvalue
        (:Is%20Valid
          (UserInterface|Viewport|AddtoViewport _returnvalue 0)
          (Utilities|IsValid (Variables|Default|GetWorldMap)
            (:Is%20Valid
              _)))
        (:Is%20Not%20Valid
          _))
      (Utilities|IsValid _value
        (:Is%20Valid
          (Utilities|Struct|SetmembersinS_AreaStatState (Variables|/Game/ModernRPG/General/GUI/Widgets/WorldMap/WorldPlace/WB_MapArea.WB_MapArea_C|GetAreaInfo _value) true))
        (:Is%20Not%20Valid
          _))
      (Utilities|IsValid (CallFunction|GetMapArea)
        (:Is%20Valid
          (Default|SetNewAreaInfo (CallFunction|GetMapArea) (Variables|Default|GetAreaInfo) false))))
    (:true
      (CallFunction|RemoveMarker))))

(event EventBeginPlay
  ;[1 1 1] Area initialization
  (Variables|Default|SetisRuntime true)
  (Rendering|SetVisibility (Variables|Default|GetAreaWidget) false false)
  (Variables|/Game/ModernRPG/General/GUI/Widgets/WorldMap/WorldPlace/WB_MapArea.WB_MapArea_C|SetAreaInfo (CallFunction|GetMapArea) (Variables|Default|GetAreaInfo))
  (Variables|/Game/ModernRPG/General/GUI/Widgets/WorldMap/WorldPlace/WB_MapArea.WB_MapArea_C|SetActor (CallFunction|GetMapArea) self))

(fn ConstructionScript
  (bind _areainfo (Variables|Default|GetAreaInfo))
  (bind (_area _discovered_ _tasks _donetasks) (Utilities|Struct|BreakS_AreaStatState _areainfo))
  (|CallParentFunction)
  (Components|Sphere|SetSphereRadius (Variables|Default|GetCasualZone) (Variables|Settings|GetSphereRadius) false)
  (if (not (Variables|Default|GetisRuntime))
    (Utilities|Array|Clear _donetasks)
    (for _array_element _tasks
      (Utilities|Array|Add _donetasks (Utilities|Struct|MakeS_pTaskList (.Task (Utilities|Struct|BreakS_pTaskList _array_element)) (LocalVariables|GetNoArray))))))

(fn GetTaskbyActorReference
  (params (Array :type Array%20of%20S%20P%20Task%20List%20Structures) (InputPin :type Object%20Object%20Reference))
  (for (_array_element _array_index) Array
    (for _array_element_2 (.Actors (Utilities|Struct|BreakS_pTaskList _array_element))
      (if (== _array_element_2 InputPin)
        (return _array_index _array_element_2))))
  (Development|PrintString "No such actor in tasks!" true true "(R=1.000000,G=0.166003,B=0.000000,A=1.000000)" 5.0))

(fn GetMapArea
  (bind _areawidget (Variables|Default|GetAreaWidget))
  (bind _returnvalue (UserInterface|GetUserWidgetObject _areawidget))
  (Utilities|IsValid _areawidget
    (:Is%20Valid
      (Utilities|IsValid _returnvalue
        (:Is%20Valid
          (bind _aswb_map_area (Utilities|Casting|CastToWB_MapArea _returnvalue))
          (return _aswb_map_area))))))

(fn RemoveMarker
  (if (Variables|/Game/ModernRPG/General/GUI/Widgets/WorldMap/WorldPlace/WB_MapArea.WB_MapArea_C|Getmarkered? (CallFunction|GetMapArea))
    (Utilities|IsValid (Variables|Default|GetWorldMap)
      (:Is%20Valid
        (Default|ToggleMarker (Default|GetAreaMapbyActor (Variables|Default|GetWorldMap) self))))))