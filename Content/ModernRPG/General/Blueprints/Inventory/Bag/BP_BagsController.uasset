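; Inventory bag manager that spawns, tracks, saves and restores BP_BagActor containers, each identified by a counter-based tag and assigned an owner.
; SpawnBag queues a unique tag, and SpawnBagEvent drains the queue newest first, 0.1 seconds apart, spawning empty bags at player 0's location.
; ReplicateBags routes through the server to a multicast that rebuilds the Bags list from world actors.
; SaveBags merges bags into BP_SaveBags by tag; LoadBags respawns them after BeginPlay.
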(event Custom|ReplicateBags%20-Server
  ;[1 1 1] Geather Bags Information
  (CallFunction|ReplicateBags-ALL))

(event Custom|ReplicateBags
  ;[1 1 1] Geather Bags Information
  (if (Ability|HasAuthority)
    (CallFunction|ReplicateBags-ALL)
    (else
      (CallFunction|ReplicateBags-Server))))

(event Custom|ReplicateBags%20-ALL
  ;[1 1 1] Geather Bags Information
  (bind _outactors (Actor|GetAllActorsOfClass "/Game/ModernRPG/General/Blueprints/Inventory/Bag/BP_BagActor.BP_BagActor_C"))
  (Variables|Default|SetBags _outactors))

(event Custom|SpawnBagEvent
  (params (BagOwner :type Actor%20Object%20Reference))
  (bind _queue (Variables|Default|GetQueue))
  (bind _returnvalue (Utilities|Array|Length _queue))
  (bind _returnvalue_2 (- _returnvalue 1))
  (if (and (not (Variables|Default|GetSpawning)) (> (Utilities|Array|Length (Variables|Default|GetQueue)) 0))
    (Variables|Default|SetSpawning true)
    (CallFunction|SpawnProcess (Utilities|Array|Get(acopy) _queue _returnvalue_2))
    (Utilities|Array|RemoveIndex (Variables|Default|GetQueue) _returnvalue_2)
    (Utilities|FlowControl|Delay 0.1)
    (Variables|Default|SetSpawning false)
    (CallFunction|SpawnBagEvent BagOwner)))

(event EventBeginPlay
  ;[1 1 1] Geather Bags Information
  (Actor|SetOwner (Game|GetPlayerCharacter 0))
  (Utilities|FlowControl|Delay 1.0)
  (CallFunction|LoadBags))

(fn ConstructionScript)

(fn LoadBags
  (bind _returnvalue (SaveGame|DoesSaveGameExist (Variables|Default|GetBagsSlot)))
  (if _returnvalue
    (bind _returnvalue_2 (SaveGame|LoadGamefromSlot (Variables|Default|GetBagsSlot)))
    (bind _asbp_save_bags (Utilities|Casting|CastToBP_SaveBags _returnvalue_2))
    (bind _output_get (LocalVariables|SetL_SaveGame _asbp_save_bags))
    (for _array_element (Variables|/Game/ModernRPG/General/Blueprints/Inventory/Bag/BP_SaveBags.BP_SaveBags_C|GetsBags _output_get)
      (if (.Spawned (Utilities|Struct|BreakS_BagsSave _array_element))
        (bind _returnvalue_3 (Game|SpawnActorfromClass "/Game/ModernRPG/General/Blueprints/Inventory/Bag/BP_BagActor.BP_BagActor_C" (Math|Transform|MakeTransform "0, 0,-500.000000" "0, 0, 0" "1.000000,1.000000,1.000000") "AlwaysSpawn" (Game|GetPlayerController 0) (.Tag (Utilities|Struct|BreakS_BagsSave _array_element)) (.Inventory (Utilities|Struct|BreakS_BagsSave _array_element)) (.Spawned (Utilities|Struct|BreakS_BagsSave _array_element)) 0))
        (Utilities|Array|Add (Variables|Default|GetBags) _returnvalue_3)
        (Default|SetBagOwner _returnvalue_3 (.Owner (Utilities|Struct|BreakS_BagsSave _array_element)))))
    (Variables|Default|SetBagsCounter (Variables|/Game/ModernRPG/General/Blueprints/Inventory/Bag/BP_SaveBags.BP_SaveBags_C|GetBagsCounter (LocalVariables|GetL_SaveGame)))))

(fn SaveBags
  (bind _returnvalue (SaveGame|DoesSaveGameExist (Variables|Default|GetBagsSlot)))
  (if _returnvalue
    (bind _returnvalue_2 (SaveGame|LoadGamefromSlot (Variables|Default|GetBagsSlot)))
    (bind _asbp_save_bags (Utilities|Casting|CastToBP_SaveBags _returnvalue_2))
    (LocalVariables|SetL_SaveGame _asbp_save_bags)
    (else
      (bind _returnvalue_3 (SaveGame|CreateSaveGameObject "/Game/ModernRPG/General/Blueprints/Inventory/Bag/BP_SaveBags.BP_SaveBags_C"))
      (LocalVariables|SetL_SaveGame _returnvalue_3)))
  (Variables|/Game/ModernRPG/General/Blueprints/Inventory/Bag/BP_SaveBags.BP_SaveBags_C|SetBagsCounter (LocalVariables|GetL_SaveGame) (Variables|Default|GetBagsCounter))
  (LocalVariables|SetL_SaveBags (Variables|/Game/ModernRPG/General/Blueprints/Inventory/Bag/BP_SaveBags.BP_SaveBags_C|GetsBags (LocalVariables|GetL_SaveGame)))
  (for _array_element (Variables|Default|GetBags)
    (if (.Result (CallFunction|HasThisTag (LocalVariables|GetL_SaveBags) (Utilities|Array|Get(acopy) (Variables|/Script/Engine.Actor|GetTags _array_element))))
      (Utilities|Array|SetArrayElem (LocalVariables|GetL_SaveBags) (.Array%20Index (CallFunction|HasThisTag (LocalVariables|GetL_SaveBags) (Utilities|Array|Get(acopy) (Variables|/Script/Engine.Actor|GetTags _array_element)))) (Utilities|Struct|MakeS_BagsSave (Utilities|Array|Get(acopy) (Variables|/Script/Engine.Actor|GetTags _array_element)) (Variables|/Game/ModernRPG/General/Blueprints/ActorComponents/Character/Inventory/AC_Inventory.AC_Inventory_C|GetInventory (Variables|/Game/ModernRPG/General/Blueprints/Inventory/Bag/BP_BagActor.BP_BagActor_C|GetAC_Inventory _array_element)) (Variables|/Game/ModernRPG/General/Blueprints/Inventory/Bag/BP_BagActor.BP_BagActor_C|GetSpawned _array_element) (Variables|/Game/ModernRPG/General/Blueprints/Inventory/Bag/BP_BagActor.BP_BagActor_C|GetBagOwner _array_element)))
      (else
        (Utilities|Array|Add (LocalVariables|GetL_SaveBags) (Utilities|Struct|MakeS_BagsSave (Utilities|Array|Get(acopy) (Variables|/Script/Engine.Actor|GetTags _array_element)) (Variables|/Game/ModernRPG/General/Blueprints/ActorComponents/Character/Inventory/AC_Inventory.AC_Inventory_C|GetInventory (Variables|/Game/ModernRPG/General/Blueprints/Inventory/Bag/BP_BagActor.BP_BagActor_C|GetAC_Inventory _array_element)) (Variables|/Game/ModernRPG/General/Blueprints/Inventory/Bag/BP_BagActor.BP_BagActor_C|GetSpawned _array_element) (Variables|/Game/ModernRPG/General/Blueprints/Inventory/Bag/BP_BagActor.BP_BagActor_C|GetBagOwner _array_element))))))
  (Variables|/Game/ModernRPG/General/Blueprints/Inventory/Bag/BP_SaveBags.BP_SaveBags_C|SetsBags (LocalVariables|GetL_SaveGame) (LocalVariables|GetL_SaveBags))
  (SaveGame|SaveGametoSlot (LocalVariables|GetL_SaveGame) (Variables|Default|GetBagsSlot)))

(fn SpawnBag
  (params (BagOwner :type Actor%20Object%20Reference))
  (Math|Integer|IncrementInt (Variables|Default|GetBagsCounter)
    (:%20%20
      (bind _output_get (LocalVariables|SetL_BagTag (Utilities|Name|MakeLiteralName (Utilities|String|StringToName (Utilities|String|ToString(Text) (Utilities|Text|FormatText "Bag_{n}" (Variables|Default|GetBagsCounter)))))))
      (CallFunction|AddUniqueQueue _output_get BagOwner)
      (CallFunction|SpawnBagEvent BagOwner)
      (return _output_get))))

(fn GetBag
  (params (Tag :type Name))
  (for _array_element (Variables|Default|GetBags)
    (Utilities|IsValid _array_element
      (:Is%20Valid
        (if (Actor|ActorHasTag _array_element Tag)
          (return _array_element)))))
  (return 0))

(fn HasThisTag
  (params (Array :type Array%20of%20S%20Bags%20Save%20Structures) (Tag :type Name))
  (for (_array_element _array_index) Array
    (if (Utilities|Name|Equal(Name) (.Tag (Utilities|Struct|BreakS_BagsSave _array_element)) Tag)
      (return (Utilities|Name|Equal(Name) (.Tag (Utilities|Struct|BreakS_BagsSave _array_element)) Tag) _array_index)))
  (return false 0))

(fn SpawnProcess
  (params (Queue :type S%20Bag%20Queue%20Structure))
  (bind _returnvalue (Game|Player|GetPlayerPawn 0))
  (Utilities|IsValid _returnvalue
    (:Is%20Valid
      (LocalVariables|SetSpawnLocation (Transformation|GetActorLocation _returnvalue)))
    (:Is%20Not%20Valid
      (LocalVariables|SetSpawnLocation "0, 0, 0")))
  (Utilities|IsValid (CallFunction|GetBagbyTag (.Name (Utilities|Struct|BreakS_BagQueue Queue)))
    (:Is%20Not%20Valid
      (bind _returnvalue_2 (Game|SpawnActorfromClass "/Game/ModernRPG/General/Blueprints/Inventory/Bag/BP_BagActor.BP_BagActor_C" (Math|Transform|MakeTransform (LocalVariables|GetSpawnLocation) "0, 0, 0" "1.000000,1.000000,1.000000") "AlwaysSpawn" (Game|GetPlayerController 0) (.Name (Utilities|Struct|BreakS_BagQueue Queue)) (Utilities|Array|MakeArray "") true 0))
      (Default|SetBagOwner _returnvalue_2 (.Owner (Utilities|Struct|BreakS_BagQueue Queue)))
      (Actor|Tick|SetActorTickEnabled _returnvalue_2)
      (Utilities|Array|Clear (Variables|/Game/ModernRPG/General/Blueprints/ActorComponents/Character/Inventory/AC_Inventory.AC_Inventory_C|GetInventory (Variables|/Game/ModernRPG/General/Blueprints/Inventory/Bag/BP_BagActor.BP_BagActor_C|GetAC_Inventory _returnvalue_2)))
      (Utilities|Array|Add (Variables|Default|GetBags) _returnvalue_2)
      (CallFunction|ReplicateBags))))

(fn AddUniqueQueue
  (params (Tag :type Name) (Owner :type Actor%20Object%20Reference))
  (for _array_element (Variables|Default|GetQueue)
    (if (Utilities|Name|Equal(Name) (.Name (Utilities|Struct|BreakS_BagQueue _array_element)) Tag)
      (return)))
  (Utilities|Array|Add (Variables|Default|GetQueue) (Utilities|Struct|MakeS_BagQueue Tag Owner)))