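; BP_BagActor is an actor representing an inventory bag, carrying its own AC_Inventory component.
; On BeginPlay it fills that component from its preset item list, replicates it, and applies its tag through a server-to-all event pair.
; Assigning a bag owner stamps that owner onto every item and copies the owner's Seller flag, while a similar event pair sets the actor's owner.
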(event Custom|SetTag%20-ALL
  ;[1 1 1] Initialize Tag
  (Utilities|Array|SetArrayElem (Variables|Actor|GetTags) 0 (Variables|Default|GetTag) true))

(event Custom|SetTag%20-Server
  ;[1 1 1] Initialize Tag
  (CallFunction|SetTag-ALL))

(event Custom|SetOwnerBag%20-Server
  (params (NewOwner :type Actor%20Object%20Reference))
  ;[1 1 1] Set Owner
  (CallFunction|SetOwner-ALL NewOwner))

(event Custom|SetOwner%20-ALL
  (params (NewOwner :type Actor%20Object%20Reference))
  ;[1 1 1] Set Owner
  (Actor|SetOwner NewOwner))

(event Custom|SetBagOwner
  (params (BagOwner :type Actor%20Object%20Reference))
  (Variables|Default|SetBagOwner BagOwner)
  (CallFunction|SetOwnertoInventory)
  (Utilities|IsValid (Variables|Default|GetBagOwner)
    (:Is%20Valid
      (Variables|/Game/ModernRPG/General/Blueprints/ActorComponents/Character/Inventory/AC_Inventory.AC_Inventory_C|SetSeller (Variables|Default|GetAC_Inventory) (Variables|/Game/ModernRPG/General/Blueprints/ActorComponents/Character/Inventory/AC_Inventory.AC_Inventory_C|GetSeller (Actor|GetComponentbyClass (Variables|Default|GetBagOwner) "/Game/ModernRPG/General/Blueprints/ActorComponents/Character/Inventory/AC_Inventory.AC_Inventory_C"))))
    (:Is%20Not%20Valid
      (Variables|/Game/ModernRPG/General/Blueprints/ActorComponents/Character/Inventory/AC_Inventory.AC_Inventory_C|SetSeller (Variables|Default|GetAC_Inventory) false))))

(event Custom|SetOwnerToInventory
  (for _array_element (Variables|/Game/ModernRPG/General/Blueprints/ActorComponents/Character/Inventory/AC_Inventory.AC_Inventory_C|GetInventory (Variables|Default|GetAC_Inventory))
    (CallFunction|SetBagOwner _array_element (Variables|Default|GetBagOwner))))

(event EventTick
  (params (DeltaSeconds :type Float%20%28single-precision%29))
  ;[1 1 1] Debug Bags Inventory
)

(event EventBeginPlay
  ;[1 1 1] Initialize Inventory
  (Variables|/Game/ModernRPG/General/Blueprints/ActorComponents/Character/Inventory/AC_Inventory.AC_Inventory_C|SetInventory (Variables|Default|GetAC_Inventory) (Variables|Default|GetInventroy))
  (Default|ReplicateInventory (Variables|Default|GetAC_Inventory))
  (CallFunction|SetTag-Server))

(fn ConstructionScript)