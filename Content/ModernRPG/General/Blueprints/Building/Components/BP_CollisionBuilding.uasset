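; BP_CollisionBuilding is a box collision actor for the building system, with configurable extent, optional location offset and a function to set collision mode.
; Its construction script, in preview mode, hides the box and spawns a preview BP_BuildingMaster child actor.
; It finds its own ChildActorComponent on the parent, passing that rotation plus the parent's to SetToNullCoordinatesPreview.
; Outside preview mode, it destroys the child component and shows the box.
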(event Collision|EventActorBeginOverlap
  (params (OtherActor :type Actor%20Object%20Reference)))

(fn ConstructionScript
  (bind _returnvalue (Actor|GetParentActor))
  (bind _returnvalue_2 (Transformation|GetActorRotation _returnvalue))
  (bind (_roll _pitch _yaw) (Math|Rotator|BreakRotator _returnvalue_2))
  (Components|Box|SetBoxExtent (Variables|Default|GetBox) (Variables|Default|GetBoxExtent) true)
  (Utilities|FlowControl|Sequence
    (:then_0
      (if (Variables|Default|GetbPreviewMode)
        (ChildActorComponent|SetChildActorClass (Variables|Default|GetChildActor) (Variables|Default|GetPreviewActorClass))
        (for _array_element (Actor|GetComponentsByClass (Actor|GetParentActor) "/Script/Engine.ChildActorComponent")
          (bind _asbp_collision_building (Utilities|Casting|CastToBP_CollisionBuilding (Variables|/Script/Engine.ChildActorComponent|GetChildActor _array_element)))
          (if (== _asbp_collision_building self)
            (bind _asbp_building_master (Utilities|Casting|CastToBP_BuildingMaster (Variables|/Script/Engine.ChildActorComponent|GetChildActor (Variables|Default|GetChildActor))))
            (Default|SettoNullCoordinatesPreview _asbp_building_master (Math|Rotator|MakeRotator (+ (.Roll (Math|Rotator|BreakRotator (Variables|/Script/Engine.SceneComponent|GetRelativeRotation _array_element))) _roll) (+ (.Pitch (Math|Rotator|BreakRotator (Variables|/Script/Engine.SceneComponent|GetRelativeRotation _array_element))) _pitch) (+ (.Yaw (Math|Rotator|BreakRotator (Variables|/Script/Engine.SceneComponent|GetRelativeRotation _array_element))) _yaw)))))))
    (:then_1
      (if (Math|Vector|NotEqual(Vector) (Variables|Default|GetOverriden%20relative%20location) "0, 0, 0" 0.0001)
        (Transformation|SetRelativeLocation (Variables|Default|GetBox) (Variables|Default|GetOverriden%20relative%20location) false true)))
    (:then_2
      (if (Variables|Default|GetbPreviewMode)
        (Rendering|SetVisibility (Variables|Default|GetBox) (not (Variables|Default|GetbPreviewMode)) false)
        (Rendering|SetVisibility (Variables|Default|GetChildActor) (Variables|Default|GetbPreviewMode) false)
        (bind _asbp_building_master_2 (Utilities|Casting|CastToBP_BuildingMaster (Variables|/Script/Engine.ChildActorComponent|GetChildActor (Variables|Default|GetChildActor))))
        (Rendering|SetVisibility (Variables|/Game/ModernRPG/General/Blueprints/InteractActors/BP_SimpleInteract.BP_SimpleInteract_C|GetInteractArea _asbp_building_master_2) (not (Variables|Default|GetbPreviewMode)) false)
        (else
          (Components|DestroyComponent (Variables|Default|GetChildActor))
          (Rendering|SetVisibility (Variables|Default|GetBox) true false))))))

(fn ControlCollision
  (params (NewType :type ECollisionEnabled%20Enum :default "NoCollision"))
  (Collision|SetCollisionEnabled (Variables|Default|GetBox) NewType))