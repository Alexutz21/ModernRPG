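; Off-screen preview actor that renders a loot box chest or character and weapon skin rewards into a UI image, with mouse-drag rotation.
; BeginPlay routes through server and multicast events to create a render target for the scene capture, fed to the image through an M_ItemPreview dynamic material.
; SetNewMesh applies the reward's meshes, materials and optional weapon animation, then UpdateScale hides the chest, fits bounds to a desired size and offsets the actor to recenter.
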(event Custom|UpdateScale
  (params (Selection :type E_ChestTypes%20Enum :default "NewEnumerator0"))
  (bind _desiredmesh (Variables|Default|GetDesiredMesh))
  (bind _weapon (Variables|Default|GetWeapon))
  (bind _desiredmesh_2 (Variables|Default|GetDesiredMesh))
  (bind _reference (Variables|Default|GetReference))
  (bind _reference_2 (Variables|Default|GetReference))
  (bind (_x _y _z) (Math|Vector|BreakVector _desiredmesh))
  (bind (_x_2 _y_2 _z_2) (Math|Vector|BreakVector _desiredmesh_2))
  ;[1 1 1] Scale object to your viewport
  (switch Utilities|FlowControl|Switch|SwitchonE_ChestTypes Selection
    (:NewEnumerator0
      (CallFunction|DerenderChest)
      (for _array_element (Utilities|Array|MakeArray (Variables|Default|GetHead) (Variables|Default|GetBody) (Variables|Default|GetTorso) (Variables|Default|GetLegs) (Variables|Default|GetFeet))
        (Variables|Default|SetCurrentExtandMesh (.BoxExtent (Collision|GetComponentBounds _reference_2)))
        (Transformation|SetWorldScale3D _array_element (Math|Vector|MakeVector (Math|Float|Absolute(Float) (.X (Math|Vector|BreakVector (- (* (Transformation|GetWorldScale _reference_2) (Math|Float|Min(Float) (/ _x (.X (Math|Vector|BreakVector (Variables|Default|GetCurrentExtandMesh)))) (/ _y (.Y (Math|Vector|BreakVector (Variables|Default|GetCurrentExtandMesh)))) (/ _z (.Z (Math|Vector|BreakVector (Variables|Default|GetCurrentExtandMesh)))))) (Variables|Default|GetScale))))) (Math|Float|Absolute(Float) (.Y (Math|Vector|BreakVector (- (* (Transformation|GetWorldScale _reference_2) (Math|Float|Min(Float) (/ _x (.X (Math|Vector|BreakVector (Variables|Default|GetCurrentExtandMesh)))) (/ _y (.Y (Math|Vector|BreakVector (Variables|Default|GetCurrentExtandMesh)))) (/ _z (.Z (Math|Vector|BreakVector (Variables|Default|GetCurrentExtandMesh)))))) (Variables|Default|GetScale))))) (Math|Float|Absolute(Float) (.Z (Math|Vector|BreakVector (- (* (Transformation|GetWorldScale _reference_2) (Math|Float|Min(Float) (/ _x (.X (Math|Vector|BreakVector (Variables|Default|GetCurrentExtandMesh)))) (/ _y (.Y (Math|Vector|BreakVector (Variables|Default|GetCurrentExtandMesh)))) (/ _z (.Z (Math|Vector|BreakVector (Variables|Default|GetCurrentExtandMesh)))))) (Variables|Default|GetScale)))))))
        (Variables|Default|SetAddActorLocalOffset (- (Transformation|GetWorldLocation _reference) (.Origin (Collision|GetComponentBounds _reference)))))
      (Transformation|AddActorLocalOffset (Variables|Default|GetAddActorLocalOffset) false true))
    (:NewEnumerator1
      (CallFunction|DerenderChest)
      (Variables|Default|SetCurrentExtandMesh (.BoxExtent (Collision|GetComponentBounds (Variables|Default|GetWeapon))))
      (Transformation|SetWorldScale3D (Variables|Default|GetWeapon) (- (* (Transformation|GetWorldScale (Variables|Default|GetWeapon)) (Math|Float|Min(Float) (/ _x_2 (.X (Math|Vector|BreakVector (Variables|Default|GetCurrentExtandMesh)))) (/ _y_2 (.Y (Math|Vector|BreakVector (Variables|Default|GetCurrentExtandMesh)))) (/ _z_2 (.Z (Math|Vector|BreakVector (Variables|Default|GetCurrentExtandMesh)))))) (Variables|Default|GetScale)))
      (Transformation|AddActorLocalOffset (- (Transformation|GetWorldLocation _weapon) (.Origin (Collision|GetComponentBounds _weapon))) false true))))

(event Custom|RenderChest
  ;[1 1 1] Toggle Chest
  (Rendering|SetVisibility (Variables|Default|GetStaticMesh) true false)
  (Class|SkinnedMeshComponent|SetSkeletalMesh (Variables|Default|GetWeapon) 0 true))

(event Custom|CreateRT%20Event
  (bind _scenecapturecomponent2d (Variables|Components|GetSceneCaptureComponent2D))
  ;[1 1 1] Create a render target
  (Networking|SwitchHasAuthority
    (:Authority
      (CallFunction|CreateRT-All _scenecapturecomponent2d))
    (:Remote
      (CallFunction|CreateRT-Server _scenecapturecomponent2d))))

(event Custom|CreateRT%20-%20Server
  (params (SceneCaptureComponent2D :type Scene%20Capture%20Component%202D%20Object%20Reference))
  ;[1 1 1] Create a render target
  (CallFunction|CreateRT-All SceneCaptureComponent2D))

(event Custom|On%20Mouse%20Move
  (params (Mouse%20Location :type Vector%202D%20Structure))
  ;[1 1 1] Add rotation to the mesh
  (if (Variables|Default|GetRotationEnabled)
    (Transformation|AddWorldRotation (Utilities|Select :Index (Variables|Default|GetRewardType) :NewEnumerator0 (Variables|Default|GetCharacterComponents) :NewEnumerator1 (Variables|Components|GetScene)) (CallFunction|GetNewRotation Mouse%20Location) false false)
    (Variables|Default|SetOnStartRotating Mouse%20Location)))

(event Custom|DerenderChest
  ;[1 1 1] Toggle Chest
  (Rendering|SetVisibility (Variables|Default|GetStaticMesh) false false))

(event Custom|On%20Click%20Start
  (params (Mouse%20Location :type Vector%202D%20Structure))
  ;[1 1 1] Mouse Events
  (Variables|Default|SetOnStartRotating Mouse%20Location)
  (Variables|Default|SetRotationEnabled true))

(event Custom|On%20Click%20End
  (params (Mouse%20Location :type Vector%202D%20Structure))
  ;[1 1 1] Mouse Events
  (Variables|Default|SetRotationEnabled false))

(event Custom|CreateRT-All
  (params (SceneCaptureComponent2D :type Scene%20Capture%20Component%202D%20Object%20Reference))
  ;[1 1 1] Create a render target
  (CallFunction|CreateRT SceneCaptureComponent2D))

(event EventBeginPlay
  ;[1 1 1] Create a render target
  (CallFunction|CreateRTEvent))

(fn ConstructionScript)

(fn SetNewMesh
  (params (Mesh :type Skeletal%20Mesh%20Object%20Reference) (Material :type Array%20of%20Material%20Interface%20Object%20References) (SetScale :type Vector) (NewAnimToPlay :type Animation%20Asset%20Object%20Reference) (Selection :type E_ChestTypes%20Enum :default "NewEnumerator0") (CharacterParts :type Array%20of%20S%20Character%20Skin%20Separated%20Structures))
  ;[1 1 1] Setting mesh and scale of recording actor when used lookable item
  (bind _output_get (Variables|Default|SetRewardType Selection))
  (switch Utilities|FlowControl|Switch|SwitchonE_ChestTypes _output_get
    (:NewEnumerator0
      (bind _output_get_2 (LocalVariables|Settemp_SK_Comps (Utilities|Array|MakeArray (Variables|Default|GetHead) (Variables|Default|GetBody) (Variables|Default|GetTorso) (Variables|Default|GetLegs) (Variables|Default|GetFeet))))
      (for (_array_element _array_index) _output_get_2
        (Transformation|SetRelativeRotation _array_element "0,0.000000, 0" false false)
        (Transformation|SetRelativeLocation _array_element "0, 0,-23.000000" false true)
        (Class|SkinnedMeshComponent|SetSkeletalMesh _array_element (.SkeletalMesh (Utilities|Struct|BreakS_CharacterSkin_Separated (Utilities|Array|Get(acopy) CharacterParts _array_index))) true)
        (for (_array_element_2 _array_index_2) (.Materials (Utilities|Struct|BreakS_CharacterSkin_Separated (Utilities|Array|Get(acopy) CharacterParts _array_index)))
          (Rendering|Material|SetMaterial _array_element _array_index_2 _array_element_2))
        (Variables|Default|SetScale SetScale)
        (CallFunction|UpdateScale "NewEnumerator0")))
    (:NewEnumerator1
      (Class|SkinnedMeshComponent|SetSkeletalMesh (Variables|Default|GetWeapon) Mesh true)
      (if (not (Utilities|IsValid NewAnimToPlay))
        _
        (else
          (Components|Animation|SetAnimationMode (Variables|Default|GetWeapon) "AnimationSingleNode")
          (Components|Animation|SetAnimation (Variables|Default|GetWeapon) NewAnimToPlay)
          (Audio|Components|Audio|Play (Variables|Default|GetWeapon) true)))
      (Transformation|SetRelativeRotation (Variables|Default|GetWeapon) "0, 0, 0" false false)
      (Transformation|SetRelativeLocation (Variables|Default|GetWeapon) "0, 0, 0" false false)
      (for (_array_element_3 _array_index_3) Material
        (Rendering|Material|SetMaterial (Variables|Default|GetWeapon) _array_index_3 _array_element_3))
      (Variables|Default|SetScale SetScale)
      (CallFunction|UpdateScale "NewEnumerator1"))))

(fn GetNewRotation
  (params (MouseLocaiton :type Vector%202D%20Structure))
  (bind _onstartrotating (Variables|Default|GetOnStartRotating))
  (bind _returnvalue (- MouseLocaiton _onstartrotating))
  (bind (_x _y) (Math|Vector2D|BreakVector2D _returnvalue))
  (return (Math|Rotator|MakeRotator 0.0 (Math|Float|SelectFloat (* (/ _y 1e+01) 1.0) 0.0 (> (Math|Float|Absolute(Float) _y) 1.0)) (Math|Float|SelectFloat (* (/ _x 1e+01) -1.0) 0.0 (> (Math|Float|Absolute(Float) _x) 1.0)))))

(fn CreateRT
  (params (SceneCaptureComponent2D :type Scene%20Capture%20Component%202D%20Object%20Reference))
  (bind _image (Variables|Default|GetImage))
  (bind _brush (Variables|/Script/UMG.Image|GetBrush _image))
  (Utilities|IsValid SceneCaptureComponent2D
    (:Is%20Valid
      (Components|Activation|Activate SceneCaptureComponent2D false)
      (bind _returnvalue (Rendering|CreateRenderTarget2D 1920 1920 "RTF_RGBA16f"))
      (Variables|/Script/Engine.SceneCaptureComponent2D|SetTextureTarget SceneCaptureComponent2D _returnvalue)
      (Utilities|IsValid (Variables|Default|GetDynamicMaterial)
        (:Is%20Valid
          (Rendering|Material|SetTextureParameterValue (Variables|Default|GetDynamicMaterial) "Render" (Variables|/Script/Engine.SceneCaptureComponent2D|GetTextureTarget SceneCaptureComponent2D)))
        (:Is%20Not%20Valid
          (Utilities|IsValid (Variables|Default|GetImage)
            (:Is%20Valid
              (bind _returnvalue_2 (Rendering|Material|CreateDynamicMaterialInstance "/Game/ModernRPG/General/GUI/Materials/ItemPreview/M_ItemPreview.M_ItemPreview" "None" "None" :!class /Script/Engine.KismetMaterialLibrary))
              (bind _output_get (Variables|Default|SetDynamicMaterial _returnvalue_2))
              (Class|Image|SetBrush _image (Utilities|Struct|MakeSlateBrush (.imagesize _brush) (.margin _brush) (.tintcolor _brush) "(CornerRadii=(X=0.000000,Y=0.000000,Z=0.000000,W=1.000000),Color=(SpecifiedColor=(R=0.000000,G=0.000000,B=0.000000,A=0.000000),ColorUseRule=UseColor_Specified),Width=0.000000,RoundingType=HalfHeightRadius,bUseBrushTransparency=False)" _output_get (.drawas _brush) (.tiling _brush) (.mirroring _brush)))
              (Class|Image|SetBrushfromMaterial (Variables|Default|GetImage) (Variables|Default|GetDynamicMaterial))
              (Rendering|Material|SetTextureParameterValue (Variables|Default|GetDynamicMaterial) "Render" (Variables|/Script/Engine.SceneCaptureComponent2D|GetTextureTarget SceneCaptureComponent2D))
              (return))
            (:Is%20Not%20Valid
              (return))))))))