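; Preview actor that renders an item or modification mesh through a scene capture into a UI image for a rotatable 3D view.
; Setters supply a skeletal or static mesh, which is scaled and offset using its bounds to fit the capture.
; CreateRT, routed through server and all-client events, feeds a new render target into an M_ItemPreview dynamic material.
; Mouse drag rotates the scene, and a toggle hides or shows the Scope bone.
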(event Custom|UpdateScaleStatic
  (bind _staticmesh (Variables|Default|GetStaticMesh))
  (bind _staticmesh_2 (Variables|Default|GetStaticMesh))
  (bind (_origin _boxextent _sphereradius) (Collision|GetComponentBounds _staticmesh_2))
  ;[1 1 1] Scale object to your viewport
  (Variables|Default|SetCurrentExtandMesh _boxextent)
  (Transformation|SetWorldScale3D (Variables|Default|GetStaticMesh) (Math|Conversions|ToVector(Float) (/ 2.0 _sphereradius)))
  (Transformation|AddActorLocalOffset (- (Transformation|GetWorldLocation _staticmesh) (.Origin (Collision|GetComponentBounds _staticmesh))) false true))

(event Custom|SetInformation
  (params (Skeletal :type Boolean) (SkeletalMesh :type Skeletal%20Mesh%20Object%20Reference) (StaticMesh :type Static%20Mesh%20Object%20Reference))
  ;[1 1 1] Initialize
  (if Skeletal
    (Class|SkinnedMeshComponent|SetSkeletalMesh (Variables|Default|GetSkeletalMesh) SkeletalMesh true)
    (Rendering|SetVisibility (Variables|Default|GetStaticMesh) false false)
    (CallFunction|UpdateScaleSkeletal)
    (else
      (Components|StaticMesh|SetStaticMesh (Variables|Default|GetStaticMesh) StaticMesh)
      (Rendering|SetVisibility (Variables|Default|GetSkeletalMesh) false false)
      (Rendering|SetVisibility (Variables|Default|GetStaticMesh) true false)
      (CallFunction|UpdateScaleStatic))))

(event Custom|CreateRT%20Event
  (bind _scenecapturecomponent2d (Variables|Components|GetSceneCaptureComponent2D))
  ;[1 1 1] Create a render target
  (Networking|SwitchHasAuthority
    (:Authority
      (CallFunction|CreateRT-All _scenecapturecomponent2d))
    (:Remote
      (CallFunction|CreateRT-Server _scenecapturecomponent2d))))

(event Custom|CreateRT%20-%20Server
  (params (SceneCaptureComponent2D :type Scene%20Capture%20Component%202D%20Object%20Reference))
  ;[1 1 1] Create a render target
  (CallFunction|CreateRT-All SceneCaptureComponent2D))

(event Custom|On%20Mouse%20Move
  (params (Mouse%20Location :type Vector%202D%20Structure))
  ;[1 1 1] Add rotation to the mesh
  (if (Variables|Default|GetRotationEnabled)
    (Transformation|AddWorldRotation (Variables|Components|GetScene) (CallFunction|GetNewRotation Mouse%20Location) false false)
    (Variables|Default|SetOnStartRotating Mouse%20Location)))

(event Custom|UpdateScaleSkeletal
  (bind _skeletalmesh (Variables|Default|GetSkeletalMesh))
  (bind _skeletalmesh_2 (Variables|Default|GetSkeletalMesh))
  (bind (_origin _boxextent _sphereradius) (Collision|GetComponentBounds _skeletalmesh))
  (bind (_origin_2 _boxextent_2 _sphereradius_2) (Collision|GetComponentBounds _skeletalmesh_2))
  ;[1 1 1] Scale object to your viewport
  (Variables|Default|SetCurrentExtandMesh _boxextent_2)
  (Transformation|SetWorldScale3D (Variables|Default|GetSkeletalMesh) (Math|Conversions|ToVector(Float) (* (/ 2.0 _sphereradius_2) 0.2)))
  (Transformation|AddActorLocalOffset (- (- (Transformation|GetWorldLocation _skeletalmesh) _origin) (Math|Vector|MakeVector 0.0 0.0 _sphereradius)) false true))

(event Custom|SetScaleRotation
  (params (NewRotation :type Rotator) (NewScale3D :type Vector))
  ;[1 1 1] Set scale and rotation
  (Transformation|SetRelativeRotation (Variables|Default|GetSkeletalMesh) NewRotation false false)
  (Transformation|SetRelativeScale3D (Variables|Default|GetStaticMesh) NewScale3D))

(event Custom|On%20Click%20Start
  (params (Mouse%20Location :type Vector%202D%20Structure))
  ;[1 1 1] Mouse Events
  (Variables|Default|SetOnStartRotating Mouse%20Location)
  (Variables|Default|SetRotationEnabled true))

(event Custom|ToggleScope
  (params (On :type Boolean))
  (bind _skeletalmesh (Variables|Default|GetSkeletalMesh))
  ;[1 1 1] Toggle Scope
  (if On
    (Components|SkinnedMesh|UnHideBonebyName _skeletalmesh "Scope")
    (else
      (Components|SkinnedMesh|HideBonebyName _skeletalmesh "Scope" "PBO_None"))))

(event Custom|On%20Click%20End
  (params (Mouse%20Location :type Vector%202D%20Structure))
  ;[1 1 1] Mouse Events
  (Variables|Default|SetRotationEnabled false))

(event Custom|CreateRT-All
  (params (SceneCaptureComponent2D :type Scene%20Capture%20Component%202D%20Object%20Reference))
  ;[1 1 1] Create a render target
  (CallFunction|CreateRT SceneCaptureComponent2D))

(event EventBeginPlay
  ;[1 1 1] Initialzie on begin play
  (Class|SkinnedMeshComponent|SetSkeletalMesh (Variables|Default|GetSkeletalMesh) (Variables|Default|GetModificationMesh) true)
  (CallFunction|CreateRTEvent))

(fn ConstructionScript)

(fn SetNewMesh
  (params (Mesh :type Skeletal%20Mesh%20Object%20Reference) (Material :type Array%20of%20Material%20Interface%20Object%20References) (SetScale :type Vector))
  ;[1 1 1] Setting mesh and scale of recording actor when used lookable item
  (Class|SkinnedMeshComponent|SetSkeletalMesh (Variables|Default|GetSkeletalMesh) Mesh true)
  (Transformation|SetRelativeRotation (Variables|Default|GetSkeletalMesh) "0, 0, 0" false false)
  (Transformation|SetRelativeLocation (Variables|Default|GetSkeletalMesh) "0, 0, 0" false false)
  (Variables|Default|SetScale SetScale)
  (CallFunction|UpdateScaleSkeletal)
  (for (_array_element _array_index) Material
    (Rendering|Material|SetMaterial (Variables|Default|GetSkeletalMesh) _array_index _array_element)))

(fn GetNewRotation
  (params (MouseLocation :type Vector%202D%20Structure))
  (bind _onstartrotating (Variables|Default|GetOnStartRotating))
  (bind _returnvalue (- MouseLocation _onstartrotating))
  (bind (_x _y) (Math|Vector2D|BreakVector2D _returnvalue))
  (return (Math|Rotator|MakeRotator 0.0 (Math|Float|SelectFloat (* (/ _y 4.0) 1.0) 0.0 (> (Math|Float|Absolute(Float) _y) 1.0)) (Math|Float|SelectFloat (* (/ _x 4.0) -1.0) 0.0 (> (Math|Float|Absolute(Float) _x) 1.0)))))

(fn CreateRT
  (params (Local :type Scene%20Capture%20Component%202D%20Object%20Reference))
  (bind _image (Variables|Default|GetImage))
  (bind _brush (Variables|/Script/UMG.Image|GetBrush _image))
  (Utilities|IsValid Local
    (:Is%20Valid
      (Components|Activation|Activate Local false)
      (bind _returnvalue (Rendering|CreateRenderTarget2D 1920 1920 "RTF_RGBA16f"))
      (Variables|/Script/Engine.SceneCaptureComponent2D|SetTextureTarget Local _returnvalue)
      (Utilities|IsValid (Variables|Default|GetDynamicMaterial)
        (:Is%20Valid
          (Rendering|Material|SetTextureParameterValue (Variables|Default|GetDynamicMaterial) "Render" (Variables|/Script/Engine.SceneCaptureComponent2D|GetTextureTarget Local)))
        (:Is%20Not%20Valid
          (Utilities|IsValid (Variables|Default|GetImage)
            (:Is%20Valid
              (bind _returnvalue_2 (Rendering|Material|CreateDynamicMaterialInstance "/Game/ModernRPG/General/GUI/Materials/ItemPreview/M_ItemPreview.M_ItemPreview" "None" "None" :!class /Script/Engine.KismetMaterialLibrary))
              (bind _output_get (Variables|Default|SetDynamicMaterial _returnvalue_2))
              (Class|Image|SetBrush _image (Utilities|Struct|MakeSlateBrush (.imagesize _brush) (.margin _brush) (.tintcolor _brush) "(CornerRadii=(X=0.000000,Y=0.000000,Z=0.000000,W=1.000000),Color=(SpecifiedColor=(R=0.000000,G=0.000000,B=0.000000,A=0.000000),ColorUseRule=UseColor_Specified),Width=0.000000,RoundingType=HalfHeightRadius,bUseBrushTransparency=False)" _output_get (.drawas _brush) (.tiling _brush) (.mirroring _brush)))
              (Class|Image|SetBrushfromMaterial (Variables|Default|GetImage) (Variables|Default|GetDynamicMaterial))
              (Rendering|Material|SetTextureParameterValue (Variables|Default|GetDynamicMaterial) "Render" (Variables|/Script/Engine.SceneCaptureComponent2D|GetTextureTarget Local))
              (return))
            (:Is%20Not%20Valid
              (return))))))))

(fn SetMaterials
  (params (Array :type Array%20of%20Material%20Interface%20Object%20References))
  (for (_array_element _array_index) Array
    (Rendering|Material|SetMaterial (Variables|Default|GetSkeletalMesh) _array_index _array_element)))