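; Backpack Blueprint that shows and hides a parachute, with its opening animation and sound.
; A server event relays the deploy state to an all-clients event, which toggles mesh visibility and the flying component.
; Cloth simulation turns on only after a short retriggerable delay, if the chute is still deployed, and switches off immediately on stow.
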(event Custom|ParachuteControl%20-%20ALL
  (params (Condition :type Boolean))
  ;[1 1 1] Deploy Parachute
  (bind _output_get (Variables|Default|SetEnableClothSimulation Condition))
  (CallFunction|ParactuteControl _output_get)
  (if (Variables|Default|GetEnableClothSimulation)
    (Utilities|FlowControl|RetriggerableDelay 1.41)
    (if (Variables|Default|GetEnableClothSimulation)
      (Variables|/Script/Engine.SkeletalMeshComponent|SetbDisableClothSimulation (Variables|Default|GetSK_Parachute) false))))

(event Custom|ParachuteControl%20-%20Server
  (params (bNewVisibility :type Boolean))
  ;[1 1 1] Deploy Parachute
  (CallFunction|ParachuteControl-ALL bNewVisibility))

(fn ConstructionScript)

(fn ParactuteControl
  (params (Condition :type Boolean))
  (Rendering|SetVisibility (Variables|Default|GetSK_Parachute) Condition false)
  (if Condition
    (Components|Animation|PlayAnimation (Variables|Default|GetSK_Parachute) "/Game/ModernRPG/Shooter/Materials/Parachute/A_ParachuteOpen.A_ParachuteOpen" false)
    (Audio|PlaySoundatLocation "/Game/ModernRPG/Shooter/Sounds/Parachute/SC_ParachuteOpen.SC_ParachuteOpen" (Transformation|GetActorLocation) "0, 0, 0" 1.0 1.0 0.0 0 0 0 0)
    (Components|Activation|Activate (Variables|Default|GetSC_ParachuteFly) false)
    (else
      (Variables|/Script/Engine.SkeletalMeshComponent|SetbDisableClothSimulation (Variables|Default|GetSK_Parachute) true)
      (Components|Activation|Deactivate (Variables|Default|GetSC_ParachuteFly)))))