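; Player character component that performs replicated kunai stealth kills on AI.
; A camera capsule trace accepts living AI in allowed behavior states facing the camera's direction.
; A random animation pair from a data table goes through server to all, unarming and locking the player, snapping them to the victim's tagged billboard.
; Paired montage notifies drive blood and damage, while the server spawns a temporary kunai and completion restores control.
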(event Custom|StealthKill
  ;[1 1 1] Replication
  (Variables|Engine|SetCurrentAnimations (CallFunction|ChooseAnimations))
  (Networking|SwitchHasAuthority
    (:Authority
      (CallFunction|StealthKill-ALL (Variables|Engine|GetCurrentAnimations)))
    (:Remote
      (CallFunction|StealthKill-Server (Variables|Engine|GetCurrentAnimations)))))

(event Custom|StealthKill%20-ALL
  (params (CurrentAnimations :type S%20Stealth%20Animations%20Structure))
  (bind (_result _outhit) (CallFunction|CanStealthKill))
  ;[1 1 1] Stealth Kill Event
  (Variables|Engine|SetCurrentAnimations CurrentAnimations)
  (if _result
    (Utilities|FlowControl|Sequence
      (:then_0
        (bind _output_get (Variables|Default|SetWasHolstered (CallFunction|IsHolstered? (Components|GetOwner))))
        (if (not _output_get)
          (CallFunction|ForceToggleWeapon (Components|GetOwner) true)))
      (:then_1
        (Variables|Engine|SetCurrentHit _outhit)
        (CallFunction|TogglePlayerControl true)
        (Default|UpdateState (Actor|GetComponentbyClass (Components|GetOwner) "/Game/ModernRPG/General/Blueprints/ActorComponents/Character/State/AC_PlayerCurrentState.AC_PlayerCurrentState_C") "NewEnumerator1")
        (bind _ascharacter (Utilities|Casting|CastToCharacter (.HitActor (Collision|BreakHitResult (Variables|Engine|GetCurrentHit))))
          (:then
            (Variables|Engine|SetCurrentKilled _ascharacter)
            (CallFunction|MESSAGETOABPStealthMode true "NewEnumerator0")
            (CallFunction|MESSAGETOABPStealthMode true "NewEnumerator1")
            (Components|MoveComponentTo (Variables|/Script/Engine.Character|GetCapsuleComponent (.AsCharacter (Utilities|Casting|CastToCharacter (Components|GetOwner)))) (Transformation|GetWorldLocation (Utilities|Array|Get(acopy) (Actor|GetComponentsbyTag (Variables|Engine|GetCurrentKilled) "/Script/Engine.BillboardComponent" "StealthKillTarget"))) (Transformation|GetActorRotation (Variables|Engine|GetCurrentKilled)) false false 0.1 false)
            (Utilities|IsValid (Variables|Engine|GetCurrentKilled)
              (:Is%20Valid
                (Utilities|IsValid (.Target (CallFunction|GetControlRotation (Variables|Engine|GetCurrentKilled)))
                  (:Is%20Valid
                    (Pawn|SetControlRotation (.Target (CallFunction|GetControlRotation (Variables|Engine|GetCurrentKilled))) (.Rotation (CallFunction|GetControlRotation (Variables|Engine|GetCurrentKilled)))))))
              (:Is%20Not%20Valid
                _))
            (Utilities|MPlayAnyMontage
              (:On%20Completed/On%20Interrupted
                (if (not (Variables|Default|GetWasHolstered))
                  (CallFunction|ForceToggleWeapon (Components|GetOwner) false)
                  (Variables|Default|SetWasHolstered false)))))
          (:CastFailed
            (CallFunction|ClearState))))
      (:then_2
        (Networking|SwitchHasAuthority
          (:Authority
            (CallFunction|SpawnKunai-Server)))))))

(event Custom|StealthKill%20-Server
  (params (CurrentAnimations :type S%20Stealth%20Animations%20Structure))
  ;[1 1 1] Replication
  (CallFunction|StealthKill-ALL CurrentAnimations))

(event Custom|SpawnKunai%20-%20Server
  ;[1 1 1] Stealth Kill Event
  (bind _returnvalue (Game|SpawnActorfromClass "/Game/ModernRPG/General/Blueprints/Weapon/SimpleAttach/BP_SimpleAttach.BP_SimpleAttach_C" (Math|Transform|MakeTransform "0, 0, 0" "0, 0, 0" "1.000000,1.000000,1.000000") "AlwaysSpawn" (Components|GetOwner) 0))
  (bind _output_get (Variables|Engine|SetBP_Kunai _returnvalue))
  (Default|Initialize _output_get "ACTIVEHAND_Kunai" 0 "/Game/ModernRPG/Shooter/Meshes/Weapon/Kunai/SK_Kunai.SK_Kunai"))

(event Custom|DestroyKunai%20-%20Server
  ;[1 1 1] Stealth Kill Event
  (Utilities|IsValid (Variables|Engine|GetBP_Kunai)
    (:Is%20Valid
      (Actor|DestroyActor (Variables|Engine|GetBP_Kunai)))))

(event EventBeginPlay
  ;[1 1 1] Initialize Player Controller
  (bind _ascharacter (Utilities|Casting|CastToCharacter (Components|GetOwner)))
  (Variables|Engine|SetPlayer _ascharacter)
  (bind _asplayer_controller (Utilities|Casting|CastToPlayerController (Pawn|GetController _ascharacter)))
  (Variables|Engine|SetPlayerController _asplayer_controller))

(fn ChooseAnimations
  (bind _outrownames (DataTable|GetDataTableRowNames (Variables|Settings|GetStealthDT)))
  (bind _returnvalue (Utilities|GetDataTableRow (Variables|Settings|GetStealthDT) (Utilities|Array|Get(acopy) _outrownames (Math|Random|RandomIntegerinRange 0 (- (Utilities|Array|Length _outrownames) 1))))
    (:then
      (return _returnvalue))))

(fn ClearState
  (Variables|/Game/ModernRPG/General/Blueprints/ActorComponents/Character/State/AC_PlayerCurrentState.AC_PlayerCurrentState_C|SetCurrentState (Actor|GetComponentbyClass (Components|GetOwner) "/Game/ModernRPG/General/Blueprints/ActorComponents/Character/State/AC_PlayerCurrentState.AC_PlayerCurrentState_C") "NewEnumerator4")
  (CallFunction|TogglePlayerControl false))

(fn TogglePlayerControl
  (params (Disable :type Boolean))
  (if Disable
    (Input|DisableInput (Components|GetOwner) (Variables|Engine|GetPlayerController))
    (bind _ascharacter (Utilities|Casting|CastToCharacter (Components|GetOwner)))
    (Variables|Member|SetREMEMBER_Use%20Controller%20Rotation%20Yaw (Variables|/Script/Engine.Pawn|GetbUseControllerRotationYaw _ascharacter))
    (Variables|Member|SetREMEMBER_Orient%20Rotation%20To%20Movement (Variables|/Script/Engine.CharacterMovementComponent|GetbOrientRotationToMovement (Variables|/Script/Engine.Character|GetCharacterMovement _ascharacter)))
    (Variables|/Script/Engine.Pawn|SetbUseControllerRotationYaw _ascharacter false)
    (Variables|/Script/Engine.CharacterMovementComponent|SetbOrientRotationToMovement (Variables|/Script/Engine.Character|GetCharacterMovement _ascharacter) false)
    (else
      (Input|EnableInput (Components|GetOwner) (Variables|Engine|GetPlayerController))
      (bind _ascharacter_2 (Utilities|Casting|CastToCharacter (Components|GetOwner)))
      (Variables|/Script/Engine.Pawn|SetbUseControllerRotationYaw _ascharacter_2 (Variables|Member|GetREMEMBER_Use%20Controller%20Rotation%20Yaw))
      (Variables|/Script/Engine.CharacterMovementComponent|SetbOrientRotationToMovement (Variables|/Script/Engine.Character|GetCharacterMovement _ascharacter_2) (Variables|Member|GetREMEMBER_Orient%20Rotation%20To%20Movement)))))

(fn CanbeHit
  (params (Actor :type Actor%20Object%20Reference))
  (bind _result (Class|BPICharacter|IsAlive?(Message) Actor))
  (if _result
    (bind _asbp_base_ai (Utilities|Casting|CastToBP_BaseAI Actor)
      (:then
        (if (Utilities|Array|ContainsItem (Variables|Settings|GetAIStealthModes) (Variables|/Game/ModernRPG/General/Blueprints/AI/Blueprints/BP_BaseAI.BP_BaseAI_C|GetCurrentBehavior _asbp_base_ai))
          (return (Math|Float|NearlyEqual(Float) (.yaw (Transformation|GetActorRotation Actor)) (.Yaw (Math|Rotator|BreakRotator (Transformation|GetWorldRotation (Utilities|Array|Get(acopy) (Actor|GetComponentsbyTag (Components|GetOwner) "/Script/Engine.CameraComponent" "Main"))))) 2e+01))
          (else
            (return false))))
      (:CastFailed
        _)))
  (return false))

(fn CanStealthKill
  (bind _player (Variables|Engine|GetPlayer))
  (bind _returnvalue (Actor|GetComponentsbyTag _player "/Script/Engine.CameraComponent" "Main"))
  (bind _returnvalue_2 (Actor|GetComponentbyClass _player "/Script/Engine.SpringArmComponent"))
  (bind _output (Utilities|Array|Get(acopy) _returnvalue))
  (bind _targetarmlength (Variables|/Script/Engine.SpringArmComponent|GetTargetArmLength _returnvalue_2))
  (bind _returnvalue_3 (Math|Vector|GetForwardVector _output))
  (bind _returnvalue_4 (Transformation|GetWorldLocation _output))
  (bind _returnvalue_5 (* _returnvalue_3 _targetarmlength))
  (bind _returnvalue_6 (+ _returnvalue_4 _returnvalue_5))
  (if (Utilities|Enum|Equal(Enum) (Variables|/Game/ModernRPG/General/Blueprints/ActorComponents/Character/State/AC_PlayerCurrentState.AC_PlayerCurrentState_C|GetCurrentState (Actor|GetComponentbyClass (Components|GetOwner) "/Game/ModernRPG/General/Blueprints/ActorComponents/Character/State/AC_PlayerCurrentState.AC_PlayerCurrentState_C")) "NewEnumerator4")
    (bind (_outhit _returnvalue_7) (Collision|CapsuleTraceByChannel _returnvalue_6 (+ _returnvalue_6 (* (Math|Vector|GetForwardVector _output) (Variables|Settings|GetStealthKillDistance))) 2e+01 1e+01 "TraceTypeQuery1" false 0 "None"))
    (if _returnvalue_7
      (if (CallFunction|CanbeHit (.HitActor (Collision|BreakHitResult _outhit)))
        (return true _outhit)
        (else
          (return false "")))
      (else
        (return false "")))
    (else
      (return false ""))))

(fn GetControlRotation
  (params (Victim :type Actor%20Object%20Reference))
  (bind _returnvalue (Components|GetOwner))
  (bind _returnvalue_2 (Transformation|GetActorLocation Victim))
  (bind _returnvalue_3 (- _returnvalue_2 "0, 0,50.000000"))
  (bind _returnvalue_4 (Transformation|GetActorLocation _returnvalue))
  (bind _instigator (Variables|/Script/Engine.Actor|GetInstigator _returnvalue))
  (bind _returnvalue_5 (Math|Rotator|FindLookatRotation _returnvalue_4 _returnvalue_3))
  (bind _returnvalue_6 (Pawn|GetControlRotation _instigator :!class /Script/Engine.Pawn))
  (return (Pawn|GetController _instigator) (Math|Rotator|MakeRotator (select false (.roll _returnvalue_5) (.roll _returnvalue_6)) (select false (.pitch _returnvalue_5) (.pitch _returnvalue_6)) (.yaw _returnvalue_5))))

(fn MESSAGETOABPStealthMode
  (params (StealthMode :type Boolean) (E_StealthModeOwner :type E_StealthModeOwner%20Enum :default "NewEnumerator0"))
  (switch Utilities|FlowControl|Switch|SwitchonE_StealthModeOwner E_StealthModeOwner
    (:NewEnumerator0
      (bind _defaultbodymesh (Class|BPIAI|GetDemoSkeletalMeshes(Message) (Variables|Engine|GetPlayer)))
      (Class|BPIABP|StealthMode(Message) (Components|SkeletalMesh|GetAnimInstance _defaultbodymesh) E_StealthModeOwner StealthMode))
    (:NewEnumerator1
      (bind _defaultbodymesh_2 (Class|BPIAI|GetDemoSkeletalMeshes(Message) (Variables|Engine|GetCurrentKilled)))
      (Class|BPIABP|StealthMode(Message) (Components|SkeletalMesh|GetAnimInstance _defaultbodymesh_2) E_StealthModeOwner StealthMode))))

(fn GetOnlyHit
  (bind _currenthit (Variables|Engine|GetCurrentHit))
  (bind (_bblockinghit _binitialoverlap _time _distance _location _impactpoint _normal _impactnormal _physmat _hitactor _hitcomponent _hitbonename _bonename _hititem _elementindex _faceindex _tracestart _traceend) (Collision|BreakHitResult _currenthit))
  (bind _bodymesh (CallFunction|GetCharacterSkeleton (Variables|Engine|GetPlayer)))
  (return (Collision|MakeHitResult _bblockinghit _binitialoverlap _time _distance (Transformation|GetSocketLocation _bodymesh "ACTIVEHAND_Kunai") (Transformation|GetSocketLocation _bodymesh "ACTIVEHAND_Kunai") _normal _impactnormal _physmat _hitactor _hitcomponent _hitbonename _bonename _hititem _elementindex _faceindex _tracestart _traceend)))

(fn SpawnBloodEmitter
  (bind _bodymesh (CallFunction|GetCharacterSkeleton (Variables|Engine|GetPlayer)))
  (Effects|SpawnEmitteratLocation "/Game/ModernRPG/Particles/BodyEffect/P_BodyBlood.P_BodyBlood" (.location (Transformation|GetSocketTransform _bodymesh "ACTIVEHAND_Kunai" "RTS_World")) (.rotation (Transformation|GetSocketTransform _bodymesh "ACTIVEHAND_Kunai" "RTS_World"))))

(fn IsTP
  (return (Variables|/Game/ModernRPG/General/Blueprints/ActorComponents/ViewSwitch/AC_ViewSwitch.AC_ViewSwitch_C|GetInThirdPerson (Actor|GetComponentbyClass (Components|GetOwner) "/Game/ModernRPG/General/Blueprints/ActorComponents/ViewSwitch/AC_ViewSwitch.AC_ViewSwitch_C"))))