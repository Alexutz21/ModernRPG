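; Demo character Blueprint for live retargeting to a UE4 body, as its name and components indicate.
; The construction script makes the head follow the UE4 body's pose through Set Master Pose Component.
; Two getters expose a fixed enum value for alternative skeleton use and the default body, head and alternative body meshes.
; The event graph holds no active logic, and the retargeting itself is not in these graphs.
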(event EventBeginPlay
  (|CallParentFunction) ; This node is disabled and will not be called.\nDrag off pins to build functionality.
)

(event Collision|EventActorBeginOverlap
  (params (OtherActor :type Actor%20Object%20Reference)))

(event EventTick
  (params (DeltaSeconds :type Float%20%28single-precision%29)))

(fn ConstructionScript
  (Class|SkinnedMeshComponent|SetMasterPoseComponent (Variables|Default|GetHead_1) (Variables|Default|GetUE4_Body) false))

(fn IsUsingAlternativeSkeleton?
  (return "NewEnumerator1"))

(fn GetDemoSkeletalMeshes
  (return (Variables|Character|GetMesh) (Variables|Default|GetHead_1) (Variables|Default|GetUE4_Body)))