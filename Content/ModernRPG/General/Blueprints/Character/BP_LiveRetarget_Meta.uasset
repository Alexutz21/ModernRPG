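; BP_LiveRetarget_Meta is a ModernRPG character Blueprint for a modular body, apparently a MetaHuman live-retarget variant.
; Construction makes Mesh the master pose for Body, Legs, Torso, Feet and Head1.
; Overrides report the alternative-skeleton setting and expose the part meshes.
; The camera override extends the parent to hide the head outside third person while enabling its hidden shadow, and prints a reminder to add eyes and hair.
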(event EventBeginPlay
  (|CallParentFunction) ; This node is disabled and will not be called.\nDrag off pins to build functionality.
)

(event Collision|EventActorBeginOverlap
  (params (OtherActor :type Actor%20Object%20Reference)))

(event EventTick
  (params (DeltaSeconds :type Float%20%28single-precision%29)))

(fn ConstructionScript
  (Class|SkinnedMeshComponent|SetMasterPoseComponent (Variables|Default|GetBody) (Variables|Character|GetMesh) false))

(fn IsUsingAlternativeSkeleton?
  (return "NewEnumerator2"))

(fn GetDemoSkeletalMeshes
  (return (Variables|Character|GetMesh) (Variables|Default|GetHead_1) (Variables|Default|GetBody) (Variables|Default|GetTorso) (Variables|Default|GetLegs) (Variables|Default|GetFeet)))

(fn ControlMeshandCamera
  (params (ThirdPerson :type Boolean))
  (bind _returnvalue (not ThirdPerson))
  (bind _head_1 (Variables|Default|GetHead_1))
  (|CallParentFunction ThirdPerson)
  (Development|PrintString "Open a \"BP_LiveRetarget_Meta\" actor class and find the function \"ControlMeshAndCamera\". Put everything you need to hide here: eyes, hair, etc..")
  (Development|SetHiddeninGame _head_1 _returnvalue false)
  (Class|PrimitiveComponent|SetCastHiddenShadow _head_1 _returnvalue))