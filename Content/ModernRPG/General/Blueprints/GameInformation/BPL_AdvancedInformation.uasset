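; BPL_AdvancedInformation is a Blueprint library of lookup helpers that resolve creature and character data table references into their row data.
; GetCreatureInfo and GetCharacterInfo each check that the passed handle's data table is valid, fetch the row by its name, and return it when found.
; Neither function explicitly handles an invalid table or a missing row.
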(fn GetCreatureInfo
  (params (Creature :type Data%20Table%20Row%20Handle%20Structure))
  (bind (_datatable _rowname) (Utilities|Struct|BreakDataTableRowHandle Creature))
  (Utilities|IsValid _datatable
    (:Is%20Valid
      (bind _returnvalue (Utilities|GetDataTableRow _datatable _rowname)
        (:then
          (bind _output_get (LocalVariables|SetL_PlaceTask _returnvalue))
          (return _output_get))))))

(fn GetCharacterInfo
  (params (Character :type Data%20Table%20Row%20Handle%20Structure))
  (bind (_datatable _rowname) (Utilities|Struct|BreakDataTableRowHandle Character))
  (Utilities|IsValid _datatable
    (:Is%20Valid
      (bind _returnvalue (Utilities|GetDataTableRow _datatable _rowname)
        (:then
          (bind _output_get (LocalVariables|SetL_PlaceTask _returnvalue))
          (return _output_get))))))