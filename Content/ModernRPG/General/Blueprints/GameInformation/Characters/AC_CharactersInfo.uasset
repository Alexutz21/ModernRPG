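; Actor component that keeps the player's codex of discovered characters, creatures and books.
; On BeginPlay it loads the lists from a BP_SaveCharacters slot and creates a WB_Notify widget; SaveCharacters writes them back.
; Character and book additions route through server/client events, while creatures are added locally and refresh their info widget.
; Duplicates are rejected by row name, and new entries start with Discovered false and trigger the notification.
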(event Custom|AddNewCharacter%20-Replicated
  (params (Character :type Data%20Table%20Row%20Handle%20Structure))
  ;[1 1 1] Replicate getting widget information
  (if (Ability|HasAuthority (Components|GetOwner))
    (CallFunction|AddNewCharacter-Client Character)
    (else
      (CallFunction|AddNewCharacter-Server Character))))

(event Custom|AddNewCharacter%20-Client
  (params (Character :type Data%20Table%20Row%20Handle%20Structure))
  ;[1 1 1] Replicate getting widget information
  (if (not (CallFunction|HasSameCharacter Character))
    (Utilities|Array|Add (Variables|Settings|GetDiscoveredCharacters) (Utilities|Struct|MakeS_CharacterDynamic Character false))
    (CallFunction|Notify)))

(event Custom|AddNewBook%20-Client
  (params (Book :type Data%20Table%20Row%20Handle%20Structure))
  ;[1 1 1] Replicate getting widget information
  (if (not (CallFunction|HasSameBook? Book))
    (Utilities|Array|Add (Variables|Settings|GetDiscoveredBooks) (Utilities|Struct|MakeS_BookDynam Book false))
    (CallFunction|Notify)))

(event Custom|AddNewCharacter%20-Server
  (params (Character :type Data%20Table%20Row%20Handle%20Structure))
  ;[1 1 1] Replicate getting widget information
  (CallFunction|AddNewCharacter-Client Character))

(event Custom|CreateWidget
  ;[1 1 1] Replicate getting widget information
  (if (Ability|HasAuthority (Components|GetOwner))
    (CallFunction|CreateWidget-Client)
    (else
      (CallFunction|CreateWidget-Server))))

(event Custom|CreateWidget%20-Server
  ;[1 1 1] Replicate getting widget information
  (CallFunction|CreateWidget-Client))

(event Custom|CreateWidget%20-Client
  ;[1 1 1] Replicate getting widget information
  (bind _returnvalue (UserInterface|CreateWidget "/Game/ModernRPG/General/GUI/Widgets/Glossary/WB_Notify.WB_Notify_C"))
  (Variables|Default|SetNotification _returnvalue))

(event Custom|AddNewBook%20-Replicated
  (params (Book :type Data%20Table%20Row%20Handle%20Structure))
  ;[1 1 1] Replicate getting widget information
  (if (Ability|HasAuthority (Components|GetOwner))
    (CallFunction|AddNewBook-Client Book)
    (else
      (CallFunction|AddNewBook-Server Book))))

(event Custom|AddNewBook%20-Server
  (params (Book :type Data%20Table%20Row%20Handle%20Structure))
  ;[1 1 1] Replicate getting widget information
  (CallFunction|AddNewBook-Client Book))

(event EventBeginPlay
  ;[1 1 1] At the start of the game you load every information you have collected in the game process
  (CallFunction|LoadCharacters)
  (CallFunction|CreateWidget))

(fn SaveCharacters
  (bind _returnvalue (SaveGame|DoesSaveGameExist (Variables|Default|GetCharactersSaveSlot)))
  (if _returnvalue
    (bind _returnvalue_2 (SaveGame|LoadGamefromSlot (Variables|Default|GetCharactersSaveSlot)))
    (bind _asbp_save_characters (Utilities|Casting|CastToBP_SaveCharacters _returnvalue_2))
    (Variables|Default|SetSaveGAme _asbp_save_characters)
    (else
      (bind _returnvalue_3 (SaveGame|CreateSaveGameObject "/Game/ModernRPG/General/Blueprints/GameInformation/BP_SaveCharacters.BP_SaveCharacters_C"))
      (Variables|Default|SetSaveGAme _returnvalue_3)))
  (Variables|/Game/ModernRPG/General/Blueprints/GameInformation/BP_SaveCharacters.BP_SaveCharacters_C|SetsCharacters (Variables|Default|GetSaveGAme) (Variables|Settings|GetDiscoveredCharacters))
  (Variables|/Game/ModernRPG/General/Blueprints/GameInformation/BP_SaveCharacters.BP_SaveCharacters_C|SetsCreatures (Variables|Default|GetSaveGAme) (Variables|Settings|GetDiscoveredCreatures))
  (Variables|/Game/ModernRPG/General/Blueprints/GameInformation/BP_SaveCharacters.BP_SaveCharacters_C|SetsBooks (Variables|Default|GetSaveGAme) (Variables|Settings|GetDiscoveredBooks))
  (SaveGame|SaveGametoSlot (Variables|Default|GetSaveGAme) (Variables|Default|GetCharactersSaveSlot)))

(fn LoadCharacters
  (bind _returnvalue (SaveGame|DoesSaveGameExist (Variables|Default|GetCharactersSaveSlot)))
  (if _returnvalue
    (bind _returnvalue_2 (SaveGame|LoadGamefromSlot (Variables|Default|GetCharactersSaveSlot)))
    (bind _asbp_save_characters (Utilities|Casting|CastToBP_SaveCharacters _returnvalue_2))
    (Variables|Settings|SetDiscoveredCharacters (Variables|/Game/ModernRPG/General/Blueprints/GameInformation/BP_SaveCharacters.BP_SaveCharacters_C|GetsCharacters _asbp_save_characters))
    (Variables|Settings|SetDiscoveredCreatures (Variables|/Game/ModernRPG/General/Blueprints/GameInformation/BP_SaveCharacters.BP_SaveCharacters_C|GetsCreatures _asbp_save_characters))
    (Variables|Settings|SetDiscoveredBooks (Variables|/Game/ModernRPG/General/Blueprints/GameInformation/BP_SaveCharacters.BP_SaveCharacters_C|GetsBooks _asbp_save_characters))))

(fn AddNewCharacter
  (params (Character :type Data%20Table%20Row%20Handle%20Structure))
  (CallFunction|AddNewCharacter-Replicated Character)
  (return))

(fn HasSameBook?
  (params (Book :type Data%20Table%20Row%20Handle%20Structure))
  (for _array_element (Variables|Settings|GetDiscoveredBooks)
    (if (Utilities|Name|Equal(Name) (.RowName (Utilities|Struct|BreakDataTableRowHandle (.BookInfo (Utilities|Struct|BreakS_BookDynam _array_element)))) (.RowName (Utilities|Struct|BreakDataTableRowHandle Book)))
      (return true)))
  (return false))

(fn AddNewCreature
  (params (Creature :type Data%20Table%20Row%20Handle%20Structure))
  (bind _returnvalue (Components|GetOwner))
  (bind _returnvalue_2 (Actor|GetComponentbyClass _returnvalue "/Game/ModernRPG/General/Blueprints/DialoguesQuests/WidgetHandler/AC_MainWidgetHandler.AC_MainWidgetHandler_C"))
  (bind _wb_creatureinfowidget (Default|GetWidgets _returnvalue_2))
  (if (CallFunction|HasSameCreature Creature)
    (return)
    (else
      (Utilities|Array|Add (Variables|Settings|GetDiscoveredCreatures) (Utilities|Struct|MakeS_CreatureDynam Creature false))
      (Utilities|IsValid _wb_creatureinfowidget
        (:Is%20Valid
          (Default|Update _wb_creatureinfowidget)
          (CallFunction|Notify)
          (return))))))

(fn AddNewBook
  (params (Book :type Data%20Table%20Row%20Handle%20Structure))
  (CallFunction|AddNewBook-Replicated Book))

(fn Notify
  (bind _notification (Variables|Default|GetNotification))
  (Utilities|IsValid (Variables|Default|GetNotification)
    (:Is%20Valid
      (if (UserInterface|Viewport|IsinViewport (Variables|Default|GetNotification))
        (Widget|RemovefromParent _notification)
        (UserInterface|Viewport|AddtoViewport _notification 0)
        (else
          (UserInterface|Viewport|AddtoViewport (Variables|Default|GetNotification) 0))))))

(fn HasSameCharacter
  (params (Character :type Data%20Table%20Row%20Handle%20Structure))
  (bind (_datatable _rowname) (Utilities|Struct|BreakDataTableRowHandle Character))
  (Utilities|IsValid _datatable
    (:Is%20Valid
      (for _array_element (Variables|Settings|GetDiscoveredCharacters)
        (if (Utilities|Name|Equal(Name) (.RowName (Utilities|Struct|BreakDataTableRowHandle (.Character (Utilities|Struct|BreakS_CharacterDynamic _array_element)))) _rowname)
          (return true)))
      (return false))
    (:Is%20Not%20Valid
      (return true))))

(fn HasSameCreature
  (params (Character :type Data%20Table%20Row%20Handle%20Structure))
  (bind (_datatable _rowname) (Utilities|Struct|BreakDataTableRowHandle Character))
  (Utilities|IsValid _datatable
    (:Is%20Valid
      (for _array_element (Variables|Settings|GetDiscoveredCreatures)
        (if (Utilities|Name|Equal(Name) (.RowName (Utilities|Struct|BreakDataTableRowHandle (.Creature (Utilities|Struct|BreakS_CreatureDynam _array_element)))) _rowname)
          (return true)))
      (return false))
    (:Is%20Not%20Valid
      (return true))))