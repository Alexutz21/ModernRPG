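; BP_AudioHelper is an audio helper Blueprint that supplies a sound for a requested type.
; GetSoundByType scans the rows of AudioDataTable for the first one with a matching Type.
; It returns a random entry from that row's Sounds array, so one type can map to several variations.
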(fn ConstructionScript)

(fn GetSoundbyType
  (params (Type :type E_AudioType%20Enum :default "NewEnumerator0"))
  (bind _outrownames (DataTable|GetDataTableRowNames (Variables|Default|GetAudioDataTable)))
  (for _array_element _outrownames
    (bind _returnvalue (Utilities|GetDataTableRow (Variables|Default|GetAudioDataTable) _array_element)
      (:then
        (if (Utilities|Enum|Equal(Enum) (.Type (Utilities|Struct|BreakS_AudioTypes _returnvalue)) Type)
          (return (Utilities|Array|Get(acopy) (.Sounds (Utilities|Struct|BreakS_AudioTypes _returnvalue)) (Math|Random|RandomIntegerinRange 0 (- (Utilities|Array|Length (.Sounds (Utilities|Struct|BreakS_AudioTypes _returnvalue))) 1)))))))))