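; AC_Craft is an actor component that runs player crafting and opens and closes the crafting widget with UI-only input.
; CanCraft checks recipe ingredients against the player's items and caches their locations in LastContains, while HasSpace checks room for the result.
; AddItem consumes those cached stacks and places the result through AC_Inventory.
; Slots that would empty are queued in DeleteIndexes and removed through their inventory widgets afterwards.
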(fn OpenCraftWidget
  (bind _returnvalue (Components|GetOwner))
  (bind _aspawn (Utilities|Casting|CastToPawn _returnvalue))
  (bind _returnvalue_2 (Pawn|GetController _aspawn))
  (bind _asplayer_controller (Utilities|Casting|CastToPlayerController _returnvalue_2))
  (bind _returnvalue_3 (UserInterface|CreateWidget (Variables|Settings|GetCraftWidget)))
  (Variables|Default|SetMainWidget _returnvalue_3)
  (UserInterface|Viewport|AddtoViewport _returnvalue_3 0)
  (Input|SetInputModeUIOnly _asplayer_controller _returnvalue_3 "DoNotLock")
  (Class|Widget|SetUserFocus _returnvalue_3 _asplayer_controller)
  (Variables|/Script/Engine.PlayerController|SetbShowMouseCursor _asplayer_controller true))

(fn AddItem
  (params (Item :type Data%20Table%20Row%20Handle%20Structure))
  (bind _out_row (CallFunction|GetCraftInfo Item))
  (bind _result (Utilities|Struct|BreakS_Craft _out_row))
  (Utilities|FlowControl|Sequence
    (:then_0
      (Utilities|FlowControl|Sequence
        (:then_0
          (for _array_element (Variables|Default|GetLastContains)
            (LocalVariables|SetL_CurAmount (.Amount (Utilities|Struct|BreakS_InvItemDyn (.Item (Utilities|Struct|BreakS_ContainsPerItem _array_element)))))
            (bind _array_element_2 (Utilities|Array|ForEachLoopwithBreak (.Contains (Utilities|Struct|BreakS_ContainsPerItem _array_element)) :!label _label)
              (:LoopBody
                (if (> (LocalVariables|GetL_CurAmount) 0)
                  (bind _array_element_3 (Utilities|Array|ForEachLoopwithBreak (.Items (Utilities|Struct|BreakS_ContainsPlayer _array_element_2)) :!label _label_2)
                    (:LoopBody
                      (if (<= (- (LocalVariables|GetL_CurAmount) (.Amount (Utilities|Struct|BreakS_IndexAmount _array_element_3))) 0)
                        (if (CallFunction|GetingtobeEmpty (.Inventory (Utilities|Struct|BreakS_ContainsPlayer _array_element_2)) (.Index (Utilities|Struct|BreakS_IndexAmount _array_element_3)) (LocalVariables|GetL_CurAmount))
                          (Utilities|Array|Add (LocalVariables|GetDeleteIndexes) (Utilities|Struct|MakeS_DeleteIndexes (.Inventory (Utilities|Struct|BreakS_ContainsPlayer _array_element_2)) (.Index (Utilities|Struct|BreakS_IndexAmount _array_element_3))))
                          (else
                            (Default|RemoveItem (.Inventory (Utilities|Struct|BreakS_ContainsPlayer _array_element_2)) (.Index (Utilities|Struct|BreakS_IndexAmount _array_element_3)) (LocalVariables|GetL_CurAmount))))
                        (LocalVariables|SetL_CurAmount 0)
                        (goto _label_2 Break)
                        (else
                          (if (CallFunction|GetingtobeEmpty (.Inventory (Utilities|Struct|BreakS_ContainsPlayer _array_element_2)) (.Index (Utilities|Struct|BreakS_IndexAmount _array_element_3)) (.Amount (Utilities|Struct|BreakS_IndexAmount _array_element_3)))
                            (Utilities|Array|Add (LocalVariables|GetDeleteIndexes) (Utilities|Struct|MakeS_DeleteIndexes (.Inventory (Utilities|Struct|BreakS_ContainsPlayer _array_element_2)) (.Index (Utilities|Struct|BreakS_IndexAmount _array_element_3))))
                            (else
                              (Default|RemoveItem (.Inventory (Utilities|Struct|BreakS_ContainsPlayer _array_element_2)) (.Index (Utilities|Struct|BreakS_IndexAmount _array_element_3)) (.Amount (Utilities|Struct|BreakS_IndexAmount _array_element_3)))))
                          (LocalVariables|SetL_CurAmount (- (LocalVariables|GetL_CurAmount) (.Amount (Utilities|Struct|BreakS_IndexAmount _array_element_3))))))))
                  (else
                    (goto _label Break)))))))
        (:then_1
          (bind (_result_2 _inventory _location _selectedslots) (Default|CanAddtoInventory (Actor|GetComponentbyClass (Components|GetOwner) "/Game/ModernRPG/General/Blueprints/ActorComponents/Character/Inventory/AC_Inventory.AC_Inventory_C") (.Size (Utilities|Struct|BreakS_InventorySlot (.InvTexture (Utilities|Struct|BreakS_InventoryItem (CallFunction|GetItemInfo (.Row (Utilities|Struct|BreakS_InvItemDyn _result))))))) _result))
          (if _result_2
            (Default|AddItem (Variables|/Game/ModernRPG/General/GUI/Widgets/Inventory/WB_Inventory.WB_Inventory_C|GetCurrentInventory _inventory) (.Result (Utilities|Struct|BreakS_Craft (CallFunction|GetCraftInfo Item))) (Components|GetOwner) _location _selectedslots (Variables|/Game/ModernRPG/General/Blueprints/ActorComponents/Character/Inventory/AC_Inventory.AC_Inventory_C|GetInventoryWidget (Variables|/Game/ModernRPG/General/GUI/Widgets/Inventory/WB_Inventory.WB_Inventory_C|GetCurrentInventory _inventory)))))))
    (:then_1
      (for _array_element_4 (LocalVariables|GetDeleteIndexes)
        (Default|RemoveSlotWidget (Variables|/Game/ModernRPG/General/Blueprints/ActorComponents/Character/Inventory/AC_Inventory.AC_Inventory_C|GetInventoryWidget (.Inventory (Utilities|Struct|BreakS_DeleteIndexes _array_element_4))) (Default|FindIndexSlot (Variables|/Game/ModernRPG/General/Blueprints/ActorComponents/Character/Inventory/AC_Inventory.AC_Inventory_C|GetInventoryWidget (.Inventory (Utilities|Struct|BreakS_DeleteIndexes _array_element_4))) (.Index (Utilities|Struct|BreakS_DeleteIndexes _array_element_4))))))))

(fn CanCraft?
  (params (Item :type Data%20Table%20Row%20Handle%20Structure))
  (Utilities|Array|Clear (Variables|Default|GetLastContains))
  (for _array_element (Utilities|Struct|BreakS_Craft (CallFunction|GetCraftInfo Item))
    (if (.Result (CallFunction|ContainsinPlayer _array_element (Components|GetOwner)))
      (Utilities|Array|Add (Variables|Default|GetLastContains) (Utilities|Struct|MakeS_ContainsPerItem _array_element (.Contains (CallFunction|ContainsinPlayer _array_element (Components|GetOwner)))))
      (else
        (return false))))
  (return true))

(fn HasSpace?
  (params (Item :type Data%20Table%20Row%20Handle%20Structure%20%28by%20ref%29))
  (bind _out_row (CallFunction|GetCraftInfo Item))
  (bind _result (Utilities|Struct|BreakS_Craft _out_row))
  (bind _result_2 (Default|CanAddtoInventory (Actor|GetComponentbyClass (Components|GetOwner) "/Game/ModernRPG/General/Blueprints/ActorComponents/Character/Inventory/AC_Inventory.AC_Inventory_C") (.Size (Utilities|Struct|BreakS_InventorySlot (.InvTexture (Utilities|Struct|BreakS_InventoryItem (CallFunction|GetItemInfo (.Row (Utilities|Struct|BreakS_InvItemDyn _result))))))) _result))
  (return _result_2))

(fn GetingtobeEmpty
  (params (Invnetory :type AC%20Inventory%20Object%20Reference) (Index :type Integer) (Amount :type Integer))
  (return (<= (- (.Amount (Utilities|Struct|BreakS_InvItemDyn (Utilities|Array|Get(acopy) (Variables|/Game/ModernRPG/General/Blueprints/ActorComponents/Character/Inventory/AC_Inventory.AC_Inventory_C|GetInventory Invnetory) Index))) Amount) 0)))

(fn CloseCraftWidget
  (bind _aswb_craft_main (Utilities|Casting|CastToWB_CraftMain (Variables|Default|GetMainWidget)))
  (Default|ExitWidget _aswb_craft_main))