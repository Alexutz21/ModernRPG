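; BP_FootstepEmitter is a short-lived actor in the footsteps system that plays a one-shot particle effect.
; On BeginPlay it spawns the emitter template at its stored location, then deactivates it after a configurable delay.
; A second later it destroys the particle component and itself, but only if that component is still valid.
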(event EventBeginPlay
  (bind _returnvalue (Effects|SpawnEmitteratLocation (Variables|Default|GetEmitter) (Variables|Default|GetLocation)))
  (Utilities|FlowControl|Delay (Variables|Default|GetDelay))
  (Utilities|IsValid _returnvalue
    (:Is%20Valid
      (Components|Activation|Deactivate _returnvalue))
    (:Is%20Not%20Valid
      _))
  (Utilities|FlowControl|Delay 1.0)
  (Utilities|IsValid _returnvalue
    (:Is%20Valid
      (Components|DestroyComponent _returnvalue)
      (Actor|DestroyActor))))

(fn ConstructionScript)