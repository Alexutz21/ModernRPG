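; Vehicle minigun component that handles automatic fire for AI-controlled or player-driven vehicles.
; Start and stop toggle ticking and a gate; each tick requires a living AI or valid driver, then passes a delay macro that paces shots from minigun settings.
; The server shot event reports noise, checks ammo, delegates the line trace to AC_WeaponVehicle and decrements shells.
; Helper functions supply socket transforms, scattered rotation and aiming state.
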(event Custom|EnterGate
  ;[1 1 1 1 40] Machine gun
  (Utilities|FlowControl|Gate true
    (:Exit
      (Utilities|FireDelay
        (:Exit
          (CallFunction|SpawnBulletMG-Server (Variables|Default|GetScatter)))))))

(event Custom|SpawnBullet_MG%20-%20Server
  (params (Scatter :type Vector))
  (bind _returnvalue (Components|GetOwner))
  ;[1 1 1 1 40] Machine gun
  (Variables|Default|SetScatter Scatter)
  (Class|AISenseHearing|ReportNoiseEvent (Transformation|GetActorLocation (Components|GetOwner)) 1.0 (Components|GetOwner) 5e+02 "Noise")
  (bind _count (Class|BPIVehicles|GetCountOfMinigunShells(Message) (Components|GetOwner)))
  (if (> _count 0)
    (Default|Shot-Linetrace (Actor|GetComponentbyClass (Components|GetOwner) "/Game/ModernRPG/Tanks/Components/ActorComponents/AC_WeaponVehicle.AC_WeaponVehicle_C") (Variables|Default|GetMinigunMesh) 2e+02 "/Game/ModernRPG/General/Blueprints/DamageTypes/BPDT_MinigunBullet.BPDT_MinigunBullet_C")
    (Class|BPIVehicles|SetCountOfShells(Message) _returnvalue -1 "NewEnumerator1" false)
    (Class|BPIVehicles|AfterShotAction(Message) _returnvalue "NewEnumerator1")))

(event Custom|MG_Stop
  ;[1 1 1 1 40] Machine gun
  (Components|Tick|SetComponentTickEnabled false)
  (Variables|Default|SetMinigunStarted false)
  (Utilities|FlowControl|Gate true) ; enters at Close
)

(event Custom|MG_Start
  (params (Scatter :type Vector))
  ;[1 1 1 1 40] Machine gun
  (Variables|Default|SetScatter Scatter)
  (Components|Tick|SetComponentTickEnabled true)
  (Variables|Default|SetMinigunStarted true)
  (Utilities|FlowControl|Gate true) ; enters at Open
)

(event EventTick
  (params (DeltaSeconds :type Float%20%28single-precision%29))
  ;[1 1 1 1 40] Machine gun
  (bind _owner (Class|BPIVehicles|GetParentOwner(Message) (Components|GetOwner)))
  (bind _isai_ (Class|BPIPlayerInfo|IsAI?(Message) _owner))
  (if _isai_
    (bind _result (Class|BPICharacter|IsAlive?(Message) _owner))
    (if _result
      (CallFunction|EnterGate))
    (else
      (bind _driver (Class|BPIVehicles|GetDriver(Message) _owner))
      (Utilities|IsValid _driver
        (:Is%20Valid
          (CallFunction|EnterGate))))))

(fn GetMinigunInfo
  (bind _minigunsettings (Class|BPIVehicles|GetMinigunSettings(Message) (Components|GetOwner)))
  (return _minigunsettings))

(fn GetShotLocation
  (return (Transformation|GetSocketLocation (Variables|Default|GetMinigunMesh) "Projectile")))

(fn GetShotRotation
  (params (inScatter :type Vector))
  (bind _returnvalue (Components|GetOwner))
  (bind (_x _y _z) (Math|Vector|BreakVector inScatter))
  (bind _returnvalue_2 (Actor|GetComponentsbyTag _returnvalue "/Script/Engine.ArrowComponent" "MinigunArrow"))
  (bind _returnvalue_3 (* -1 _x))
  (bind _returnvalue_4 (* -1 _y))
  (bind _returnvalue_5 (* -1 _z))
  (bind _output (Utilities|Array|Get(acopy) _returnvalue_2))
  (bind _returnvalue_6 (Math|Random|RandomFloatinRange _returnvalue_5 _z))
  (bind _returnvalue_7 (Math|Random|RandomFloatinRange _returnvalue_3 _x))
  (bind _returnvalue_8 (Math|Random|RandomFloatinRange _returnvalue_4 _y))
  (bind _relativerotation (Variables|/Script/Engine.SceneComponent|GetRelativeRotation _output))
  (bind _returnvalue_9 (Math|Vector|MakeVector _returnvalue_7 _returnvalue_8 _returnvalue_6))
  (bind (_roll _pitch _yaw) (Math|Rotator|BreakRotator _relativerotation))
  (bind (_x_2 _y_2 _z_2) (Math|Vector|BreakVector _returnvalue_9))
  (Variables|Default|SetScatterCalculated _returnvalue_9)
  (return (Math|Rotator|MakeRotator (+ _x_2 _roll) (+ _y_2 _pitch) (+ _z_2 _yaw))))

(fn GetShellLocation
  (return (Transformation|GetSocketLocation (Variables|Default|GetMinigunMesh) "Shell")))

(fn GetShellRotation
  (return (Transformation|GetSocketRotation (Variables|Default|GetMinigunMesh) "Shell")))

(fn IsAiming
  (bind _isaiming (Class|BPIVehicles|IsAiming(Message) (Components|GetOwner)))
  (return _isaiming))