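; Tank lamp part that provides a switchable pair of spotlights on a configurable mesh.
; Toggle, on and off requests run the All events directly with authority, or route through Server events from remote machines.
; The All events set both spotlights' intensity, track the On state and swap the mesh material.
; Tank interface functions return empty, zero or false defaults, except GetParentOwner, which returns the owner.
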(event Custom|ToggleLight%20-%20Server
  (CallFunction|ToggleLight-All))

(event Custom|ToggleLight%20-%20All
  (bind _index (Variables|Default|Getindex))
  (if (Variables|Default|GetOn?)
    (Rendering|Components|Light|SetIntensity (Variables|Default|GetSpotLight) 0.0)
    (Variables|Default|SetOn? false)
    (Rendering|Material|SetMaterial (Variables|Default|GetMesh) _index (Variables|Default|GetDefaultMat))
    (else
      (Rendering|Components|Light|SetIntensity (Variables|Default|GetSpotLight) 1e+05)
      (Variables|Default|SetOn? true)
      (Rendering|Material|SetMaterial (Variables|Default|GetMesh) _index (Variables|Default|GetOnMaterial)))))

(event Custom|TurnOn%20-%20All
  (Rendering|Components|Light|SetIntensity (Variables|Default|GetSpotLight) 1e+05)
  (Variables|Default|SetOn? true)
  (Rendering|Material|SetMaterial (Variables|Default|GetMesh) (Variables|Default|Getindex) (Variables|Default|GetOnMaterial)))

(event Custom|TurnOn%20-%20Server
  (CallFunction|Turnon-All))

(event Custom|TurnOff%20-%20All
  (Rendering|Components|Light|SetIntensity (Variables|Default|GetSpotLight) 0.0)
  (Variables|Default|SetOn? false)
  (Rendering|Material|SetMaterial (Variables|Default|GetMesh) (Variables|Default|Getindex) (Variables|Default|GetDefaultMat)))

(event Custom|TurnOff%20-%20Server
  (CallFunction|TurnOff-All))

(event EventToggleLight
  (Networking|SwitchHasAuthority
    (:Authority
      (CallFunction|ToggleLight-All))
    (:Remote
      (CallFunction|ToggleLight-Server))))

(event EventTurnOff
  (Networking|SwitchHasAuthority
    (:Authority
      (CallFunction|TurnOff-All))
    (:Remote
      (CallFunction|TurnOff-Server))))

(event EventTurnon
  (Networking|SwitchHasAuthority
    (:Authority
      (CallFunction|Turnon-All))
    (:Remote
      (CallFunction|Turnon-Server))))

(fn ConstructionScript
  (Components|StaticMesh|SetStaticMesh (Variables|Default|GetMesh) (Variables|Default|GetMeshLamp)))

(fn CanHit
  (return false))

(fn CanShot?
  (return false))

(fn GetCannonSettings
  (return ""))

(fn GetCannonSound
  (return 0))

(fn GetCountOfCannonShells
  (return 0))

(fn GetCountOfMinigunShells
  (return 0))

(fn GetDriver
  (return 0))

(fn GetDriverPlace
  (return 0))

(fn GetForward/SideSpeed
  (return 0.0 0.0 0.0))

(fn GetHeight
  (return 0.0))

(fn GetHitDecalClass
  (return 0))

(fn GetMinigunSettings
  (return ""))

(fn GetMinimapArrow
  (return 0))

(fn GetParentOwner
  (return (Components|GetOwner)))

(fn GetPassengers
  (return 0))

(fn GetReloadTime
  (return 0.0))

(fn GetSmokeSettings
  (return ""))

(fn GetWBTank
  (return 0))

(fn HitCharacterVelocity
  (return 0.0 0))

(fn IsAiming
  (return false))

(fn IsBOMBLOAD
  (return false))

(fn IsComponentAllright
  (return false))

(fn IsDrone
  (return false))

(fn IsItTrack
  (return false))

(fn IsShell
  (return false))

(fn IsSiucideMode
  (return false))

(fn IsTankValid
  (return false))

(fn IsVehicleActive
  (return false))