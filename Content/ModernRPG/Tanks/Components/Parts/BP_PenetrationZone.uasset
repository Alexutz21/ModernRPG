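; Damageable hit zone for one part of an owning vehicle, turning point and radial damage into penetration results.
; Damage is reduced by the zone's protection, filtered by weakness list and self-damage checks, then routed to the owner's AC_VehicleHit.
; Outcomes include instant ammo explosion, chance-based penetration or ricochet, broken tracks, and vehicle destruction after repeated bullet hits on fuel.
; A few interface queries forward to the owner; most are empty stubs.
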(event Custom|PlaySound_OC
  (params (Sound :type Sound%20Base%20Object%20Reference) (Location :type Vector))
  (Audio|PlaySoundatLocation Sound Location "0, 0, 0" 1.0 1.0 0.0 0 0 0 0))

(event EventBeginPlay
  (if (Variables|Settings|GetShouldHasImpact)
    (Class|PrimitiveComponent|SetPhysMaterialOverride (Variables|Default|GetZone) (Variables|Settings|GetPhysOverridenMat))
    (Variables|Default|SetTags (Utilities|Array|MakeArray "BulletDetector" "ShouldImpact"))))

(event Game|Damage|EventPointDamage
  (params (Damage :type Float%20%28single-precision%29) (DamageType :type Damage%20Type%20Object%20Reference) (HitLocation :type Vector :default "0, 0, 0") (HitNormal :type Vector :default "0, 0, 0") (HitComponent :type Primitive%20Component%20Object%20Reference) (BoneName :type Name :default "None") (ShotFromDirection :type Vector :default "0, 0, 0") (InstigatedBy :type Controller%20Object%20Reference) (DamageCauser :type Actor%20Object%20Reference) (HitInfo :type Hit%20Result%20Structure%20%28by%20ref%29))
  (CallFunction|PointDamageEvent DamageType DamageCauser (* Damage (- 1.0 (Variables|Settings|GetDegree%20of%20protection)))))

(event Game|Damage|EventRadialDamage
  (params (DamageReceived :type Float%20%28single-precision%29) (DamageType :type Damage%20Type%20Object%20Reference) (Origin :type Vector :default "0, 0, 0") (HitInfo :type Hit%20Result%20Structure%20%28by%20ref%29) (InstigatedBy :type Controller%20Object%20Reference) (DamageCauser :type Actor%20Object%20Reference))
  (CallFunction|DamageEvent DamageType DamageCauser (* DamageReceived (- 1.0 (Variables|Settings|GetDegree%20of%20protection)))))

(fn ConstructionScript)

(fn RandomLocation
  (bind _returnvalue (Transformation|GetActorLocation))
  (bind (_x _y _z) (Math|Vector|BreakVector _returnvalue))
  (return (Math|Vector|MakeVector (+ _x (Math|Random|RandomFloatinRange -1.5e+02 1.5e+02)) (+ _y (Math|Random|RandomFloatinRange -1.5e+02 1.5e+02)) (+ _z (Math|Random|RandomFloatinRange -1.5e+02 1.5e+02)))))

(fn GetOwners
  (params (OtherActor :type Actor%20Object%20Reference))
  (bind _returnvalue (Components|GetOwner OtherActor))
  (bind _owner (CallFunction|GetParentOwner))
  (bind _e_pawntype (Class|BPIAI|GetPawnType(Message) _returnvalue))
  (switch Utilities|FlowControl|Switch|SwitchonE_PawnType _e_pawntype
    (:NewEnumerator3
      (bind _owner_2 (Class|BPIVehicles|GetParentOwner(Message) _returnvalue))
      (return _owner _owner_2))
    (:NewEnumerator0
      (return _owner _returnvalue))
    (:NewEnumerator1
      (bind _owner_3 (Class|BPIVehicles|GetParentOwner(Message) (Components|GetOwner OtherActor)))
      (return _owner _owner_3))
    (:NewEnumerator2
      (bind _owner_4 (Class|BPIVehicles|GetParentOwner(Message) (Components|GetOwner OtherActor)))
      (return _owner _owner_4))))

(fn HitAmmunition
  (params (Killer/Shell :type Actor%20Object%20Reference) (ParentOwner :type Actor%20Object%20Reference)))

(fn GetHitOwners)

(fn PointDamageHit
  (bind _owner (CallFunction|GetParentOwner))
  (LocalVariables|SetSelfOwner _owner))

(fn PointDamageEvent
  (params (DamageT :type Damage%20Type%20Object%20Reference) (DamageC :type Actor%20Object%20Reference) (Damage :type Float%20%28double-precision%29))
  (bind _e_damagetype (CallFunction|GetDamageType DamageT))
  (if (!= (Components|GetOwner) DamageC)
    (bind _owner (Class|BPIVehicles|GetParentOwner(Message) DamageC))
    (Utilities|IsValid _owner
      (:Is%20Valid
        (if (!= (Components|GetOwner) _owner)
          (bind _driver (Class|BPIVehicles|GetDriver(Message) (Components|GetOwner)))
          (Utilities|IsValid _driver
            (:Is%20Valid
              (bind _owner_2 (Class|BPIVehicles|GetParentOwner(Message) DamageC))
              (if (!= _owner_2 _driver)
                (if (Utilities|Array|ContainsItem (Variables|Settings|GetListOfWeakness) _e_damagetype) :!label _label
                  (LocalVariables|SetE_DamageType _e_damagetype)
                  (bind _e_pawntype (Class|BPIAI|GetPawnType(Message) (Components|GetOwner)))
                  (switch Utilities|FlowControl|Switch|SwitchonE_PawnType _e_pawntype
                    (:NewEnumerator0
                      (switch Utilities|FlowControl|Switch|SwitchonE_DamageType (LocalVariables|GetE_DamageType) :!label _label_2
                        (:NewEnumerator0
                          (bind _e_pawntype_2 (Class|BPIAI|GetPawnType(Message) DamageC))
                          (switch Utilities|FlowControl|Switch|SwitchonE_PawnType _e_pawntype_2
                            (:NewEnumerator0
                              (CallFunction|FuelEvent (LocalVariables|GetE_DamageType) DamageC))
                            (:NewEnumerator1
                              (bind _driver_2 (Class|BPIVehicles|GetDriver(Message) DamageC :!label _label_3))
                              (CallFunction|FuelEvent (LocalVariables|GetE_DamageType) _driver_2))
                            (:NewEnumerator2
                              (goto _label_3))))
                        (:NewEnumerator2
                          (bind _driver_3 (Class|BPIVehicles|GetDriver(Message) DamageC :!label _label_4))
                          (CallFunction|DamageEvent DamageT _driver_3 Damage))))
                    (:NewEnumerator1
                      (goto _label_2))
                    (:NewEnumerator2
                      (bind _e_pawntype_3 (Class|BPIAI|GetPawnType(Message) DamageC :!label _label_5))
                      (switch Utilities|FlowControl|Switch|SwitchonE_PawnType _e_pawntype_3
                        (:NewEnumerator0
                          (CallFunction|DamageEvent DamageT DamageC Damage))
                        (:NewEnumerator1
                          (goto _label_4))
                        (:NewEnumerator2
                          (goto _label_4))))
                    (:NewEnumerator4
                      (goto _label_5))))))
            (:Is%20Not%20Valid
              (goto _label)))))
      (:Is%20Not%20Valid
        (goto _label)))))

(fn FuelEvent
  (params (Selection :type E_DamageType%20Enum :default "NewEnumerator0") (Killer :type Actor%20Object%20Reference))
  (switch Utilities|FlowControl|Switch|SwitchonE_DamageType Selection
    (:NewEnumerator0
      _)
    (:NewEnumerator3
      _))
  (if (== (Variables|Settings|GetE_Part) (Utilities|Enum|LiteralenumE_TankPart "NewEnumerator7"))
    (bind _output_get (Variables|Default|SetFuelHitCounter (+ (Variables|Default|GetFuelHitCounter) 1)))
    (if (== _output_get 10)
      (Default|DestroyVehicleTrace (Actor|GetComponentbyClass (Components|GetOwner) "/Game/ModernRPG/General/Blueprints/ActorComponents/Machinery/AC_VehicleHit.AC_VehicleHit_C") Selection Killer false)
      (return true)
      (else
        (return true)))
    (else
      (return false))))

(fn DamageEvent
  (params (DamageT :type Damage%20Type%20Object%20Reference) (DamageC :type Actor%20Object%20Reference) (Damage :type Float%20%28double-precision%29))
  (bind _returnvalue (Components|GetOwner))
  (bind _returnvalue_2 (Components|GetOwner))
  (bind _returnvalue_3 (Components|GetOwner))
  (bind _returnvalue_4 (Actor|GetComponentbyClass _returnvalue "/Game/ModernRPG/General/Blueprints/ActorComponents/Machinery/AC_VehicleHit.AC_VehicleHit_C"))
  (bind _returnvalue_5 (Actor|GetComponentbyClass _returnvalue_3 "/Game/ModernRPG/General/Blueprints/ActorComponents/Machinery/AC_VehicleHit.AC_VehicleHit_C"))
  (bind _returnvalue_6 (Actor|GetComponentbyClass _returnvalue_2 "/Game/ModernRPG/General/Blueprints/ActorComponents/Machinery/AC_VehicleHit.AC_VehicleHit_C"))
  (if (Utilities|Array|ContainsItem (Variables|Settings|GetListOfWeakness) (CallFunction|GetDamageType DamageT))
    (bind _isdestroyed (Class|BPIAI|IsDestroyed(Message) (Components|GetOwner)))
    (if (not _isdestroyed)
      (if (!= (Components|GetOwner) DamageC)
        (bind _owner (Class|BPIVehicles|GetParentOwner(Message) DamageC))
        (Utilities|IsValid _owner
          (:Is%20Valid
            (if (!= (Components|GetOwner) _owner)
              (bind _driver (Class|BPIVehicles|GetDriver(Message) (Components|GetOwner)))
              (Utilities|IsValid _driver
                (:Is%20Valid
                  (bind _owner_2 (Class|BPIVehicles|GetParentOwner(Message) DamageC))
                  (if (!= _owner_2 _driver)
                    (bind _e_pawntype (Class|BPIAI|GetPawnType(Message) (Components|GetOwner) :!label _label))
                    (switch Utilities|FlowControl|Switch|SwitchonE_PawnType _e_pawntype
                      (:NewEnumerator3
                        _)
                      (:NewEnumerator1
                        _)
                      (:NewEnumerator2
                        _)
                      (:NewEnumerator4
                        _)
                      (:NewEnumerator5
                        _))
                    (if (Variables|Settings|GetbImmediatelyDestroy)
                      (Default|AmmunitionExplosion (Actor|GetComponentbyClass (Components|GetOwner) "/Game/ModernRPG/General/Blueprints/ActorComponents/Machinery/AC_VehicleHit.AC_VehicleHit_C") (CallFunction|GetDamageType DamageT) DamageC self)
                      (elif (Math|Boolean|ORBoolean (== (CallFunction|GetDamageType DamageT) (Utilities|Enum|LiteralenumE_DamageType "NewEnumerator7")) (== (CallFunction|GetDamageType DamageT) (Utilities|Enum|LiteralenumE_DamageType "NewEnumerator2")) (== (CallFunction|GetDamageType DamageT) (Utilities|Enum|LiteralenumE_DamageType "NewEnumerator10")))
                        (Default|NewHit (Actor|GetComponentbyClass (Components|GetOwner) "/Game/ModernRPG/General/Blueprints/ActorComponents/Machinery/AC_VehicleHit.AC_VehicleHit_C") Damage (CallFunction|GetDamageType DamageT) DamageC)
                        (else
                          (switch Utilities|FlowControl|Switch|SwitchonE_TankPart (Variables|Settings|GetE_Part)
                            (:NewEnumerator2
                              (if (Math|Integer|InRange(Integer) (Math|Random|RandomIntegerinRange 0 100) 0 (Variables|Settings|GetChance%20of%20Breaking%20Through)) :!label _label_2
                                (Utilities|IsValid _returnvalue_5
                                  (:Is%20Valid
                                    (Default|NewHit _returnvalue_5 Damage (CallFunction|GetDamageType DamageT) DamageC)))
                                (else
                                  (CallFunction|PlaySoundOC "/Game/ModernRPG/Tanks/Sounds/Noise/Effects/SC_Ricochet.SC_Ricochet" (Transformation|GetActorLocation))
                                  (Utilities|IsValid _returnvalue_4
                                    (:Is%20Valid
                                      (Default|NoPenetration _returnvalue_4 (CallFunction|GetDamageType DamageT) DamageC))))))
                            (:NewEnumerator3
                              (goto _label_2))
                            (:NewEnumerator4
                              (Class|BPIVehicles|BreakTracks(Message) (Components|GetOwner))
                              (Utilities|IsValid _returnvalue_6
                                (:Is%20Valid
                                  (Default|NewHit _returnvalue_6 0.0 (CallFunction|GetDamageType DamageT) DamageC))))))))))
                (:Is%20Not%20Valid
                  (goto _label)))))
          (:Is%20Not%20Valid
            (goto _label)))))))

(fn BulletDamage
  (return 0.0))

(fn CanHit
  (return false))

(fn CanShot?
  (return false))

(fn GetMinigunShellPlace
  (return 0))

(fn GetTankSettings
  (return ""))

(fn GetActiveCamera
  (return "NewEnumerator0"))

(fn GetAllWeapons
  (return "NewEnumerator0"))

(fn GetArrowBarrel
  (return 0))

(fn GetArrowMinigun
  (return 0))

(fn GetArrowSmoke
  (return 0))

(fn GetAudioAmmunitionExplosion
  (return 0))

(fn GetBarrel
  (return 0))

(fn GetBlackboardRef
  (return 0))

(fn GetBody
  (return 0 0))

(fn GetBodyCamera
  (return 0))

(fn GetBreakThroughSound
  (return 0))

(fn GetCameraAimInside
  (return 0))

(fn GetCameraMinigun
  (return 0))

(fn GetCameraTurret
  (return 0))

(fn GetCannonSettings
  (return ""))

(fn GetCannonSound
  (return 0))

(fn GetCountOfCannonShells
  (return 0))

(fn GetCountOfMachineGun
  (return 0))

(fn GetCountOfMinigunShells
  (return 0))

(fn GetCountOfShells
  (return 0))

(fn GetCountOfSmokes
  (return 0))

(fn GetDefaultAim
  (return 0))

(fn GetDemoSkeletalMeshes
  (return 0 0))

(fn GetDestroyedTankParticle
  (return 0))

(fn GetDestroyedTankSmokeParticle
  (return 0))

(fn GetDetectionDistance[Fighter]
  (return 0.0))

(fn GetDriver
  (return 0))

(fn GetDriverInside
  (return 0))

(fn GetDriverPlace
  (return 0))

(fn GetForward/SideSpeed
  (return 0.0 0.0 0.0))

(fn GetHealth
  (return 0.0 0.0))

(fn GetHeight
  (return 0.0))

(fn GetHitDecalClass
  (return 0))

(fn GetHitWidget
  (return 0))

(fn GetLastActiveWeapon
  (return "NewEnumerator0"))

(fn GetLastWheels
  (return 0))

(fn GetLeftWheels
  (return 0))

(fn GetMainCamera
  (return 0))

(fn GetMainShotParticle
  (return 0))

(fn GetMainSpringArm
  (return 0))

(fn GetMaxSpeed
  (return 0.0))

(fn GetMinigunAim
  (return 0))

(fn GetMinigunSettings
  (return ""))

(fn GetMiniGunTurret
  (return 0))

(fn GetMinimapArrow
  (return 0))

(fn GetName
  (return ""))

(fn GetParentOwner
  (bind _owner (Class|BPIVehicles|GetParentOwner(Message) (Components|GetOwner)))
  (return _owner))

(fn GetPassengers
  (return 0))

(fn GetPawnType
  (bind _owner (CallFunction|GetParentOwner))
  (bind _e_pawntype (Class|BPIAI|GetPawnType(Message) _owner))
  (return _e_pawntype))

(fn GetPlaceforAmmunitionExplosionParticle
  (return 0))

(fn GetPlaneSettings
  (return ""))

(fn GetPointtoShot
  (return 0))

(fn GetPredictAim
  (return 0))

(fn GetReloadTime
  (return 0.0))

(fn GetRicochetSound
  (return 0))

(fn GetRightWheels
  (return 0))

(fn GetSecondShotParticle
  (return 0))

(fn GetShellDamage
  (return 0.0))

(fn GetShotAudio
  (return 0))

(fn GetSmokeSettings
  (return ""))

(fn GetSpeed
  (return 0.0))

(fn GetSplineL
  (return 0))

(fn GetSplineR
  (return 0))

(fn GetSusp
  (return 0))

(fn GetSuspensions
  (return 0))

(fn GetTarget
  (return 0))

(fn GetTeam
  (return "NewEnumerator2"))

(fn GetTrackL
  (return 0))

(fn GetTrackR
  (return 0))

(fn GetTurret
  (return 0))

(fn GetVehicleHealthInfo
  (return ""))

(fn GetWBTank
  (return 0))

(fn HitCharacterVelocity
  (return 0.0 0))

(fn IamParent
  (return false))

(fn IsAiming
  (return false))

(fn IsAlive?
  (bind _result (Class|BPICharacter|IsAlive?(Message) (Components|GetOwner)))
  (return _result))

(fn IsBOMBLOAD
  (return false))

(fn IsComponentAllright
  (return false))

(fn IsDestroyed
  (return false))

(fn IsDrone
  (return false))

(fn IsHeatTrap
  (return false))

(fn IsItTrack
  (return false))

(fn IsShell
  (return false))

(fn IsSiucideMode
  (return false))

(fn IsTank
  (return false))

(fn IsTankActive
  (return false))

(fn IsTankValid
  (return false))

(fn IsVehicleActive
  (return false))

(fn IsVehicleTarget
  (bind _owner (CallFunction|GetParentOwner))
  (bind _istarget (Class|BPIAI|IsVehicleTarget(Message) _owner))
  (return _istarget))

(fn NoImpulse
  (return false))

(fn Person?
  (return false))

(fn PlaceforShotSound
  (return 0))

(fn PointtoMove
  (return false))

(fn Sensible
  (return false))

(fn TankStarted
  (return false))

(fn TypeOfShell
  (return "NewEnumerator0"))